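; BP_Apollo_SaveObject is a save data object that holds the summary of a player's save slot.
; UpdateData stores location, key card level, slot name, difficulty and play time, and stamps the current date and time.
; GetStaticData returns all of those fields together for other code to read.
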(fn UpdateData
  (params (CurrentLocation :type String) (KeyCardLevel :type Integer) (SlotName :type String) (GameDifficulty :type EGameDifficultySetting%20Enum :default "Beginner") (CurrentPlayTime :type Timespan%20Structure))
  (Variables|Default|SetCurrentLocation CurrentLocation)
  (Variables|Default|SetKeyCardLevel KeyCardLevel)
  (Variables|Default|SetSlotName SlotName)
  (Variables|Default|SetCurrentDateTime (Math|DateTime|Now))
  (Variables|Default|SetGameDifficulty GameDifficulty)
  (Variables|Default|SetCurrentPlayTime CurrentPlayTime))

(fn GetStaticData
  (return (Variables|Default|GetSlotName) (Variables|Default|GetCurrentDateTime) (Variables|Default|GetCurrentLocation) (Variables|Default|GetKeyCardLevel) (Variables|Default|GetGameDifficulty) (Variables|Default|GetCurrentPlayTime)))