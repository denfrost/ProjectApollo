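; Game mode Blueprint for CheekyFPS that stores the current game type and exposes game-state queries.
; UpdateGameType sets CurrentGameType, which GetCurrentGameType returns, while GetMissionPracticeStatus reads the IsMissionPractice flag.
; Alert status, alert time left, reflex status, level music player and actor-to-weapon-class conversion are stubs returning fixed defaults or nothing.
; BeginPlay, Tick and the construction script do no work.
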(event EventBeginPlay)

(event EventTick
  (params (DeltaSeconds :type Float%20%28single-precision%29)))

(event EventUpdateGameType
  (params (NewGameType :type E_EGameType%20Enum :default "NewEnumerator0"))
  (Variables|Default|SetCurrentGameType NewGameType))

(fn ConstructionScript)

(fn ConvertActortoWeaponClass
  (params (InActor :type Actor%20Class%20Reference))
  (return 0))

(fn GetAlertStatus
  (return "NewEnumerator0"))

(fn GetAlertStatusTimeLeft
  (return 0.0))

(fn GetCurrentGameType
  (return (Variables|Default|GetCurrentGameType)))

(fn GetLevelMusicPlayer
  (return 0))

(fn GetMissionPracticeStatus
  (return (Variables|Default|GetbIsMissionPractice?)))

(fn GetReflexStatus
  (return false))