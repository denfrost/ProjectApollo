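; Gameplay game mode for CheekyFPS that handles setup when play begins.
; On BeginPlay it runs the parent logic, then switches the first player controller to game-only input.
; It also copies the practice flag from BP_ApolloGameInstance into IsMissionPractice.
; Tick is disabled, and the construction script only calls its parent.
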(event EventBeginPlay
  (|CallParentFunction)
  (Input|SetInputModeGameOnly (Game|GetPlayerController 0))
  (Variables|Default|SetbIsMissionPractice? (Variables|/Game/CheekyFPS/Blueprints/Game/BP_ApolloGameInstance.BP_ApolloGameInstance_C|GetIs%20Practice? (.AsBP%20Apollo%20Game%20Instance (Utilities|Casting|CastToBP_ApolloGameInstance (Game|GetGameInstance))))))

(event EventTick
  (params (DeltaSeconds :type Float%20%28single-precision%29))
  (|CallParentFunction DeltaSeconds) ; This node is disabled and will not be called.\nDrag off pins to build functionality.
)

(fn ConstructionScript
  (|CallParentFunction))