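; Game instance for the Apollo FPS that manages saving, loading, new-game starts and session-wide data.
; On init it scans save slots, resets settings if no gamepad type is set, sets difficulty and builds level-name and weapon lookup maps.
; Saves use Rama Save with a static data object from the game state plus a screenshot.
; Loads read that static data to open the saved level, with most-recent-save lookup by file timestamp.
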(event EventInit
  (|CallParentFunction)
  (CallFunction|GetValidSaveNames)
  (Utilities|FlowControl|Sequence
    (:then_0
      (if (Utilities|Enum|Equal(Enum) (Class|ApolloPlayerSettingsLibrary|GetPlayerGamepadType) "None")
        (Class|ApolloPlayerSettingsLibrary|ResetGameSettingstoDefault)
        (Development|PrintString "Reset Game Settings!")))
    (:then_1
      (Variables|Default|SetSupportsDLSS? (Class|DLSSLibrary|IsDLSSSupported))
      (Class|ApolloGameInstance|SetGameDifficulty "Medium")
      (CallFunction|GetLevelNames))
    (:then_2
      (Utilities|FlowControl|Delay 0.5)
      (for _array_element (Variables|Default|GetDataTableRowArray)
        (bind _returnvalue (Utilities|GetDataTableRow (Variables|Default|GetWeaponLookupTable) _array_element)
          (:then
            (Utilities|Map|Add (Variables|Default|GetWeapons) (.WeaponName (Utilities|Struct|BreakPlayerWeaponStruct _returnvalue)) (.WeaponBlueprint (Utilities|Struct|BreakPlayerWeaponStruct _returnvalue))))))
      (bind _values (Utilities|Map|Values (Variables|Default|GetWeapons)))
      (for _array_element_2 _values
        _))))

(event EventSavePlayerData
  (params (NewFilePath :type String))
  (bind _returnvalue (Game|GetGameState))
  (bind _asissgame_state_base (Utilities|Casting|CastToISSGameStateBase _returnvalue))
  (bind _apollorso (Variables|/Game/CheekyFPS/Blueprints/Game/ISSGameStateBase.ISSGameStateBase_C|GetApolloRSO _asissgame_state_base))
  (CallFunction|UpdateCurrentSaveSlotName (CallFunction|GetSaveSlotName NewFilePath))
  (Default|UpdateStaticData _asissgame_state_base)
  (bind _fileiosuccess (Class|RamaSaveLibrary|RamaSaveSaveOnlyStatictoFile NewFilePath _apollorso))
  (if _fileiosuccess
    (Development|PrintString "Static Data Saved!")
    (bind (_fileiosuccess_2 _allcomponentssaved) (Class|RamaSaveLibrary|RamaSaveSavetoFile NewFilePath "" false _apollorso))
    (if (and _fileiosuccess_2 _allcomponentssaved)
      (CallFunction|CaptureSaveSlotScreenshot (Game|GetPlayerController 0) self)
      (Development|PrintString "Saved!")
      (Development|PrintString NewFilePath true true "(R=1.000000,G=0.897364,B=0.000000,A=1.000000)"))))

(event EventLoadMostRecentSave
  (bind _returnvalue (CallFunction|GetMostRecentSave))
  (CallFunction|LoadPlayerData _returnvalue)
  (CallFunction|LoadtoNewLevelfromSave _returnvalue))

(event EventLoadPlayerData
  (params (NewFilePath :type String))
  (if (Class|RamaSaveLibrary|RamaSaveFileExists NewFilePath)
    (bind _fileiosuccess (Class|RamaSaveLibrary|RamaSaveLoadfromFile NewFilePath true false true))
    (if _fileiosuccess
      (Development|PrintString "Loaded!"))))

(event EventIsStartingNewGame?
  (params (bStartingNewGame? :type Boolean) (NewGameDifficulty :type EGameDifficultySetting%20Enum :default "Beginner"))
  (Variables|Default|SetbStartingNewGame? bStartingNewGame?)
  (CallFunction|SetNewGameDifficulty NewGameDifficulty)
  (Development|PrintString (Utilities|String|EnumtoString NewGameDifficulty))
  (Game|OpenLevel(byName) "ActOneMap"))

(event EventLoadtoNewLevelfromSave
  (params (SaveFilePath :type String))
  (if (Class|RamaSaveLibrary|RamaSaveFileExists SaveFilePath)
    (bind (_fileiosuccess _returnvalue) (Class|RamaSaveLibrary|RamaSaveLoadStaticDatafromFile SaveFilePath))
    (if _fileiosuccess
      (CallFunction|LoadNewLevel (Utilities|String|StringToName (Variables|/Game/CheekyFPS/Blueprints/Game/BP_Apollo_SaveObject.BP_Apollo_SaveObject_C|GetCurrentLocation (.AsBP%20Apollo%20Save%20Object (Utilities|Casting|CastToBP_Apollo_SaveObject _returnvalue)))))
      (Development|PrintString (Utilities|String|EnumtoString (Class|ApolloGameInstance|GetGameDifficulty))))))

(event EventUpdateCurrentSaveSlotName
  (params (NewSaveSlotName :type String))
  (Class|ApolloGameInstance|SetCurrentSaveSlot NewSaveSlotName))

(event EventSetNewGameDifficulty
  (params (NewDifficulty :type EGameDifficultySetting%20Enum :default "Beginner"))
  (Class|ApolloGameInstance|SetGameDifficulty NewDifficulty))

(event EventRefreshSaveSlots
  (CallFunction|GetValidSaveNames))

(event EventLoadGamefromMenu
  (params (NewFilePath :type String))
  (CallFunction|LoadPlayerData NewFilePath)
  (CallFunction|LoadtoNewLevelfromSave NewFilePath)
  (Development|PrintString "Loaded from Menu!"))

(fn UpdatePlayerStruct
  (params (CurrentHealth :type Float%20%28single-precision%29) (MaxHealth :type Float%20%28single-precision%29) (CurrentItemInventory :type Array%20of%20BP%20Item%20Base%20Object%20References) (CurrentWeaponInventory :type Map%20of%20Integers%20to%20Objects)))

(fn GetPlayerStructData
  (return 0.0 0.0 0 0))

(fn GetValidSaveNames
  (for _array_element (Class|ApolloGameInstance|GetPossibleManualSaveSlots)
    (if (Class|RamaSaveLibrary|RamaSaveFileExists (Class|VictoryBPFunctionLibrary|AppendMultiple (CallFunction|GetSaveLocation) _array_element ".sav"))
      (Utilities|Array|AddUnique (Variables|Default|GetCurrentSaveSlotsArray) (Class|VictoryBPFunctionLibrary|AppendMultiple (CallFunction|GetSaveLocation) _array_element ".sav"))
      (else
        (Class|ApolloGameInstance|SetCurrentSaveSlotFilePath (Class|VictoryBPFunctionLibrary|AppendMultiple (CallFunction|GetSaveLocation) "SaveSlotA" ".sav")))))
  (Class|ApolloGameInstance|SetCurrentManualSaves (Variables|Default|GetCurrentSaveSlotsArray))
  (CallFunction|GetValidStaticData)
  (for _array_element_2 (Class|ApolloGameInstance|GetPossibleAutoSaveSlots)
    (if (Class|RamaSaveLibrary|RamaSaveFileExists (Class|VictoryBPFunctionLibrary|AppendMultiple (CallFunction|GetSaveLocation) _array_element_2 ".sav"))
      (Utilities|Array|AddUnique (LocalVariables|GetLocal_AutoSaveSlotArray) _array_element_2)))
  (Class|ApolloGameInstance|SetCurrentAutoSaves (LocalVariables|GetLocal_AutoSaveSlotArray))
  (for _array_element_3 (Variables|Default|GetCurrentSaveSlotsArray)
    (Utilities|Array|AddUnique (LocalVariables|GetLocal_AllSavesArray) _array_element_3))
  (for _array_element_4 (LocalVariables|GetLocal_AutoSaveSlotArray)
    (Utilities|Array|AddUnique (LocalVariables|GetLocal_AllSavesArray) _array_element_4))
  (Class|ApolloGameInstance|SetAllCurrentSaves (LocalVariables|GetLocal_AllSavesArray)))

(fn GetValidStaticData
  (for _array_element (Variables|Default|GetCurrentSaveSlotsArray)
    (bind (_fileiosuccess _returnvalue) (Class|RamaSaveLibrary|RamaSaveLoadStaticDatafromFile _array_element))
    (if _fileiosuccess
      (Utilities|Map|Add (Variables|Default|GetStaticDataArray) (CallFunction|GetSaveSlotName _array_element) (.AsBP%20Apollo%20Save%20Object (Utilities|Casting|CastToBP_Apollo_SaveObject _returnvalue))))))

(fn GetMostRecentSave
  (bind _localsavedatetimemap (LocalVariables|GetLocalSaveDateTimeMap))
  (for _array_element (Class|ApolloGameInstance|GetAllSavesonDisk)
    (Utilities|Map|Add (LocalVariables|GetLocalSaveDateTimeMap) (Class|RamaSaveLibrary|RamaSaveGetFileTimeStamp _array_element) _array_element))
  (bind _keys (Utilities|Map|Keys _localsavedatetimemap))
  (if (.ReturnValue (Utilities|Map|Find _localsavedatetimemap (.MaxValue (Class|LowEntryExtendedStandardLibrary|MaxOfDateTimeArray _keys))))
    (return (.Value (Utilities|Map|Find _localsavedatetimemap (.MaxValue (Class|LowEntryExtendedStandardLibrary|MaxOfDateTimeArray _keys)))))))

(fn GetMostRecentManualSave
  (for _array_element (Class|ApolloGameInstance|GetCurrentManualSaveSlots)
    (if (not (Utilities|String|Contains _array_element "AutoSave"))
      (if (>= (Class|RamaSaveLibrary|RamaSaveGetFileTimeStamp _array_element) (Math|DateTime|Now))
        (return _array_element)))))

(fn GetLevelNames
  (for _array_element (Variables|Default|GetBaseLevelFolderNames)
    (LocalVariables|SetInCategoryName _array_element)
    (bind _returnvalue (Class|GetAllMapNamesPluginBPLibrary|GetAllMapNamesbyFolder (LocalVariables|GetInCategoryName)))
    (for (_array_element_2 _array_index) _returnvalue
      (LocalVariables|SetLocalArrayIndex _array_index)
      (LocalVariables|SetLocalLevelName _array_element_2)
      (switch string (LocalVariables|GetInCategoryName)
        (:Campaign
          (Utilities|Map|Add (Variables|Default|GetCampaignLevelNames) (LocalVariables|GetLocalArrayIndex) (.RightS (Utilities|String|Split (LocalVariables|GetLocalLevelName) "/"))))
        (:Stealth
          (Utilities|Map|Add (Variables|Default|GetStealthLevelNames) _array_index (.RightS (Utilities|String|Split _array_element_2 "/"))))))))

(fn GetCurrentGameDifficulty
  (return (Class|ApolloGameInstance|GetGameDifficulty)))

(fn GetCurrentStaticSaveHeader
  (return 0))

(fn GetNewGameStatus
  (return (Variables|Default|GetbStartingNewGame?)))