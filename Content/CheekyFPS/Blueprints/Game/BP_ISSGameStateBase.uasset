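; Game state for the FPS that owns the Calm/Warning/Alert alarm status, driving alarm events, music and a pausable cooldown timer.
; BeginPlay creates the save object, music player and Chameleon effects actor, and finds the next stealth level.
; Detection can trigger Reflex slow motion via global time dilation before escalating to Alert.
; It also tracks play time, updates save data, spawns backup enemies and places a failure endpoint when stealth missions fail.
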(event Custom|IncrementMissionPlayTime
  (Variables|Default|SetCurrentMissionPlayTime (+ (Variables|Default|GetCurrentMissionPlayTime) (Math|Timespan|MakeTimespan 0 0 0 0 1))))

(event Custom|UpdateStaticData
  (params (RamaSaveComponent :type Rama%20Save%20Component%20Object%20Reference))
  (bind _returnvalue (CallFunction|GetCurrentSaveSlotName))
  (bind _returnvalue_2 (Game|GetGameInstance))
  (bind _returnvalue_3 (Game|Player|GetPlayerPawn 0))
  (bind _apollorso (Variables|Default|GetApolloRSO))
  (bind _current_play_time (Variables|Default|GetCurrent%20Play%20Time))
  (bind _returnvalue_4 (Actor|GetComponentbyClass _returnvalue_3 "/Game/CheekyFPS/Blueprints/Components/BP_InventoryComponent.BP_InventoryComponent_C"))
  (bind _currentkeycard (Variables|/Game/CheekyFPS/Blueprints/Components/BP_InventoryComponent.BP_InventoryComponent_C|GetCurrentKeyCard _returnvalue_4))
  (Utilities|IsValid _apollorso
    (:Is%20Valid
      (bind _returnvalue_5 (Game|GetCurrentLevelName true))
      (Utilities|IsValid _currentkeycard
        (:Is%20Valid
          (bind _returnvalue_6 (Class|BPISaveLoad|GetCurrentGameDifficulty(Message) _returnvalue_2))
          (Default|UpdateData _apollorso _returnvalue_5 (Variables|/Game/CheekyFPS/Blueprints/Interaction/Items/BP_ItemBase.BP_ItemBase_C|GetItemLevel _currentkeycard) _returnvalue _returnvalue_6 _current_play_time))
        (:Is%20Not%20Valid
          (bind _returnvalue_7 (Class|BPISaveLoad|GetCurrentGameDifficulty(Message) _returnvalue_2))
          (Default|UpdateData _apollorso _returnvalue_5 0 _returnvalue _returnvalue_7 _current_play_time))))))

(event Custom|IncrementPlayTime
  (Variables|Default|SetCurrent%20Play%20Time (+ (Variables|Default|GetCurrent%20Play%20Time) (Math|Timespan|MakeTimespan 0 0 0 1))))

(event Custom|SetStatusToCalm
  (CallFunction|StartCalmStatus))

(event Custom|OnMissionEndEvent
  (params (bWasSuccessful? :type Boolean))
  (if (not bWasSuccessful?)
    (switch Utilities|FlowControl|Switch|SwitchonE_EGameType (Variables|Default|GetCurrentGameType)
      (:NewEnumerator2
        (Game|SpawnActorfromClass "/Game/CheekyFPS/Blueprints/Interaction/Mission/BP_MissionEndpoint.BP_MissionEndpoint_C" (Transformation|GetActorTransform (Game|Player|GetPlayerPawn 0)) "Undefined" 0 false 0)))))

(event EventBeginPlay
  (bind _returnvalue (Game|GetGameMode))
  (bind _returnvalue_2 (Game|ConstructObjectfromClass "/Game/CheekyFPS/Blueprints/Game/BP_Apollo_SaveObject.BP_Apollo_SaveObject_C" self))
  (Variables|Default|SetApolloRSO _returnvalue_2)
  (Utilities|FlowControl|Sequence
    (:then_0
      (EventDispatchers|BindEventtoOnPlayerLost (EventDispatchers|CreateEvent :!event PauseAlarmTimer))
      (EventDispatchers|BindEventtoOnPlayerDetected (EventDispatchers|CreateEvent :!event UnpauseAlarmTimer))
      (bind _returnvalue_3 (Class|BPIGameEvents|GetCurrentGameType(Message) _returnvalue))
      (bind _output_get (Variables|Default|SetCurrentGameType _returnvalue_3))
      (EventDispatchers|BindEventtoOnMissionEnd (.AsBP%20ISSCheeky%20Game%20Mode (Utilities|Casting|CastToBP_ISSCheekyGameMode _returnvalue)) (EventDispatchers|CreateEvent :!event Custom|OnMissionEndEvent))
      (switch Utilities|FlowControl|Switch|SwitchonE_EGameType _output_get
        (:NewEnumerator2
          (CallFunction|NewFunction0 (Variables|/Game/CheekyFPS/Blueprints/Game/BP_ApolloGameInstance.BP_ApolloGameInstance_C|GetStealthLevelNames (.AsBP%20Apollo%20Game%20Instance (Utilities|Casting|CastToBP_ApolloGameInstance (Game|GetGameInstance))))))))
    (:then_1
      (if (not (Utilities|IsValid (Variables|Default|GetChamReference)))
        (bind _returnvalue_4 (Game|SpawnActorfromClass "/Game/CheekyFPS/Chameleon/ISS_Chameleon.ISS_Chameleon_C" (Math|Transform|MakeTransform "0, 0, 0") "Undefined" 0 0))
        (Variables|Default|SetChamReference _returnvalue_4)))
    (:then_2
      (bind _returnvalue_5 (Game|SpawnActorfromClass "/Game/CheekyFPS/Blueprints/Game/BP_MusicPlayer.BP_MusicPlayer_C" (Math|Transform|MakeTransform "0, 0, 0") "Undefined" 0 true 0))
      (Variables|Default|SetBGMPlayerRef _returnvalue_5))
    (:then_3
      (if (< (Class|GameplayStatics|GetGlobalTimeDilation) 1.0)
        (Utilities|Time|SetGlobalTimeDilation 1.0)))))

(event EventSecurityAlarmInterface
  (params (SendAlarm :type Boolean) (NewAlertStatus :type E_EAlertStatus%20Enum :default "NewEnumerator0"))
  (Variables|Default|SetCurrentAlertStatus NewAlertStatus)
  (CallFunction|UpdateAlertStatus)
  (Default|CallOnPlayerDetected))

(event EventUpdateSpawners
  (params (NewSpawners :type Array%20of%20BP%20Spawner%20Object%20References))
  (for _array_element NewSpawners
    (Utilities|Array|AddUnique (Variables|Default|GetEnemySpawners) _array_element)))

(event EventShouldSpawnBackup?
  (params (bRequestApproved? :type Boolean))
  (if (and bRequestApproved? (not (Variables|Default|GetbHaveNewEnemiesHaveSpawned?)))
    (for _array_element (Variables|Default|GetEnemySpawners)
      (bind _returnvalue (Default|SpawnNewEnemy _array_element (Transformation|GetActorLocation _array_element) (Transformation|GetActorRotation _array_element) "/Game/CheekyFPS/Blueprints/Enemies/Humanoids/BP_GruntEnemy.BP_GruntEnemy_C"))
      (AI|Components|Blackboard|SetValueasVector (AI|GetBlackboard (AI|GetAIController _returnvalue)) (Utilities|Name|MakeLiteralName "PointOfInterest") (Transformation|GetActorLocation (Game|GetPlayerCharacter 0)))
      (Variables|Default|SetbHaveNewEnemiesHaveSpawned? true))))

(event EventClearSpawners
  (Utilities|Array|Clear (Variables|Default|GetEnemySpawners))
  (Variables|Default|SetbHaveNewEnemiesHaveSpawned? false))

(event EventFindSpawners
  (bind _outactors (Actor|GetAllActorswithTag "Spawner"))
  (for _array_element _outactors
    (if (Utilities|IsValid (.AsBP%20Spawner (Utilities|Casting|CastToBP_Spawner _array_element)))
      (Utilities|Array|AddUnique (Variables|Default|GetEnemySpawners) (.AsBP%20Spawner (Utilities|Casting|CastToBP_Spawner _array_element))))))

(event EventToggleFreezeEffect?
  (params (bActivateEffect? :type Boolean))
  (Default|ToggleFreezeEffect (Variables|Default|GetChamReference) bActivateEffect?))

(event EventToggleSonarEffect?
  (params (bActivateEffect? :type Boolean))
  (Default|ToggleSonarEffect (Variables|Default|GetChamReference) bActivateEffect?)
  (Class|BPIChameleon|ToggleSonarEffect?(Message) (Game|GetPlayerCharacter 0) bActivateEffect?))

(event EventTick
  (params (DeltaSeconds :type Float%20%28single-precision%29))
  (bind _alertstatusresettimer (Variables|Default|GetAlertStatusResetTimer))
  (Utilities|FlowControl|Sequence
    (:then_0
      (Utilities|IsValid (Variables|Default|GetApolloRSO)
        (:Is%20Not%20Valid
          (bind _returnvalue (Game|ConstructObjectfromClass "/Game/CheekyFPS/Blueprints/Game/BP_Apollo_SaveObject.BP_Apollo_SaveObject_C" self))
          (Variables|Default|SetApolloRSO _returnvalue))))
    (:then_1
      (if (and (Utilities|Time|IsTimerActivebyHandle _alertstatusresettimer) (not (Class|KismetSystemLibrary|IsTimerPausedHandle _alertstatusresettimer)))
        (Variables|Default|SetAlertStatusRemainingTime (Utilities|Time|GetTimerRemainingTimebyHandle _alertstatusresettimer))))))

(event EventResetAlertStatus
  (CallFunction|StartCalmStatus))

(event EventPlayReflex
  (CallFunction|PlayReflexEffect))

(event EventUnpauseAlarmTimer
  (bind _alertstatusresettimer (Variables|Default|GetAlertStatusResetTimer))
  (if (Class|KismetSystemLibrary|IsTimerPausedHandle _alertstatusresettimer)
    (Utilities|Time|UnpauseTimerbyHandle _alertstatusresettimer)))

(event EventPauseAlarmTimer
  (bind _alertstatusresettimer (Variables|Default|GetAlertStatusResetTimer))
  (if (Utilities|Time|IsTimerActivebyHandle _alertstatusresettimer)
    (Utilities|Time|PauseTimerbyHandle _alertstatusresettimer)
    (Variables|Default|SetAlertStatusRemainingTime 99.0)))

(event EventToggleScopeEffect?
  (params (bActivateEffect? :type Boolean))
  (Default|ToggleScopeEffect (Variables|Default|GetChamReference) bActivateEffect?))

(event EventStopReflexFX
  (params (bTriggerAlarm? :type Boolean))
  (if bTriggerAlarm?
    (CallFunction|EndReflexEffect)
    (Variables|Default|SetCurrentAlertStatus "NewEnumerator2")
    (else
      (CallFunction|EndReflexEffect)))
  (CallFunction|UpdateAlertStatus))

(fn ConstructionScript)

(fn PlayReflexEffect
  (if (not (Utilities|Enum|Equal(Enum) (Variables|Default|GetCurrentAlertStatus) "NewEnumerator3"))
    (if (Utilities|Enum|NotEqual(Enum) (Variables|Default|GetCurrentAlertStatus) "NewEnumerator2")
      (Utilities|Time|SetGlobalTimeDilation 0.5)
      (bind _output_get (Variables|Default|SetIsReflexActive? true))
      (Default|ToggleReflexEffect (Variables|Default|GetChamReference) _output_get)
      (CallFunction|ResetReflexEffect))))

(fn ResetReflexEffect
  (Utilities|Time|SetTimerbyEvent (EventDispatchers|CreateEvent :!event EndReflexEffect) 5.0))

(fn EndReflexEffect
  (Utilities|Time|SetGlobalTimeDilation 1.0)
  (bind _output_get (Variables|Default|SetIsReflexActive? false))
  (Default|ToggleReflexEffect (Variables|Default|GetChamReference) _output_get))

(fn StartAlertStatus
  (Default|CallOnAlarmActivate)
  (bind _output_get (Variables|Default|SetCurrentAlertStatus "NewEnumerator2"))
  (Default|PlayStatusMusic (Variables|Default|GetBGMPlayerRef) _output_get))

(fn UpdateAlertStatus
  (switch Utilities|FlowControl|Switch|SwitchonE_EAlertStatus (Variables|Default|GetCurrentAlertStatus)
    (:NewEnumerator0
      (CallFunction|StartCalmStatus)
      (Variables|Default|SetbHaveNewEnemiesHaveSpawned? false))
    (:NewEnumerator2
      (CallFunction|StartAlertStatus)
      (CallFunction|SetAlertCooldownTimer))
    (:NewEnumerator3
      (CallFunction|StartWarningStatus))))

(fn StartCalmStatus
  (Default|CallOnAlarmDeactivate)
  (bind _output_get (Variables|Default|SetCurrentAlertStatus "NewEnumerator0"))
  (Default|PlayStatusMusic (Variables|Default|GetBGMPlayerRef) _output_get))

(fn SetAlertCooldownTimer
  (bind _returnvalue (Utilities|Time|SetTimerbyEvent (EventDispatchers|CreateEvent :!event Custom|SetStatusToCalm) 6e+01))
  (Variables|Default|SetAlertStatusResetTimer _returnvalue))

(fn GetRemainingAlertTime
  (return (Variables|Default|GetAlertStatusRemainingTime)))

(fn NewFunction0
  (params (TargetMap :type Map%20of%20Integers%20to%20Strings))
  (bind _returnvalue (Game|GetCurrentLevelName true))
  (Variables|Default|SetCurrentLevelName _returnvalue)
  (bind _values (Utilities|Map|Values TargetMap))
  (for (_array_element _array_index) _values
    (if (Utilities|Enum|Equal(Enum) _array_element (Variables|Default|GetCurrentLevelName))
      (bind _output_get (LocalVariables|SetArray%20Index _array_index))
      (bind _result (Math|Integer|IncrementInt _output_get)
        (:%20%20
          (bind _output_get_2 (LocalVariables|SetNextLevelIndex _result))
          (if (.ReturnValue (Utilities|Map|Find TargetMap _output_get_2))
            (Variables|Default|SetNextLevelName (.Value (Utilities|Map|Find TargetMap _output_get_2)))))))))

(fn StartWarningStatus
  (bind _output_get (Variables|Default|SetCurrentAlertStatus "NewEnumerator3"))
  (Default|PlayStatusMusic (Variables|Default|GetBGMPlayerRef) _output_get))

(fn ConvertActortoWeaponClass
  (params (InActor :type Actor%20Class%20Reference))
  (return 0))

(fn GetAlertStatus
  (return (Variables|Default|GetCurrentAlertStatus)))

(fn GetAlertStatusTimeLeft
  (return (CallFunction|GetRemainingAlertTime)))

(fn GetCurrentAlertStatus
  (return (Variables|Default|GetCurrentAlertStatus)))

(fn GetCurrentAlertTime
  (return (CallFunction|GetRemainingAlertTime)))

(fn GetCurrentGameDifficulty
  (return "Beginner"))

(fn GetCurrentGameType
  (return "NewEnumerator0"))

(fn GetCurrentMissionTime
  (return (Variables|Default|GetCurrentMissionPlayTime)))

(fn GetCurrentStaticSaveHeader
  (bind _apollorso (Variables|Default|GetApolloRSO))
  (Utilities|IsValid _apollorso
    (:Is%20Valid
      (return _apollorso))))

(fn GetLevelMusicPlayer
  (return (Variables|Default|GetBGMPlayerRef)))

(fn GetMissionPracticeStatus
  (return false))

(fn GetNewGameStatus
  (return false))

(fn GetReflexStatus
  (return (Variables|Default|GetIsReflexActive?)))

(fn SceneCaptureActivation
  (params (Activation :type Boolean))
  (return 0))