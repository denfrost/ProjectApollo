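; Game state that coordinates the alarm status, reflex slow motion and save-header data.
; On BeginPlay it creates the Apollo save object and spawns the Chameleon effects actor and music player.
; Alert broadcasts the alarm, switches music and starts a pausable cooldown timer, whose remaining time Tick records.
; Reflex halves global time dilation with a Chameleon effect, while static-data updates write level, keycard, slot, difficulty and play time to the save object.
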(event Custom|IncrementPlayTime
  (Variables|Default|SetCurrent%20Play%20Time (+ (Variables|Default|GetCurrent%20Play%20Time) (Math|Timespan|MakeTimespan 0 0 0 1))))

(event Custom|UpdateStaticData
  (params (RamaSaveComponent :type Rama%20Save%20Component%20Object%20Reference))
  (bind _returnvalue (Game|GetGameInstance))
  (bind _returnvalue_2 (CallFunction|GetCurrentSaveSlotName))
  (bind _returnvalue_3 (Game|Player|GetPlayerPawn 0))
  (bind _apollorso (Variables|Default|GetApolloRSO))
  (bind _current_play_time (Variables|Default|GetCurrent%20Play%20Time))
  (bind _returnvalue_4 (Actor|GetComponentbyClass _returnvalue_3 "/Game/CheekyFPS/Blueprints/Components/InventoryComponent.InventoryComponent_C"))
  (bind _currentkeycard (Variables|/Game/CheekyFPS/Blueprints/Components/InventoryComponent.InventoryComponent_C|GetCurrentKeyCard _returnvalue_4))
  (Utilities|IsValid _apollorso
    (:Is%20Valid
      (bind _returnvalue_5 (Game|GetCurrentLevelName true))
      (Utilities|IsValid _currentkeycard
        (:Is%20Valid
          (bind _returnvalue_6 (Class|BPISaveLoad|GetCurrentGameDifficulty(Message) _returnvalue))
          (Default|UpdateData _apollorso _returnvalue_5 (Variables|/Game/CheekyFPS/Blueprints/Interaction/Items/BP_ItemBase.BP_ItemBase_C|GetItemLevel _currentkeycard) _returnvalue_2 _returnvalue_6 _current_play_time))
        (:Is%20Not%20Valid
          (bind _returnvalue_7 (Class|BPISaveLoad|GetCurrentGameDifficulty(Message) _returnvalue))
          (Default|UpdateData _apollorso _returnvalue_5 0 _returnvalue_2 _returnvalue_7 _current_play_time))))))

(event Custom|SetStatusToCalm
  (CallFunction|StartCalmStatus))

(event EventBeginPlay
  (bind _returnvalue (Game|ConstructObjectfromClass "/Game/CheekyFPS/Blueprints/Game/BP_Apollo_SaveObject.BP_Apollo_SaveObject_C" self))
  (Variables|Default|SetApolloRSO _returnvalue)
  (Utilities|FlowControl|Sequence
    (:then_0
      (if (not (Utilities|IsValid (Variables|Default|GetChamReference)))
        (bind _returnvalue_2 (Game|SpawnActorfromClass "/Game/CheekyFPS/Chameleon/ISS_Chameleon.ISS_Chameleon_C" (Math|Transform|MakeTransform "0, 0, 0") "Undefined" 0 0))
        (Variables|Default|SetChamReference _returnvalue_2)))
    (:then_1
      (bind _returnvalue_3 (Game|SpawnActorfromClass "/Game/CheekyFPS/Blueprints/Game/BP_MusicPlayer.BP_MusicPlayer_C" (Math|Transform|MakeTransform "0, 0, 0") "Undefined" 0 0))
      (Variables|Default|SetBGMPlayerRef _returnvalue_3))))

(event EventSecurityAlarmInterface
  (params (SendAlarm :type Boolean) (NewAlertStatus :type EAlertStatus%20Enum :default "NewEnumerator0"))
  (bind _bgmplayerref (Variables|Default|GetBGMPlayerRef))
  (Variables|/Game/CheekyFPS/Blueprints/Game/BP_MusicPlayer.BP_MusicPlayer_C|SetCurrentAlertStatus _bgmplayerref NewAlertStatus)
  (if SendAlarm
    (Default|PlayStatusMusic _bgmplayerref "NewEnumerator2")
    (else
      (Default|PlayStatusMusic _bgmplayerref "NewEnumerator0"))))

(event EventToggleSonarEffect?
  (params (bActivateEffect? :type Boolean))
  (Default|ToggleSonarEffect (Variables|Default|GetChamReference) bActivateEffect?))

(event EventTick
  (params (DeltaSeconds :type Float%20%28single-precision%29))
  (bind _alertstatusresettimer (Variables|Default|GetAlertStatusResetTimer))
  (Utilities|FlowControl|Sequence
    (:then_0
      (Utilities|IsValid (Variables|Default|GetApolloRSO)
        (:Is%20Not%20Valid
          (bind _returnvalue (Game|ConstructObjectfromClass "/Game/CheekyFPS/Blueprints/Game/BP_Apollo_SaveObject.BP_Apollo_SaveObject_C" self))
          (Variables|Default|SetApolloRSO _returnvalue))))
    (:then_1
      (if (and (Utilities|Time|IsTimerActivebyHandle _alertstatusresettimer) (not (Class|KismetSystemLibrary|IsTimerPausedHandle _alertstatusresettimer)))
        (Variables|Default|SetAlertStatusRemainingTime (Utilities|Time|GetTimerRemainingTimebyHandle _alertstatusresettimer))))))

(event EventSaveStaticObjectData
  (params (NewFilePath :type String) (RamaSaveComponent :type Rama%20Save%20Component%20Object%20Reference)))

(event EventPlayReflex
  (CallFunction|PlayReflexEffect))

(event EventUnpauseAlarmTimer
  (bind _alertstatusresettimer (Variables|Default|GetAlertStatusResetTimer))
  (if (Class|KismetSystemLibrary|IsTimerPausedHandle _alertstatusresettimer)
    (Utilities|Time|UnpauseTimerbyHandle _alertstatusresettimer)))

(event EventPauseAlarmTimer
  (bind _alertstatusresettimer (Variables|Default|GetAlertStatusResetTimer))
  (if (Utilities|Time|IsTimerActivebyHandle _alertstatusresettimer)
    (Utilities|Time|PauseTimerbyHandle _alertstatusresettimer)
    (Variables|Default|SetAlertStatusRemainingTime 99.0)))

(event EventStopReflexFX
  (params (bTriggerAlarm? :type Boolean))
  (if bTriggerAlarm?
    (CallFunction|EndReflexEffect)
    (Variables|Default|SetCurrentAlertStatus "NewEnumerator2")
    (else
      (CallFunction|EndReflexEffect)))
  (CallFunction|UpdateAlertStatus))

(fn ConstructionScript)

(fn PlayReflexEffect
  (Utilities|Time|SetGlobalTimeDilation 0.5)
  (Default|ToggleReflexEffect (Variables|Default|GetChamReference) true)
  (CallFunction|ResetReflexEffect))

(fn ResetReflexEffect
  (Utilities|Time|SetTimerbyEvent (EventDispatchers|CreateEvent :!event EndReflexEffect) 5.0))

(fn EndReflexEffect
  (Utilities|Time|SetGlobalTimeDilation 1.0)
  (Default|ToggleReflexEffect (Variables|Default|GetChamReference) false))

(fn StartAlertStatus
  (Default|CallOnAlarmActivate)
  (bind _output_get (Variables|Default|SetCurrentAlertStatus "NewEnumerator2"))
  (Default|PlayStatusMusic (Variables|Default|GetBGMPlayerRef) _output_get))

(fn UpdateAlertStatus
  (switch Utilities|FlowControl|Switch|SwitchonEAlertStatus (Variables|Default|GetCurrentAlertStatus)
    (:NewEnumerator2
      (CallFunction|StartAlertStatus)
      (CallFunction|SetAlertCooldownTimer))))

(fn StartCalmStatus
  (Default|CallOnAlarmDeactivate)
  (bind _output_get (Variables|Default|SetCurrentAlertStatus "NewEnumerator0"))
  (Default|PlayStatusMusic (Variables|Default|GetBGMPlayerRef) _output_get))

(fn SetAlertCooldownTimer
  (bind _returnvalue (Utilities|Time|SetTimerbyEvent (EventDispatchers|CreateEvent :!event Custom|SetStatusToCalm) 99.0))
  (Variables|Default|SetAlertStatusResetTimer _returnvalue))

(fn GetRemainingAlertTime
  (return (Variables|Default|GetAlertStatusRemainingTime)))

(fn GetAlertStatusTimeLeft
  (return (CallFunction|GetRemainingAlertTime)))

(fn GetCurrentGameDifficulty
  (return "Beginner"))

(fn GetCurrentStaticSaveHeader
  (bind _apollorso (Variables|Default|GetApolloRSO))
  (Utilities|IsValid _apollorso
    (:Is%20Valid
      (return _apollorso))))

(fn GetNewGameStatus
  (return false))

(fn SceneCaptureActivation
  (params (Activation :type Boolean))
  (return 0))