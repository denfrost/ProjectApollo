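; Gameplay game state that restores saved game data through the Rama Save System when play begins.
; On BeginPlay, it checks for a file at the save slot location, loads it and prints a debug message on success.
; Disconnected, unused logic remains for spawning the player's starting inventory when empty and for loading only Pickup and Player tagged actors.
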(event EventBeginPlay
  (bind _returnvalue (CallFunction|GetSaveSlotLocation))
  (|CallParentFunction)
  (Utilities|FlowControl|Sequence
    (:then_0
      (if (Class|RamaSaveLibrary|RamaSaveFileExists _returnvalue)
        (bind _fileiosuccess (Class|RamaSaveLibrary|RamaSaveLoadfromFile _returnvalue true false true))
        (if _fileiosuccess
          (Development|PrintString "Loaded!"))))))

(fn ConstructionScript
  (|CallParentFunction))