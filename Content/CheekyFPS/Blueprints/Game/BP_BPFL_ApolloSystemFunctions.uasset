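; Blueprint function library of shared helpers for The Apollo Project, covering saves, level loading, input icons and ray tracing.
; Save helpers read and write slot names, full .sav paths and manual or mission slot lists on ApolloGameInstance, with slot screenshots captured by HighResShot.
; Icon lookups use player controller 0's gamepad and keyboard/mouse data, while ray tracing toggles run console commands.
; LoadNewLevel clears any new-game flag before opening the level.
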(fn GetSaveLocation
  (return (Class|VictoryBPFunctionLibrary|AppendMultiple (Class|RamaSaveLibrary|GetDocumentsFolder) "My Games/The Apollo Project/")))

(fn BPGetCurrentSaveSlotFilePath
  (return (Class|ApolloGameInstance|GetCurrentSaveSlotFilePath (.AsApollo%20Game%20Instance (Utilities|Casting|CastToApolloGameInstance (Game|GetGameInstance))))))

(fn GetCurrentSaveSlotName
  (bind _returnvalue (Game|GetGameInstance))
  (bind _asapollo_game_instance (Utilities|Casting|CastToApolloGameInstance _returnvalue))
  (bind _returnvalue_2 (Class|ApolloGameInstance|GetCurrentSaveSlot _asapollo_game_instance))
  (if (Utilities|Enum|NotEqual(Enum) _returnvalue_2 "")
    (return _returnvalue_2)
    (else
      (Development|PrintString 0 (Class|VictoryBPFunctionLibrary|AppendMultiple "No valid Save name!" " " "Defaulting to SaveSlotA") true true "(R=1.000000,G=0.081818,B=0.000000,A=1.000000)" 5.0)
      (return (I/O|UpdateSaveSlotNametoFilePath "SaveSlotA")))))

(fn GetValidManualSaveSlots
  (return (Class|ApolloGameInstance|GetCurrentManualSaveSlots (.AsApollo%20Game%20Instance (Utilities|Casting|CastToApolloGameInstance (Game|GetGameInstance))))))

(fn CaptureSaveSlotScreenshot
  (params (SpecificPlayer :type Player%20Controller%20Object%20Reference) (WorldContextObject :type Object%20Object%20Reference))
  (bind _returnvalue (Class|ApolloBlueprintFunctionLibrary|GetGameResolution))
  (bind _returnvalue_2 (Class|KismetMathLibrary|ToIntPoint(Vector2D) _returnvalue))
  (bind (_x _y) (Utilities|Struct|BreakIntPoint _returnvalue_2))
  (Development|ExecuteConsoleCommand WorldContextObject (Utilities|String|Append "HighResShot " (Utilities|String|Append (Utilities|String|ToString(Integer) _x) "x" (Utilities|String|ToString(Integer) _y)) " filename=\"" (Utilities|String|Append (Screenshot|GetScreenShotsLocation) (I/O|GetCurrentSaveSlotName)) "\"") SpecificPlayer))

(fn GetScreenshot
  (params (FullFilePath :type String) (WorldContextObject :type Object%20Object%20Reference))
  (bind _returnvalue (Class|KismetRenderingLibrary|ImportFileasTexture2D WorldContextObject FullFilePath))
  (return (Utilities|IsValid _returnvalue) _returnvalue (Class|BlueprintPathsLibrary|GetBaseFilename FullFilePath true) FullFilePath))

(fn GetSaveSlotName
  (params (FilePathName :type String))
  (return (.LeftS (Utilities|String|Split (.RightS (Utilities|String|Split FilePathName "The Apollo Project/")) ".sav"))))

(fn GetScreenShotsLocation
  (return (Utilities|String|Append (Class|VictoryBPFunctionLibrary|VictoryPathsSavedDir) "Screenshots/")))

(fn DoSavesExist?
  (for _array_element (I/O|GetValidManualSaveSlots)
    (return (Class|RamaSaveLibrary|RamaSaveFileExists _array_element))))

(fn UpdateSaveSlotNametoFilePath
  (params (SaveSlotName :type String))
  (bind _returnvalue (Game|GetGameInstance))
  (bind _returnvalue_2 (I/O|GetSaveLocation))
  (bind _returnvalue_3 (Utilities|String|Append _returnvalue_2 SaveSlotName))
  (bind _asapollo_game_instance (Utilities|Casting|CastToApolloGameInstance _returnvalue))
  (bind _returnvalue_4 (Utilities|String|Append _returnvalue_3 ".sav"))
  (if (Utilities|Enum|NotEqual(Enum) SaveSlotName "")
    (if (Utilities|String|Contains SaveSlotName _returnvalue_2)
      (Class|ApolloGameInstance|SetCurrentSaveSlotFilePath _asapollo_game_instance SaveSlotName)
      (return SaveSlotName)
      (elif (Utilities|String|Contains _returnvalue_3 ".sav")
        (Class|ApolloGameInstance|SetCurrentSaveSlotFilePath _asapollo_game_instance _returnvalue_3)
        (return _returnvalue_3)
        (else
          (Class|ApolloGameInstance|SetCurrentSaveSlotFilePath _asapollo_game_instance _returnvalue_4)
          (return _returnvalue_4))))
    (else
      (Class|ApolloGameInstance|SetCurrentSaveSlotFilePath _asapollo_game_instance)
      (return ""))))

(fn GetManualSaveSlots
  (return (Variables|/Script/ApolloGame.ApolloGameInstance|GetManualSaveSlotsList (.AsApollo%20Game%20Instance (Utilities|Casting|CastToApolloGameInstance (Game|GetGameInstance))))))

(fn LoadNewLevel
  (params (NewLevelName :type Name))
  (bind _returnvalue (Game|GetGameInstance))
  (bind _bstartnewgame_ (Class|BPISaveLoad|GetNewGameStatus(Message) _returnvalue))
  (if _bstartnewgame_
    (Class|BPISaveLoad|IsStartingNewGame?(Message) _returnvalue false "Beginner"))
  (Game|OpenLevel(byName) 0 NewLevelName))

(fn UpdateCurrentSaveSlotName
  (params (NewSaveSlot :type String))
  (Class|ApolloGameInstance|SetCurrentSaveSlot (.AsApollo%20Game%20Instance (Utilities|Casting|CastToApolloGameInstance (Game|GetGameInstance))) NewSaveSlot))

(fn GetActionIcon(byKey)
  (params (InputAction :type Key%20Structure :default "None") (bIsGamepad :type Boolean))
  (bind _returnvalue (Game|GetPlayerController 0))
  (bind _asapollo_player_controller_base (Utilities|Casting|CastToBP_Apollo_PlayerController_Base _returnvalue))
  (return (Class|ApolloPlayerSettingsLibrary|GetIconforActionbyKey InputAction (Variables|/Script/ApolloGame.ISSPlayerController|GetCurrentGamepadIconData _asapollo_player_controller_base) (Variables|/Script/ApolloGame.ISSPlayerController|GetKBMIconData _asapollo_player_controller_base) bIsGamepad)))

(fn GetActionIcon(byName)
  (params (InputActionName :type Name) (bIsGamepad :type Boolean))
  (bind _returnvalue (Game|GetPlayerController 0))
  (bind _returnvalue_2 (Class|BPIPlayer|GetGamepadIconDataTable(Message) _returnvalue))
  (bind _returnvalue_3 (Class|BPIPlayer|GetKBMIconDataTable(Message) _returnvalue))
  (return (Class|ApolloPlayerSettingsLibrary|GetIconforActionbyName InputActionName _returnvalue_2 _returnvalue_3 bIsGamepad)))

(fn IsPlayerUsingGamepad?
  (return (Variables|/Game/CheekyFPS/Blueprints/Player/BP_Apollo_PlayerController_Base.BP_Apollo_PlayerController_Base_C|GetIsUsingGamepad? (.AsApollo%20Player%20Controller%20Base (Utilities|Casting|CastToBP_Apollo_PlayerController_Base (Game|GetPlayerController 0))))))

(fn ToggleGlobalRayTracingEffects
  (params (EnableEffects? :type Boolean))
  (if EnableEffects?
    (Development|ExecuteConsoleCommand 0 "r.RayTracing.GlobalIllumination 1" 0)
    (Development|ExecuteConsoleCommand 0 "r.RayTracing.AmbientOcclusion 1" 0)
    (Development|ExecuteConsoleCommand 0 "r.RayTracing.Reflections 1" 0)
    (Development|ExecuteConsoleCommand 0 "r.RayTracing.Shadows 1" 0)
    (Development|ExecuteConsoleCommand 0 "r.RayTracing.Translucency 1" 0)
    (else
      (Development|ExecuteConsoleCommand 0 "r.RayTracing.GlobalIllumination 0" 0)
      (Development|ExecuteConsoleCommand 0 "r.RayTracing.AmbientOcclusion 0" 0)
      (Development|ExecuteConsoleCommand 0 "r.RayTracing.Reflections 0" 0)
      (Development|ExecuteConsoleCommand 0 "r.RayTracing.Shadows 0" 0)
      (Development|ExecuteConsoleCommand 0 "r.RayTracing.Translucency 0" 0))))

(fn EnableRTGlobalIllumination
  (params (EnableEffect? :type Boolean))
  (if EnableEffect?
    (Development|ExecuteConsoleCommand 0 "r.RayTracing.GlobalIllumination 1" 0)
    (else
      (Development|ExecuteConsoleCommand 0 "r.RayTracing.GlobalIllumination 0" 0))))

(fn EnableRTAO
  (params (EnableEffect? :type Boolean))
  (if EnableEffect?
    (Development|ExecuteConsoleCommand 0 "r.RayTracing.AmbientOcclusion 1" 0)
    (else
      (Development|ExecuteConsoleCommand 0 "r.RayTracing.AmbientOcclusion 0" 0))))

(fn EnableRTReflections
  (params (EnableEffect? :type Boolean))
  (if EnableEffect?
    (Development|ExecuteConsoleCommand 0 "r.RayTracing.Reflections 1" 0)
    (else
      (Development|ExecuteConsoleCommand 0 "r.RayTracing.Reflections 0" 0))))

(fn EnableRTShadows
  (params (EnableEffect? :type Boolean))
  (if EnableEffect?
    (Development|ExecuteConsoleCommand 0 "r.RayTracing.Shadows 1" 0)
    (else
      (Development|ExecuteConsoleCommand 0 "r.RayTracing.Shadows 0" 0))))

(fn EnableRTTranslucency
  (params (EnableEffect? :type Boolean))
  (if EnableEffect?
    (Development|ExecuteConsoleCommand 0 "r.RayTracing.Translucency 1" 0)
    (else
      (Development|ExecuteConsoleCommand 0 "r.RayTracing.Translucency 0" 0))))

(fn GetMainMenuName
  (return "ApolloMainMenu"))

(fn GetMissionSaveSlots
  (return (Variables|/Script/ApolloGame.ApolloGameInstance|GetMissionSaveSlotsList (.AsApollo%20Game%20Instance (Utilities|Casting|CastToApolloGameInstance (Game|GetGameInstance))))))

(fn GetValidMissionSaveSlots
  (return (Variables|/Script/ApolloGame.ApolloGameInstance|GetCurrentMissionSaveSlotsList (.AsApollo%20Game%20Instance (Utilities|Casting|CastToApolloGameInstance (Game|GetGameInstance))))))