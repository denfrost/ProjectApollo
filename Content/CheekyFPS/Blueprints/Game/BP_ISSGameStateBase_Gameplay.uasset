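; Gameplay game state base that starts play-time timers and triggers player data loading when play begins.
; The game mode's game type selects either a one-second looping play-time timer or, outside mission practice, a millisecond-interval mission timer.
; Unless the game instance reports a new game, it loads player data from the current save slot.
; EndPlay clears only the general play-time timer handle.
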(event EventBeginPlay
  (bind _returnvalue (Game|GetGameInstance))
  (|CallParentFunction)
  (Utilities|FlowControl|Sequence
    (:then_0
      (bind _returnvalue_2 (Class|BPIGameEvents|GetCurrentGameType(Message) (Game|GetGameMode)))
      (if (Utilities|Enum|Equal(Enum) _returnvalue_2 "NewEnumerator1")
        (bind _returnvalue_3 (Utilities|Time|SetTimerbyEvent (EventDispatchers|CreateEvent :!event IncrementPlayTime) 1.0 true))
        (Variables|Default|SetPlayTimeIncrementHandle _returnvalue_3)
        (else
          (bind _returnvalue_4 (Class|BPIGameEvents|GetMissionPracticeStatus(Message) (Game|GetGameMode)))
          (if (not _returnvalue_4)
            (bind _returnvalue_5 (Utilities|Time|SetTimerbyEvent (EventDispatchers|CreateEvent :!event IncrementMissionPlayTime) 0.001 true))
            (Variables|Default|SetMissionPlayTimeIncrementHandle _returnvalue_5)))))
    (:then_1
      (bind _bstartnewgame_ (Class|BPISaveLoad|GetNewGameStatus(Message) _returnvalue))
      (if (not _bstartnewgame_)
        (Class|BPISaveLoad|LoadPlayerData(Message) _returnvalue (CallFunction|GetCurrentSaveSlotFilePath))))))

(event EventEndPlay
  (params (EndPlayReason :type EEndPlayReason%20Enum :default "Destroyed"))
  (Utilities|Time|ClearandInvalidateTimerbyHandle (Variables|Default|GetPlayTimeIncrementHandle))
  (|CallParentFunction EndPlayReason))

(fn ConstructionScript
  (|CallParentFunction))