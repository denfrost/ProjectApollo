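; BP_MusicPlayer is an actor that switches background music between a stealth cue and an alarm cue according to alert status.
; PlayStatusMusic routes Calm to StartCalmMusic, and both Alert and Warning to StartAlertMusic.
; Each starter rechecks CurrentAlertStatus, which the alarm one requires to equal Alert, and restarts the Audio component only when its cue differs.
; Events are empty, so playback depends on external calls.
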(event EventBeginPlay)

(event Collision|EventActorBeginOverlap
  (params (OtherActor :type Actor%20Object%20Reference)))

(event EventTick
  (params (DeltaSeconds :type Float%20%28single-precision%29)))

(fn ConstructionScript)

(fn StartAlertMusic
  (bind _audio (Variables|Default|GetAudio))
  (if (Utilities|Enum|Equal(Enum) (Variables|Default|GetCurrentAlertStatus) "NewEnumerator2")
    (if (!= (Variables|/Script/Engine.AudioComponent|GetSound _audio) "/Game/CheekyFPS/External/Assets/Audio/Blueprint_Music_Alarm02_Cue.Blueprint_Music_Alarm02_Cue")
      (Audio|Components|Audio|SetSound _audio "/Game/CheekyFPS/External/Assets/Audio/Blueprint_Music_Alarm02_Cue.Blueprint_Music_Alarm02_Cue")
      (Audio|Components|Audio|Play _audio 0.0))))

(fn StartCalmMusic
  (bind _audio (Variables|Default|GetAudio))
  (if (Utilities|Enum|Equal(Enum) (Variables|Default|GetCurrentAlertStatus) "NewEnumerator0")
    (if (!= (Variables|/Script/Engine.AudioComponent|GetSound _audio) "/Game/CheekyFPS/External/Assets/Audio/Blueprint_Music_Stealth01_Cue.Blueprint_Music_Stealth01_Cue")
      (Audio|Components|Audio|SetSound _audio "/Game/CheekyFPS/External/Assets/Audio/Blueprint_Music_Stealth01_Cue.Blueprint_Music_Stealth01_Cue")
      (Audio|Components|Audio|Play _audio 0.0))))

(fn PlayStatusMusic
  (params (CurrentAlertStatus :type EAlertStatus%20Enum :default "NewEnumerator0"))
  (switch Utilities|FlowControl|Switch|SwitchonEAlertStatus CurrentAlertStatus
    (:NewEnumerator0
      (CallFunction|StartCalmMusic))
    (:NewEnumerator2
      (CallFunction|StartAlertMusic :!label _label))
    (:NewEnumerator3
      (goto _label))))