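; BP_CamModifier_Pain is a camera modifier that gives a pain effect on screen and in the view.
; Its post process pass applies a red scene tint, a strong vignette and a blur material, weighted by the modifier's Alpha.
; Its camera pass narrows the FOV slightly in proportion to the same Alpha, leaving location and rotation untouched.
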(fn BlueprintModifyPostProcess
  (params (DeltaTime :type Float%20%28single-precision%29))
  (return (Variables|CameraModifier|GetAlpha) (Utilities|Struct|MakePostProcessSettings "(R=1.000000,G=0.000000,B=0.031044,A=1.000000)" 1.0 0.8 (Utilities|Struct|MakeWeightedBlendables (Utilities|Array|MakeArray (Utilities|Struct|MakeWeightedBlendable 1.0 "/Game/CheekyFPS/Materials/PostProcess/PP_Blur.PP_Blur"))))))

(fn BlueprintModifyCamera
  (params (DeltaTime :type Float%20%28single-precision%29) (ViewLocation :type Vector :default "0, 0, 0") (ViewRotation :type Rotator :default "0, 0, 0") (FOV :type Float%20%28single-precision%29))
  (return ViewLocation ViewRotation (- FOV (* 5.0 (Variables|CameraModifier|GetAlpha)))))