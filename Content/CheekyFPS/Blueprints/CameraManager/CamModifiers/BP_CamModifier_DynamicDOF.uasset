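; Camera modifier that drives dynamic depth of field, keeping focus on whatever lies at the center of the view.
; BlueprintModifyCamera caches the view location and rotation, passing the camera through unchanged.
; BlueprintModifyPostProcess line-traces forward from that view, ignoring the player character, and smoothly interpolates focal distance toward the hit, or a far default on a miss.
; The override uses an enlarged sensor width to exaggerate blur, blended by the modifier's alpha.
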(fn BlueprintModifyPostProcess
  (params (DeltaTime :type Float%20%28single-precision%29))
  (bind _viewlocation (Variables|Default|GetViewLocation))
  (bind (_outhit _returnvalue) (Collision|LineTraceByChannel _viewlocation (+ _viewlocation (* (Math|Vector|GetForwardVector (Variables|Default|GetViewRotation)) 5e+03)) "TraceTypeQuery1" true (Utilities|Array|MakeArray (Game|GetPlayerCharacter 0)) "None"))
  (Utilities|FlowControl|Sequence
    (:then_1
      (Variables|Default|SetFocalDistance (Math|Interpolation|FInterpTo (Variables|Default|GetFocalDistance) (select _returnvalue (.Distance (Collision|BreakHitResult _outhit)) 5e+03) (Utilities|Time|GetWorldDeltaSeconds) 1e+01))
      (return (Variables|CameraModifier|GetAlpha) (Utilities|Struct|MakePostProcessSettings 6e+01 (Variables|Default|GetFocalDistance))))))

(fn BlueprintModifyCamera
  (params (DeltaTime :type Float%20%28single-precision%29) (ViewLocation :type Vector :default "0, 0, 0") (ViewRotation :type Rotator :default "0, 0, 0") (FOV :type Float%20%28single-precision%29))
  (Variables|Default|SetViewLocation ViewLocation)
  (Variables|Default|SetViewRotation ViewRotation)
  (return ViewLocation ViewRotation FOV))