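; BP_CamModifier_QuakeRoll is a camera modifier that adds a Quake-style view roll as the player strafes.
; It projects the character's last movement input onto the actor's right vector to set a target roll, scaled by a maximum angle.
; Roll moves toward that target at a constant rate, faster during input than when returning to level.
; The result, weighted by the modifier's Alpha, is added to view roll, leaving location and FOV untouched.
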(fn BlueprintModifyCamera
  (params (DeltaTime :type Float%20%28single-precision%29) (ViewLocation :type Vector :default "0, 0, 0") (ViewRotation :type Rotator :default "0, 0, 0") (FOV :type Float%20%28single-precision%29))
  (bind (_roll _pitch _yaw) (Math|Rotator|BreakRotator ViewRotation))
  ;[0 0.4238 1] Get player character
  (if (Variables|RuntimeStuff|GetbHasInitialised)
    _
    (else
      (Variables|RuntimeStuff|SetPlayerCharacter (Game|GetPlayerCharacter 0))
      (Variables|RuntimeStuff|SetbHasInitialised true)))
  ;[1 0.4502 0] Is player trying to move?
  (Variables|RuntimeStuff|SetbIsInputActive (> (Math|Vector|VectorLength (Pawn|Components|PawnMovement|GetLastInputVector (Variables|/Script/Engine.Character|GetCharacterMovement (Variables|RuntimeStuff|GetPlayerCharacter)))) 0.1))
  (Variables|RuntimeStuff|SetRollRotation (Math|Interpolation|FInterptoConstant (Variables|RuntimeStuff|GetRollRotation) (* (Math|Float|Clamp(Float) (Math|Vector|DotProduct (Math|Vector|GetRightVector (Transformation|GetActorRotation (Variables|RuntimeStuff|GetPlayerCharacter))) (Pawn|Components|PawnMovement|GetLastInputVector (Variables|/Script/Engine.Character|GetCharacterMovement (Variables|RuntimeStuff|GetPlayerCharacter)))) -1.0) (Variables|Default|GetRollAngleMax)) DeltaTime (select (Variables|RuntimeStuff|GetbIsInputActive) 8.0 3.0)))
  (return ViewLocation (Math|Rotator|MakeRotator (+ _roll (* (Variables|RuntimeStuff|GetRollRotation) (Variables|CameraModifier|GetAlpha))) _pitch _yaw) FOV))