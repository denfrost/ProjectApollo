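; Camera modifier that adds first-person headbob and jump/landing bounce to the player's view.
; Ground speed and stride length advance a looping cycle that samples position and rotation curves, faded by speed, and also drives the footstep component.
; A damped spring fed by vertical velocity changes adds landing dip and tilt.
; The combined offset is applied relative to view rotation, scaled by modifier alpha and the player's headbob setting.
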(fn BlueprintModifyCamera
  (params (DeltaTime :type Float%20%28single-precision%29) (ViewLocation :type Vector :default "0, 0, 0") (ViewRotation :type Rotator :default "0, 0, 0") (FOV :type Float%20%28single-precision%29))
  (bind _headbobrotation (Variables|Default|GetHeadbobRotation))
  (bind (_roll _pitch _yaw) (Math|Rotator|BreakRotator ViewRotation))
  ;[0 0.4238 1] Get player character
  (if (Variables|Default|GetbHasInitialised)
    _
    (else
      (bind _output_get (Variables|Default|SetPlayerCharacter (Game|GetPlayerCharacter 0)))
      (Variables|Default|SetFootstepComponent (Actor|GetComponentbyClass _output_get "/Game/CheekyFPS/Blueprints/Footsteps/BP_CheekyFootstepComponent.BP_CheekyFootstepComponent_C"))
      (Variables|Default|SetPlayerSettingsManager (Actor|GetComponentbyClass _output_get "/Game/CheekyFPS/Blueprints/BP_CheekyPlayerSettingsManager.BP_CheekyPlayerSettingsManager_C"))
      (Variables|Default|SetbHasInitialised true)))
  (CallFunction|HeadbobSpring DeltaTime)
  (return (Math|Vector|Lerp(Vector) ViewLocation (+ ViewLocation (Math|Transform|TransformLocation (Math|Transform|MakeTransform "0, 0, 0" ViewRotation) (Variables|Default|GetHeadbobLocation))) (* (Variables|CameraModifier|GetAlpha) (Variables|/Game/CheekyFPS/Blueprints/BP_CheekyPlayerSettingsManager.BP_CheekyPlayerSettingsManager_C|GetHeadbobScale (Variables|Default|GetPlayerSettingsManager)))) (Math|Rotator|Lerp(Rotator) ViewRotation (Math|Rotator|MakeRotator (+ _roll (.roll _headbobrotation)) (+ _pitch (.pitch _headbobrotation)) (+ _yaw (.yaw _headbobrotation))) (* (Variables|CameraModifier|GetAlpha) (Variables|/Game/CheekyFPS/Blueprints/BP_CheekyPlayerSettingsManager.BP_CheekyPlayerSettingsManager_C|GetHeadbobScale (Variables|Default|GetPlayerSettingsManager))) true) FOV))

(fn HeadbobSpring
  (params (DeltaTime :type Float%20%28single-precision%29))
  (Utilities|FlowControl|Sequence
    (:then_0
      ;[0.1638 1 0.1602] Velocity Update
      (LocalVariables|SetVelocity (/ (Pawn|Components|CharacterMovement|GetLastUpdateVelocity (Variables|/Script/Engine.Character|GetCharacterMovement (Variables|Default|GetPlayerCharacter))) 1e+02))
      (LocalVariables|SetVelocityChange (- (LocalVariables|GetVelocity) (Variables|HeadbobSpring|Runtime|GetPrevVeloc)))
      (Variables|HeadbobSpring|Runtime|SetPrevVeloc (LocalVariables|GetVelocity)) ; GLOBAL Var
    )
    (:then_1
      ;[1 0.2552 0.1955] Springy-ma-jig For Jumping / Landing
      (Variables|HeadbobSpring|Runtime|SetSpringVelocity (* (- (- (Variables|HeadbobSpring|Runtime|GetSpringVelocity) (.z (LocalVariables|GetVelocityChange))) (* (Variables|HeadbobSpring|Runtime|GetSpringPosition) (Variables|HeadbobSpring|GetSpringElasticity))) (Variables|HeadbobSpring|GetSpringDampening)))
      (Variables|HeadbobSpring|Runtime|SetSpringPosition (Math|Float|Clamp(Float) (+ (Variables|HeadbobSpring|Runtime|GetSpringPosition) (* (Variables|HeadbobSpring|Runtime|GetSpringVelocity) DeltaTime)) -0.32 0.32))
      ;[0.2804 0.7348 1] Set Spring Position / Pitch
      (LocalVariables|SetSpringPosZ (* (Variables|HeadbobSpring|Runtime|GetSpringPosition) (Variables|HeadbobSpring|GetLandingMovement)))
      (LocalVariables|SetSpringPitch (* (Variables|HeadbobSpring|Runtime|GetSpringPosition) (Variables|HeadbobSpring|GetLandingTilt))))
    (:then_2
      ;[1 0 0.6197] Ground Velocity
      (LocalVariables|SetGroundVelocity (select (AI|Components|NavMovement|IsMovingonGround (Variables|/Script/Engine.Character|GetCharacterMovement (Variables|Default|GetPlayerCharacter))) (Math|Vector|VectorLength (LocalVariables|GetVelocity)) 0.0))
      ;[0.1808 0.4349 1] Stride Length (Affects Headbob Cycle speed)
      (LocalVariables|SetStrideLengthen (+ 1.0 (* (LocalVariables|GetGroundVelocity) (Variables|HeadbobSpring|GetStrideLengthFactor))))
      ;[1 0.3647 0] Increment Headbob Cycle
      (Variables|HeadbobSpring|Runtime|SetHeadBobCycle (select (>= (+ (Variables|HeadbobSpring|Runtime|GetHeadBobCycle) (* (/ (LocalVariables|GetGroundVelocity) (LocalVariables|GetStrideLengthen)) (/ DeltaTime 2.0))) 2.0) 0.0 (+ (Variables|HeadbobSpring|Runtime|GetHeadBobCycle) (* (/ (LocalVariables|GetGroundVelocity) (LocalVariables|GetStrideLengthen)) (/ DeltaTime 2.0)))))
      ;[0 1 0.6315] Headbob Fade
      (bind _output_get (Variables|HeadbobSpring|Runtime|SetHeadBobFade (Math|Interpolation|FInterptoConstant (Variables|HeadbobSpring|Runtime|GetHeadBobFade) (Math|Float|Clamp(Float) (/ (* (LocalVariables|GetGroundVelocity) 1.4e+02) (Variables|/Script/Engine.CharacterMovementComponent|GetMaxWalkSpeed (Variables|/Script/Engine.Character|GetCharacterMovement (Variables|Default|GetPlayerCharacter))))) DeltaTime (Variables|HeadbobSpring|GetHeadbobFadeSpeed))))
      ;;[1 0 0.7367 1 15] This used to reset the headbob cylce when the player stops moving, but it seems unnecessary - you can add it back in if required.
      (if (== _output_get 0.0)
        (Variables|HeadbobSpring|Runtime|SetHeadBobCycle 0.0))
      (Default|FootstepCycle (Variables|Default|GetFootstepComponent) (Variables|HeadbobSpring|Runtime|GetHeadBobCycle)))
    (:then_3
      ;[0.9309 0 1] Headbob Animation
      (LocalVariables|SetHeadbobPos (* (Math|Curves|GetVectorValue (Variables|Default|GetHeadbobCurvePosition) (Variables|HeadbobSpring|Runtime|GetHeadBobCycle)) (Variables|HeadbobSpring|Runtime|GetHeadBobFade)))
      (LocalVariables|SetHeadbobRot (* (Math|Curves|GetVectorValue (Variables|Default|GetHeadbobCurveRotation) (Variables|HeadbobSpring|Runtime|GetHeadBobCycle)) (Variables|HeadbobSpring|Runtime|GetHeadBobFade))))
    (:then_4
      ;[1 0.1442 0.5944] Final Headbob Position (Used in BlueprintModifyCamera)
      (Variables|Default|SetHeadbobLocation (Math|Vector|MakeVector (.X (Math|Vector|BreakVector (LocalVariables|GetHeadbobPos))) (.Y (Math|Vector|BreakVector (LocalVariables|GetHeadbobPos))) (+ (.Z (Math|Vector|BreakVector (LocalVariables|GetHeadbobPos))) (LocalVariables|GetSpringPosZ))))
      ;[1 0.3315 0] Final Headbob Rotation (Used in BlueprintModifyCamera)
      (Variables|Default|SetHeadbobRotation (Math|Rotator|MakeRotator (.X (Math|Vector|BreakVector (LocalVariables|GetHeadbobRot))) (+ (.Y (Math|Vector|BreakVector (LocalVariables|GetHeadbobRot))) (LocalVariables|GetSpringPitch)) (.Z (Math|Vector|BreakVector (LocalVariables|GetHeadbobRot)))))
      (return))))