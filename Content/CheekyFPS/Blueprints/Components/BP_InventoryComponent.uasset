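; Inventory component that stores the player's item actors and tracks the current key card, plus a grenade inventory.
; SpawnItem creates hidden actors from classes, adds them to the inventory and records the class, uniquely for stackables.
; Adding a KeyCard-tagged item rescans for the key, and removing the last of a class notifies the player controller.
; Grenades live in a map looked up by key or index, alongside a current selection index.
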(event EventBeginPlay
  (CallFunction|GetKeyCard))

(fn AddItem
  (params (NewItem :type BP%20Item%20Base%20Object%20Reference%20%28by%20ref%29))
  (bind _iteminventory (Variables|Default|GetItemInventory))
  (Utilities|IsValid NewItem
    (:Is%20Valid
      (bind _returnvalue (Utilities|Array|Add _iteminventory NewItem))
      (Utilities|IsValid (Utilities|Array|Get(acopy) _iteminventory _returnvalue)
        (:Is%20Valid
          (Utilities|FlowControl|Sequence
            (:then_0
              (Development|PrintString "Successfully added item!"))
            (:then_1
              (if (Actor|ActorHasTag NewItem "KeyCard")
                (CallFunction|GetKeyCard)))))
        (:Is%20Not%20Valid
          (Development|PrintString "Unable to add item!"))))))

(fn RemoveItem
  (params (Item :type BP%20Item%20Base%20Object%20Reference%20%28by%20ref%29))
  (bind _returnvalue (Utilities|Array|RemoveItem (Variables|Default|GetItemInventory) Item))
  (if _returnvalue
    (Development|PrintString "Successfully removed item!")
    (if (<= (CallFunction|GetNumOfIteminArray (Utilities|GetClass Item)) 0)
      (Class|BPIPlayer|OnItemConsumed(Message) (Game|GetPlayerController 0)))
    (else
      (Development|PrintString "Unable to remove item!"))))

(fn GetKeyCard
  (for _array_element (Variables|Default|GetItemInventory)
    (if (.bSuccess (Utilities|Casting|CastToBP_KeyItem _array_element))
      (Utilities|IsValid (.AsBP%20Key%20Item (Utilities|Casting|CastToBP_KeyItem _array_element))
        (:Is%20Valid
          (bind _output_get (Variables|Default|SetCurrentKeyCard (.AsBP%20Key%20Item (Utilities|Casting|CastToBP_KeyItem _array_element))))
          (if (Utilities|IsValid _output_get)
            (Development|PrintString "Found key card!")
            (else
              (Development|PrintString "Could not find key card!")))
          (return))))))

(fn SpawnItem
  (params (NewItem :type BP%20Item%20Base%20Class%20Reference))
  (bind _spawniteminventory (Variables|Default|GetSpawnItemInventory))
  (bind _returnvalue (Game|SpawnActorfromClass NewItem (Math|Transform|MakeTransform "0, 0, 0") "AlwaysSpawn" 0 0))
  (Rendering|SetActorHiddenInGame _returnvalue true)
  (CallFunction|AddItem _returnvalue)
  (if (Variables|/Game/CheekyFPS/Blueprints/Interaction/Items/BP_ItemBase.BP_ItemBase_C|GetbIsStackable? _returnvalue)
    (Utilities|Array|AddUnique _spawniteminventory NewItem)
    (return)
    (else
      (Utilities|Array|Add _spawniteminventory NewItem)
      (return))))

(fn GetNumOfIteminArray
  (params (FilterClass :type Actor%20Class%20Reference))
  (bind _filteredarray (Utilities|Array|FilterArray (Variables|Default|GetItemInventory) FilterClass))
  (return (Utilities|Array|Length _filteredarray)))

(fn FindGrenade(ByMapKey)
  (params (InName :type String%20%28by%20ref%29))
  (bind _grenadeinventory (Variables|Default|GetGrenadeInventory))
  (bind (_value _returnvalue) (Utilities|Map|Find _grenadeinventory InName))
  (if _returnvalue
    (return _value)))

(fn GetGrenadeInventory
  (return (Variables|Default|GetGrenadeInventory)))

(fn FindGrenade(ByIndex)
  (params (NewIndex :type Integer))
  (bind _values (Utilities|Map|Values (Variables|Default|GetGrenadeInventory)))
  (return (.IsUnlocked? (Utilities|Struct|BreakGrenadeInventoryStruct (Utilities|Array|Get(acopy) _values NewIndex))) (.GrenadeCooldownLength (Utilities|Struct|BreakGrenadeInventoryStruct (Utilities|Array|Get(acopy) _values NewIndex)))))

(fn SetCurrentGrenadeIndex
  (params (NewIndex :type Integer))
  (Variables|Default|SetCurrentGrenadeIndex NewIndex))

(fn GetCurrentGrenadeIndex
  (return (Variables|Default|GetCurrentGrenadeIndex)))