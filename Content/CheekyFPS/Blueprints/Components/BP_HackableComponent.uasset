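; BP_HackableComponent lets the player take control of its owning pawn after a successful drone hack.
; At BeginPlay it caches the owner and its AI controller, then on hack success flags player control, blends the view and has the player controller possess the pawn.
; ReturntoPlayer blends back to the character stored in BP_ISSGameStateBase, repossesses it and hands the pawn back to its AI, without clearing the control flag.
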(event EventBeginPlay
  (bind _output_get (Variables|Default|SetOwnerRef (Components|GetOwner)))
  (Variables|Default|SetAICON_Ref (AI|GetAIController _output_get)))

(event EventTick
  (params (DeltaSeconds :type Float%20%28single-precision%29)))

(event EventOnDroneHackSucceeded
  (params (bWasAssaultDrone? :type Boolean))
  (bind _returnvalue (Game|GetPlayerController 0))
  (bind _returnvalue_2 (Components|GetOwner))
  (Variables|Default|SetbIsControlledByPlayer? true)
  (Game|Player|SetViewTargetwithBlend _returnvalue _returnvalue_2 3.0 "VTBlend_Linear" 0.0 false)
  (Pawn|UnPossess _returnvalue)
  (Pawn|Possess _returnvalue (.AsPawn (Utilities|Casting|CastToPawn _returnvalue_2))))

(event EventReturntoPlayer
  (bind _returnvalue (Game|GetPlayerController 0))
  (bind _returnvalue_2 (Game|GetGameState))
  (bind _asbp_issgame_state_base (Utilities|Casting|CastToBP_ISSGameStateBase _returnvalue_2))
  (bind _playercharacterreference (Variables|/Game/CheekyFPS/Blueprints/Game/BP_ISSGameStateBase.BP_ISSGameStateBase_C|GetPlayerCharacterReference _asbp_issgame_state_base))
  (Game|Player|SetViewTargetwithBlend _returnvalue _playercharacterreference 3.0 "VTBlend_Linear" 0.0 false)
  (Pawn|UnPossess _returnvalue)
  (Pawn|Possess (Game|GetPlayerController 0) _playercharacterreference)
  (Pawn|Possess (Variables|Default|GetAICON_Ref) (.AsPawn (Utilities|Casting|CastToPawn (Variables|Default|GetOwnerRef)))))

(fn IsPossessedbyPlayer
  (return (Variables|Default|GetbIsControlledByPlayer?)))