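; First-person player character with walk, run, sneak, stances, stamina, jumping with parkour, zoom and weapons.
; Input events drive movement, smoothed look and components for weapons, leaning, interaction and parkour, plus debug keys for damage and RamaSave.
; A 0.1-second timer updates movement state, normalised speed and stamina instead of Tick.
; Stance changes retry on a looping timer, sphere-tracing headroom to rise, while Tick interpolates capsule and camera height.
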(event OnThingDead(HealthComponent)
  (CallFunction|PlayDeathAnimation))

(event Custom|PlayerUpdates
  ;[0.05719 0.2929 1] Things to run frequently - but not tick
  ;;[1 0.4446 0.1392] Movement
  (Movement|CalculateMovementState)
  (Movement|CalculatePlayerSpeed)
  (Movement|UpdateStamina))

(event EventBeginPlay
  (Utilities|Time|SetTimerbyEvent (delegate Custom|PlayerUpdates) 0.1 true)
  (CallFunction|PlayCameraShake "/Game/CheekyFPS/Blueprints/CameraManager/CamShakes/CamShake_Idle.CamShake_Idle_C" 1.0 false)
  ;[1 1 1] Set MaxWalkSpeed to = Run Speed
  (Variables|/Script/Engine.CharacterMovementComponent|SetMaxWalkSpeed (Variables|Character|GetCharacterMovement) (Variables|Movement|Speed|GetBaseRunSpeed))
  (Variables|Default|SetMyABP (Components|SkeletalMesh|GetAnimInstance (Variables|Character|GetMesh)))
  (Variables|Default|SetOriginalAttachLocation (Variables|/Script/Engine.SceneComponent|GetRelativeLocation (Variables|Default|GetWeaponAttachPoint))))

(event EventTick
  (params (DeltaSeconds :type Float%20%28single-precision%29))
  ;[0 0.2977 1] Interp Player / Camera Height by Stance
  (Components|Capsule|SetCapsuleHalfHeight (Variables|Collision|GetCapsuleComponent) (Math|Interpolation|FInterpTo (Variables|/Script/Engine.CapsuleComponent|GetCapsuleHalfHeight (Variables|Collision|GetCapsuleComponent)) (Utilities|Select :Index (Variables|Stance|GetCurrentPlayerStance) :NewEnumerator0 (Variables|Stance|GetPlayerHalfHeight) :NewEnumerator1 (Variables|Stance|GetPlayerCrouchedHeight) :NewEnumerator2 (Variables|Stance|GetPlayerProneHeight)) DeltaSeconds (Variables|Stance|GetStanceChangeSpeed)) true)
  (Transformation|SetRelativeLocation (Variables|Default|GetSpringArm) (Math|Interpolation|VInterpTo (Variables|/Script/Engine.SceneComponent|GetRelativeLocation (Variables|Default|GetSpringArm)) (Math|Vector|MakeVector 0.0 0.0 (* (Variables|/Script/Engine.CapsuleComponent|GetCapsuleHalfHeight (Variables|Collision|GetCapsuleComponent)) 0.7)) DeltaSeconds 5.0) false false))

(event Input|KeyboardEvents|Divide
  (params (Key :type Key%20Structure))
  (:Pressed
    (Game|Damage|ApplyDamage self 1e+01 0 0)))

(event Input|ActionEvents|InputAction[CHEEKY]Jump
  (params (Key :type Key%20Structure))
  ;[0.1944 1 0.4592] Movement Actions
  (:Pressed
    (CallFunction|JumpStart))
  (:Released
    (CallFunction|JumpEnd)))

(event Input|ActionEvents|InputActionAttack
  (params (Key :type Key%20Structure))
  (bind _bp_weaponcomponent (Variables|Default|GetBP_WeaponComponent))
  (bind _currentweapon (Variables|/Game/CheekyFPS/Blueprints/Components/BP_WeaponComponent.BP_WeaponComponent_C|GetCurrentWeapon _bp_weaponcomponent))
  (:Pressed
    (Utilities|IsValid _currentweapon
      (:Is%20Valid
        (bind _remainingammo (Default|Fire _currentweapon))
        (Default|CallOnFiredWeapon _remainingammo)
        (Class|BPIAnimation|OnCharacterAttack(Message) (Variables|Default|GetMyABP) (Default|GetWeaponType _currentweapon))))))

(event Input|ActionEvents|InputActionSelectWeapon2
  (params (Key :type Key%20Structure))
  (:Pressed
    (CallFunction|EquipWeapon 1)))

(event Input|ActionEvents|InputActionSelectWeapon3
  (params (Key :type Key%20Structure))
  (:Pressed
    (CallFunction|EquipWeapon 2)))

(event Input|ActionEvents|InputAction[CHEEKY]Interact
  (params (Key :type Key%20Structure))
  (bind _inventorycomponent (Variables|Default|GetInventoryComponent))
  (bind _cheekytracecomponent (Variables|Default|GetCheekyTraceComponent))
  (bind _currentkeycard (Variables|/Game/CheekyFPS/Blueprints/Components/InventoryComponent.InventoryComponent_C|GetCurrentKeyCard _inventorycomponent))
  ;[0.6979 0 1] Interaction
  (:Pressed
    (Default|InteractInput _cheekytracecomponent true "NewEnumerator0")
    (Utilities|IsValid _currentkeycard
      (:Is%20Valid
        (Class|BPIDoors|AttemptDoorUnlock(Message) (Variables|/Game/CheekyFPS/Blueprints/Interaction/CheekyTraceComponent.CheekyTraceComponent_C|GetCurrentInteractionComponent _cheekytracecomponent) (Variables|/Game/CheekyFPS/Blueprints/Interaction/Items/BP_KeyItem.BP_KeyItem_C|GetCurrentLevel _currentkeycard)))))
  (:Released
    (Default|InteractInput _cheekytracecomponent false "NewEnumerator0")))

(event Input|ActionEvents|InputAction[CHEEKY]Crouch
  (params (Key :type Key%20Structure))
  (bind _myabp (Variables|Default|GetMyABP))
  (bind _playersettingsmanager (Variables|Default|GetPlayerSettingsManager))
  (bind _bcrouchtoggle (Variables|/Game/CheekyFPS/Blueprints/CheekyPlayerSettingsManager.CheekyPlayerSettingsManager_C|GetbCrouchToggle _playersettingsmanager))
  ;[1 0 0.7882] Crouching
  (:Pressed
    (if _bcrouchtoggle
      (if (Utilities|Enum|Equal(Enum) (Variables|Stance|GetTargetPlayerStance) "NewEnumerator1")
        (CallFunction|ChangeStance "NewEnumerator0" :!label _label)
        (Class|BPIAnimation|OnCharacterCrouch(Message) _myabp false)
        (else
          (CallFunction|ChangeStance "NewEnumerator1" :!label _label_2)
          (Class|BPIAnimation|OnCharacterCrouch(Message) _myabp true)))
      (else
        (goto _label_2))))
  (:Released
    (if (not _bcrouchtoggle)
      (goto _label))))

(event Input|ActionEvents|InputAction[CHEEKY]Zoom
  (params (Key :type Key%20Structure))
  ;[1 0.3846 0] Zoom
  (:Pressed
    (CallFunction|ZoomView true))
  (:Released
    (CallFunction|ZoomView false)))

(event Input|ActionEvents|InputAction[CHEEKY]Sneak
  (params (Key :type Key%20Structure))
  ;[0.1944 1 0.4592] Movement Actions
  (:Pressed
    (Variables|Movement|SetbIsTryingToSneak true))
  (:Released
    (Variables|Movement|SetbIsTryingToSneak false)))

(event Input|ActionEvents|InputAction[CHEEKY]Run
  (params (Key :type Key%20Structure))
  (bind _playersettingsmanager (Variables|Default|GetPlayerSettingsManager))
  (bind _bruntoggle (Variables|/Game/CheekyFPS/Blueprints/CheekyPlayerSettingsManager.CheekyPlayerSettingsManager_C|GetbRunToggle _playersettingsmanager))
  ;[0.04337 0.127 1] Running
  (:Pressed
    (if _bruntoggle
      (Variables|Movement|SetbIsTryingToRun (not (Variables|Movement|GetbIsTryingToRun)))
      (else
        (Variables|Movement|SetbIsTryingToRun true))))
  (:Released
    (if (not _bruntoggle)
      (Variables|Movement|SetbIsTryingToRun false))))

(event Input|ActionEvents|InputAction[CHEEKY]Prone
  (params (Key :type Key%20Structure))
  (bind _playersettingsmanager (Variables|Default|GetPlayerSettingsManager))
  (bind _bpronetoggle (Variables|/Game/CheekyFPS/Blueprints/CheekyPlayerSettingsManager.CheekyPlayerSettingsManager_C|GetbProneToggle _playersettingsmanager))
  ;[1 0 0.7882] Prone
  (:Pressed
    (if _bpronetoggle
      (if (Utilities|Enum|Equal(Enum) (Variables|Stance|GetTargetPlayerStance) "NewEnumerator2")
        (CallFunction|ChangeStance "NewEnumerator0" :!label _label)
        (else
          (CallFunction|ChangeStance "NewEnumerator2" :!label _label_2)))
      (else
        (goto _label_2))))
  (:Released
    (if (not _bpronetoggle)
      (goto _label))))

(event Input|ActionEvents|InputActionReload
  (params (Key :type Key%20Structure))
  (bind _bp_weaponcomponent (Variables|Default|GetBP_WeaponComponent))
  (bind _currentweapon (Variables|/Game/CheekyFPS/Blueprints/Components/BP_WeaponComponent.BP_WeaponComponent_C|GetCurrentWeapon _bp_weaponcomponent))
  (:Pressed
    (Utilities|IsValid _currentweapon
      (:Is%20Valid
        (bind (_currentammo _remaininginvammo) (Default|Reload _currentweapon))
        (Default|CallOnReloadedWeapon _currentammo _remaininginvammo)))))

(event Input|ActionEvents|InputActionSelectWeapon1
  (params (Key :type Key%20Structure))
  (:Pressed
    (CallFunction|EquipWeapon)))

(event Input|AxisEvents|InputAxis[FPS]MoveRight
  (params (AxisValue :type Float%20%28single-precision%29))
  ;[0.1175 0.1248 1] Movement
  (CallFunction|MoveRightInput AxisValue))

(event Input|AxisEvents|InputAxis[FPS]MoveForward
  (params (AxisValue :type Float%20%28single-precision%29))
  ;[0.1175 0.1248 1] Movement
  (CallFunction|MoveForwardInput AxisValue))

(event Input|AxisEvents|InputAxis[FPS]LeanRight
  (params (AxisValue :type Float%20%28single-precision%29))
  ;[0.1686 0.2777 1] Leaning
  (Default|UpdateLeanfromAxis (Variables|Default|GetLeanComponent) AxisValue))

(event Input|AxisEvents|InputAxisLookUp
  (params (AxisValue :type Float%20%28single-precision%29))
  ;[1 0.1188 0.6025] Mouselook
  (CallFunction|LookVertical (* AxisValue -1.0) false))

(event Input|AxisEvents|InputAxisLookRight
  (params (AxisValue :type Float%20%28single-precision%29))
  ;[1 0.1188 0.6025] Mouselook
  (CallFunction|LookHorizontal AxisValue false))

(event Input|GamepadEvents|GamepadLeftX
  (params (AxisValue :type Float%20%28single-precision%29))
  (CallFunction|MoveRightInput AxisValue))

(event Input|GamepadEvents|GamepadRightY
  (params (AxisValue :type Float%20%28single-precision%29))
  ;[1 0.1357 0.3162] Gamepad Look
  (CallFunction|LookVertical AxisValue true))

(event Input|GamepadEvents|GamepadRightX
  (params (AxisValue :type Float%20%28single-precision%29))
  ;[1 0.1357 0.3162] Gamepad Look
  (CallFunction|LookHorizontal AxisValue true))

(event Input|KeyboardEvents|G
  (params (Key :type Key%20Structure))
  (:Pressed
    (bind _allcomponentssaved (Class|RamaSaveLibrary|RamaSaveSavetoFile (CallFunction|GetSaveSlotLocation) "" false 0))
    (if _allcomponentssaved
      (Development|PrintString "Saved!"))))

(event Input|KeyboardEvents|NumPadTwo
  (params (Key :type Key%20Structure))
  (:Pressed
    (Class|RamaSaveLibrary|RamaSaveDeleteFile (CallFunction|GetSaveSlotLocation))))

(event Input|KeyboardEvents|H
  (params (Key :type Key%20Structure))
  (:Pressed
    (bind _fileiosuccess (Class|RamaSaveLibrary|RamaSaveLoadfromFile (CallFunction|GetSaveSlotLocation) true false true))
    (if _fileiosuccess
      (Development|PrintString "Loaded!"))))

(event OnCrouch(CheekyParkourComponent)
  ;[0 1 0.1289] Change Stance - Note the actual stance changing (e.g modifying player height) happens on Event Tick
  (Variables|Stance|SetTargetPlayerStance "NewEnumerator1")
  (Utilities|Time|ClearTimerbyFunctionName 0 "ChangeStanceTarget")
  (Utilities|Time|SetTimerbyFunctionName 0 "ChangeStanceTarget" 0.1 true) ; This will keep looping until the player can transition to\nthe target stance, and it will then stop itself
)

(event OnChangePlayerMovementLock(CheekyTraceComponent)
  (params (bAllowLook :type Boolean) (bAllowMove :type Boolean))
  ;[0 1 0.3113] Lock / Unlock player look and movement from interactors
  ;
  ; (Note - if multiple systems are trying to manage this, then you'd need to add more delegation)
  (Variables|Movement|SetbAllowLook bAllowLook)
  (Variables|Movement|SetbAllowMovement bAllowMove))

(event OnParkour(CheekyParkourComponent)
  ;[1 0.0205 0.9536] Jump / Landing
  (Character|StopJumping)
  (Utilities|Time|ClearandInvalidateTimerbyHandle (Variables|Default|GetParkourTimerCheck)))

(event Custom|MoveForwardInput
  (params (Axis :type Float%20%28single-precision%29))
  ;[0.03282 0.338 1] Move Forward
  (Pawn|Input|AddMovementInput (Transformation|GetActorForwardVector) (* Axis (Variables|Movement|Speed|GetNormalisedMovementSpeed) (select (< Axis 0.0) (Variables|Movement|Speed|GetBackwardsPenalty) 1.0) (Math|Conversions|ToFloat(Boolean) (Variables|Movement|GetbAllowMovement))) false))

(event Custom|MoveRightInput
  (params (Axis :type Float%20%28single-precision%29))
  ;[0.03282 0.338 1] Move Right
  (Pawn|Input|AddMovementInput (Transformation|GetActorRightVector) (* Axis (Variables|Movement|Speed|GetNormalisedMovementSpeed) (Variables|Movement|Speed|GetSidewaysPenalty) (Math|Conversions|ToFloat(Boolean) (Variables|Movement|GetbAllowMovement))) false))

(event Custom|ChangeStance
  (params (NewStance :type EPlayerStances%20Enum :default "NewEnumerator0"))
  ;[0 1 0.1289] Change Stance - Note the actual stance changing (e.g modifying player height) happens on Event Tick
  (Variables|Stance|SetTargetPlayerStance NewStance)
  (Utilities|Time|ClearTimerbyFunctionName 0 "ChangeStanceTarget")
  (Utilities|Time|SetTimerbyFunctionName 0 "ChangeStanceTarget" 0.1 true) ; This will keep looping until the player can transition to\nthe target stance, and it will then stop itself
)

(event Custom|LookHorizontal
  (params (Axis :type Float%20%28single-precision%29) (bIsGamepad :type Boolean))
  (bind _playersettingsmanager (Variables|Default|GetPlayerSettingsManager))
  ;[1 0.2764 0.6413] Look Horizontal
  ;;[0.2562 0.541 1] Smooth Axis Input
  (bind _output_get (Variables|Movement|Look|SetSmoothHorizontalLook (Math|Interpolation|FInterpTo (Variables|Movement|Look|GetSmoothHorizontalLook) Axis (Utilities|Time|GetWorldDeltaSeconds) (Default|GetLookSmooth (Variables|Default|GetPlayerSettingsManager) bIsGamepad))))
  ;;[1 0.3819 0.2215] Apply settings, apply to controller
  (Pawn|Input|AddControllerYawInput (* _output_get (Math|Float|SelectFloat -1.0 1.0 (Default|GetLookInvertY _playersettingsmanager bIsGamepad)) (Default|GetLookSensY _playersettingsmanager bIsGamepad) (Math|Conversions|ToFloat(Boolean) (Variables|Movement|GetbAllowLook)))))

(event Custom|CheckForParkour
  ;[1 0.0205 0.9536] Jump / Landing
  ;;[1 0.1179 0] Check for Parkour while jumping
  (bind _bparkouractionperformed (Default|JumpAction (Variables|Default|GetCheekyParkourComponent)))
  (if _bparkouractionperformed
    (Utilities|Time|ClearandInvalidateTimerbyHandle (Variables|Default|GetParkourTimerCheck))))

(event Custom|LookVertical
  (params (Axis :type Float%20%28single-precision%29) (bIsGamepad :type Boolean))
  (bind _playersettingsmanager (Variables|Default|GetPlayerSettingsManager))
  ;[1 0.2764 0.6413] Look Vertical
  ;;[0.2562 0.541 1] Smooth Axis Input
  (bind _output_get (Variables|Movement|Look|SetSmoothVerticalLook (Math|Interpolation|FInterpTo (Variables|Movement|Look|GetSmoothVerticalLook) Axis (Utilities|Time|GetWorldDeltaSeconds) (Default|GetLookSmooth (Variables|Default|GetPlayerSettingsManager) bIsGamepad))))
  ;;[1 0.3819 0.2215] Apply settings, apply to controller
  (Pawn|Input|AddControllerPitchInput (* _output_get (Math|Float|SelectFloat -1.0 1.0 (Default|GetLookInvertY _playersettingsmanager bIsGamepad)) (Default|GetLookSensY _playersettingsmanager bIsGamepad) (Math|Conversions|ToFloat(Boolean) (Variables|Movement|GetbAllowLook)))))

(event Custom|JumpStart
  ;[1 0.0205 0.9536] Jump / Landing
  ;;[1 0.3939 0.1205] Make sure we're standing and not already mid-parkour
  (if (and (Utilities|Enum|Equal(Enum) (Variables|Stance|GetCurrentPlayerStance) "NewEnumerator0") (not (Variables|/Game/CheekyFPS/Blueprints/CheekyParkourComponent.CheekyParkourComponent_C|GetbIsParkouring (Variables|Default|GetCheekyParkourComponent))))
    ;;[0 0.2579 1] Parkour stuff
    (bind _bparkouractionperformed (Default|JumpAction (Variables|Default|GetCheekyParkourComponent)))
    (if (not _bparkouractionperformed)
      (Character|Jump)
      (Default|PlayFootstep (Variables|Default|GetFootstepComponent) "NewEnumerator3" 1 1.0)
      (bind _returnvalue (Utilities|Time|SetTimerbyEvent (delegate Custom|CheckForParkour) 0.1 true))
      (Variables|Default|SetParkourTimerCheck _returnvalue))))

(event Custom|JumpEnd
  ;[1 0.0205 0.9536] Jump / Landing
  (Character|StopJumping)
  (Utilities|Time|ClearandInvalidateTimerbyHandle (Variables|Default|GetParkourTimerCheck)))

(event EventOnLanded
  (params (Hit :type Hit%20Result%20Structure%20%28by%20ref%29))
  (bind _charactermovement (Variables|Character|GetCharacterMovement))
  (bind _returnvalue (Pawn|Components|CharacterMovement|GetLastUpdateVelocity _charactermovement))
  (bind _z (Math|Vector|BreakVector _returnvalue))
  (bind _returnvalue_2 (Math|Float|Absolute(Float) _z))
  ;[0 1 0.5457] Land Event
  (Default|OnLanded (Variables|Default|GetHealthComponent) _returnvalue_2)
  (Default|PlayFootstep (Variables|Default|GetFootstepComponent) "NewEnumerator5" 1 (Math|Float|Clamp(Float) (/ _returnvalue_2 8e+02) 0.5)))

(event Custom|ZoomView
  (params (bStart :type Boolean))
  ;[1 0.31 0.6422] Zoom / Focus Mode
  (if bStart
    (Utilities|IsValid (Variables|Default|GetCameraModifierZoom)
      (:Is%20Valid
        _)
      (:Is%20Not%20Valid
        (bind _returnvalue (Game|Player|AddNewCameraModifier (Game|GetPlayerCameraManager 0) "/Game/CheekyFPS/Blueprints/CameraManager/CamModifiers/CamModifier_InspectZoom.CamModifier_InspectZoom_C")) ; This should only happen the first time the player uses zoom
        (Variables|Default|SetCameraModifierZoom _returnvalue)))
    (CameraModifier|EnableModifier (Variables|Default|GetCameraModifierZoom))
    (Variables|Default|SetbIsInZoomMode true)
    (Utilities|IsValid (Variables|/Game/CheekyFPS/Blueprints/Components/BP_WeaponComponent.BP_WeaponComponent_C|GetCurrentWeapon (Variables|Default|GetBP_WeaponComponent))
      (:Is%20Valid
        (Components|Timeline|PlayfromStart (Variables|Default|GetWeaponZoomTimeline))))
    (else
      (Utilities|IsValid (Variables|Default|GetCameraModifierZoom)
        (:Is%20Valid
          (CameraModifier|DisableModifier (Variables|Default|GetCameraModifierZoom) false)
          (Variables|Default|SetbIsInZoomMode false)
          (Utilities|IsValid (Variables|/Game/CheekyFPS/Blueprints/Components/BP_WeaponComponent.BP_WeaponComponent_C|GetCurrentWeapon (Variables|Default|GetBP_WeaponComponent))
            (:Is%20Valid
              (Components|Timeline|ReversefromEnd (Variables|Default|GetWeaponZoomTimeline)))))
        (:Is%20Not%20Valid
          (Variables|Default|SetbIsInZoomMode false))))))

(event Custom|EndZoom
  ;[1 0.31 0.6422] Zoom / Focus Mode
  (Utilities|IsValid (Variables|Default|GetCameraModifierZoom)
    (:Is%20Valid
      (CameraModifier|DisableModifier (Variables|Default|GetCameraModifierZoom) false)
      (Variables|Default|SetbIsInZoomMode false)
      (Utilities|IsValid (Variables|/Game/CheekyFPS/Blueprints/Components/BP_WeaponComponent.BP_WeaponComponent_C|GetCurrentWeapon (Variables|Default|GetBP_WeaponComponent))
        (:Is%20Valid
          (Components|Timeline|ReversefromEnd (Variables|Default|GetWeaponZoomTimeline)))))
    (:Is%20Not%20Valid
      (Variables|Default|SetbIsInZoomMode false))))

(fn ConstructionScript)

(fn PlayCameraShake
  (params (ShakeClass :type Matinee%20Camera%20Shake%20Class%20Reference) (Scale :type Float%20%28single-precision%29) (bIgnoreHeadbobSettings :type Boolean))
  (Class|PlayerCameraManager|StartMatineeCameraShake (Game|GetPlayerCameraManager 0) ShakeClass (select bIgnoreHeadbobSettings Scale (* Scale (Variables|/Game/CheekyFPS/Blueprints/CheekyPlayerSettingsManager.CheekyPlayerSettingsManager_C|GetHeadbobScale (Variables|Default|GetPlayerSettingsManager)))) "CameraLocal" "0, 0, 0")
  (return))

(fn CalculateMovementState
  (bind _output_get (LocalVariables|SetCurrentVelocity (Math|Vector|VectorLength (Pawn|Components|CharacterMovement|GetLastUpdateVelocity (Variables|Character|GetCharacterMovement)))))
  ;[1 1 1] This is generally useful for other systems
  (bind _output_get_2 (Variables|Movement|SetbIsPlayerMoving (and (AI|Components|NavMovement|IsMovingonGround (Variables|Character|GetCharacterMovement)) (not (Math|Float|NearlyEqual(Float) _output_get 0.0 3.0)))))
  ;[0.3236 0.2872 1] If run toggle is on, and the player stops moving, cancel running
  (if (and (not _output_get_2) (Variables|/Game/CheekyFPS/Blueprints/CheekyPlayerSettingsManager.CheekyPlayerSettingsManager_C|GetbRunToggle (Variables|Default|GetPlayerSettingsManager)))
    (Variables|Movement|SetbIsTryingToRun false))
  ;[1 1 1] Can player run?
  (LocalVariables|SetCanPlayerRun (and (not (Variables|Movement|Stamina|GetbIsPlayStaminaOnCooldown)) (> (LocalVariables|GetCurrentVelocity) 1e+02)))
  ;[1 1 1] Final movement state
  (Variables|Movement|SetMovementState (select (and (Variables|Movement|GetbIsTryingToRun) (LocalVariables|GetCanPlayerRun)) "NewEnumerator2" (select (Variables|Movement|GetbIsTryingToSneak) "NewEnumerator1" "NewEnumerator0")))
  (return))

(fn CalculatePlayerSpeed
  (LocalVariables|SetMovementPenalties (* 1.0 (select (Variables|Default|GetbIsInZoomMode) (Variables|Movement|Speed|GetZoomPenalty) 1.0)))
  ;[1 1 1] Calculate Normalised Speed - this could be more efficient by precalculating values
  (Variables|Movement|Speed|SetNormalisedMovementSpeed (* (Utilities|Select :Index (Variables|Stance|GetCurrentPlayerStance) :NewEnumerator0 (Utilities|Select :Index (Variables|Movement|GetMovementState) :NewEnumerator0 (/ (Variables|Movement|Speed|GetBaseWalkSpeed) (Variables|Movement|Speed|GetBaseRunSpeed)) :NewEnumerator1 (/ (Variables|Movement|Speed|GetBaseSneakSpeed) (Variables|Movement|Speed|GetBaseRunSpeed)) :NewEnumerator2 1.0) :NewEnumerator1 (/ (Variables|Movement|Speed|GetBaseCrouchSpeed) (Variables|Movement|Speed|GetBaseRunSpeed)) :NewEnumerator2 (/ (Variables|Movement|Speed|GetBaseProneSpeed) (Variables|Movement|Speed|GetBaseRunSpeed))) (LocalVariables|GetMovementPenalties)))
  (return))

(fn UpdateStamina
  (if (Variables|Movement|Stamina|GetbUseStamina?)
    (bind _output_get (Variables|Movement|Stamina|SetStamina (Math|Float|Clamp(Float) (+ (Variables|Movement|Stamina|GetStamina) (/ (select (Variables|Movement|GetbIsPlayerMoving) (Utilities|Select :Index (Variables|Movement|GetMovementState) :NewEnumerator0 4.0 :NewEnumerator1 6.0 :NewEnumerator2 -1e+01) 7.0) 1e+01)) 0.0 1e+02)))
    ;[1 1 1] If stamina hits 0, enable cooldown
    (if (== _output_get 0.0)
      (Variables|Movement|Stamina|SetbIsPlayStaminaOnCooldown true)
      (return)
      (else
        ;[1 1 1] If stamina is above 20, make sure cooldown is off
        (if (>= _output_get (Variables|Movement|Stamina|GetStaminaCooldownThreshold))
          (Variables|Movement|Stamina|SetbIsPlayStaminaOnCooldown false)
          (return)
          (else
            ;[1 1 1] Do not change stamina state
            (return)))))))

(fn ChangeStanceTarget
  (switch Utilities|FlowControl|Switch|SwitchonEPlayerStances (Variables|Stance|GetCurrentPlayerStance)
    (:NewEnumerator0
      ;[0.8045 0 1] Standing > Any other stance is always ok
      (switch Utilities|FlowControl|Switch|SwitchonEPlayerStances (Variables|Stance|GetTargetPlayerStance)
        (:NewEnumerator0
          (Variables|Stance|SetCurrentPlayerStance "NewEnumerator0"))
        (:NewEnumerator1
          (Variables|Stance|SetCurrentPlayerStance "NewEnumerator1")
          (CallFunction|PlayCameraShake "/Game/CheekyFPS/Blueprints/CameraManager/CamShakes/CamShake_CrouchDown.CamShake_CrouchDown_C" 0.8 false)
          (Audio|SpawnSoundAttached (Variables|Stance|GetCrouchSound) (Variables|Collision|GetCapsuleComponent) "None" "0, 0, 0" "0, 0, 0" "KeepRelativeOffset" false 1.0 1.0 0.0 0 0))
        (:NewEnumerator2
          (Variables|Stance|SetCurrentPlayerStance "NewEnumerator2")
          (CallFunction|PlayCameraShake "/Game/CheekyFPS/Blueprints/CameraManager/CamShakes/CamShake_CrouchDown.CamShake_CrouchDown_C" 1.0 false)
          (Audio|SpawnSoundAttached (Variables|Stance|GetProneSound) (Variables|Collision|GetCapsuleComponent) "None" "0, 0, 0" "0, 0, 0" "KeepRelativeOffset" false 1.0 1.0 0.0 0 0)))
      (Utilities|Time|ClearTimerbyFunctionName 0 "ChangeStanceTarget")
      (return))
    (:NewEnumerator1
      ;[0 1 0.847] Crouch to other stances
      (switch Utilities|FlowControl|Switch|SwitchonEPlayerStances (Variables|Stance|GetTargetPlayerStance)
        (:NewEnumerator0
          (Utilities|CanPlayerChangeStance (Variables|Stance|GetPlayerHalfHeight)
            (:Yes
              (Variables|Stance|SetCurrentPlayerStance "NewEnumerator0")
              (CallFunction|PlayCameraShake "/Game/CheekyFPS/Blueprints/CameraManager/CamShakes/CamShake_CrouchUp.CamShake_CrouchUp_C" 1.0 false)
              (Audio|SpawnSoundAttached (Variables|Stance|GetStandSound) (Variables|Collision|GetCapsuleComponent) "None" "0, 0, 0" "0, 0, 0" "KeepRelativeOffset" false 1.0 1.0 0.0 0 0))
            (:No
              (return))))
        (:NewEnumerator1
          _)
        (:NewEnumerator2
          (Variables|Stance|SetCurrentPlayerStance "NewEnumerator2")
          (CallFunction|PlayCameraShake "/Game/CheekyFPS/Blueprints/CameraManager/CamShakes/CamShake_CrouchDown.CamShake_CrouchDown_C" 0.5 false)
          (Audio|SpawnSoundAttached (Variables|Stance|GetProneSound) (Variables|Collision|GetCapsuleComponent) "None" "0, 0, 0" "0, 0, 0" "KeepRelativeOffset" false 1.0 1.0 0.0 0 0)))
      (Utilities|Time|ClearTimerbyFunctionName 0 "ChangeStanceTarget")
      (return))
    (:NewEnumerator2
      ;[1 0.6367 0.2282] Prone to other stances
      (switch Utilities|FlowControl|Switch|SwitchonEPlayerStances (Variables|Stance|GetTargetPlayerStance)
        (:NewEnumerator0
          (Utilities|CanPlayerChangeStance (Variables|Stance|GetPlayerHalfHeight)
            (:Yes
              (Variables|Stance|SetCurrentPlayerStance "NewEnumerator0")
              (CallFunction|PlayCameraShake "/Game/CheekyFPS/Blueprints/CameraManager/CamShakes/CamShake_CrouchUp.CamShake_CrouchUp_C" 1.0 false)
              (Audio|SpawnSoundAttached (Variables|Stance|GetStandSound) (Variables|Collision|GetCapsuleComponent) "None" "0, 0, 0" "0, 0, 0" "KeepRelativeOffset" false 1.0 1.0 0.0 0 0))
            (:No
              (return))))
        (:NewEnumerator1
          (Utilities|CanPlayerChangeStance (Variables|Stance|GetPlayerProneHeight)
            (:Yes
              (Variables|Stance|SetCurrentPlayerStance "NewEnumerator1")
              (CallFunction|PlayCameraShake "/Game/CheekyFPS/Blueprints/CameraManager/CamShakes/CamShake_CrouchUp.CamShake_CrouchUp_C" 0.5 false)
              (Audio|SpawnSoundAttached (Variables|Stance|GetCrouchSound) (Variables|Collision|GetCapsuleComponent) "None" "0, 0, 0" "0, 0, 0" "KeepRelativeOffset" false 1.0 1.0 0.0 0 0))
            (:No
              (return))))
        (:NewEnumerator2
          (Variables|Stance|SetCurrentPlayerStance "NewEnumerator2")))
      (Utilities|Time|ClearTimerbyFunctionName 0 "ChangeStanceTarget")
      (return))))

(fn EquipWeapon
  (params (Key :type Integer))
  (bind _bp_weaponcomponent (Variables|Default|GetBP_WeaponComponent))
  (bind _bp_weaponcomponent_2 (Variables|Default|GetBP_WeaponComponent))
  (bind _weaponinventory (Variables|/Game/CheekyFPS/Blueprints/Components/BP_WeaponComponent.BP_WeaponComponent_C|GetWeaponInventory _bp_weaponcomponent))
  (bind (_value _returnvalue) (Utilities|Map|Find _weaponinventory Key))
  (Utilities|FlowControl|Sequence
    (:then_0
      (Utilities|IsValid (Variables|/Game/CheekyFPS/Blueprints/Components/BP_WeaponComponent.BP_WeaponComponent_C|GetCurrentWeapon _bp_weaponcomponent)
        (:Is%20Valid
          (Rendering|SetActorHiddenInGame (Variables|/Game/CheekyFPS/Blueprints/Components/BP_WeaponComponent.BP_WeaponComponent_C|GetCurrentWeapon _bp_weaponcomponent) true)
          (Variables|/Game/CheekyFPS/Blueprints/Components/BP_WeaponComponent.BP_WeaponComponent_C|SetCurrentWeapon _bp_weaponcomponent 0))))
    (:then_1
      (if _returnvalue
        (Utilities|IsValid _value
          (:Is%20Valid
            (Default|AttachtoOwner _bp_weaponcomponent_2 _value (Variables|Default|GetWeaponAttachPoint) "None")
            (bind _output_get (Variables|/Game/CheekyFPS/Blueprints/Components/BP_WeaponComponent.BP_WeaponComponent_C|SetCurrentWeapon _bp_weaponcomponent_2 _value))
            (Rendering|SetActorHiddenInGame _output_get false)
            (Variables|Default|SetbHasWeaponEquipped? true)
            (Class|BPIPlayer|UpdateWeaponHUD(Message) (Game|GetPlayerController 0))
            (Class|BPIAnimation|OnCharacterEquipWeapon(Message) (Variables|Default|GetMyABP) (Default|GetWeaponType _output_get))))))))

(fn DropItem
  (params (DroppedItem :type Actor%20Class%20Reference))
  (Game|SpawnActorfromClass DroppedItem (Math|Transform|MakeTransform (Transformation|GetActorLocation) (Transformation|GetActorRotation) "1,1,1") "AdjustIfPossibleButAlwaysSpawn" 0 0))

(fn PlayDeathAnimation
  (bind _self self)
  (bind _returnvalue (AI|GetAIController _self))
  (Class|BPIAnimation|OnCharacterPlayDeath(Message) (Variables|Default|GetMyABP) true)
  (if (!= _self (Game|GetPlayerCharacter 0))
    (Utilities|IsValid _returnvalue
      (:Is%20Valid
        (AI|Navigation|StopMovement _returnvalue)
        (Class|Pawn|DetachfromControllerPendingDestroy)))))

(fn MoveDroppedItem
  (params (Target :type Actor%20Object%20Reference) (NewTransform :type Transform%20%28by%20ref%29))
  (Transformation|SetActorTransform Target NewTransform))