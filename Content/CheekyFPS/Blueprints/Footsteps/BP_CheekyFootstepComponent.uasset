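; Footstep component that plays surface-specific step sounds for its owning character and reports them as noise events.
; FootstepCycle accumulates changes in a looping cycle input, ignoring wrap jumps, and triggers alternating left/right walk steps.
; PlayFootstep line-traces from a foot offset, matches the physical material to surface data, then passes the cue and step type to the owner's audio.
; Player noise depends on stance and run intent.
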(event EventBeginPlay)

(event EventTick
  (params (DeltaSeconds :type Float%20%28single-precision%29)))

(fn PlayFootstep
  (params (Type :type EFootstepTypes%20Enum :default "NewEnumerator0") (Position :type Integer) (OverrideVolume :type Float%20%28single-precision%29))
  (bind _returnvalue (Components|GetOwner))
  (bind _returnvalue_2 (Components|GetOwner))
  (bind _returnvalue_3 (Components|GetOwner))
  (bind _returnvalue_4 (Components|GetOwner))
  (bind _footseperation (Variables|Default|GetFootSeperation))
  (bind _returnvalue_5 (Transformation|GetActorRotation _returnvalue_4))
  (bind _returnvalue_6 (* _footseperation -1.0))
  (bind _asbp_cheeky_character (Utilities|Casting|CastToBP_CheekyCharacter _returnvalue))
  (bind _rootcomponent (Variables|/Script/Engine.Actor|GetRootComponent _returnvalue_4))
  (bind _returnvalue_7 (Transformation|GetWorldLocation _rootcomponent))
  (bind _returnvalue_8 (Math|Vector|GetRightVector _returnvalue_5))
  (bind _returnvalue_9 (Utilities|Select :Index Position :Option%200 _returnvalue_6 :Option%201 0.0 :Option%202 _footseperation))
  (bind _returnvalue_10 (* _returnvalue_8 _returnvalue_9))
  (bind _returnvalue_11 (+ _returnvalue_7 _returnvalue_10))
  ;[0.09387 1 0.08132] Line Trace - Find out what surface is below the player
  (bind (_outhit _returnvalue_12) (Collision|LineTraceByChannel _returnvalue_11 (* _returnvalue_11 "0, 0,-200.000000") "TraceTypeQuery1" false (Utilities|Array|MakeArray (Components|GetOwner)) (select (Variables|Default|GetbDebug) "ForDuration" "None")))
  (if _returnvalue_12
    (LocalVariables|SetHitLocation (.Location (Collision|BreakHitResult _outhit)))
    (LocalVariables|SetPhysMat (.PhysMat (Collision|BreakHitResult _outhit)))
    ;[1 0.54 0] Find surface data
    (for _array_element (Variables|SurfaceData|GetFootstepSurfaces)
      (if (== (.PhysicalMaterial (Utilities|Struct|BreakSFootstepSurface _array_element)) (LocalVariables|GetPhysMat))
        (LocalVariables|SetFootstepSurface _array_element)
        (LocalVariables|SetbFoundFootstepSurface true)
        ;;[1 0.303 0.4129] Debug
        (if (Variables|Default|GetbDebug)
          (Development|PrintString (Utilities|String|Append "Found footstep surface data for " (Utilities|GetDisplayName (LocalVariables|GetPhysMat)))))))
    (if (LocalVariables|GetbFoundFootstepSurface)
      (Variables|Default|SetCurrentFootstepType Type)
      (else
        (LocalVariables|SetFootstepSurface (Variables|SurfaceData|GetDefaultFootstepSurface))))
    (Utilities|FlowControl|Sequence
      (:then_0
        ;[1 0 0.1066] Play Sound
        (Utilities|IsValid (.soundcue (LocalVariables|GetFootstepSurface))
          (:Is%20Valid
            (Class|BPIAnimation|OnCharacterMove(Message) _returnvalue_3 (.soundcue (LocalVariables|GetFootstepSurface)) OverrideVolume)
            (bind _returnvalue_13 (Class|BPIAnimation|GetFootstepAudioComponent(Message) _returnvalue_3))
            (Effects|Components|ParticleSystem|SetIntParameter _returnvalue_13 "FootstepType" (Utilities|Select :Index Type :NewEnumerator0 0 :NewEnumerator7 1 :NewEnumerator6 2 :NewEnumerator2 3 :NewEnumerator3 4 :NewEnumerator5 5 :NewEnumerator8 6))
            (if (== _returnvalue (Game|GetPlayerCharacter 0))
              (if (Utilities|Enum|Equal(Enum) (Variables|/Game/CheekyFPS/Blueprints/BP_CheekyCharacter.BP_CheekyCharacter_C|GetTargetPlayerStance _asbp_cheeky_character) "NewEnumerator0")
                (if (Variables|/Game/CheekyFPS/Blueprints/BP_CheekyCharacter.BP_CheekyCharacter_C|GetbIsTryingToRun _asbp_cheeky_character)
                  (Class|AISenseHearing|ReportNoiseEvent (LocalVariables|GetHitLocation) 2.0 _returnvalue_2 0.0 "Player")
                  (else
                    (Class|AISenseHearing|ReportNoiseEvent (LocalVariables|GetHitLocation) 1.0 _returnvalue_2 0.0 "Player"))))
              (else
                (Class|AISenseHearing|ReportNoiseEvent (LocalVariables|GetHitLocation) 1.0 (Components|GetOwner) 0.0 "None"))))))
      (:then_1
        (return)))
    (else
      (return))))

(fn FootstepCycle
  (params (CycleInput :type Float%20%28single-precision%29))
  (if (> (Variables|FootstepCycle|GetNextStep) 0.25)
    (Variables|FootstepCycle|SetNextStep -0.25)
    (CallFunction|PlayFootstep "NewEnumerator0" (select (Variables|FootstepCycle|GetbWasLastFootstepRight) 0 2) 1.0)
    (Variables|FootstepCycle|SetbWasLastFootstepRight (not (Variables|FootstepCycle|GetbWasLastFootstepRight)))
    (return)
    (else
      (Variables|FootstepCycle|SetNextStep (+ (Variables|FootstepCycle|GetNextStep) (select (> (Math|Float|Absolute(Float) (- CycleInput (Variables|FootstepCycle|GetLastCycle))) 1.0) 0.0 (- CycleInput (Variables|FootstepCycle|GetLastCycle)))))
      (Variables|FootstepCycle|SetLastCycle CycleInput)
      (return))))