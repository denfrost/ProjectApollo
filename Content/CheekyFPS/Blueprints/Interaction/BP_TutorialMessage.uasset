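; BP_TutorialMessage is a trigger actor that shows an input tutorial prompt when the player character overlaps it and CanPlayerExecuteAction is true.
; It creates a WBP_TutorialMessage_Input widget from its input action name, hold-button flag and action text.
; RemoveExistingWidgets clears other top-level prompts of that class, then the new one reaches the viewport after a short retriggerable delay.
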(event EventBeginPlay)

(event Collision|EventActorBeginOverlap
  (params (OtherActor :type Actor%20Object%20Reference))
  (if (== OtherActor (Game|GetPlayerCharacter 0))
    (if (Variables|WidgetSettings|GetCanPlayerExecuteAction?)
      (bind _returnvalue (UserInterface|CreateWidget "/Game/CheekyFPS/Blueprints/UMG/Gameplay/Tutorials/WBP_TutorialMessage_Input.WBP_TutorialMessage_Input_C" 0 (Variables|WidgetSettings|GetNew%20Input%20Action%20Name) (Variables|WidgetSettings|GetShould%20Hold%20Button) (Variables|WidgetSettings|GetIn%20Action%20Text)))
      (Variables|Default|SetWBPReference _returnvalue)
      (CallFunction|RemoveExistingWidgets)
      (Utilities|FlowControl|RetriggerableDelay 0.2)
      (UserInterface|Viewport|AddtoViewport _returnvalue 0))))

(fn ConstructionScript)

(fn RemoveExistingWidgets
  (bind _foundwidgets (Widget|GetAllWidgetsOfClass "/Game/CheekyFPS/Blueprints/UMG/Gameplay/Tutorials/WBP_TutorialMessage_Input.WBP_TutorialMessage_Input_C" true))
  (for _array_element _foundwidgets
    (if (!= _array_element (Variables|Default|GetWBPReference))
      (Widget|RemovefromParent _array_element))))