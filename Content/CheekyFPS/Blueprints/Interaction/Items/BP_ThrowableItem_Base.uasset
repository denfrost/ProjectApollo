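; Base throwable physics item that the player can pick up, carry, drop or throw, making noise on impact to distract listeners.
; The interact component tints it red when selected and grabs it with the player's PhysicsHandle, which Tick keeps at a camera-relative offset.
; HoldStyle chooses whether an Interact press or release drops it, while right mouse releases it with a forward impulse.
; Impacts report "Distract" noise, with a DoOnce-gated sound rearmed while held.
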(event OnBeginSelected(CheekyInteractComponent)
  ;[1 0.8053 0] Selection Colour
  (if (not (Variables|Default|GetbHoldingItem))
    (Rendering|Material|SetVectorParameterValue (Variables|Default|GetMaterialInstance) "Color" "(R=1.000000,G=0.000000,B=0.000000,A=1.000000)" :!class /Script/Engine.MaterialInstanceDynamic)))

(event OnEndSelection(CheekyInteractComponent)
  ;[1 0.8053 0] Selection Colour
  (if (not (Variables|Default|GetbHoldingItem))
    (Rendering|Material|SetVectorParameterValue (Variables|Default|GetMaterialInstance) "Color" "(R=1.000000,G=1.000000,B=1.000000,A=1.000000)" :!class /Script/Engine.MaterialInstanceDynamic)))

(event OnBeginInteraction(CheekyInteractComponent)
  (params (Type :type EInteractionTypes%20Enum :default "NewEnumerator0"))
  (bind _staticmesh (Variables|Default|GetStaticMesh))
  ;[0.09549 1 0.2229] Pickup
  (bind _output_get (Variables|Default|SetPhysicsHandle (Actor|GetComponentbyClass (Game|GetPlayerCharacter 0) "/Script/Engine.PhysicsHandleComponent")))
  (Utilities|IsValid _output_get
    (:Is%20Valid
      (Variables|Default|SetbHoldingItem true)
      (Physics|Components|PhysicsHandle|GrabComponentatLocationwithRotation (Variables|Default|GetPhysicsHandle) (Variables|Default|GetStaticMesh) "None" (Physics|GetCenterOfMass _staticmesh "None") (Transformation|GetWorldRotation _staticmesh))
      (Actor|Tick|SetActorTickEnabled true)
      (Input|EnableInput (Game|GetPlayerController 0))
      (Collision|SetCollisionResponsetoChannel (Variables|Default|GetStaticMesh) "ECC_Pawn" "ECR_Ignore")
      (Rendering|Material|SetVectorParameterValue (Variables|Default|GetMaterialInstance) "Color" "(R=1.000000,G=1.000000,B=1.000000,A=1.000000)" :!class /Script/Engine.MaterialInstanceDynamic))))

(event OnComponentHit(StaticMesh)
  (params (HitComponent :type Primitive%20Component%20Object%20Reference) (OtherActor :type Actor%20Object%20Reference) (OtherComp :type Primitive%20Component%20Object%20Reference) (NormalImpulse :type Vector :default "0, 0, 0") (Hit :type Hit%20Result%20Structure%20%28by%20ref%29))
  (bind _returnvalue (Game|GetPlayerCharacter 0))
  (bind (_bblockinghit _binitialoverlap _time _distance _location _impactpoint _normal _impactnormal _physmat _hitactor) (Collision|BreakHitResult Hit))
  (bind _returnvalue_2 (!= _hitactor _returnvalue))
  (if _bblockinghit
    (Variables|Default|SetHitPoint _impactpoint)
    (if _returnvalue_2
      (Utilities|FlowControl|Sequence
        (:then_0
          (if (Variables|Default|GetbHoldingItem)
            (goto _label Reset)
            (else
              (Utilities|FlowControl|DoOnce false :!label _label
                (:Completed
                  (if _returnvalue_2
                    (Audio|PlaySoundatLocation "/Game/CheekyFPS/Sounds/tada-fanfare-g.tada-fanfare-g" (Variables|Default|GetHitPoint) "0, 0, 0" 1.0 1.0 0.0 0 0 0)))))))
        (:then_1
          (Class|AISenseHearing|ReportNoiseEvent (Variables|Default|GetHitPoint) 1.0 self 0.0 "Distract"))
        (:then_2
          (Development|PrintString (Utilities|GetDisplayName _hitactor)))))))

(event Custom|Release
  ;[1 0 0.8797] Release Actions
  (Physics|Components|PhysicsHandle|ReleaseComponent (Variables|Default|GetPhysicsHandle))
  (Variables|Default|SetbHoldingItem false)
  (Actor|Tick|SetActorTickEnabled false)
  (Input|DisableInput (Game|GetPlayerController 0))
  (Collision|SetCollisionResponsetoChannel (Variables|Default|GetStaticMesh) "ECC_Pawn" "ECR_Ignore"))

(event EventTick
  (params (DeltaSeconds :type Float%20%28single-precision%29))
  (bind _returnvalue (Game|GetPlayerCameraManager 0))
  (bind _holdoffset (Variables|Default|GetHoldOffset))
  (bind _returnvalue_2 (Camera|GetCameraRotation _returnvalue))
  ;[0.958 0.1102 1] Holds the object in front of and just below the player camera
  (Class|PhysicsHandleComponent|SetTargetLocationandRotation (Variables|Default|GetPhysicsHandle) (+ (Camera|GetCameraLocation _returnvalue) (* (Math|Vector|GetForwardVector _returnvalue_2) (.x _holdoffset)) (* (Math|Vector|GetRightVector _returnvalue_2) (.y _holdoffset)) (* (Math|Vector|GetUpVector _returnvalue_2) (.z _holdoffset))) _returnvalue_2))

(event Input|ActionEvents|InputAction[CHEEKY]Interact
  (params (Key :type Key%20Structure :default "None"))
  ;[1 0 0.8797] Release Actions
  (:Pressed
    (if (and (Variables|Default|GetbHoldStyle) (Variables|Default|GetbHoldingItem))
      (Physics|Components|PhysicsHandle|ReleaseComponent (Variables|Default|GetPhysicsHandle) :!label _label)
      (Variables|Default|SetbHoldingItem false)
      (Actor|Tick|SetActorTickEnabled false)
      (Input|DisableInput (Game|GetPlayerController 0))
      (Collision|SetCollisionResponsetoChannel (Variables|Default|GetStaticMesh) "ECC_Pawn" "ECR_Ignore")))
  (:Released
    (if (Variables|Default|GetbHoldingItem)
      (if (not (Variables|Default|GetbHoldStyle))
        (goto _label)))))

(event Input|MouseEvents|RightMouseButton
  (params (Key :type Key%20Structure :default "None"))
  ;[0.05725 0 1] Throw
  (:Pressed
    (if (Variables|Default|GetbHoldingItem)
      (CallFunction|Release)
      (Physics|AddImpulse (Variables|Default|GetStaticMesh) (* (Math|Vector|GetForwardVector (Camera|GetCameraRotation (Game|GetPlayerCameraManager 0))) (Variables|Default|GetThrowForce)) "None" false))))

(fn ConstructionScript
  ;[1 1 1] Create dynamic material instance for the cube
  (bind _returnvalue (Rendering|Material|CreateDynamicMaterialInstance (Variables|Default|GetStaticMesh) 0 (Rendering|Material|GetMaterial (Variables|Default|GetStaticMesh) 0) "None" :!class /Script/Engine.PrimitiveComponent))
  (Variables|Default|SetMaterialInstance _returnvalue))