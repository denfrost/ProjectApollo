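; Throwable smoke grenade item that spawns smoke and reduces AI sight range around its impact point.
; A hit on a static-mesh actor stores the impact point, triggers Explode after a short delay and activates the grenade.
; Explode spawns the smoke, starts a looping timer and sets a lifespan.
; TraceForTargets sphere-traces forward from impact, shrinking the hit AI's sight range or sending a delayed sight-reset message if that fails.
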(event OnComponentHit(StaticMesh)
  (params (HitComponent :type Primitive%20Component%20Object%20Reference) (OtherActor :type Actor%20Object%20Reference) (OtherComp :type Primitive%20Component%20Object%20Reference) (NormalImpulse :type Vector :default "0, 0, 0") (Hit :type Hit%20Result%20Structure%20%28by%20ref%29))
  (bind (_bblockinghit _binitialoverlap _time _distance _location _impactpoint _normal _impactnormal _physmat _hitactor) (Collision|BreakHitResult Hit))
  (if _bblockinghit
    (Utilities|IsValid (Actor|GetComponentbyClass _hitactor "/Script/Engine.StaticMeshComponent")
      (:Is%20Valid
        (Variables|Default|SetHitPoint _impactpoint)
        (Utilities|FlowControl|RetriggerableDelay 0.2)
        (CallFunction|Explode)
        (if (not (Variables|Default|GetbIsActivated?))
          (Variables|Default|SetbIsActivated? true))))))

(event Custom|TraceForTargets
  (bind _hitpoint (Variables|Default|GetHitPoint))
  (if (Variables|Default|GetbIsActivated?)
    (if (not (Variables|Default|GetbHoldingItem))
      (bind _outhit (Collision|SphereTraceForObjects _hitpoint (+ _hitpoint (* (Math|Vector|GetForwardVector (Transformation|GetActorRotation)) 1.5e+03)) 5.4e+02 (Utilities|Array|MakeArray "ObjectTypeQuery3" "ObjectTypeQuery2") true 0 "ForDuration"))
      (if (.bBlockingHit (Collision|BreakHitResult _outhit))
        (Utilities|IsValid (Class|ApolloAIBlueprintLibrary|GetPerceptionSenseConfig (AI|GetAIController (.HitActor (Collision|BreakHitResult _outhit))) "/Script/AIModule.AISense_Sight")
          (:Is%20Valid
            (bind _returnvalue (Class|ApolloAIBlueprintLibrary|SetSightRange (AI|GetAIController (.HitActor (Collision|BreakHitResult _outhit))) 5e+01))
            (if _returnvalue
              (Development|PrintString "Modified Sight Range!")
              (else
                (Utilities|FlowControl|Delay 2.0)
                (Class|BPIEnemy|OnResetSight(Message) (AI|GetAIController (.HitActor (Collision|BreakHitResult _outhit))))))))))))

(event EventBeginPlay
  (|CallParentFunction)
  (Variables|Default|SetbIsActivated? false))

(event Collision|EventActorBeginOverlap
  (params (OtherActor :type Actor%20Object%20Reference))
  (|CallParentFunction OtherActor) ; This node is disabled and will not be called.\nDrag off pins to build functionality.
)

(event EventTick
  (params (DeltaSeconds :type Float%20%28single-precision%29))
  (|CallParentFunction DeltaSeconds))

(event EventExplode
  (|CallParentFunction)
  (Utilities|FlowControl|RetriggerableDelay 1.0)
  (Effects|SpawnEmitteratLocation "/Game/CheekyFPS/External/StarterContent/Particles/P_Smoke.P_Smoke" (Variables|Default|GetHitPoint) (Transformation|GetActorRotation) "3.000000,3.000000,3.000000")
  (Utilities|Time|SetTimerbyEvent (EventDispatchers|CreateEvent :!event Custom|TraceForTargets) 0.5 true)
  (Actor|SetLifeSpan 12.0))

(fn ConstructionScript
  (|CallParentFunction))