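; Throwable grenade item that spawns an explosion effect and defines radial damage.
; When its health component reports death, Explode spawns a scaled-up emitter at the hit point, using a flag so it only fires once.
; DealRadialDamage applies falloff damage around the grenade, crediting the instigator's controller, but nothing in this graph calls it.
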(event OnThingDead(CheekyHealthComponent)
  (CallFunction|Explode))

(event EventBeginPlay
  (|CallParentFunction))

(event Collision|EventActorBeginOverlap
  (params (OtherActor :type Actor%20Object%20Reference))
  (|CallParentFunction OtherActor) ; This node is disabled and will not be called.\nDrag off pins to build functionality.
)

(event EventTick
  (params (DeltaSeconds :type Float%20%28single-precision%29))
  (|CallParentFunction DeltaSeconds) ; This node is disabled and will not be called.\nDrag off pins to build functionality.
)

(fn ConstructionScript
  (|CallParentFunction))

(fn Explode
  (if (not (Variables|Default|GetbSpawnVFX?))
    (Effects|SpawnEmitteratLocation (Variables|Feedback|GetExplosionFX) (Variables|Default|GetHitPoint) (Transformation|GetActorRotation) "3.000000,3.000000,3.000000")
    (Variables|Default|SetbSpawnVFX? true)))

(fn DealRadialDamage
  (Class|GameplayStatics|ApplyRadialDamagewithFalloff (Variables|Damage|GetBaseDamage) (Variables|Damage|GetMinimumDamage) (Transformation|GetActorLocation) (Variables|Radius|GetMaximumDamageRadius) (Variables|Radius|GetMinimumDamageRadius) 1.0 (Variables|Type|GetGrenadeDamageType) 0 self (Game|GetInstigatorController) "ECC_Visibility"))