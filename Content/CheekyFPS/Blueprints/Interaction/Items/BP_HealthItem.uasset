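; BP_HealthItem is an inventory item that heals the player when activated.
; ActivateItem gets player 0's CheekyCharacter, adds RecoverAmount to its HealthComponent and fires the health update notification with the new current HP.
; It then removes itself from the character's InventoryComponent.
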(event EventBeginPlay
  (|CallParentFunction) ; This node is disabled and will not be called.\nDrag off pins to build functionality.
)

(event Collision|EventActorBeginOverlap
  (params (OtherActor :type Actor%20Object%20Reference))
  (|CallParentFunction OtherActor) ; This node is disabled and will not be called.\nDrag off pins to build functionality.
)

(event EventTick
  (params (DeltaSeconds :type Float%20%28single-precision%29))
  (|CallParentFunction DeltaSeconds) ; This node is disabled and will not be called.\nDrag off pins to build functionality.
)

(event EventActivateItem
  (bind _returnvalue (Game|GetPlayerCharacter 0))
  (bind _ascheeky_character (Utilities|Casting|CastToCheekyCharacter _returnvalue))
  (bind _healthcomponent (Variables|/Game/CheekyFPS/Blueprints/CheekyCharacter.CheekyCharacter_C|GetHealthComponent _ascheeky_character))
  (Default|AddHealth _healthcomponent (Variables|Default|GetRecoverAmount))
  (Default|CallOnUpdateHealth _healthcomponent (.CurrentHP (Default|GetHealth _healthcomponent)))
  (Default|RemoveItem (Variables|/Game/CheekyFPS/Blueprints/CheekyCharacter.CheekyCharacter_C|GetInventoryComponent _ascheeky_character) self))

(fn ConstructionScript
  (|CallParentFunction))