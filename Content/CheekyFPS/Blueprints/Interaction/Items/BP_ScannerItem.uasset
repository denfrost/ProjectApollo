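; BP_ScannerItem is an interaction item that switches a sonar effect on and off.
; ActivateItem runs the parent logic, flips IsItemActive and sends the new state through ToggleSonarEffectMessage to the game state and player character 0.
; Switching off also fires the OnDeactivated dispatcher, while switching on has no matching call.
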(event EventBeginPlay
  (|CallParentFunction) ; This node is disabled and will not be called.\nDrag off pins to build functionality.
)

(event Collision|EventActorBeginOverlap
  (params (OtherActor :type Actor%20Object%20Reference))
  (|CallParentFunction OtherActor) ; This node is disabled and will not be called.\nDrag off pins to build functionality.
)

(event EventTick
  (params (DeltaSeconds :type Float%20%28single-precision%29))
  (|CallParentFunction DeltaSeconds) ; This node is disabled and will not be called.\nDrag off pins to build functionality.
)

(event EventActivateItem
  (bind _returnvalue (Game|GetGameState))
  (bind _returnvalue_2 (Game|GetPlayerCharacter 0))
  (|CallParentFunction)
  (if (Variables|Default|GetIsItemActive?)
    (bind _output_get (Variables|Default|SetIsItemActive? false))
    (Class|BPIChameleon|ToggleSonarEffect?(Message) _returnvalue _output_get)
    (Class|BPIChameleon|ToggleSonarEffect?(Message) _returnvalue_2 _output_get)
    (Default|CallOnDeactivated)
    (else
      (bind _output_get_2 (Variables|Default|SetIsItemActive? true))
      (Class|BPIChameleon|ToggleSonarEffect?(Message) _returnvalue _output_get_2)
      (Class|BPIChameleon|ToggleSonarEffect?(Message) _returnvalue_2 _output_get_2))))

(fn ConstructionScript
  (|CallParentFunction))