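; BP_DistractionItem is an item actor that, when activated, places a copy of itself near the player as a distraction.
; ActivateItem spawns a new BP_DistractionItem from the player pawn's transform, offset along world X rather than the pawn's forward vector.
; It then immediately starts an interaction on the new actor's CheekyInteractComponent.
; The actor has no other active logic.
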(event EventBeginPlay
  (|CallParentFunction) ; This node is disabled and will not be called.\nDrag off pins to build functionality.
)

(event Collision|EventActorBeginOverlap
  (params (OtherActor :type Actor%20Object%20Reference))
  (|CallParentFunction OtherActor) ; This node is disabled and will not be called.\nDrag off pins to build functionality.
)

(event EventTick
  (params (DeltaSeconds :type Float%20%28single-precision%29))
  (|CallParentFunction DeltaSeconds) ; This node is disabled and will not be called.\nDrag off pins to build functionality.
)

(event EventActivateItem
  (bind _returnvalue (Game|Player|GetPlayerPawn 0))
  (bind _returnvalue_2 (Transformation|GetActorTransform _returnvalue))
  (bind _returnvalue_3 (Game|SpawnActorfromClass "BP_DistractionItem_C" (Math|Transform|MakeTransform (+ (.location _returnvalue_2) "100.000000, 0, 0") (.rotation _returnvalue_2) (.scale _returnvalue_2)) "Undefined" 0 0))
  (Default|Interaction (Variables|/Game/CheekyFPS/Blueprints/Interaction/Items/BP_ThrowableItem_Base.BP_ThrowableItem_Base_C|GetCheekyInteractComponent _returnvalue_3) true "NewEnumerator0"))

(fn ConstructionScript
  (|CallParentFunction))