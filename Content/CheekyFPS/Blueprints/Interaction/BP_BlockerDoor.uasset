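; BP_BlockerDoor is a toggleable barrier with particle effects and sound that hurts and repels the player on contact.
; A box hit by the player applies a small fixed damage and launches them opposite their facing direction with a velocity-change impulse.
; ToggleVisibility switches collision, both particle systems and audio together.
; The construction script applies it from IsEnabled, while BeginPlay always stops the audio.
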(event OnComponentHit(Box)
  (params (HitComponent :type Primitive%20Component%20Object%20Reference) (OtherActor :type Actor%20Object%20Reference) (OtherComp :type Primitive%20Component%20Object%20Reference) (NormalImpulse :type Vector :default "0, 0, 0") (Hit :type Hit%20Result%20Structure%20%28by%20ref%29))
  (bind _returnvalue (Game|GetPlayerCharacter 0))
  (if (== OtherActor _returnvalue)
    (Game|Damage|ApplyDamage (Game|Player|GetPlayerPawn 0) 5.0 0 self "/Game/CheekyFPS/Blueprints/Weapons/DamageTypes/BP_StandardDamageType.BP_StandardDamageType_C")
    (Physics|AddImpulse (Variables|/Script/Engine.Character|GetCharacterMovement _returnvalue) (* (Math|Vector|NegateVector (Math|Vector|GetForwardVector (Transformation|GetActorRotation _returnvalue))) 8e+03) true)))

(event EventBeginPlay
  (Audio|Components|Audio|Stop (Variables|Default|GetAudio)))

(event Collision|EventActorBeginOverlap
  (params (OtherActor :type Actor%20Object%20Reference)))

(fn ConstructionScript
  (CallFunction|ToggleVisibility (Variables|Default|GetbIsEnabled?)))

(fn ToggleVisibility
  (params (ToggleStatus :type Boolean))
  (bind _box (Variables|Default|GetBox))
  (if ToggleStatus
    (Variables|Default|SetbIsEnabled? true)
    (Collision|SetCollisionEnabled _box "QueryAndPhysics")
    (Rendering|SetVisibility (Variables|Default|GetParticleSystem) true true)
    (Audio|Components|Audio|Play (Variables|Default|GetAudio) 0.0)
    (else
      (Variables|Default|SetbIsEnabled? false)
      (Collision|SetCollisionEnabled _box "NoCollision")
      (Rendering|SetVisibility (Variables|Default|GetParticleSystem) false true)
      (Audio|Components|Audio|Stop (Variables|Default|GetAudio)))))