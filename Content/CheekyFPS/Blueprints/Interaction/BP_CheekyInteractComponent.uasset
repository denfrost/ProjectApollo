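; BP_CheekyInteractComponent is an interaction component that holds interactable state and relays selection, interaction, hold and message changes through event dispatchers.
; Setter functions store the selected, interacting and message values and fire matching begin, end or update dispatchers, passing along interaction type or hold success.
; Hold progress is broadcast as the supplied timer divided by HoldTime, so the component does no timing or ticking itself.
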(event EventBeginPlay)

(event EventTick
  (params (DeltaSeconds :type Float%20%28single-precision%29)))

(fn IsEnabled?
  (return (Variables|Default|GetbEnabled)))

(fn SetSelected
  (params (bIsSelected :type Boolean))
  (bind _output_get (Variables|Runtime|SetbIsSelected bIsSelected))
  (if _output_get
    (Default|CallOnBeginSelected)
    (else
      (Default|CallOnEndSelection)))
  (return))

(fn Interaction
  (params (bStart :type Boolean) (InteractionType :type EInteractionTypes%20Enum :default "NewEnumerator0"))
  (if bStart
    (Default|CallOnBeginInteraction InteractionType)
    (Variables|Runtime|SetbIsBeingInteractedWith true)
    (return)
    (else
      (Default|CallOnEndInteraction InteractionType)
      (Variables|Runtime|SetbIsBeingInteractedWith false)
      (return))))

(fn UpdateMessage
  (params (MessageText :type Text))
  (bind _output_get (Variables|Default|SetMessageText MessageText))
  (Default|CallOnMessageUpdated _output_get)
  (return))

(fn UpdateHoldState
  (params (bBegin :type Boolean) (bSuccessful :type Boolean))
  (if bBegin
    (Default|CallOnBeginHold)
    (else
      (Default|CallOnEndHold bSuccessful)))
  (return))

(fn UpdateHoldProgress
  (params (Timer :type Float%20%28single-precision%29))
  (Default|CallOnHoldUpdate (/ Timer (Variables|HoldInteraction|GetHoldTime)))
  (return))