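; Level streaming trigger actor that loads or unloads a named level as the player crosses its box.
; The LoadNewLevel flag sets its role: load on entering the box, or unload on leaving it.
; Each action fires a loaded or unloaded dispatcher.
; BeginPlay binds to the unloaded dispatcher, and a ClearSpawnersOnUnload event messages the GameState to clear spawners.
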(event OnComponentBeginOverlap(Box)
  (params (OverlappedComponent :type Primitive%20Component%20Object%20Reference) (OtherActor :type Actor%20Object%20Reference) (OtherComp :type Primitive%20Component%20Object%20Reference) (OtherBodyIndex :type Integer) (bFromSweep :type Boolean) (SweepResult :type Hit%20Result%20Structure%20%28by%20ref%29))
  (if (CallFunction|PlayerCollisionCheck OtherActor OtherComp)
    (if (Variables|Settings|GetbLoadNewLevel?)
      (Game|LoadStreamLevel(byName) (Variables|Settings|GetNewLevelName) (Variables|Settings|GetbMake%20Visible%20After%20Load?) (Variables|Settings|GetShould%20Block%20on%20Load?))
      (Default|CallOnNewLevelLoaded))))

(event OnComponentEndOverlap(Box)
  (params (OverlappedComponent :type Primitive%20Component%20Object%20Reference) (OtherActor :type Actor%20Object%20Reference) (OtherComp :type Primitive%20Component%20Object%20Reference) (OtherBodyIndex :type Integer))
  (if (CallFunction|PlayerCollisionCheck OtherActor OtherComp)
    (if (not (Variables|Settings|GetbLoadNewLevel?))
      (Game|UnloadStreamLevel(byName) (Variables|Settings|GetNewLevelName) false)
      (Default|CallOnNewLevelUnloaded))))

(event Custom|ClearSpawnersOnUnload
  (Class|BPIGameEvents|ClearSpawners(Message) (Game|GetGameState)))

(event EventBeginPlay
  (EventDispatchers|BindEventtoOnNewLevelUnloaded (EventDispatchers|CreateEvent :!event Custom|ClearSpawnersOnUnload)))

(event Collision|EventActorBeginOverlap
  (params (OtherActor :type Actor%20Object%20Reference)))

(event EventTick
  (params (DeltaSeconds :type Float%20%28single-precision%29)))

(fn ConstructionScript)