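; BP_Elevator is an elevator actor that moves between floors using an InterpToMovement component.
; Up and down events restart that movement as OneShot or OneShotReverse and call OnElevatorActivated.
; When the player character overlaps the Box while IsActive is set, it moves up and sweeps the player to the Scene component's location.
; ToggleElevatorStatus sets IsActive, and logic for building control points from actor location is left unconnected.
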(event OnComponentBeginOverlap(Box)
  (params (OverlappedComponent :type Primitive%20Component%20Object%20Reference) (OtherActor :type Actor%20Object%20Reference) (OtherComp :type Primitive%20Component%20Object%20Reference) (OtherBodyIndex :type Integer) (bFromSweep :type Boolean) (SweepResult :type Hit%20Result%20Structure%20%28by%20ref%29))
  (bind _returnvalue (Game|GetPlayerCharacter 0))
  (if (== OtherActor _returnvalue)
    (if (Variables|Default|GetbIsActive?)
      (CallFunction|MovetoNextFloor)
      (Transformation|SetActorLocation _returnvalue (Transformation|GetWorldLocation (Variables|Default|GetScene)) true false))))

(event EventBeginPlay)

(event EventTick
  (params (DeltaSeconds :type Float%20%28single-precision%29)))

(event EventMoveElevatorDown
  (CallFunction|MovetoPreviousFloor))

(event EventMoveElevatorUp
  (CallFunction|MovetoNextFloor))

(event EventToggleElevatorStatus
  (params (isActive? :type Boolean))
  (Variables|Default|SetbIsActive? isActive?))

(fn ConstructionScript)

(fn MovetoNextFloor
  (bind _interptomovement (Variables|Default|GetInterpToMovement))
  (Components|Activation|SetActive _interptomovement true true)
  (Class|InterptoMovementComponent|RestartMovement _interptomovement 1.0)
  (Variables|/Script/Engine.InterpToMovementComponent|SetBehaviourType _interptomovement "OneShot")
  (Default|CallOnElevatorActivated))

(fn MovetoPreviousFloor
  (bind _interptomovement (Variables|Default|GetInterpToMovement))
  (Components|Activation|SetActive (Variables|Default|GetInterpToMovement) true true)
  (Class|InterptoMovementComponent|RestartMovement _interptomovement 1.0)
  (Variables|/Script/Engine.InterpToMovementComponent|SetBehaviourType _interptomovement "OneShot_Reverse")
  (Default|CallOnElevatorActivated))