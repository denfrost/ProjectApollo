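; Base interactive door that opens, closes, locks and jiggles when locked, starting locked if it requires a key card level.
; Debounced interaction checks the player's key card for an exact level match, while incoming name signals can also drive open and lock states.
; Timelines animate it, with swing direction from a player-facing dot product, and opening or closing sends outgoing signals.
; RamaSave load replays opening for doors saved open.
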(event OnBeginInteraction(CheekyInteractComponent)
  (params (Type :type EInteractionTypes%20Enum :default "NewEnumerator0"))
  (bind _returnvalue (Game|GetPlayerCharacter 0))
  (bind _ascheeky_character (Utilities|Casting|CastToCheekyCharacter _returnvalue))
  (bind _inventorycomponent (Variables|/Game/CheekyFPS/Blueprints/CheekyCharacter.CheekyCharacter_C|GetInventoryComponent _ascheeky_character))
  (bind _currentkeycard (Variables|/Game/CheekyFPS/Blueprints/Components/InventoryComponent.InventoryComponent_C|GetCurrentKeyCard _inventorycomponent))
  ;[0.2158 1 0.0831] Interaction
  (Utilities|FlowControl|DoOnce false ; Stops the player spamming inputs
    (:Completed
      (Utilities|FlowControl|Sequence
        (:then_0
          (if (Variables|Default|GetbDoorIsLocked)
            (Utilities|IsValid _currentkeycard
              (:Is%20Valid
                (CallFunction|AttemptDoorUnlock (Variables|/Game/CheekyFPS/Blueprints/Interaction/Items/BP_KeyItem.BP_KeyItem_C|GetCurrentLevel _currentkeycard))))))
        (:then_1
          (if (and (Variables|Default|GetbDoorIsLocked) (not (Variables|Default|GetbDoorIsOpen)))
            ;[0.3135 0.1534 1] Door locked
            (CallFunction|LockedJiggle)
            (CallFunction|UpdateMessage)
            (CallFunction|ResetDelay)
            (else
              ;[1 0.004513 0.2253] Open / Close door
              (if (Variables|Default|GetbDoorIsOpen)
                (CallFunction|CloseDoor)
                (else
                  (CallFunction|OpenDoor)))
              (CallFunction|ResetDelay))))))))

(event OnNameSignal(SignalTranscieverComponent)
  (params (Sender :type Actor%20Object%20Reference) (ReceivedName :type Name :default "None"))
  ;[0.02832 1 0] Name Signals
  (switch name ReceivedName
    (:Default
      (if (Variables|Default|GetbDoorIsOpen) :!label _label
        (if (Variables|Default|GetbDoorIsOpen) :!label _label_2 ; Don't try and close the door\nif it's already closed...
          (CallFunction|CloseDoor))
        (else
          (if (Variables|Default|GetbDoorIsLocked) :!label _label_3
            (CallFunction|LockedJiggle)
            (else
              (CallFunction|OpenDoor))))))
    (:Open
      (goto _label_3))
    (:Close
      (goto _label_2))
    (:Toggle
      (goto _label))
    (:Lock
      (CallFunction|LockToggle true))
    (:Unlock
      (CallFunction|LockToggle false))
    (:ToggleLock
      (CallFunction|LockToggle (not (Variables|Default|GetbDoorIsLocked))))))

(event Custom|ResetDelay
  (bind _returnvalue (Game|GetPlayerCharacter 0))
  (bind _ascheeky_character (Utilities|Casting|CastToCheekyCharacter _returnvalue))
  (bind _inventorycomponent (Variables|/Game/CheekyFPS/Blueprints/CheekyCharacter.CheekyCharacter_C|GetInventoryComponent _ascheeky_character))
  (bind _currentkeycard (Variables|/Game/CheekyFPS/Blueprints/Components/InventoryComponent.InventoryComponent_C|GetCurrentKeyCard _inventorycomponent))
  (Utilities|FlowControl|Delay 0.3)
  (Utilities|FlowControl|DoOnce false) ; enters at Reset
)

(event EventAttemptDoorUnlock
  (params (CurrentKeyCardLevel :type EKeyCardLevel%20Enum :default "NewEnumerator6"))
  (bind _output_get (Variables|Default|SetIncomingCardLevel CurrentKeyCardLevel))
  (CallFunction|UnlockDoor(WithKey) _output_get))

(event EventBeginPlay
  (EventDispatchers|BindEventtoOnDoorUnlock (EventDispatchers|CreateEvent :!event UnlockDoor(WithoutKey))))

(event RamaSaveEventActorFullyLoaded(RamaSave)
  (params (RamaSaveComponent :type Rama%20Save%20Component%20Object%20Reference) (LevelPackageName :type String))
  (Utilities|FlowControl|Sequence
    (:then_0
      (if (Variables|Default|GetbDoorIsOpen)
        (CallFunction|AttemptDoorOpen)))
    (:then_1
      (bind _returnvalue (Game|GetCurrentLevelName true)))))

(event Custom|LockedJiggle
  ;[1 0.463 0] Locked Jiggle
  (Audio|SpawnSoundAttached (Variables|Sounds|GetLockedRattleSound) (Variables|Default|GetDoor) "None" "100.000000, 0,100.000000" "0, 0, 0" "KeepRelativeOffset" false 1.0 1.0 0.0 0 0)
  (bind _jiggleanim (Timeline|JiggleTimeline PlayFromStart)
    (:Update
      (Transformation|SetRelativeRotation (Variables|Default|GetDoor) (Math|Rotator|MakeRotator 0.0 0.0 (* _jiggleanim 2.0)) false false))))

(event Custom|OpenDoor
  (bind _movesound (Variables|Sounds|GetMoveSound))
  ;[0 1 0.1847] Open Door
  (Audio|SpawnSoundAttached _movesound (Variables|Default|GetDoor) "None" "0, 0,100.000000" "0, 0, 0" "KeepRelativeOffset" false 1.0 (/ (Variables|/Script/Engine.SoundBase|GetDuration _movesound) (Variables|Default|GetCloseSpeed)) 0.0 0 0) ; Movement sound
  (Audio|SpawnSoundAttached (Variables|Sounds|GetOpenSound) (Variables|Default|GetDoor) "None" "100.000000, 0,100.000000" "0, 0, 0" "KeepRelativeOffset" false 1.0 1.0 0.0 0 0) ; Open sound
  (CallFunction|SetTimelineDuration (Variables|Default|GetDoorTimeline) (Variables|Default|GetOpenSpeed))
  (Default|SendNameArray (Variables|Default|GetSignalTranscieverComponent) (Variables|Signals|GetOpenSignals))
  (bind _bopeningforwards (CallFunction|DeterminePlayerDirection))
  (Variables|Default|SetbDoorOpenForwards _bopeningforwards)
  (Audio|Components|Audio|Play (Variables|Default|GetDoorTimeline)))

(event Custom|CloseDoor
  (bind _movesound (Variables|Sounds|GetMoveSound))
  ;[1 0.1159 0] Close Door
  (Audio|SpawnSoundAttached _movesound (Variables|Default|GetDoor) "None" "0, 0,100.000000" "0, 0, 0" "KeepRelativeOffset" false 1.0 (/ (Variables|/Script/Engine.SoundBase|GetDuration _movesound) (Variables|Default|GetCloseSpeed)) 0.0 0 0) ; Movement sound
  (CallFunction|SetTimelineDuration (Variables|Default|GetDoorTimeline) (Variables|Default|GetCloseSpeed))
  (Default|SendNameArray (Variables|Default|GetSignalTranscieverComponent) (Variables|Signals|GetCloseSignals))
  (Utilities|String|Reverse (Variables|Default|GetDoorTimeline)))

(event Custom|LockToggle
  (params (bLock :type Boolean))
  ;[1 0 0.3133] Toggle Lock State
  (Audio|SpawnSoundAttached (select bLock (Variables|Sounds|GetLockSound) (Variables|Sounds|GetUnlockSound)) (Variables|Default|GetDoor) "None" "100.000000, 0,100.000000" "0, 0, 0" "KeepRelativeOffset" false 1.0 1.0 0.0 0 0)
  (Variables|Default|SetbDoorIsLocked bLock))

(event EventAttemptDoorOpen
  (bind _movesound (Variables|Sounds|GetMoveSound))
  ;[0 1 0.1847] Open Door
  (Audio|SpawnSoundAttached _movesound (Variables|Default|GetDoor) "None" "0, 0,100.000000" "0, 0, 0" "KeepRelativeOffset" false 1.0 (/ (Variables|/Script/Engine.SoundBase|GetDuration _movesound) (Variables|Default|GetCloseSpeed)) 0.0 0 0) ; Movement sound
  (Audio|SpawnSoundAttached (Variables|Sounds|GetOpenSound) (Variables|Default|GetDoor) "None" "100.000000, 0,100.000000" "0, 0, 0" "KeepRelativeOffset" false 1.0 1.0 0.0 0 0) ; Open sound
  (CallFunction|SetTimelineDuration (Variables|Default|GetDoorTimeline) (Variables|Default|GetOpenSpeed))
  (Default|SendNameArray (Variables|Default|GetSignalTranscieverComponent) (Variables|Signals|GetOpenSignals))
  (bind _bopeningforwards (CallFunction|DeterminePlayerDirection))
  (Variables|Default|SetbDoorOpenForwards _bopeningforwards)
  (Audio|Components|Audio|Play (Variables|Default|GetDoorTimeline)))

(fn ConstructionScript
  (CallFunction|UpdateMessage)
  (if (Utilities|Enum|NotEqual(Enum) (Variables|Default|GetRequiredCardLevel) "NewEnumerator0")
    (Variables|Default|SetbDoorIsLocked true)))

(fn UpdateMessage
  (Default|UpdateMessage (Variables|Default|GetCheekyInteractComponent) (select (Variables|Default|GetbDoorIsLocked) (Utilities|Select :Index (Math|Random|RandomInteger 4) :Option%200 "It's Locked" :Option%201 "Won't Budge" :Option%202 "Can't Open It" :Option%203 "Jammed") (select (Variables|Default|GetbDoorIsOpen) "Close Door" "Open Door")))
  (return))

(fn DeterminePlayerDirection
  (return (> (Math|Vector|DotProduct (Math|Vector|GetForwardVector (Transformation|GetWorldRotation (Variables|Default|GetArrow))) (Math|Vector|GetForwardVector (Transformation|GetWorldRotation (Variables|/Script/Engine.Actor|GetRootComponent (Game|GetPlayerCharacter 0))))) 0.0)))

(fn UnlockDoor(WithKey)
  (params (InputCardLevel :type EKeyCardLevel%20Enum :default "NewEnumerator0"))
  (if (Utilities|Enum|Equal(Enum) InputCardLevel (Variables|Default|GetRequiredCardLevel))
    (Variables|Default|SetbDoorIsLocked false)
    (if (Variables|Default|GetbDoorIsOpen)
      (CallFunction|CloseDoor)
      (else
        (CallFunction|OpenDoor)))
    (CallFunction|ResetDelay)
    (Default|UpdateMessage (Variables|Default|GetCheekyInteractComponent) "Door Unlocked!")
    (else
      (Variables|Default|SetbDoorIsLocked true)
      (CallFunction|LockedJiggle)
      (CallFunction|UpdateMessage)
      (CallFunction|ResetDelay)
      (Utilities|FlowControl|Sequence
        (:then_0
          (if (or (Utilities|Enum|Equal(Enum) InputCardLevel "NewEnumerator6") (Utilities|Enum|Equal(Enum) InputCardLevel "NewEnumerator0"))
            (Development|PrintString "Player does not have a key!" true true "(R=1.000000,G=0.000000,B=0.000000,A=1.000000)")))
        (:then_1
          (Development|PrintString "And/Or Player 's key card is not the correct level!" true true "(R=1.000000,G=0.161888,B=0.000000,A=1.000000)"))))))

(fn FinishEvent
  (params (Selection :type ETimelineDirection%20Enum :default "Forward"))
  (switch Utilities|FlowControl|Switch|SwitchonETimelineDirection Selection
    (:Forward
      (Variables|Default|SetbDoorIsOpen true))
    (:Backward
      (Variables|Default|SetbDoorIsOpen false)
      (Audio|SpawnSoundAttached (Variables|Sounds|GetCloseSound) (Variables|Default|GetDoor) "None" "100.000000, 0,100.000000" "0, 0, 0" "KeepRelativeOffset" false 1.0 1.0 0.0 0 0)))
  (CallFunction|UpdateMessage))

(fn UnlockDoor(WithoutKey)
  (if (Variables|Default|GetbDoorIsLocked)
    (Variables|Default|SetbDoorIsLocked false)
    (if (Variables|Default|GetbDoorIsOpen)
      (CallFunction|CloseDoor)
      (else
        (CallFunction|OpenDoor)))
    (CallFunction|ResetDelay)
    (Default|UpdateMessage (Variables|Default|GetCheekyInteractComponent) "Door Unlocked!")
    (else
      (Variables|Default|SetbDoorIsLocked true)
      (CallFunction|LockedJiggle)
      (CallFunction|UpdateMessage)
      (CallFunction|ResetDelay))))