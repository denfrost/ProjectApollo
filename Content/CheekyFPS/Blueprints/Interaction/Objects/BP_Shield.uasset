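; BP_Shield is a shield actor with health that reflects damage visually and switches off when depleted.
; Each tick it feeds current HP into the emissive power of a dynamic material on StaticMesh1, and sets both meshes to a fixed world scale below half health.
; When CheekyHealthComponent reports death, it hides the actor and disables collision on both meshes instead of destroying it.
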(event OnThingDead(CheekyHealthComponent)
  (Rendering|SetActorHiddenInGame true)
  (Collision|SetCollisionEnabled (Variables|Default|GetStaticMesh) "NoCollision"))

(event EventBeginPlay
  (bind _staticmesh1 (Variables|Default|GetStaticMesh1))
  (bind _returnvalue (Rendering|Material|CreateDynamicMaterialInstance _staticmesh1 0 (Rendering|Material|GetMaterial _staticmesh1 0) "None" :!class /Script/Engine.PrimitiveComponent))
  (Variables|Default|SetSparksMI _returnvalue))

(event Collision|EventActorBeginOverlap
  (params (OtherActor :type Actor%20Object%20Reference)))

(event EventTick
  (params (DeltaSeconds :type Float%20%28single-precision%29))
  (bind _cheekyhealthcomponent (Variables|Default|GetCheekyHealthComponent))
  (Rendering|Material|SetScalarParameterValue (Variables|Default|GetSparksMI) "EmissivePower" (.CurrentHP (Default|GetHealth _cheekyhealthcomponent)) :!class /Script/Engine.MaterialInstanceDynamic)
  (if (< (Default|GetHealthPercentage _cheekyhealthcomponent) 0.5)
    (Transformation|SetWorldScale3D (Variables|Default|GetStaticMesh) "4.000000,4.000000,4.000000")))

(fn ConstructionScript)