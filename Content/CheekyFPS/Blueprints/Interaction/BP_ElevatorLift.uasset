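; Interactable elevator actor with two swinging doors that open and close as the player enters or leaves a trigger.
; Tick steps door yaw and raises the lift to a target Z, reopening the doors after arrival.
; Interaction toggles movement and can stream in a level, while ToggleElevatorStatus sets power and unlocks it, refreshing the prompt.
; MoveToFloor maps floors to heights but is uncalled here, and the MoveReady Tick branch does nothing.
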(event OnBeginInteraction(CheekyInteractComponent)
  (params (Type :type EInteractionTypes%20Enum :default "NewEnumerator0"))
  (bind _newlevelname (Variables|Default|GetNewLevelName))
  (CallFunction|UpdateMessage)
  (if (Variables|Default|GetisActive?)
    (if (Utilities|Name|NotEqual(Name) _newlevelname "None")
      (Game|LoadStreamLevel(byName) _newlevelname true true))
    (Variables|Default|SetMove (not (Variables|Default|GetMove)))))

(event OnComponentBeginOverlap(MoveCollision)
  (params (OverlappedComponent :type Primitive%20Component%20Object%20Reference) (OtherActor :type Actor%20Object%20Reference) (OtherComp :type Primitive%20Component%20Object%20Reference) (OtherBodyIndex :type Integer) (bFromSweep :type Boolean) (SweepResult :type Hit%20Result%20Structure%20%28by%20ref%29))
  (if (== OtherActor (Game|GetPlayerCharacter 0))
    (if (Variables|Default|GetisActive?)
      (Variables|Default|SetMoveReady true))))

(event OnComponentEndOverlap(Collision)
  (params (OverlappedComponent :type Primitive%20Component%20Object%20Reference) (OtherActor :type Actor%20Object%20Reference) (OtherComp :type Primitive%20Component%20Object%20Reference) (OtherBodyIndex :type Integer))
  ;[1 1 1] AutoOpenAndColseDoor
  (if (== OtherActor (Game|GetPlayerCharacter 0))
    (Variables|Default|SetAutoClose true)
    (Variables|Default|SetAutoOpen false)
    (Variables|Default|SetbDoorIsOpen false)))

(event OnComponentBeginOverlap(Collision)
  (params (OverlappedComponent :type Primitive%20Component%20Object%20Reference) (OtherActor :type Actor%20Object%20Reference) (OtherComp :type Primitive%20Component%20Object%20Reference) (OtherBodyIndex :type Integer) (bFromSweep :type Boolean) (SweepResult :type Hit%20Result%20Structure%20%28by%20ref%29))
  ;[1 1 1] AutoOpenAndColseDoor
  (if (== OtherActor (Game|GetPlayerCharacter 0))
    (if (Variables|Default|GetisActive?)
      (Variables|Default|SetAutoClose false)
      (Variables|Default|SetAutoOpen true))))

(event EventBeginPlay
  (Variables|Default|SetMoveVector_Z (.z (Variables|Default|GetMoveVector))))

(event EventToggleElevatorStatus
  (params (isActive? :type Boolean))
  (bind _output_get (Variables|Default|SetisActive? isActive?))
  (Variables|Default|SetbDoorIsLocked false)
  (CallFunction|UpdateMessage))

(event EventTick
  (params (DeltaSeconds :type Float%20%28single-precision%29))
  (if (Variables|Default|GetisActive?)
    (Utilities|FlowControl|Sequence
      (:then_0
        ;[1 1 1] AutoOpenAndColseDoor
        (if (Variables|Default|GetAutoDoor)
          (if (Variables|Default|GetAutoOpen)
            (Math|Float|CompareFloat (Variables|Default|GetDoorPosition) 27.0
              (:>
                (Variables|Default|SetDoorPosition 27.0 :!label _label)
                (Variables|Default|SetAutoOpen false))
              (:==
                (goto _label))
              (:<
                (Variables|Default|SetDoorPosition (+ (Variables|Default|GetDoorPosition) 0.5))
                (Transformation|SetRelativeRotation (Variables|Default|GetLift02Door02) (Math|Rotator|MakeRotator 0.0 0.0 (Variables|Default|GetDoorPosition)) false false :!label _label_2)
                (Transformation|SetRelativeRotation (Variables|Default|GetLift02Door01) (Math|Rotator|MakeRotator 0.0 0.0 (* (Variables|Default|GetDoorPosition) -1.0)) false false)
                (Variables|Default|SetbDoorIsOpen true)))
            (elif (Variables|Default|GetAutoClose)
              (Math|Float|CompareFloat (Variables|Default|GetDoorPosition) 0.0
                (:>
                  (Variables|Default|SetDoorPosition (- (Variables|Default|GetDoorPosition) 0.5))
                  (goto _label_2))
                (:==
                  _)
                (:<
                  _))
              (Variables|Default|SetDoorPosition 0.0)
              (Variables|Default|SetAutoClose false)))))
      (:then_1
        (if (not (Variables|Default|GetAutoOpen))
          (if (not (Variables|Default|GetAutoClose))
            (if (Variables|Default|GetMoveReady)
              _))))
      (:then_2
        (if (Variables|Default|GetMove)
          (Math|Float|CompareFloat (Variables|Default|GetMovePosition) (Variables|Default|GetMoveVector_Z)
            (:>
              (Variables|Default|SetMovePosition (Variables|Default|GetMoveVector_Z) :!label _label_3)
              (Variables|Default|SetMove false)
              (Utilities|FlowControl|Delay 1.0)
              (Variables|Default|SetAutoOpen true)
              (Variables|Default|SetMoveReady false))
            (:==
              (goto _label_3))
            (:<
              (Variables|Default|SetMovePosition (+ (Variables|Default|GetMovePosition) 5.0))
              (Transformation|SetRelativeLocation (Variables|Default|GetLift02) (Math|Vector|MakeVector 0.0 0.0 (* (Variables|Default|GetMovePosition) 1.0)) false false)
              (Utilities|FlowControl|Delay 5.0)
              (Transformation|SetRelativeRotation (Variables|Default|GetLift02) (Math|Rotator|MakeRotator 0.0 0.0 (* (Variables|Default|GetMoveRotation_Z) 1.0)) false false))))))))

(fn ConstructionScript
  (bind _doorposition (Variables|Default|GetDoorPosition))
  (bind _lift02door01 (Variables|Default|GetLift02Door01))
  (Utilities|FlowControl|Sequence
    (:then_0
      (if (not (Variables|Default|GetisActive?))
        (Variables|Default|SetbDoorIsLocked true)))
    (:then_1
      ;[1 1 1] Movement
      (CallFunction|UpdateMessage)
      (Transformation|SetRelativeRotation (Variables|Default|GetLift02Door02) (Math|Rotator|MakeRotator 0.0 0.0 _doorposition) false false)
      (Transformation|SetRelativeRotation _lift02door01 (Math|Rotator|MakeRotator 0.0 0.0 (* _doorposition -1.0)) false false)
      ;[1 1 1] Material
      (Rendering|Material|SetMaterial _lift02door01 0 (Variables|Default|GetMaterial)))))

(fn UpdateMessage
  (Default|UpdateMessage (Variables|Default|GetCheekyInteractComponent) (select (Variables|Default|GetbDoorIsLocked) (Utilities|Select :Index (Math|Random|RandomInteger 4) :Option%200 "It's Locked" :Option%201 "Won't Budge" :Option%202 "Can't Open It" :Option%203 "Jammed") (select (Variables|Default|GetbDoorIsOpen) "Close Door" "Call Elevator")))
  (return))

(fn MovetoFloor
  (switch Utilities|FlowControl|Switch|SwitchonEElevatorLevels (Variables|Default|GetCurrentElevatorLevel)
    (:NewEnumerator0
      (Variables|Default|SetMoveVector_Z (Variables|Default|GetLevel0_ZPosition)))
    (:NewEnumerator2
      (Variables|Default|SetMoveVector_Z (Variables|Default|GetLevel1_ZPosition)))
    (:NewEnumerator3
      (Variables|Default|SetMoveVector_Z (Variables|Default|GetLevel2_ZPosition)))
    (:NewEnumerator4
      (Variables|Default|SetMoveVector_Z (Variables|Default|GetLevel3_ZPosition)))))