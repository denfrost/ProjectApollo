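; Mission endpoint trigger that shows the mission end screen when the player reaches it.
; A Box overlap passing PlayerCollisionCheck creates WBP_MissionEndScreen with WasSuccessful and hands it to the player controller through OnAddWidgetToViewportMessage.
; The construction script tints the particle system from Color, and BeginPlay debug-prints the game state's NextLevelName after a short delay.
; The game mode's CallOnMissionEnd call is disconnected and never runs.
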(event OnComponentBeginOverlap(Box)
  (params (OverlappedComponent :type Primitive%20Component%20Object%20Reference) (OtherActor :type Actor%20Object%20Reference) (OtherComp :type Primitive%20Component%20Object%20Reference) (OtherBodyIndex :type Integer) (bFromSweep :type Boolean) (SweepResult :type Hit%20Result%20Structure%20%28by%20ref%29))
  (if (CallFunction|PlayerCollisionCheck OtherActor OtherComp)
    (Development|PrintString "Hello")
    (bind _returnvalue (UserInterface|CreateWidget "/Game/CheekyFPS/Blueprints/UMG/Gameplay/Mission/WBP_MissionEndScreen.WBP_MissionEndScreen_C" 0 (Variables|Default|GetWas%20Successful?)))
    (Variables|Default|SetWBP _returnvalue)
    (Class|BPIPlayer|OnAddWidgettoViewport(Message) (Game|GetPlayerController 0) _returnvalue)))

(event EventBeginPlay
  (Utilities|FlowControl|Delay 1.0)
  (Development|PrintString (Variables|/Game/CheekyFPS/Blueprints/Game/ISSGameStateBase.ISSGameStateBase_C|GetNextLevelName (.AsISSGame%20State%20Base (Utilities|Casting|CastToISSGameStateBase (Game|GetGameState)))) true true "(R=1.000000,G=0.000000,B=0.000000,A=1.000000)"))

(event Collision|EventActorBeginOverlap
  (params (OtherActor :type Actor%20Object%20Reference)))

(event EventTick
  (params (DeltaSeconds :type Float%20%28single-precision%29)))

(fn ConstructionScript
  (Effects|Components|ParticleSystem|SetVectorParameter (Variables|Default|GetParticleSystem) "color" (Math|Conversions|ToVector(LinearColor) (Variables|Default|Getcolor))))