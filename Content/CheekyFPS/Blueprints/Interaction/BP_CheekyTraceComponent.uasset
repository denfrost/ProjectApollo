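; Trace component that detects and drives player interaction with actors carrying a BP_CheekyInteractComponent.
; A looping timer line-traces forward, selecting the enabled component hit, showing its message widget and ending holds or interactions when the target is lost.
; InteractInput starts either simple or timed hold interactions, with optional progress widget.
; Dispatchers report selection changes and player look/move locks set by the interacted component.
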(event Custom|TraceEvent
  ;[0 0.4442 1] Perform trace
  (Variables|Default|SetLastSelectedComponent (Variables|Default|GetCurrentSelectedComponent))
  (bind _result (CallFunction|LineTrace))
  (bind _output_get (Variables|Default|SetCurrentSelectedComponent _result))
  (Utilities|IsValid _output_get
    (:Is%20Valid
      (Variables|Default|SetbHasValidTarget true)
      (Utilities|IsValid (Variables|Default|GetLastSelectedComponent)
        (:Is%20Valid
          ;[0.01239 1 0.3792] If there was a different actor selected last, then deselect it first
          ; (If current = last, then we're still selecting the same actor, and don't need to do anything)
          (if (not (== (Variables|Default|GetCurrentSelectedComponent) (Variables|Default|GetLastSelectedComponent)))
            (Default|SetSelected (Variables|Default|GetLastSelectedComponent) false)
            ;[0 0.291 1 1 28] Select the new actor
            (Default|SetSelected (Variables|Default|GetCurrentSelectedComponent) true :!label _label)
            (Default|CallOnBeginSelection (Components|GetOwner (Variables|Default|GetCurrentSelectedComponent)))
            (Interface|AddMessageWidget (Variables|Default|GetCurrentSelectedComponent))))
        (:Is%20Not%20Valid
          (goto _label))))
    (:Is%20Not%20Valid
      ;[1 0.1254 0] Lost selection
      (Variables|Default|SetbHasValidTarget false)
      (Utilities|FlowControl|Sequence
        (:then_0
          (Utilities|IsValid (Variables|Default|GetLastSelectedComponent)
            (:Is%20Valid
              (Default|SetSelected (Variables|Default|GetLastSelectedComponent) false)
              (Default|CallOnLostSelection (Components|GetOwner (Variables|Default|GetLastSelectedComponent)))
              (Interface|ClearMessageWidget))))
        (:then_1
          ;[1 0 0.06703] Stop any hold progress
          (if (Variables|HoldInteraction|GetbIsInHoldWait)
            (HoldInteraction|EndHoldInput)))
        (:then_2
          ;[1 0.7589 0] Stop any remaining interaction
          (CallFunction|EndInteraction "NewEnumerator0"))))))

(event EventBeginPlay
  ;[0.1816 0.1744 1] Start trace event
  (Utilities|Time|SetTimerbyEvent (delegate Custom|TraceEvent) (Variables|Configuration|GetTraceInterval) true))

(fn LineTrace
  (bind _returnvalue (Transformation|GetWorldLocation))
  ;[1 0.0625 0.0625] Line Trace
  (bind (_outhit _returnvalue_2) (Collision|LineTraceByChannel _returnvalue (+ _returnvalue (* (Math|Vector|GetForwardVector) (Variables|Configuration|GetInteractionRange))) "TraceTypeQuery1" true (Utilities|Array|MakeArray (Components|GetOwner)) (select (Variables|Configuration|GetDrawDebugTrace) "ForDuration" "None") true "(R=1.000000,G=0.000000,B=0.000000,A=1.000000)" "(R=0.000000,G=1.000000,B=0.000000,A=1.000000)" 1.0))
  (if _returnvalue_2
    ;[0.01289 1 0.2456] Is this something we can interact with?
    (Utilities|IsValid (.HitActor (Collision|BreakHitResult _outhit)) ; Because not everything we hit will be an actor
      (:Is%20Valid
        (Utilities|IsValid (Actor|GetComponentbyClass (.HitActor (Collision|BreakHitResult _outhit)) "/Game/CheekyFPS/Blueprints/Interaction/BP_CheekyInteractComponent.BP_CheekyInteractComponent_C")
          (:Is%20Valid
            (if (Default|IsEnabled? (Actor|GetComponentbyClass (.HitActor (Collision|BreakHitResult _outhit)) "/Game/CheekyFPS/Blueprints/Interaction/BP_CheekyInteractComponent.BP_CheekyInteractComponent_C"))
              (return (Actor|GetComponentbyClass (.HitActor (Collision|BreakHitResult _outhit)) "/Game/CheekyFPS/Blueprints/Interaction/BP_CheekyInteractComponent.BP_CheekyInteractComponent_C"))
              (else
                _)))
          (:Is%20Not%20Valid
            _)))
      (:Is%20Not%20Valid
        _)))
  (return 0))

(fn InteractInput
  (params (bStart :type Boolean) (InteractionType :type EInteractionTypes%20Enum :default "NewEnumerator0"))
  (bind _currentselectedcomponent (Variables|Default|GetCurrentSelectedComponent))
  (if bStart
    ;[0.06453 1 0.3054] If we're starting a new interaction, set the component
    (Utilities|IsValid _currentselectedcomponent
      (:Is%20Valid
        (Variables|Default|SetCurrentInteractionComponent _currentselectedcomponent)
        (if (Variables|/Game/CheekyFPS/Blueprints/Interaction/BP_CheekyInteractComponent.BP_CheekyInteractComponent_C|GetbUseHoldInteraction (Variables|Default|GetCurrentInteractionComponent)) :!label _label
          ;[1 0 0] Start / End Hold Input
          (if bStart
            (HoldInteraction|BeginHoldWait InteractionType)
            (return)
            (else
              (HoldInteraction|EndHoldInput)
              (return)))
          (else
            ;[0.1563 0 1] Start / End Simple Input
            (if bStart
              (CallFunction|BeginInteraction InteractionType)
              (return)
              (else
                (CallFunction|EndInteraction InteractionType)
                (return))))))
      (:Is%20Not%20Valid
        _))
    (else
      (Utilities|IsValid (Variables|Default|GetCurrentInteractionComponent)
        (:Is%20Valid
          (goto _label))
        (:Is%20Not%20Valid
          _))))
  (return))

(fn AddMessageWidget
  (params (Component :type BP%20Cheeky%20Interact%20Component%20Object%20Reference))
  (bind _messagetext (Variables|/Game/CheekyFPS/Blueprints/Interaction/BP_CheekyInteractComponent.BP_CheekyInteractComponent_C|GetMessageText Component))
  (Utilities|IsValid (Variables|Interface|GetMessageWidget)
    (:Is%20Valid
      (Interface|ClearMessageWidget))
    (:Is%20Not%20Valid
      _))
  (if (Utilities|Text|TextIsEmpty _messagetext) ; Don't create a widget if initial text\nis empty
    (return)
    (else
      (bind _returnvalue (UserInterface|CreateWidget "/Game/CheekyFPS/Blueprints/Interaction/UI/WBP_InteractionMessage.WBP_InteractionMessage_C" (Game|GetPlayerController 0) _messagetext Component))
      (bind _output_get (Variables|Interface|SetMessageWidget _returnvalue))
      (UserInterface|Viewport|AddtoViewport _output_get (Variables|Configuration|GetWidgetZOrder))
      (return))))

(fn ClearMessageWidget
  (bind _messagewidget (Variables|Interface|GetMessageWidget))
  (Utilities|IsValid _messagewidget
    (:Is%20Valid
      (Default|Close _messagewidget)
      (return))
    (:Is%20Not%20Valid
      (return))))

(fn AddHoldWidget
  (bind _returnvalue (UserInterface|CreateWidget "/Game/CheekyFPS/Blueprints/Interaction/UI/WBP_InteractCircleFill.WBP_InteractCircleFill_C" (Game|GetPlayerController 0) self))
  (bind _output_get (Variables|Interface|SetHoldProgressWidget _returnvalue))
  (UserInterface|Viewport|AddtoViewport _output_get (Variables|Configuration|GetWidgetZOrder))
  (return))

(fn ClearHoldWidget
  (Utilities|IsValid (Variables|Interface|GetHoldProgressWidget)
    (:Is%20Valid
      (Default|Close (Variables|Interface|GetHoldProgressWidget))
      (return))
    (:Is%20Not%20Valid
      (return))))

(fn BeginHoldWait
  (params (InteractionType :type EInteractionTypes%20Enum :default "NewEnumerator0"))
  (bind _currentinteractioncomponent (Variables|Default|GetCurrentInteractionComponent))
  (Variables|HoldInteraction|SetPendingHoldInteractionType InteractionType)
  (Variables|HoldInteraction|SetbIsInHoldWait true)
  ;[1 1 1] Reset each time
  (Variables|HoldInteraction|SetHoldTimeCurrent 0.0)
  (Variables|HoldInteraction|SetbHoldInteractionSuccessful false)
  (Default|UpdateHoldState _currentinteractioncomponent true false)
  (Default|CallOnChangePlayerMovementLock (not (Variables|/Game/CheekyFPS/Blueprints/Interaction/BP_CheekyInteractComponent.BP_CheekyInteractComponent_C|GetbLockPlayerViewDuringHold _currentinteractioncomponent)) (not (Variables|/Game/CheekyFPS/Blueprints/Interaction/BP_CheekyInteractComponent.BP_CheekyInteractComponent_C|GetbLockPlayerMoveDuringHold _currentinteractioncomponent)))
  (Variables|HoldInteraction|SetHoldTimeTarget (Variables|/Game/CheekyFPS/Blueprints/Interaction/BP_CheekyInteractComponent.BP_CheekyInteractComponent_C|GetHoldTime _currentinteractioncomponent))
  (if (Variables|/Game/CheekyFPS/Blueprints/Interaction/BP_CheekyInteractComponent.BP_CheekyInteractComponent_C|GetbShowProgress _currentinteractioncomponent)
    (Interface|AddHoldWidget))
  (Utilities|Time|SetTimerbyFunctionName 0 "IncrementHoldTimer" 0.1 true)
  (return))

(fn IncrementHoldTimer
  ;[1 0.04114 0.03119] Increment hold timer and send update to component
  (bind _output_get (Variables|HoldInteraction|SetHoldTimeCurrent (+ (Variables|HoldInteraction|GetHoldTimeCurrent) 0.1)))
  (Default|UpdateHoldProgress (Variables|Default|GetCurrentInteractionComponent) _output_get)
  (if (>= _output_get (Variables|HoldInteraction|GetHoldTimeTarget))
    (HoldInteraction|SuccessfulHoldWait))
  (return))

(fn SuccessfulHoldWait
  (Variables|HoldInteraction|SetbHoldInteractionSuccessful true)
  (Utilities|Time|ClearTimerbyFunctionName 0 "IncrementHoldTimer")
  (Default|CallOnEndHold (Variables|Default|GetCurrentInteractionComponent) true)
  (Interface|ClearHoldWidget)
  (CallFunction|BeginInteraction (Variables|HoldInteraction|GetPendingHoldInteractionType))
  (return))

(fn EndHoldInput
  (Variables|HoldInteraction|SetbIsInHoldWait false)
  (Default|CallOnChangePlayerMovementLock true true)
  (if (Variables|Default|GetbIsInteracting)
    (CallFunction|EndInteraction (Variables|HoldInteraction|GetPendingHoldInteractionType))
    (return)
    (else
      ;[0.2402 0.2814 1] This path will be taken if the player began a hold but ended it before anything was interacted with
      (Default|UpdateHoldState (Variables|Default|GetCurrentInteractionComponent) false false)
      (Interface|ClearHoldWidget)
      (Utilities|Time|ClearTimerbyFunctionName 0 "IncrementHoldTimer")
      (return))))

(fn EndInteraction
  (params (InteractionType :type EInteractionTypes%20Enum :default "NewEnumerator0"))
  (Utilities|IsValid (Variables|Default|GetCurrentInteractionComponent)
    (:Is%20Valid
      (Default|Interaction (Variables|Default|GetCurrentInteractionComponent) false InteractionType)
      (Variables|Default|SetCurrentInteractionComponent 0))
    (:Is%20Not%20Valid
      _))
  (Variables|Default|SetbIsInteracting false)
  (Default|CallOnChangePlayerMovementLock true true)
  (return))

(fn BeginInteraction
  (params (InteractionType :type EInteractionTypes%20Enum :default "NewEnumerator0"))
  (bind _currentinteractioncomponent (Variables|Default|GetCurrentInteractionComponent))
  (Utilities|IsValid _currentinteractioncomponent
    (:Is%20Valid
      (Default|Interaction _currentinteractioncomponent true InteractionType)
      (Variables|Default|SetbIsInteracting true)
      (Default|CallOnChangePlayerMovementLock (not (Variables|/Game/CheekyFPS/Blueprints/Interaction/BP_CheekyInteractComponent.BP_CheekyInteractComponent_C|GetbLockPlayerViewDuringInteraction _currentinteractioncomponent)) (not (Variables|/Game/CheekyFPS/Blueprints/Interaction/BP_CheekyInteractComponent.BP_CheekyInteractComponent_C|GetbLockPlayerMoveDuringInteraction _currentinteractioncomponent)))
      (return))
    (:Is%20Not%20Valid
      (return))))