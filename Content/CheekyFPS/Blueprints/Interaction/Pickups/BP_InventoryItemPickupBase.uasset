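; Base pickup actor that gives the player an inventory item.
; On BeginPlay it binds to OnPickedUp; GiveItem spawns ItemToPickup through player 0's BP_InventoryComponent, plays a pickup sound, then hides the actor and disables its collision.
; RamaSave integration re-runs GiveItem on load if HasBeenPickedUp is set, so a collected pickup grants its item again and stays hidden.
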(event RamaSaveEventActorFullyLoaded(RamaSave)
  (params (RamaSaveComponent :type Rama%20Save%20Component%20Object%20Reference) (LevelPackageName :type String))
  (if (Variables|Default|GetbHasBeenPickedUp?)
    (CallFunction|GiveItem)))

(event Custom|GiveItem
  (Default|SpawnItem (Actor|GetComponentbyClass (Game|GetPlayerCharacter 0) "/Game/CheekyFPS/Blueprints/Components/BP_InventoryComponent.BP_InventoryComponent_C") (Variables|Default|GetItemToPickup))
  (Audio|PlaySound2D "/Game/CheekyFPS/Sounds/A_Proto_Pickup.A_Proto_Pickup" 1.0 1.0 0.0 0 0)
  (Variables|Default|SetbHasBeenPickedUp? true)
  (Collision|SetActorEnableCollision false)
  (Rendering|SetActorHiddenInGame true))

(event EventBeginPlay
  (|CallParentFunction)
  (EventDispatchers|BindEventtoOnPickedUp (EventDispatchers|CreateEvent :!event Custom|GiveItem)))

(event Collision|EventActorBeginOverlap
  (params (OtherActor :type Actor%20Object%20Reference))
  (|CallParentFunction OtherActor) ; This node is disabled and will not be called.\nDrag off pins to build functionality.
)

(event EventTick
  (params (DeltaSeconds :type Float%20%28single-precision%29))
  (|CallParentFunction DeltaSeconds) ; This node is disabled and will not be called.\nDrag off pins to build functionality.
)

(fn ConstructionScript
  (|CallParentFunction))