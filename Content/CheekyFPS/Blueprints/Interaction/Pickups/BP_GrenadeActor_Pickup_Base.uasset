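; Base grenade pickup actor that hands a grenade type to the player character when collected.
; On BeginPlay it binds to the inherited OnPickedUp event.
; SetGrenadeToSpawn casts the other actor to BP_CheekyCharacter and sends UnlockNewGrenade with the grenade and IsUnlocked false.
; It then flags itself as picked up, disables collision and hides rather than destroying itself.
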(event Custom|SetGrenadeToSpawn
  (Class|BPICharacter|UnlockNewGrenade(Message) (.AsBP%20Cheeky%20Character (Utilities|Casting|CastToBP_CheekyCharacter (Variables|Default|GetOther%20Actor))) false (Variables|Default|GetIn%20Grenade))
  (Variables|Default|SetbHasBeenPickedUp? true)
  (Collision|SetActorEnableCollision false)
  (Rendering|SetActorHiddenInGame true))

(event EventBeginPlay
  (|CallParentFunction)
  (EventDispatchers|BindEventtoOnPickedUp (EventDispatchers|CreateEvent :!event Custom|SetGrenadeToSpawn)))

(event Collision|EventActorBeginOverlap
  (params (OtherActor :type Actor%20Object%20Reference)))

(event EventTick
  (params (DeltaSeconds :type Float%20%28single-precision%29)))

(fn ConstructionScript
  (|CallParentFunction))