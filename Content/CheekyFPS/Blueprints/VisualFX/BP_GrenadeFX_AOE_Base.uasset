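; Base actor for grenade area-of-effect FX, providing a smoke check that cuts enemy AI perception.
; SmokeSphereTrace runs a single Visibility sphere trace forward from the actor, with one-frame debug drawing.
; A hit actor implementing BPI_Enemy is cast directly to AIController, whose sight range is shrunk and hearing range zeroed, with no restore here.
; The event graph is empty, so nothing in this Blueprint calls the trace.
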(event EventBeginPlay
  (|CallParentFunction) ; This node is disabled and will not be called.\nDrag off pins to build functionality.
)

(event Collision|EventActorBeginOverlap
  (params (OtherActor :type Actor%20Object%20Reference)))

(event EventTick
  (params (DeltaSeconds :type Float%20%28single-precision%29)))

(fn ConstructionScript
  (|CallParentFunction))

(fn SmokeSphereTrace
  (bind _returnvalue (Transformation|GetActorLocation))
  (bind (_outhit _returnvalue_2) (Collision|SphereTraceByChannel _returnvalue (+ _returnvalue (* (Math|Vector|GetForwardVector (Transformation|GetActorRotation)) 512.0)) 3.6e+02 "TraceTypeQuery1" false 0 "ForOneFrame"))
  (if _returnvalue_2
    (if (Utilities|DoesObjectImplementInterface (.HitActor (Collision|BreakHitResult _outhit)) "/Game/CheekyFPS/Blueprints/Interfaces/BPI_Enemy.BPI_Enemy_C")
      (Class|ApolloAIBlueprintLibrary|SetSightRange (.AsAIController (Utilities|Casting|CastToAIController (.HitActor (Collision|BreakHitResult _outhit)))) 5.0)
      (Class|ApolloAIBlueprintLibrary|SetHearingRange (.AsAIController (Utilities|Casting|CastToAIController (.HitActor (Collision|BreakHitResult _outhit)))) 0.0))))