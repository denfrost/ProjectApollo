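; Base AI controller that runs a behavior tree and gives enemies a stealth-style detection meter for the player and distractions.
; Perception updates store the stimulus location and drive a looping timer that fills the meter while the player is visible; losing the stimulus zeroes it and starts a line-of-sight timer.
; A full meter sets alert Blackboard keys and plays a sting, while Tick scales audio volume with meter progress.
; Delayed events restore original sight and hearing ranges.
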(event OnTargetPerceptionUpdated(AIPerception)
  (params (Actor :type Actor%20Object%20Reference) (Stimulus :type AI%20Stimulus%20Structure))
  (bind (_stimuluslocation _tag _bsuccessfullysensed) (Utilities|Struct|BreakAIStimulus Stimulus))
  (Utilities|IsValid Actor
    (:Is%20Valid
      (Variables|Default|SetDetectedActor Actor)
      (if (and (Math|Boolean|ORBoolean (Actor|ActorHasTag Actor "Player") (Utilities|Name|Equal(Name) _tag "Player") (Utilities|Name|Equal(Name) _tag "Distract")) _bsuccessfullysensed)
        (CallFunction|UpdatePOIKey _stimuluslocation)
        (if (not (Variables|Default|GetbIsAlerted?))
          (Utilities|Time|ClearandInvalidateTimerbyHandle (Variables|Default|GetLowerPerceptionTimer))
          (bind _returnvalue (Utilities|Time|SetTimerbyEvent (EventDispatchers|CreateEvent :!event Custom|RaisePerception) 0.01 true))
          (Variables|Default|SetRaisePerceptionTimer _returnvalue))
        (else
          (Utilities|Time|SetTimerbyEvent (EventDispatchers|CreateEvent :!event Custom|StartEnemyTimer) (Variables|Default|GetLOSTimer))
          (Utilities|Time|ClearandInvalidateTimerbyHandle (Variables|Default|GetRaisePerceptionTimer))
          (Variables|Default|SetCurrentPerception 0.0))))))

(event Custom|RaisePerception
  (bind _audio (Variables|Default|GetAudio))
  (bind _returnvalue (CallFunction|CanSeePlayer?))
  (Utilities|FlowControl|Sequence
    (:then_0
      (if _returnvalue
        (bind _output_get (Variables|Default|SetCurrentPerception (+ (Variables|Default|GetPerceptionIncreaseAmount) (Variables|Default|GetCurrentPerception))))
        (Utilities|FlowControl|Sequence
          (:then_0
            (if (not (Audio|Components|Audio|IsPlaying _audio))
              (Audio|Components|Audio|Play _audio 0.0)))
          (:then_1
            (if (>= _output_get (Variables|Default|GetPerceptionLimit))
              (Variables|Default|SetCurrentPerception (Variables|Default|GetPerceptionLimit))
              (Variables|Default|SetbIsAlerted? true)
              (AI|Components|Blackboard|SetValueasBool (Variables|Default|GetBlackboard) (Variables|Default|GetDetectedEnemyKey) true)
              (AI|Components|Blackboard|SetValueasObject (Variables|Default|GetBlackboard) (Variables|Default|GetEnemyActorKey) (Variables|Default|GetDetectedActor))
              (Audio|PlaySound2D "/Game/CheekyFPS/Sounds/Perception/Alert/413641__djlprojects__metal-gear-solid-inspired-alert-surprise-sfx.413641__djlprojects__metal-gear-solid-inspired-alert-surprise-sfx" 1.0 1.0 0.0 0 0)
              (Utilities|Time|ClearandInvalidateTimerbyHandle (Variables|Default|GetRaisePerceptionTimer)))))))
    (:then_1
      (AI|Components|Blackboard|SetValueasBool (Variables|Default|GetBlackboard) (Variables|Default|GetLOSKey) _returnvalue))))

(event Custom|LowerPerception
  (bind _audio (Variables|Default|GetAudio))
  (if (not (Variables|Default|GetbIsAlerted?))
    (bind _output_get (Variables|Default|SetCurrentPerception (- (Variables|Default|GetCurrentPerception) (Variables|Default|GetPerceptionIncreaseAmount))))
    (Utilities|FlowControl|Sequence
      (:then_0
        (if (Audio|Components|Audio|IsPlaying _audio)
          (Audio|Components|Audio|Stop _audio))
        (Audio|Components|Audio|SetSound _audio "/Game/CheekyFPS/Sounds/Perception/Alert/Alert_Status_Lower.Alert_Status_Lower")
        (Audio|Components|Audio|Play _audio 0.0))
      (:then_1
        (if (<= _output_get 0.0)
          (Variables|Default|SetCurrentPerception 0.0)
          (Variables|Default|SetbIsAlerted? false)
          (AI|Components|Blackboard|SetValueasBool (Variables|Default|GetBlackboard) (Variables|Default|GetDetectedEnemyKey) false)
          (CallFunction|ClearKey (Variables|Default|GetPOIKey))
          (CallFunction|ClearKey (Variables|Default|GetEnemyActorKey))
          (Utilities|Time|ClearandInvalidateTimerbyHandle (Variables|Default|GetLowerPerceptionTimer)))))))

(event Custom|CustomEvent_0)

(event Custom|StartEnemyTimer
  (bind _blackboard (Variables|Default|GetBlackboard))
  (AI|Components|Blackboard|SetValueasBool _blackboard (Variables|Default|GetLOSKey) false)
  (AI|Components|Blackboard|SetValueasObject _blackboard (Variables|Default|GetEnemyActorKey) 0)
  (Variables|Default|SetbIsAlerted? false)
  (CallFunction|ClearKey (Variables|Default|GetPOIKey))
  (CallFunction|ClearKey (Variables|Default|GetDetectedEnemyKey)))

(event EventBeginPlay
  (bind _self self)
  (EventDispatchers|BindEventtoOnRaisePerception (delegate Custom|CustomEvent_0))
  (Audio|Components|Audio|Stop (Variables|Default|GetAudio))
  (bind _output_get (Variables|Default|SetOriginalSightRange (Class|ApolloAIBlueprintLibrary|GetSightRange _self)))
  (bind _output_get_2 (Variables|Default|SetOriginalHearingRange (Class|ApolloAIBlueprintLibrary|GetHearingRange _self)))
  (Development|PrintString (Utilities|String|Append (Utilities|GetDisplayName (Pawn|GetControlledPawn)) " has sight range of " (Utilities|String|ToString(Float) _output_get) " " "and a hearing range of " (Utilities|String|ToString(Float) _output_get_2))))

(event EventTick
  (params (DeltaSeconds :type Float%20%28single-precision%29))
  (bind _audio (Variables|Default|GetAudio))
  (if (Audio|Components|Audio|IsPlaying _audio)
    (Audio|Components|Audio|SetVolumeMultiplier _audio (Math|Float|Lerp 0.01 0.95 (CallFunction|GetPerceptionPercentage)) :!class /Script/Engine.AudioComponent)))

(event EventPossess
  (params (PossessedPawn :type Pawn%20Object%20Reference))
  (AI|RunBehaviorTree (Variables|Default|GetStartingBehaviorTree)))

(event EventOnResetHearing
  (Utilities|FlowControl|Delay 4.0)
  (CallFunction|ResetHearingRange))

(event EventOnResetSight
  (Utilities|FlowControl|Delay 4.0)
  (CallFunction|ResetSightRange))

(fn ConstructionScript)

(fn SetStartingStats
  (params (FloatValue :type Float%20%28single-precision%29))
  (AI|Components|Blackboard|SetValueasFloat (AI|GetBlackboard self) (Utilities|Name|MakeLiteralName "CurrentHealth") FloatValue))

(fn GetPerceptionPercentage
  (bind _output_get (Variables|Default|SetPerceptionPercentage (/ (Variables|Default|GetCurrentPerception) (Variables|Default|GetPerceptionLimit))))
  (return _output_get))

(fn UpdatePOIKey
  (params (StimulusLocation :type Vector))
  (bind _output_get (Variables|Default|SetStimulusLocation StimulusLocation))
  (AI|Components|Blackboard|SetValueasVector (Variables|Default|GetBlackboard) (Variables|Default|GetPOIKey) _output_get))

(fn ClearKey
  (params (KeyName :type Name))
  (AI|Components|Blackboard|ClearValue (Variables|Default|GetBlackboard) KeyName))

(fn CanSeePlayer?
  (for _array_element (Class|AIPerceptionComponent|GetCurrentlyPerceivedActors (Variables|Default|GetAIPerception) "/Script/AIModule.AISense_Sight")
    (return (== _array_element (Game|GetPlayerCharacter 0)))))

(fn ResetSightRange
  (bind _returnvalue (Class|ApolloAIBlueprintLibrary|SetSightRange self (Variables|Default|GetOriginalSightRange)))
  (if _returnvalue
    (Development|PrintString (Utilities|String|Append "Reset Sight Range for " (Utilities|GetDisplayName (Pawn|GetControlledPawn))))))

(fn ResetHearingRange
  (bind _returnvalue (Class|ApolloAIBlueprintLibrary|SetHearingRange self (Variables|Default|GetOriginalHearingRange)))
  (if _returnvalue
    (Development|PrintString (Utilities|String|Append "Reset Hearing Range for " (Utilities|GetDisplayName (Pawn|GetControlledPawn))))))