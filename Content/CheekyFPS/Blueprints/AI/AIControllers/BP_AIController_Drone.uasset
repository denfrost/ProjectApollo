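; AI controller for the drone that turns perception updates into Blackboard values.
; A perceived player, matched by pawn or "Player" tag, becomes the enemy actor.
; Any other actor clears the enemy key, and one with an identification component on a different team also sets the point of interest to the stimulus location.
; The sense type and whether sensing succeeded are not checked.
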(event OnTargetPerceptionUpdated(AIPerception)
  (params (Actor :type Actor%20Object%20Reference) (Stimulus :type AI%20Stimulus%20Structure))
  (bind _returnvalue (Actor|GetComponentbyClass Actor "/Game/CheekyFPS/Blueprints/Components/BP_IdentificationComponent.BP_IdentificationComponent_C"))
  (bind _blackboard (Variables|Default|GetBlackboard))
  (if (or (== Actor (Game|GetPlayerCharacter 0)) (Actor|ActorHasTag Actor "Player"))
    (AI|Components|Blackboard|SetValueasObject _blackboard (Variables|Default|GetEnemyActorKey) Actor)
    (else
      (Utilities|FlowControl|Sequence
        (:then_0
          (if (Utilities|IsValid _returnvalue)
            (bind _returnvalue_2 (Class|BPIEnemy|GetGenericTeamID(Message) (Pawn|GetControlledPawn)))
            (if (!= (Default|GetOwnerTeamID _returnvalue) _returnvalue_2)
              (AI|Components|Blackboard|SetValueasVector _blackboard (Variables|Default|GetPOIKey) (.StimulusLocation (Utilities|Struct|BreakAIStimulus Stimulus))))))
        (:then_1
          (AI|Components|Blackboard|SetValueasObject (Variables|Default|GetBlackboard) (Variables|Default|GetEnemyActorKey) 0))))))

(event EventBeginPlay)

(event EventTick
  (params (DeltaSeconds :type Float%20%28single-precision%29)))

(fn ConstructionScript)