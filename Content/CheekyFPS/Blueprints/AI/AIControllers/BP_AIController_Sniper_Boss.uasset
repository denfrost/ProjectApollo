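; AI controller for the sniper boss that feeds the player to the Blackboard and tracks health phases.
; Every tick sets the player as enemy, while AI perception flags detection when it senses the player.
; Tick also polls the pawn's health component, firing a one-time desperation move below quarter health.
; The half-health flag is cleared unconditionally later in the same tick, so it never persists.
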(event OnTargetPerceptionUpdated(AIPerception)
  (params (Actor :type Actor%20Object%20Reference) (Stimulus :type AI%20Stimulus%20Structure))
  (bind _blackboard (Variables|Default|GetBlackboard))
  (if (and (== Actor (Game|GetPlayerCharacter 0)) (.bSuccessfullySensed (Utilities|Struct|BreakAIStimulus Stimulus)))
    (AI|Components|Blackboard|SetValueasObject _blackboard (Variables|Default|GetEnemyActorKey) Actor)
    (AI|Components|Blackboard|SetValueasBool _blackboard (Variables|Default|GetDetectedEnemyKey) true)))

(event EventBeginPlay
  (|CallParentFunction) ; This node is disabled and will not be called.\nDrag off pins to build functionality.
)

(event EventTick
  (params (DeltaSeconds :type Float%20%28single-precision%29))
  (bind _returnvalue (Pawn|GetControlledPawn))
  (bind _returnvalue_2 (Actor|GetComponentbyClass _returnvalue "/Game/CheekyFPS/Blueprints/Health/BP_CheekyHealthComponent.BP_CheekyHealthComponent_C"))
  (bind _returnvalue_3 (Default|GetHealthPercentage _returnvalue_2))
  (|CallParentFunction DeltaSeconds)
  (AI|Components|Blackboard|SetValueasObject (Variables|Default|GetBlackboard) (Variables|Default|GetEnemyActorKey) (Game|GetPlayerCharacter 0))
  (Utilities|FlowControl|Sequence
    (:then_0
      (Variables|Default|SetAtHalfHealth (<= _returnvalue_3 0.45)))
    (:then_1
      (Variables|Default|SetAtQuarterHealth (< _returnvalue_3 0.25))
      (Variables|Default|SetAtHalfHealth false)
      (if (Variables|Default|GetAtQuarterHealth)
        (if (not (Variables|Default|GetHasUsedDesperationMove?))
          (Default|CallOnDesperationMove)
          (Variables|Default|SetHasUsedDesperationMove? true))))))

(fn ConstructionScript
  (|CallParentFunction))