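; Base AI controller for CheekyFPS enemies that runs a behavior tree and turns AI Perception stimuli into detection and alert state.
; Looping timers raise or lower a perception meter with audio cues, writing line of sight, enemy and alert status to the Blackboard.
; Full detection triggers a reflex effect and delayed stun check.
; It syncs with the game-state alarm, fails missions when the player is seen, and offers partner-follow and sense-range reset helpers.
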(event OnTargetPerceptionUpdated(AIPerception)
  (params (Actor :type Actor%20Object%20Reference) (Stimulus :type AI%20Stimulus%20Structure))
  (CallFunction|UpdateNewStimulus Stimulus Actor))

(event Custom|LowerPerception
  (bind _audiocomp (Variables|Default|GetAudioComp))
  (bind _blackboard (Variables|Default|GetBlackboard))
  (if (Variables|Status|GetbIsStunned?)
    (CallFunction|ClearPerceptiononStun)
    (elif (and (not (Variables|Status|GetbIsAlerted?)) (not (CallFunction|CanSeePlayer?)))
      (bind _output_get (Variables|Perception|SetCurrentPerception (- (Variables|Perception|GetCurrentPerception) (Variables|Perception|GetPerceptionIncreaseAmount))))
      (Class|BPIEnemy|HasDetectedEnemy?(Message) (Pawn|GetControlledPawn) false)
      (Utilities|FlowControl|Sequence
        (:then_0
          (if (Audio|Components|Audio|IsPlaying _audiocomp)
            (Audio|Components|Audio|Stop _audiocomp)
            (Utilities|FlowControl|Delay 0.2))
          (Audio|Components|Audio|SetSound _audiocomp "/Game/CheekyFPS/Sounds/Perception/Alert/A_Alert_Status_Lower.A_Alert_Status_Lower")
          (Audio|Components|Audio|Play _audiocomp 0.0))
        (:then_1
          (if (<= _output_get 0.0)
            (Variables|Perception|SetCurrentPerception 0.0)
            (Variables|Status|SetbIsAlerted? false)
            (AI|Components|Blackboard|SetValueasBool (Variables|Default|GetBlackboard) (Variables|Keys|GetDetectedEnemyKey) false)
            (AI|Components|Blackboard|SetValueasObject _blackboard (Variables|Keys|GetEnemyActorKey) 0)
            (AI|Components|Blackboard|SetValueasBool _blackboard (Variables|Keys|GetIsInCombatKey) false)
            (Utilities|Time|ClearandInvalidateTimerbyHandle (Variables|Behavior|GetLowerPerceptionTimer))))))))

(event Custom|ActivateAlarm
  (bind _returnvalue (Game|GetGameState))
  (bind _raiseperceptiontimer (Variables|Behavior|GetRaisePerceptionTimer))
  (Utilities|FlowControl|Sequence
    (:then_0
      (AI|Components|Blackboard|SetValueasBool (Variables|Default|GetBlackboard) (Variables|Keys|GetIsInCombatKey) true)
      (CallFunction|UpdateAlertStatus "NewEnumerator3"))
    (:then_1
      (if (Utilities|Time|IsTimerActivebyHandle _raiseperceptiontimer)
        (Utilities|Time|ClearandInvalidateTimerbyHandle _raiseperceptiontimer)))
    (:then_2
      (if (Utilities|Enum|NotEqual(Enum) (Variables|/Game/CheekyFPS/Blueprints/Game/BP_ISSGameStateBase.BP_ISSGameStateBase_C|GetCurrentAlertStatus (.AsBP%20ISSGame%20State%20Base (Utilities|Casting|CastToBP_ISSGameStateBase _returnvalue))) "NewEnumerator2")
        (Class|BPISecurityAlarmInterface|SecurityAlarmInterface(Message) _returnvalue true "NewEnumerator2")
        (Utilities|FlowControl|DoOnce false :!label _label
          (:Completed
            (Audio|PlaySound2D "/Game/CheekyFPS/Sounds/Perception/Alert/A_413641__djlprojects__metal-gear-solid-inspired-alert-surprise-sfx.A_413641__djlprojects__metal-gear-solid-inspired-alert-surprise-sfx" 1.0 1.0 0.0 0 0)))
        (else
          (goto _label Reset))))))

(event Custom|StartEnemyTimer
  (bind _blackboard (Variables|Default|GetBlackboard))
  (bind _blackboard_2 (Variables|Default|GetBlackboard))
  (AI|Components|Blackboard|SetValueasBool _blackboard (Variables|Keys|GetLOSKey) false)
  (AI|Components|Blackboard|SetValueasObject _blackboard (Variables|Keys|GetEnemyActorKey) 0)
  (Variables|Status|SetbIsAlerted? false)
  (AI|Components|Blackboard|SetValueasVector _blackboard_2 (Variables|Keys|GetPOIKey) "0, 0, 0")
  (AI|Components|Blackboard|SetValueasBool _blackboard_2 (Variables|Keys|GetDetectedEnemyKey) false))

(event Custom|CheckStunStatus
  (bind _returnvalue (Game|GetGameState))
  (if (Variables|Status|GetbIsStunned?)
    (Class|BPIGameEvents|StopReflexFX(Message) _returnvalue false)
    (CallFunction|SetBoolValue (Variables|Keys|GetIsInCombatKey) false)
    (else
      (Class|BPIGameEvents|StopReflexFX(Message) _returnvalue true)
      (bind _returnvalue_2 (Utilities|Time|SetTimerbyEvent (EventDispatchers|CreateEvent :!event Custom|CheckAlarmResetStatus) 0.5 true))
      (Variables|Default|SetAlarmResetCheckStatus _returnvalue_2)))
  (Utilities|Time|ClearandInvalidateTimerbyHandle (Variables|Default|GetStunStatusTimer)))

(event Custom|CheckAlarmResetStatus
  (bind _returnvalue (Game|GetGameState))
  (if (CallFunction|CanSeePlayer?)
    (Class|BPIGameEvents|PauseAlarmTimer(Message) _returnvalue)
    (else
      (Utilities|FlowControl|Delay 3.0)
      (Class|BPIGameEvents|UnpauseAlarmTimer(Message) _returnvalue))))

(event EventBeginPlay
  (bind _returnvalue (Pawn|GetControlledPawn))
  (bind _self self)
  (bind _returnvalue_2 (Actor|GetComponentbyClass _returnvalue "/Game/CheekyFPS/Blueprints/Health/BP_CheekyHealthComponent.BP_CheekyHealthComponent_C"))
  (CallFunction|SetKeyNames)
  (Audio|Components|Audio|Stop (Variables|Default|GetAudioComp))
  (bind _output_get (Variables|Behavior|SetOriginalSightRange (Class|ApolloAIBlueprintLibrary|GetSightRange _self)))
  (bind _output_get_2 (Variables|Behavior|SetOriginalHearingRange (Class|ApolloAIBlueprintLibrary|GetHearingRange _self)))
  (Utilities|FlowControl|Sequence
    (:then_0
      (EventDispatchers|BindEventtoOnAlarmActivate (.AsBP%20ISSGame%20State%20Base (Utilities|Casting|CastToBP_ISSGameStateBase (Game|GetGameState))) (EventDispatchers|CreateEvent :!event Custom|ActivateAlarm))
      (Audio|Components|Audio|Stop (Variables|Default|GetAudioComp)))
    (:then_1
      (Utilities|IsValid _returnvalue_2
        (:Is%20Valid
          (Variables|Default|SetPawnHealthComponent _returnvalue_2))))))

(event EventTick
  (params (DeltaSeconds :type Float%20%28single-precision%29))
  (bind _audiocomp (Variables|Default|GetAudioComp))
  (Utilities|FlowControl|Sequence
    (:then_0
      (if (Audio|Components|Audio|IsPlaying _audiocomp)
        (Audio|Components|Audio|SetVolumeMultiplier _audiocomp (Math|Float|Lerp 0.0 0.95 (CallFunction|GetPerceptionPercentage)) :!class /Script/Engine.AudioComponent)))
    (:then_1
      (bind _returnvalue (Class|BPISecurityAlarmInterface|GetCurrentAlertStatus(Message) (Game|GetGameState)))
      (if (Utilities|Enum|Equal(Enum) _returnvalue "NewEnumerator2")
        (if (not (Default|IsDead? (Variables|Default|GetPawnHealthComponent)))
          (bind _returnvalue_2 (Class|BPIEnemy|GetCurrentAlertState(Message) (Pawn|GetControlledPawn)))
          (if (Utilities|Enum|NotEqual(Enum) _returnvalue_2 "NewEnumerator3")
            (CallFunction|UpdateAlertStatus "NewEnumerator3")))))))

(event EventPossess
  (params (PossessedPawn :type Pawn%20Object%20Reference))
  (|CallParentFunction 0)
  (AI|RunBehaviorTree (Variables|Behavior|GetStartingBehaviorTree)))

(event EventOnResetHearing
  (Utilities|FlowControl|Delay 4.0)
  (CallFunction|ResetHearingRange))

(event EventOnResetSight
  (Utilities|FlowControl|Delay 4.0)
  (CallFunction|ResetSightRange))

(event EventSetBoolKey
  (params (KeyName :type Name :default "None") (ToggleStatus :type Boolean))
  (CallFunction|SetBoolValue KeyName ToggleStatus))

(fn ConstructionScript)

(fn UpdatePOIKey
  (params (StimulusLocation :type Vector))
  (bind _output_get (Variables|Default|SetStimulusLocation StimulusLocation))
  (AI|Components|Blackboard|SetValueasVector (Variables|Default|GetBlackboard) (Variables|Keys|GetPOIKey) _output_get))

(fn GetPerceptionPercentage
  (bind _output_get (Variables|Perception|SetPerceptionPercentage (/ (Variables|Perception|GetCurrentPerception) (Variables|Perception|GetPerceptionLimit))))
  (return _output_get))

(fn CanSeePlayer?
  (for _array_element (Class|AIPerceptionComponent|GetCurrentlyPerceivedActors (Variables|Default|GetAIPerception) "/Script/AIModule.AISense_Sight")
    (return (and (== _array_element (Game|GetPlayerCharacter 0)) (Actor|ActorHasTag _array_element "Player")))))

(fn ResetHearingRange
  (bind _returnvalue (Class|ApolloAIBlueprintLibrary|SetHearingRange self (Variables|Behavior|GetOriginalHearingRange)))
  (if _returnvalue
    (Development|PrintString (Utilities|String|Append "Reset Hearing Range for " (Utilities|GetDisplayName (Pawn|GetControlledPawn))))))

(fn ResetSightRange
  (bind _returnvalue (Class|ApolloAIBlueprintLibrary|SetSightRange self (Variables|Behavior|GetOriginalSightRange)))
  (if _returnvalue
    (Development|PrintString (Utilities|String|Append "Reset Sight Range for " (Utilities|GetDisplayName (Pawn|GetControlledPawn))))))

(fn SetStartingStats
  (params (FloatValue :type Float%20%28single-precision%29))
  (AI|Components|Blackboard|SetValueasFloat (AI|GetBlackboard self) (Utilities|Name|MakeLiteralName "CurrentHealth") FloatValue))

(fn ClearPerceptiononStun
  (bind _returnvalue (Game|GetGameState))
  (Variables|Perception|SetCurrentPerception 0.0)
  (CallFunction|UpdateAlertStatus "NewEnumerator6")
  (Variables|Status|SetbIsStunned? true)
  (bind _returnvalue_2 (Class|BPIGameEvents|GetReflexStatus(Message) _returnvalue))
  (if _returnvalue_2
    (Class|BPIGameEvents|StopReflexFX(Message) _returnvalue false)))

(fn SetBoolValue
  (params (KeyName :type Name%20%28by%20ref%29) (BoolValue :type Boolean))
  (AI|Components|Blackboard|SetValueasBool (Variables|Default|GetBlackboard) KeyName BoolValue))

(fn ClearAlarmResetTimer
  (bind _alarmresetcheckstatus (Variables|Default|GetAlarmResetCheckStatus))
  (if (Utilities|Time|IsTimerActivebyHandle _alarmresetcheckstatus)
    (Utilities|Time|ClearandInvalidateTimerbyHandle _alarmresetcheckstatus)))

(fn CheckMissionStatus
  (bind _returnvalue (Class|BPIGameEvents|GetCurrentGameType(Message) (Game|GetGameMode)))
  (bind _output_get (Variables|Default|SetbIsMission? (Utilities|Enum|NotEqual(Enum) _returnvalue "NewEnumerator1")))
  (return _output_get))

(fn SetKeyNames
  (Utilities|FlowControl|Sequence
    (:then_0
      (bind _output_get (Variables|Keys|SetPOIKey "PointOfInterest"))
      (bind _output_get_2 (Variables|Keys|SetEnemyActorKey "CurrentEnemy"))
      (bind _output_get_3 (Variables|Keys|SetLOSKey "HasLOS"))
      (bind _output_get_4 (Variables|Keys|SetDetectedEnemyKey "HasDetectedEnemy"))
      (bind _output_get_5 (Variables|Keys|SetStunnedKey "IsStunned"))
      (bind _output_get_6 (Variables|Keys|SetIsInCombatKey "IsInCombat"))
      (bind _output_get_7 (Variables|Keys|SetAlertStatusKey "CurrentAlertStatus"))
      (bind _output_get_8 (Variables|Keys|SetPartnerKey "PartnerActor"))
      (bind _output_get_9 (Variables|Keys|SetLeaderKey "IsLeader"))
      (CallFunction|UpdateAlertStatus "NewEnumerator1"))
    (:then_1
      (CallFunction|CheckKeyNameStatus _output_get)
      (CallFunction|CheckKeyNameStatus _output_get_2)
      (CallFunction|CheckKeyNameStatus _output_get_3)
      (CallFunction|CheckKeyNameStatus _output_get_4)
      (CallFunction|CheckKeyNameStatus _output_get_5)
      (CallFunction|CheckKeyNameStatus _output_get_6)
      (CallFunction|CheckKeyNameStatus _output_get_7)
      (CallFunction|CheckKeyNameStatus _output_get_8)
      (CallFunction|CheckKeyNameStatus _output_get_9))))

(fn CheckKeyNameStatus
  (params (InputName :type Name))
  (if (not (Utilities|Name|NotEqual(Name) InputName "None"))
    (Development|PrintString "A key is missing a name value!")))

(fn UpdateAllAItoPlayerLocation
  (bind _returnvalue (Game|Player|GetPlayerPawn 0))
  (bind _outactors (Actor|GetAllActorsOfClass "/Game/CheekyFPS/Blueprints/Enemies/Humanoids/BP_BaseEnemy.BP_BaseEnemy_C"))
  (for _array_element _outactors
    (if (Utilities|Enum|NotEqual(Enum) (Variables|/Game/CheekyFPS/Blueprints/Enemies/Humanoids/BP_BaseEnemy.BP_BaseEnemy_C|GetSoldierType _array_element) "NewEnumerator2")
      (CallFunction|UpdatePOIKey (.AsBP%20AIController%20Base (Utilities|Casting|CastToBP_AIController_Base (AI|GetAIController _array_element))) (Transformation|GetActorLocation _returnvalue))
      (AI|Components|Blackboard|SetValueasObject (AI|GetBlackboard _array_element) (Variables|Keys|GetEnemyActorKey) _returnvalue))))

(fn UpdateNewStimulus
  (params (AIStimulus :type AI%20Stimulus%20Structure%20%28by%20ref%29) (DetectedActor :type Actor%20Object%20Reference))
  (bind (_stimuluslocation _tag) (Utilities|Struct|BreakAIStimulus AIStimulus))
  (bind _blackboard (Variables|Default|GetBlackboard))
  (bind _output_get (Variables|Behavior|SetDetectedActor DetectedActor))
  (if (Math|Boolean|ORBoolean (Actor|ActorHasTag _output_get "Player") (Utilities|Name|Equal(Name) _tag "Player") (Utilities|Name|Equal(Name) _tag "Distract") (Utilities|Name|Equal(Name) _tag "Weapon"))
    (Utilities|FlowControl|Sequence
      (:then_0
        (CallFunction|UpdatePOIKey _stimuluslocation)
        (if (not (Variables|Status|GetbIsAlerted?))
          (Utilities|Time|ClearandInvalidateTimerbyHandle (Variables|Behavior|GetLowerPerceptionTimer))
          (bind _returnvalue (Utilities|Time|SetTimerbyEvent (EventDispatchers|CreateEvent :!event RaisePerception) 0.01 true))
          (Variables|Behavior|SetRaisePerceptionTimer _returnvalue)))
      (:then_2
        (if (== DetectedActor (Game|Player|GetPlayerPawn 0))
          (if (and (CallFunction|CheckMissionStatus) (CallFunction|CanSeePlayer?))
            (Class|BPIGameEvents|OnMissionFail(Message) (Game|GetGameMode))))))
    (else
      (Utilities|FlowControl|Sequence
        (:then_0
          (Utilities|Time|ClearandInvalidateTimerbyHandle (Variables|Behavior|GetRaisePerceptionTimer) :!label _label)
          (if (or (Variables|Status|GetbIsAlerted?) (ScalableFloat|GetValueasBool (Variables|Default|GetBlackboard) (Variables|Keys|GetIsInCombatKey)))
            (if (!= (AI|Components|Blackboard|GetValueasObject (Variables|Default|GetBlackboard) (Variables|Keys|GetEnemyActorKey)) 0)
              (AI|Components|Blackboard|SetValueasBool _blackboard (Variables|Keys|GetLOSKey) false)
              (AI|Components|Blackboard|SetValueasObject _blackboard (Variables|Keys|GetEnemyActorKey) 0)
              (Variables|Behavior|SetDetectedActor 0))
            (else
              (bind _returnvalue_2 (Utilities|Time|SetTimerbyEvent (EventDispatchers|CreateEvent :!event Custom|LowerPerception) 0.01 true))
              (Variables|Behavior|SetLowerPerceptionTimer _returnvalue_2)
              (AI|Components|Blackboard|SetValueasBool (Variables|Default|GetBlackboard) (Variables|Keys|GetLOSKey) false))))
        (:then_1
          (if (and (Actor|ActorHasTag DetectedActor "Enemy") (!= DetectedActor (Pawn|GetControlledPawn self)))
            (AI|Components|Blackboard|SetValueasObject (Variables|Default|GetBlackboard) (Variables|Keys|GetPartnerKey) DetectedActor)
            (else
              (goto _label))))))))

(fn GetNormalizedDistancetoPOI
  (bind _blackboard (Variables|Default|GetBlackboard))
  (if (ScalableFloat|GetValueasBool _blackboard (Variables|Keys|GetLOSKey))
    (return (Math|Float|NormalizetoRange (Math|Vector|Distance(Vector) (AI|Components|Blackboard|GetValueasVector _blackboard (Variables|Keys|GetPOIKey)) (Transformation|GetActorLocation (Pawn|GetControlledPawn))) 1.0 1e+04))
    (else
      (return 0.0))))

(fn FollowTarget
  (params (TargetToFollow :type Actor%20Object%20Reference))
  (bind _returnvalue (Pawn|GetControlledPawn))
  (bind _returnvalue_2 (Transformation|GetActorLocation TargetToFollow))
  (bind _returnvalue_3 (Transformation|GetActorLocation _returnvalue))
  (bind _returnvalue_4 (AI|Navigation|MovetoLocation (Math|Vector|Lerp(Vector) _returnvalue_3 _returnvalue_2 (Math|Vector|Distance(Vector) _returnvalue_2 _returnvalue_3)) -1.0 true true true true 0))
  (switch Utilities|FlowControl|Switch|SwitchonEPathFollowingRequestResult _returnvalue_4
    (:Failed
      (Development|PrintString "Move Failed"))
    (:RequestSuccessful
      (Development|PrintString "Move Success"))))

(fn UpdateAlertStatus
  (params (NewState :type E_EnemyAlertStatus%20Enum :default "NewEnumerator1"))
  (bind _returnvalue (Pawn|GetControlledPawn))
  (bind _returnvalue_2 (Pawn|GetControlledPawn))
  (bind _blackboard (Variables|Default|GetBlackboard))
  (bind _blackboard_2 (Variables|Default|GetBlackboard))
  (bind _blackboard_3 (Variables|Default|GetBlackboard))
  (bind _blackboard_4 (Variables|Default|GetBlackboard))
  (Utilities|FlowControl|Sequence
    (:then_0
      (Class|BPIEnemy|UpdateAlertState(Message) (Pawn|GetControlledPawn) NewState)
      (Utilities|IsValid _blackboard_4
        (:Is%20Valid
          (AI|Components|Blackboard|SetValueasEnum _blackboard_4 (Variables|Keys|GetAlertStatusKey) NewState))))
    (:then_1
      (if (!= (AI|Components|Blackboard|GetValueasObject _blackboard_3 (Variables|Keys|GetEnemyActorKey)) 0)
        (bind _returnvalue_3 (Class|BPIEnemy|GetCurrentAlertState(Message) _returnvalue))
        (if (or (Utilities|Enum|NotEqual(Enum) _returnvalue_3 "NewEnumerator1") (Utilities|Enum|NotEqual(Enum) _returnvalue_3 "NewEnumerator2"))
          (Class|BPIEnemy|UpdateAlertState(Message) _returnvalue "NewEnumerator3")
          (Utilities|IsValid _blackboard
            (:Is%20Valid
              (AI|Components|Blackboard|SetValueasEnum _blackboard (Variables|Keys|GetAlertStatusKey) _returnvalue_3))))))
    (:then_2
      (if (Math|Vector|NotEqual(Vector) (AI|Components|Blackboard|GetValueasVector _blackboard_3 (Variables|Keys|GetPOIKey)) "0, 0, 0" 0.0001)
        (bind _returnvalue_4 (Class|BPIEnemy|GetCurrentAlertState(Message) _returnvalue_2))
        (if (or (Utilities|Enum|NotEqual(Enum) _returnvalue_4 "NewEnumerator1") (Utilities|Enum|NotEqual(Enum) _returnvalue_4 "NewEnumerator3"))
          (Class|BPIEnemy|UpdateAlertState(Message) _returnvalue_2 "NewEnumerator2")
          (Utilities|IsValid _blackboard_2
            (:Is%20Valid
              (AI|Components|Blackboard|SetValueasEnum _blackboard_2 (Variables|Keys|GetAlertStatusKey) _returnvalue_4))))))))

(fn MovetoPartnerTarget
  (bind _returnvalue (Pawn|GetControlledPawn))
  (bind _partnerkey (Variables|Keys|GetPartnerKey))
  (bind _blackboard (Variables|Default|GetBlackboard))
  (bind _leaderkey (Variables|Keys|GetLeaderKey))
  (bind _blackboard_2 (Variables|Default|GetBlackboard))
  (bind _returnvalue_2 (AI|Components|Blackboard|GetValueasObject _blackboard _partnerkey))
  (bind _asactor (Utilities|Casting|CastToActor _returnvalue_2))
  (Utilities|FlowControl|Sequence
    (:then_0
      (if (not (ScalableFloat|GetValueasBool _blackboard_2 _leaderkey))
        (AI|Components|Blackboard|SetValueasBool _blackboard_2 _leaderkey true)))
    (:then_1
      (if (ScalableFloat|GetValueasBool (Variables|Default|GetBlackboard) (Variables|Keys|GetLeaderKey))
        (Utilities|IsValid _asactor
          (:Is%20Valid
            (AI|Navigation|MovetoLocation (Math|Interpolation|VInterpTo (Transformation|GetActorLocation _returnvalue) (+ (Transformation|GetActorLocation _asactor) (* (Transformation|GetActorForwardVector _returnvalue) -1.5e+02)) (Utilities|Time|GetWorldDeltaSeconds) 3.0) -1.0 true true false true 0)))))))

(fn RaisePerception
  (bind _returnvalue (CallFunction|CanSeePlayer?))
  (bind _audiocomp (Variables|Default|GetAudioComp))
  (bind _returnvalue_2 (Class|BPIGameEvents|GetAlertStatus(Message) (Game|GetGameState)))
  (if (and (Utilities|Enum|NotEqual(Enum) _returnvalue_2 "NewEnumerator2") (not (Utilities|Enum|Equal(Enum) _returnvalue_2 "NewEnumerator3")))
    (if (not (Utilities|Enum|Equal(Enum) (Variables|/Game/CheekyFPS/Blueprints/Enemies/Components/BP_AlertComponent.BP_AlertComponent_C|GetAlertState (Actor|GetComponentbyClass (Pawn|GetControlledPawn) "/Game/CheekyFPS/Blueprints/Enemies/Components/BP_AlertComponent.BP_AlertComponent_C")) "NewEnumerator1"))
      (if _returnvalue
        (CallFunction|UpdateAlertStatus "NewEnumerator2")
        (AI|Components|Blackboard|SetValueasBool (Variables|Default|GetBlackboard) (Variables|Keys|GetLOSKey) _returnvalue)
        (bind _output_get (Variables|Perception|SetCurrentPerception (+ (Variables|Perception|GetPerceptionIncreaseAmount) (Variables|Perception|GetCurrentPerception))))
        (Class|BPIEnemy|HasDetectedEnemy?(Message) (Pawn|GetControlledPawn) true)
        (Utilities|FlowControl|Sequence
          (:then_0
            (if (Audio|Components|Audio|IsPlaying _audiocomp)
              (Audio|Components|Audio|Stop _audiocomp))
            (Audio|Components|Audio|SetSound _audiocomp "/Game/CheekyFPS/Sounds/Perception/Alert/A_Alert_Status_Rise.A_Alert_Status_Rise")
            (Audio|Components|Audio|Play _audiocomp 0.0))
          (:then_1
            (if (>= _output_get (Variables|Perception|GetPerceptionLimit))
              (Variables|Perception|SetCurrentPerception (Variables|Perception|GetPerceptionLimit))
              (bind _output_get_2 (Variables|Status|SetbIsAlerted? true))
              (AI|Components|Blackboard|SetValueasBool (Variables|Default|GetBlackboard) (Variables|Keys|GetDetectedEnemyKey) _output_get_2)
              (AI|Components|Blackboard|SetValueasObject (Variables|Default|GetBlackboard) (Variables|Keys|GetEnemyActorKey) (Variables|Behavior|GetDetectedActor))
              (Class|BPIGameEvents|PlayReflex(Message) (Game|GetGameState))
              (bind _returnvalue_3 (Utilities|Time|SetTimerbyEvent (EventDispatchers|CreateEvent :!event Custom|CheckStunStatus) 5.0))
              (Variables|Default|SetStunStatusTimer _returnvalue_3)
              (Utilities|Time|ClearandInvalidateTimerbyHandle (Variables|Behavior|GetRaisePerceptionTimer)))))
        (else
          (AI|Components|Blackboard|SetValueasBool (Variables|Default|GetBlackboard) (Variables|Keys|GetLOSKey) false))))
    (else
      (Variables|Perception|SetCurrentPerception (Variables|Perception|GetPerceptionLimit))
      (Utilities|Time|ClearandInvalidateTimerbyHandle (Variables|Behavior|GetRaisePerceptionTimer)))))

(fn GetCurrentAlertState
  (return "NewEnumerator1"))

(fn GetGenericTeamID
  (return (.teamid (Variables|Default|GetTeamId))))