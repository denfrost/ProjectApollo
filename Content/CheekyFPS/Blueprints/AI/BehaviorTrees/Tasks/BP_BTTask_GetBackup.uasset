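; Behavior tree task that recruits another enemy as backup for the AI pawn running it.
; On execute, it line-traces on Visibility from the pawn's eye viewpoint along its view direction, out to the controller's sight range, with debug drawing enabled.
; If the hit actor implements BPI_Enemy, its BP_AIController_Base is told to follow the calling pawn.
; The graph never calls FinishExecute.
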(event EventReceiveExecuteAI
  (params (OwnerController :type AI%20Controller%20Object%20Reference) (ControlledPawn :type Pawn%20Object%20Reference))
  (bind (_outlocation _outrotation) (Actor|GetActorEyesViewPoint ControlledPawn))
  (bind (_outhit _returnvalue) (Collision|LineTraceByChannel _outlocation (+ _outlocation (* (Math|Vector|GetForwardVector _outrotation) (Class|ApolloAIBlueprintLibrary|GetSightRange OwnerController))) "TraceTypeQuery1" true 0 "ForDuration"))
  (if _returnvalue
    (if (Utilities|DoesObjectImplementInterface (.HitActor (Collision|BreakHitResult _outhit)) "/Game/CheekyFPS/Blueprints/Interfaces/BPI_Enemy.BPI_Enemy_C")
      (Default|FollowTarget (.AsBP%20AIController%20Base (Utilities|Casting|CastToBP_AIController_Base (AI|GetAIController (.HitActor (Collision|BreakHitResult _outhit))))) ControlledPawn))))