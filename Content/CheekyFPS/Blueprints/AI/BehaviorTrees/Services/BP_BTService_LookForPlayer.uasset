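; Behavior tree service that checks on each tick whether the player is directly in the AI pawn's line of sight.
; It traces the visibility channel forward from the pawn's eye viewpoint, out to the controller's sight range.
; A hit on the player character starts the find-player EQS query, while any other hit starts the find-POI query.
; No query runs when the trace hits nothing, and the service does not read the query results.
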(event EventReceiveTickAI
  (params (OwnerController :type AI%20Controller%20Object%20Reference) (ControlledPawn :type Pawn%20Object%20Reference) (DeltaSeconds :type Float%20%28single-precision%29))
  (bind (_outlocation _outrotation) (Actor|GetActorEyesViewPoint ControlledPawn))
  (bind (_outhit _returnvalue) (Collision|LineTraceByChannel _outlocation (+ _outlocation (* (Math|Vector|GetForwardVector _outrotation) (Class|ApolloAIBlueprintLibrary|GetSightRange OwnerController))) "TraceTypeQuery1" true 0 "None"))
  (if _returnvalue
    (if (== (.HitActor (Collision|BreakHitResult _outhit)) (Game|GetPlayerCharacter 0))
      (AI|EQS|RunEQSQuery "/Game/CheekyFPS/Blueprints/AI/BehaviorTrees/EQS_FindPlayer.EQS_FindPlayer" OwnerController "SingleResult")
      (else
        (AI|EQS|RunEQSQuery "/Game/CheekyFPS/Blueprints/AI/BehaviorTrees/EQS_FindPOI.EQS_FindPOI" OwnerController "SingleResult")))))