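; CheekyPlayerSettingsManager caches the player's control settings for the CheekyFPS game.
; On BeginPlay it copies crouch, prone, run and walk toggles, mouse and gamepad look options, and gamepad type from config getters into variables.
; Look getters pick the mouse or gamepad sensitivity, inversion or smoothing value from an IsGamepad flag.
; The smoothing getter inverts and scales the stored value, so a higher setting returns a lower number.
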(event EventBeginPlay
  (CallFunction|UpdatePlayerSettingsfromConfig))

(event EventTick
  (params (DeltaSeconds :type Float%20%28single-precision%29)))

(fn GetLookSmooth
  (params (bIsGamepad :type Boolean))
  (return (- 5e+01 (* (select bIsGamepad (Variables|Contol|Gamepad|GetGamepadSmooth) (Variables|Contol|Mouse|GetMouseSmooth)) 2e+01))))

(fn GetLookInvertY
  (params (bIsGamepad :type Boolean))
  (return (select bIsGamepad (Variables|Contol|Gamepad|GetbInvertGamepadY) (Variables|Contol|Mouse|GetbInvertMouseY))))

(fn GetLookInvertX
  (params (bIsGamepad :type Boolean))
  (return (select bIsGamepad (Variables|Contol|Gamepad|GetbInvertGamepadX) (Variables|Contol|Mouse|GetbInvertMouseX))))

(fn GetLookSensY
  (params (bIsGamepad :type Boolean))
  (return (select bIsGamepad (Variables|Contol|Gamepad|GetGamepadSensY) (Variables|Contol|Mouse|GetMouseSensY))))

(fn GetLookSensX
  (params (bIsGamepad :type Boolean))
  (return (select bIsGamepad (Variables|Contol|Gamepad|GetGamepadSensX) (Variables|Contol|Mouse|GetMouseSensX))))

(fn UpdatePlayerSettingsfromConfig
  (Variables|Default|SetbCrouchToggle (Class|ApolloPlayerSettingsLibrary|GetCrouchToggleSetting))
  (Variables|Default|SetbProneToggle (Class|ApolloPlayerSettingsLibrary|GetProneToggleSetting))
  (Variables|Default|SetbRunToggle (Class|ApolloPlayerSettingsLibrary|GetRunToggleSetting))
  (Variables|Default|SetbWalkToggle (Class|ApolloPlayerSettingsLibrary|GetWalkToggleSetting))
  (Variables|Contol|Mouse|SetbInvertMouseX (Class|ApolloPlayerSettingsLibrary|GetMouseInvertXSetting))
  (Variables|Contol|Mouse|SetbInvertMouseY (Class|ApolloPlayerSettingsLibrary|GetMouseInvertYSetting))
  (Variables|Contol|Gamepad|SetbInvertGamepadX (Class|ApolloPlayerSettingsLibrary|GetGamepadInvertXSetting))
  (Variables|Contol|Gamepad|SetbInvertGamepadY (Class|ApolloPlayerSettingsLibrary|GetGamepadInvertYSetting))
  (Variables|Contol|Mouse|SetMouseSensX (Class|ApolloPlayerSettingsLibrary|GetMouseXSensitivitySetting))
  (Variables|Contol|Mouse|SetMouseSensY (Class|ApolloPlayerSettingsLibrary|GetMouseYSensitivitySetting))
  (Variables|Contol|Mouse|SetMouseSmooth (Class|ApolloPlayerSettingsLibrary|GetMouseSmoothRateSetting))
  (Variables|Contol|Gamepad|SetGamepadSensX (Class|ApolloPlayerSettingsLibrary|GetGamepadXSensitivitySetting))
  (Variables|Contol|Gamepad|SetGamepadSensY (Class|ApolloPlayerSettingsLibrary|GetGamepadYSensitivitySetting))
  (Variables|Contol|Gamepad|SetGamepadSmooth (Class|ApolloPlayerSettingsLibrary|GetGamepadSmoothRateSetting))
  (Variables|Default|SetGamepadType (Class|ApolloPlayerSettingsLibrary|GetPlayerGamepadType)))