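; Base player controller for CheekyFPS that manages modal UI and gamepad-aware input, built on UINavigation hooks.
; Opening a widget pauses the game, disables character input and headbob, and shows the cursor for keyboard or mouse; removal restores game-only input.
; Any key press refreshes the gamepad icon set, served through data-table getters.
; Hotkeys toggle the elevator panel, fast-forward time, and delete the current save before reloading the level.
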(event EventBeginPlay
  (Class|SwitcherooBlueprintLibrary|SetInputDetectionEnabled true)
  (Development|PrintString (Utilities|String|ToString(Boolean) (Class|SwitcherooBlueprintLibrary|IsInputDetectionEnabled))))

(event EventTick
  (params (DeltaSeconds :type Float%20%28single-precision%29)))

(event EventOnAddWidgettoViewport
  (params (InWidget :type User%20Widget%20Object%20Reference))
  (CallFunction|OnCreateNewWidget InWidget))

(event EventOnSelect)

(event EventOnRootWidgetRemoved
  (bind _currentwbp (Variables|Default|GetCurrentWBP))
  (Variables|Default|SetbShowMouseCursor false)
  (Input|ResetIgnoreLookInput)
  (Input|ResetIgnoreMoveInput)
  (Input|SetInputModeGameOnly self)
  (Game|SetGamePaused false)
  (Utilities|IsValid _currentwbp
    (:Is%20Valid
      (CallFunction|RemoveWidget _currentwbp))))

(event EventOnReturn)

(event EventOnPrevious)

(event EventOnNext)

(event EventOnNavigated
  (params (NavigationDirection :type ENavigationDirection%20Enum :default "None")))

(event EventOnInputChanged
  (params (From :type EInputType%20Enum :default "None") (To :type EInputType%20Enum :default "None")))

(event EventUpdateIcons
  (Class|ISSPlayerController|UpdateGamepadIconSet (Class|ApolloPlayerSettingsLibrary|GetPlayerGamepadType)))

(event Input|KeyboardEvents|I
  (params (Key :type Key%20Structure))
  (:Pressed
    (Utilities|IsValid (Variables|Default|GetElevatorWBP)
      (:Is%20Valid
        (CallFunction|RemoveWidget (Variables|Default|GetElevatorWBP)))
      (:Is%20Not%20Valid
        (bind _returnvalue (UserInterface|CreateWidget "/Game/CheekyFPS/Blueprints/UMG/Menus/Prompts/WBP_ElevatorPanel.WBP_ElevatorPanel_C"))
        (bind _output_get (Variables|Default|SetElevatorWBP _returnvalue))
        (CallFunction|OnCreateNewWidget _output_get)))))

(event Input|KeyboardEvents|NumPadTwo
  (params (Key :type Key%20Structure))
  (:Pressed
    (bind _returnvalue (Class|RamaSaveLibrary|RamaSaveDeleteFile (CallFunction|GetCurrentSaveSlotFilePath)))
    (if _returnvalue
      (bind _returnvalue_2 (Game|GetCurrentLevelName true))
      (Game|OpenLevel(byName) (Utilities|String|StringToName _returnvalue_2)))))

(event Input|KeyboardEvents|AnyKey
  (params (Key :type Key%20Structure))
  (:Pressed
    (Utilities|FlowControl|Sequence
      (:then_0
        (Class|ISSPlayerController|UpdateGamepadIconSet (Class|ApolloPlayerSettingsLibrary|GetPlayerGamepadType)))
      (:then_1
        (Variables|Default|SetIsUsingGamepad? (Class|KismetInputLibrary|KeyIsGamepadKey Key))))))

(event Input|KeyboardEvents|NumPadOne
  (params (Key :type Key%20Structure))
  (:Pressed
    (Utilities|Time|SetGlobalTimeDilation 1e+01))
  (:Released
    (Utilities|Time|SetGlobalTimeDilation 1.0)))

(fn ConstructionScript)

(fn OnCreateNewWidget
  (params (NewWidget :type User%20Widget%20Object%20Reference))
  (Input|SetInputModeGameandUI self 0 "DoNotLock" false)
  (Game|SetGamePaused true)
  (UserInterface|Viewport|AddtoViewport NewWidget 0)
  (Input|DisableInput (Game|GetPlayerCharacter 0) self)
  (Utilities|FlowControl|Sequence
    (:then_0
      (for _array_element (Variables|/Game/CheekyFPS/Blueprints/CameraManager/BP_CheekyCameraManager.BP_CheekyCameraManager_C|GetCurrentCameraModifiers (.AsCheeky%20Camera%20Manager (Utilities|Casting|CastToBP_CheekyCameraManager (Game|GetPlayerCameraManager 0))))
        (if (== _array_element "/Game/CheekyFPS/Blueprints/CameraManager/CamModifiers/BP_CamModifier_Headbob.BP_CamModifier_Headbob")
          (CameraModifier|DisableModifier _array_element true))))
    (:then_1
      (switch Utilities|FlowControl|Switch|SwitchonEInputType (Class|UINavPCComponent|GetCurrentInputType (Variables|Default|GetUINavPC))
        (:Keyboard
          _)
        (:Mouse
          _))
      (Variables|Default|SetbShowMouseCursor true))))

(fn RemoveWidget
  (params (Widget :type Widget%20Object%20Reference))
  (bind _self self)
  (Widget|RemovefromParent Widget)
  (bind _output_get (Variables|Default|SetbShowMouseCursor false))
  (Game|SetGamePaused _output_get)
  (Input|SetInputModeGameOnly _self)
  (Class|Controller|ResetIgnoreInputFlags)
  (Input|EnableInput (Game|GetPlayerCharacter 0) _self))

(fn GetCurrentItem
  (return 0))

(fn GetGamepadIconDataTable
  (return (Variables|Default|GetCurrentGamepadIconData)))

(fn GetJoystickDirection
  (params (Stick :type EJoystickTypes%20Enum :default "NewEnumerator0"))
  (switch Utilities|FlowControl|Switch|SwitchonEJoystickTypes Stick
    (:NewEnumerator0
      (return (Math|Vector2D|MakeVector2D (Class|Actor|GetInputAxisKeyValue) (* (Class|Actor|GetInputAxisKeyValue) -1.0))))
    (:NewEnumerator1
      (return (Math|Vector2D|MakeVector2D (Class|Actor|GetInputAxisKeyValue) (Class|Actor|GetInputAxisKeyValue))))))

(fn GetKBMIconDataTable
  (return (Variables|Default|GetKBMIconData)))