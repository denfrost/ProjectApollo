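; Player objective component that tracks objectives and codex entries in two maps keyed by short name.
; Functions add entries to either map, return whole maps, and look up an objective's struct or title.
; Status updates set the completion flag on the found map value without re-adding it.
; The description getter returns the description when complete and the completion message otherwise, which looks inverted.
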(event EventBeginPlay)

(event EventTick
  (params (DeltaSeconds :type Float%20%28single-precision%29)))

(fn AddNewObjective
  (params (ObjectiveShortName :type String%20%28by%20ref%29) (NewObjectiveStructEntry :type S%20Player%20Objective%20Structure%20%28by%20ref%29))
  (Utilities|Map|Add (Variables|Objectives|GetObjectiveList) ObjectiveShortName NewObjectiveStructEntry))

(fn UpdateObjectiveStatus
  (params (ObjectiveShortName :type String%20%28by%20ref%29) (IsObjectiveComplete? :type Boolean))
  (bind _objectivelist (Variables|Objectives|GetObjectiveList))
  (bind (_value _returnvalue) (Utilities|Map|Find _objectivelist ObjectiveShortName))
  (if _returnvalue
    (Utilities|Struct|SetmembersinS_PlayerObjective _value IsObjectiveComplete?)))

(fn GetObjectiveDescription
  (params (ObjectiveShortName :type String%20%28by%20ref%29))
  (bind _returnvalue (CallFunction|GetObjective ObjectiveShortName))
  (bind (_isobjectivecomplete_ _objectivetitle _objectivedescription _objectivecompletemessage) (Utilities|Struct|BreakS_PlayerObjective _returnvalue))
  (if _isobjectivecomplete_
    (return _objectivedescription)
    (else
      (return _objectivecompletemessage))))

(fn GetObjective
  (params (ObjectiveShortName :type String%20%28by%20ref%29))
  (bind _objectivelist (Variables|Objectives|GetObjectiveList))
  (bind (_value _returnvalue) (Utilities|Map|Find _objectivelist ObjectiveShortName))
  (if _returnvalue
    (return _value)))

(fn GetObjectiveTitle
  (params (ObjectiveShortName :type String%20%28by%20ref%29))
  (return (.ObjectiveTitle (Utilities|Struct|BreakS_PlayerObjective (CallFunction|GetObjective ObjectiveShortName)))))

(fn GetObjectiveList
  (return (Variables|Objectives|GetObjectiveList)))

(fn AddNewCodexEntry
  (params (EntryShortName :type String%20%28by%20ref%29) (NewCodexStructEntry :type S%20Player%20Objective%20Structure%20%28by%20ref%29))
  (Utilities|Map|Add (Variables|Objectives|GetCodexList) EntryShortName NewCodexStructEntry))

(fn GetCodexList
  (return (Variables|Objectives|GetCodexList)))