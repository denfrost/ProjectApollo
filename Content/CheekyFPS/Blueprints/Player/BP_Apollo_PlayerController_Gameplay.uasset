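; Gameplay player controller that owns the HUD, minimap and scope widgets and runs the pause and character menus.
; Menu inputs toggle through FlipFlops, each checking the other menu's visibility, and opening either pauses the game.
; Hit and crit events drive timelines that tint the reticle red or gold, reversed after a retriggerable delay.
; Other events refresh weapon info, hide consumed-item HUD, toggle the scope and hide the HUD when new widgets are created.
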(event EventBeginPlay
  (|CallParentFunction)
  (bind _returnvalue (UserInterface|CreateWidget "/Game/CheekyFPS/Blueprints/UMG/WBP_GameplayHUD.WBP_GameplayHUD_C" 0 (.AsCheeky%20Character (Utilities|Casting|CastToBP_CheekyCharacter (Game|GetPlayerCharacter 0)))))
  (bind _output_get (Variables|Default|SetGameplayHUDWBP _returnvalue))
  (UserInterface|Viewport|AddtoViewport _returnvalue 0)
  (Variables|Default|SetMinimapWBP (Variables|/Game/CheekyFPS/Blueprints/UMG/WBP_GameplayHUD.WBP_GameplayHUD_C|GetWBP_Minimap _output_get))
  (bind _returnvalue_2 (UserInterface|CreateWidget "/Game/CheekyFPS/Blueprints/UMG/Gameplay/WBP_Scope.WBP_Scope_C"))
  (Variables|Default|SetScopeWBP _returnvalue_2)
  (Input|SetInputModeGameOnly self))

(event EventRegisterPlayerHit
  (bind _hittimeline (Variables|Default|GetHitTimeline))
  (Audio|Components|Audio|Play _hittimeline)
  (Utilities|FlowControl|RetriggerableDelay 0.6)
  (Utilities|String|Reverse _hittimeline))

(event EventUpdateWeaponHUD
  (Default|GetCurrentWeaponInfo (Variables|Default|GetGameplayHUDWBP)))

(event EventRegisterPlayerCritHit
  (bind _crithittimeline (Variables|Default|GetCritHitTimeline))
  (Audio|Components|Audio|Play _crithittimeline)
  (Utilities|FlowControl|RetriggerableDelay 0.6)
  (Utilities|String|Reverse _crithittimeline))

(event EventOnRootWidgetRemoved
  (|CallParentFunction)
  (Utilities|FlowControl|Sequence
    (:then_0
      (Utilities|IsValid (Variables|Default|GetPauseMenuWBP)
        (:Is%20Valid
          (CallFunction|RemoveWidget (Variables|Default|GetPauseMenuWBP))
          (Variables|Default|SetPauseMenuWBP 0))))))

(event EventOnItemConsumed
  (bind _gameplayhudwbp (Variables|Default|GetGameplayHUDWBP))
  (Default|ToggleBoxVisibility _gameplayhudwbp (Variables|/Game/CheekyFPS/Blueprints/UMG/WBP_GameplayHUD.WBP_GameplayHUD_C|GetItemImage _gameplayhudwbp) "Hidden")
  (Default|ToggleBoxVisibility _gameplayhudwbp (Variables|/Game/CheekyFPS/Blueprints/UMG/WBP_GameplayHUD.WBP_GameplayHUD_C|GetItemInfoBox _gameplayhudwbp) "Hidden"))

(event EventOnPlayerScopeZoom
  (params (ShowScope? :type Boolean))
  (bind _scopewbp (Variables|Default|GetScopeWBP))
  (if ShowScope?
    (UserInterface|Viewport|AddtoViewport _scopewbp 0)
    (else
      (Widget|RemovefromParent _scopewbp))))

(event Input|ActionEvents|InputActionCharacterMenu
  (params (Key :type Key%20Structure))
  (bind _returnvalue (Game|GetPlayerController 0))
  (bind _pausemenuwbp (Variables|Default|GetPauseMenuWBP))
  (:Pressed
    (Utilities|IsValid _pausemenuwbp
      (:Is%20Valid
        (if (not (Widget|IsVisible _pausemenuwbp))
          (Utilities|FlowControl|FlipFlop :!label _label
            (:A
              (bind _returnvalue_2 (UserInterface|CreateWidget "/Game/CheekyFPS/Blueprints/UMG/Gameplay/WBP_CharMenu.WBP_CharMenu_C"))
              (bind _output_get (Variables|Default|SetCharMenuWBP _returnvalue_2))
              (UserInterface|Viewport|AddtoViewport _returnvalue_2 0)
              (Input|SetInputModeGameandUI _returnvalue _output_get "DoNotLock" false)
              (bind _returnvalue_3 (Game|SetGamePaused true))
              (Variables|/Script/Engine.PlayerController|SetbShowMouseCursor _returnvalue _returnvalue_3))
            (:B
              (Widget|RemovefromParent (Variables|Default|GetCharMenuWBP))
              (Game|SetGamePaused false)
              (Variables|/Script/Engine.PlayerController|SetbShowMouseCursor (Game|GetPlayerController 0) false)
              (Input|SetInputModeGameOnly _returnvalue)
              (Variables|Default|SetCharMenuWBP 0)))))
      (:Is%20Not%20Valid
        (goto _label)))))

(event Input|ActionEvents|InputActionPause
  (params (Key :type Key%20Structure))
  (bind _charmenuwbp (Variables|Default|GetCharMenuWBP))
  (:Pressed
    (Utilities|IsValid _charmenuwbp
      (:Is%20Valid
        (if (not (Widget|IsVisible _charmenuwbp))
          (Utilities|FlowControl|FlipFlop :!label _label
            (:A
              (Variables|Default|SetbShowMouseCursor true)
              (Variables|Default|SetCurrentWBP (Variables|Default|GetPauseMenuWBP))
              (bind _returnvalue (UserInterface|CreateWidget "/Game/CheekyFPS/Blueprints/UMG/Gameplay/WBP_PauseMenu.WBP_PauseMenu_C"))
              (UserInterface|Viewport|AddtoViewport _returnvalue 0)
              (Input|SetInputModeGameandUI self 0 "DoNotLock" false)
              (Game|SetGamePaused true))
            (:B
              (CallFunction|RemoveWidget _returnvalue)
              (Variables|Default|SetPauseMenuWBP 0)))))
      (:Is%20Not%20Valid
        (goto _label)))))

(fn ConstructionScript
  (|CallParentFunction))

(fn OnCreateNewWidget
  (params (NewWidget :type User%20Widget%20Object%20Reference))
  (bind _gameplayhudwbp (Variables|Default|GetGameplayHUDWBP))
  (if (Widget|IsVisible _gameplayhudwbp)
    (Widget|SetVisibility _gameplayhudwbp "Hidden")
    (Widget|SetVisibility (Variables|/Game/CheekyFPS/Blueprints/UMG/WBP_GameplayHUD.WBP_GameplayHUD_C|GetWBP_Minimap _gameplayhudwbp) "HitTestInvisible")
    (|CallParentFunction NewWidget)
    (else
      (|CallParentFunction NewWidget))))