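; Gameplay player controller that owns the HUD and handles pausing in CheekyFPS.
; On BeginPlay it creates the gameplay HUD for the player's CheekyCharacter, and UpdateWeaponHUD refreshes its weapon info.
; Pause opens the pause menu, showing the cursor, ignoring look and move input and pausing the game.
; If an item wheel or pause menu exists, Pause instead removes the item wheel widget, clears the menu reference and resumes game-only input.
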(event EventBeginPlay
  (|CallParentFunction)
  (bind _returnvalue (UserInterface|CreateWidget "/Game/CheekyFPS/Blueprints/UMG/WBP_GameplayHUD.WBP_GameplayHUD_C" 0 (.AsCheeky%20Character (Utilities|Casting|CastToCheekyCharacter (Game|GetPlayerCharacter 0)))))
  (UserInterface|Viewport|AddtoViewport _returnvalue 0)
  (Variables|Default|SetGameplayHUD_WBP _returnvalue))

(event EventTick
  (params (DeltaSeconds :type Float%20%28single-precision%29))
  (|CallParentFunction DeltaSeconds) ; This node is disabled and will not be called.\nDrag off pins to build functionality.
)

(event EventUpdateWeaponHUD
  (Default|GetCurrentWeaponInfo (Variables|Default|GetGameplayHUD_WBP)))

(event Input|ActionEvents|InputActionPause
  (params (Key :type Key%20Structure :default "None"))
  (bind _itemwheelwbp (Variables|Default|GetItemWheelWBP))
  (:Pressed
    (Utilities|IsValid _itemwheelwbp
      (:Is%20Valid
        (Widget|RemovefromParent _itemwheelwbp :!label _label)
        (Game|SetGamePaused false)
        (Input|SetInputModeGameOnly self)
        (Variables|Default|SetPauseMenuWBP 0))
      (:Is%20Not%20Valid
        (Utilities|IsValid (Variables|Default|GetPauseMenuWBP)
          (:Is%20Valid
            (goto _label))
          (:Is%20Not%20Valid
            (Variables|Default|SetbShowMouseCursor true)
            (Input|SetIgnoreLookInput true)
            (Input|SetIgnoreMoveInput true)
            (bind _returnvalue (UserInterface|CreateWidget "/Game/CheekyFPS/Blueprints/UMG/WBP_PauseMenu.WBP_PauseMenu_C"))
            (bind _output_get (Variables|Default|SetPauseMenuWBP _returnvalue))
            (UserInterface|Viewport|AddtoViewport _output_get 0)
            (Input|SetInputModeGameandUI self 0 "DoNotLock" false)
            (Game|SetGamePaused true)))))))

(fn ConstructionScript
  (|CallParentFunction))