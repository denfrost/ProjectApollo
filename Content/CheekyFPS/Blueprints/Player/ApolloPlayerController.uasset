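; Player controller for the Apollo player that runs hold-to-open weapon and item radial menus.
; Pressing a menu input creates its wheel widget, pauses the game and switches to Game and UI input; releasing removes it and restores play.
; Interact forwards a select message to the item wheel only.
; GetJoystickDirection returns either stick's axes as a 2D vector, inverting Y for the left stick.
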(event EventBeginPlay)

(event EventTick
  (params (DeltaSeconds :type Float%20%28single-precision%29)))

(event Input|ActionEvents|InputActionWeaponMenu
  (params (Key :type Key%20Structure :default "None"))
  (bind _self self)
  (:Pressed
    (Utilities|IsValid (Variables|Default|GetWeaponWheelWBP)
      (:Is%20Not%20Valid
        (bind _returnvalue (UserInterface|CreateWidget "/Game/CheekyFPS/Blueprints/UI/WBP_WeaponWheel.WBP_WeaponWheel_C"))
        (Variables|Default|SetWeaponWheelWBP _returnvalue)
        (UserInterface|Viewport|AddtoViewport _returnvalue 0)
        (Game|SetGamePaused true)
        (Input|SetInputModeGameandUI _self 0 "DoNotLock" true))))
  (:Released
    (Widget|RemovefromParent (Variables|Default|GetWeaponWheelWBP))
    (Game|SetGamePaused false)
    (Input|SetInputModeGameOnly _self)
    (Variables|Default|SetWeaponWheelWBP 0)))

(event Input|ActionEvents|InputActionItemMenu
  (params (Key :type Key%20Structure :default "None"))
  (bind _self self)
  (:Pressed
    (Utilities|IsValid (Variables|Default|GetItemWheelWBP)
      (:Is%20Not%20Valid
        (bind _returnvalue (UserInterface|CreateWidget "/Game/CheekyFPS/Blueprints/UI/WBP_ItemWheel.WBP_ItemWheel_C"))
        (Variables|Default|SetItemWheelWBP _returnvalue)
        (UserInterface|Viewport|AddtoViewport _returnvalue 0)
        (Game|SetGamePaused true)
        (Input|SetInputModeGameandUI _self 0 "DoNotLock" true))))
  (:Released
    (Widget|RemovefromParent (Variables|Default|GetItemWheelWBP))
    (Game|SetGamePaused false)
    (Input|SetInputModeGameOnly _self)
    (Variables|Default|SetItemWheelWBP 0)))

(event Input|ActionEvents|InputAction[CHEEKY]Interact
  (params (Key :type Key%20Structure :default "None"))
  (:Pressed
    (Class|BPIPlayer|PlayerSelect(Message) (Variables|Default|GetItemWheelWBP))))

(fn ConstructionScript)

(fn GetJoystickDirection
  (params (Stick :type EJoystickTypes%20Enum :default "NewEnumerator0"))
  (switch Utilities|FlowControl|Switch|SwitchonEJoystickTypes Stick
    (:NewEnumerator0
      (return (Math|Vector2D|MakeVector2D (Class|Actor|GetInputAxisKeyValue) (* (Class|Actor|GetInputAxisKeyValue) -1.0))))
    (:NewEnumerator1
      (return (Math|Vector2D|MakeVector2D (Class|Actor|GetInputAxisKeyValue) (Class|Actor|GetInputAxisKeyValue))))))