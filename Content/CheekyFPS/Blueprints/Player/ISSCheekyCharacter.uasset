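; Player character for CheekyFPS, extending a parent character with grapple, dash and cloak abilities.
; Grapple line-traces from the camera and uses looping timers, with grip strength that drains and recovers.
; Dash applies directional impulses, while cloak swaps the first-person material and unregisters AI sight stimuli.
; It also forwards weapon, power, objective, codex and photo-mode calls to components, tracks kill stats, and restores position and inventory through RamaSave.
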(event RamaSaveEventPreSave(RamaSave)
  (params (RamaSaveComponent :type Rama%20Save%20Component%20Object%20Reference))
  (bind _returnvalue (Game|GetCurrentLevelName true))
  (Variables|Default|SetPlayerSavedLevel _returnvalue)
  (Variables|Default|SetPlayerCurrentTransform (Transformation|GetActorTransform)))

(event RamaSaveEventActorFullyLoaded(RamaSave)
  (params (RamaSaveComponent :type Rama%20Save%20Component%20Object%20Reference) (LevelPackageName :type String))
  (bind _playercurrenttransform (Variables|Default|GetPlayerCurrentTransform))
  (bind _returnvalue (Game|GetCurrentLevelName true))
  (if (Utilities|Enum|Equal(Enum) _returnvalue (Variables|Default|GetPlayerSavedLevel))
    (Transformation|Teleport (.location _playercurrenttransform) (.rotation _playercurrenttransform))))

(event OnComponentBeginOverlap(CapsuleComponent)
  (params (OverlappedComponent :type Primitive%20Component%20Object%20Reference) (OtherActor :type Actor%20Object%20Reference) (OtherComp :type Primitive%20Component%20Object%20Reference) (OtherBodyIndex :type Integer) (bFromSweep :type Boolean) (SweepResult :type Hit%20Result%20Structure%20%28by%20ref%29))
  (if (and (Utilities|Enum|Equal(Enum) (Variables|Default|GetCurrentPlayerStance) "NewEnumerator5") (Actor|ActorHasTag OtherActor "Grapple"))
    (Variables|Default|SetIsGrappling? true)
    (else
      (Variables|Default|SetIsGrappling? false))))

(event Custom|ReloadPlayerItemData
  (params (RamaSaveComponent :type Rama%20Save%20Component%20Object%20Reference))
  (bind _returnvalue (Game|GetPlayerController 0))
  (bind _returnvalue_2 (Pawn|GetControlledPawn _returnvalue))
  (bind _asisscheeky_character (Utilities|Casting|CastToISSCheekyCharacter _returnvalue_2))
  (bind _inventorycomponent (Variables|/Game/CheekyFPS/Blueprints/CheekyCharacter.CheekyCharacter_C|GetInventoryComponent _asisscheeky_character))
  (for _array_element (Variables|/Game/CheekyFPS/Blueprints/Components/InventoryComponent.InventoryComponent_C|GetSpawnItemInventory _inventorycomponent)
    (if (Utilities|IsValidClass _array_element)
      (Default|SpawnItem _inventorycomponent _array_element)))
  (Development|PrintString "Done respawning items!"))

(event Custom|ReloadPlayerWeaponData
  (params (RamaSaveComponent :type Rama%20Save%20Component%20Object%20Reference))
  (bind _returnvalue (Game|GetPlayerController 0))
  (bind _returnvalue_2 (Pawn|GetControlledPawn _returnvalue))
  (bind _asisscheeky_character (Utilities|Casting|CastToISSCheekyCharacter _returnvalue_2))
  (bind _bp_weaponcomponent (Variables|/Game/CheekyFPS/Blueprints/CheekyCharacter.CheekyCharacter_C|GetBP_WeaponComponent _asisscheeky_character))
  (for _array_element (Variables|/Game/CheekyFPS/Blueprints/Components/BP_WeaponComponent.BP_WeaponComponent_C|GetSpawnedWeaponsInventory _bp_weaponcomponent)
    (Default|SpawnWeapon _bp_weaponcomponent _array_element)))

(event Custom|GetRelaxedState
  (params (Relax :type Boolean))
  (bind _output_get (Variables|Default|SetIsRelaxed Relax))
  (Class|BPAnimInterface|UpdateRelaxedState(Message) (Variables|Default|GetArmsAnimInstance) _output_get))

(event EventBeginPlay
  (bind _ramasave (Variables|Default|GetRamaSave))
  (bind _healthcomponent (Variables|Default|GetHealthComponent))
  (bind _apollopowercomponent (Variables|Default|GetApolloPowerComponent))
  (|CallParentFunction)
  (Variables|/Game/CheekyFPS/Blueprints/Health/CheekyHealthComponent.CheekyHealthComponent_C|SetbUseFallDamage _healthcomponent false)
  (bind _output_get (Variables|/Game/CheekyFPS/Blueprints/Health/CheekyHealthComponent.CheekyHealthComponent_C|SetMaxHP _healthcomponent 2e+02))
  (Variables|/Game/CheekyFPS/Blueprints/Health/CheekyHealthComponent.CheekyHealthComponent_C|SetCurrentHP _healthcomponent _output_get)
  (Utilities|FlowControl|Sequence
    (:then_0
      (Variables|Default|SetDashVectorInAirMultiplier (/ (Variables|Default|GetDashVectorMultiplier) 3.25))
      (bind _output_get_2 (Variables|Default|SetDefaultMeshMaterial (Rendering|Material|GetMaterial (Variables|Default|GetFPMesh) 0)))
      (bind _returnvalue (Rendering|Material|CreateDynamicMaterialInstance (Variables|Default|GetFPMesh) 0 _output_get_2 "None" :!class /Script/Engine.PrimitiveComponent))
      (Variables|Default|SetFPMeshDynMat _returnvalue)
      (EventDispatchers|BindEventtoRamaSaveEventPreLoadDestroy _ramasave (EventDispatchers|CreateEvent :!event Custom|ReloadPlayerWeaponData))
      (EventDispatchers|BindEventtoRamaSaveEventPreLoadDestroy _ramasave (EventDispatchers|CreateEvent :!event Custom|ReloadPlayerItemData))
      (Default|Initialization (Variables|Default|GetPhotoModeComponent) self (Variables|Default|GetCamera) (Variables|Default|GetSpringArm) (Game|GetPlayerController 0))
      (Variables|Default|SetCurrentGripStrength (Variables|Default|GetMaxGripStrength)))
    (:then_1
      (if (Utilities|IsValid (Variables|Default|GetBP_WeaponComponent))
        (CallFunction|EquipWeapon(byKey))
        (Development|SetHiddeninGame (Variables|Character|GetMesh) true false)))
    (:then_2
      (Default|SetNewPower _apollopowercomponent (Default|FindPower _apollopowercomponent "TacticalCloak"))
      (Default|SetNewAbility _apollopowercomponent (Default|FindAbility _apollopowercomponent (Utilities|String|MakeLiteralString "Dash"))))))

(event EventAttemptDash
  (CallFunction|ActivateDash))

(event EventAttemptCloak
  (CallFunction|ActivateCloak))

(event EventStopCloak
  (CallFunction|DeactivateCloak))

(event EventUpdateWeaponAmmoCount
  (params (RemainingAmmo :type Integer))
  (Default|CallOnFiredWeapon RemainingAmmo))

(event EventToggleRelaxState
  (params (bIsRelaxed? :type Boolean))
  (CallFunction|GetRelaxedState bIsRelaxed?))

(event EventPlayerUnequipWeapon
  (Class|BPAnimInterface|UnequipWeapon(Message) (Variables|Default|GetMyABP))
  (Utilities|FlowControl|Delay 0.5)
  (CallFunction|UnequipWeapon)
  (CallFunction|ToggleRelaxState true))

(event EventOnPlayerKilledEnemy
  (params (bIsBoss? :type Boolean))
  (bind _playerprofilestruct (Variables|Default|GetPlayerProfileStruct))
  (bind (_numenemieskilled _numenemiescritkilled _numbosseskilled) (Utilities|Struct|BreakInGameStatsStruct _playerprofilestruct))
  (if bIsBoss?
    (Utilities|Struct|SetmembersinInGameStatsStruct _playerprofilestruct (+ _numbosseskilled 1))
    (else
      (Utilities|Struct|SetmembersinInGameStatsStruct _playerprofilestruct (+ _numenemieskilled 1)))))

(event EventOnPlayerCritKilledEnemy
  (params (bIsBoss? :type Boolean))
  (bind _playerprofilestruct (Variables|Default|GetPlayerProfileStruct))
  (bind (_numenemieskilled _numenemiescritkilled _numbosseskilled) (Utilities|Struct|BreakInGameStatsStruct _playerprofilestruct))
  (if bIsBoss?
    (Utilities|Struct|SetmembersinInGameStatsStruct _playerprofilestruct (+ _numenemiescritkilled 1))
    (else
      (Utilities|Struct|SetmembersinInGameStatsStruct _playerprofilestruct (+ _numbosseskilled 1)))))

(event EventOnPlayerUseRecoveryItem
  (bind _playerprofilestruct (Variables|Default|GetPlayerProfileStruct))
  (Utilities|Struct|SetmembersinInGameStatsStruct _playerprofilestruct (+ (.NumRecoveryItemsUsed (Utilities|Struct|BreakInGameStatsStruct _playerprofilestruct)) 1)))

(event EventOnJumped
  (bind _charactermovement (Variables|Character|GetCharacterMovement))
  (if (<= (Variables|/Script/Engine.CharacterMovementComponent|GetGravityScale _charactermovement) 0.0)
    (Variables|/Script/Engine.CharacterMovementComponent|SetGravityScale _charactermovement 1.0)))

(event EventTick
  (params (DeltaSeconds :type Float%20%28single-precision%29))
  (|CallParentFunction DeltaSeconds)
  (Utilities|FlowControl|Sequence
    (:then_1
      (bind _output_get (Variables|Default|SetisMovingForward? (Math|Conversions|ToBoolean(Integer) (Math|Float|Round (Input|AxisValues|GetMoveForward)))))
      (if _output_get
        _))
    (:then_2
      (bind _output_get_2 (Variables|Default|SetisMovingRight? (Math|Conversions|ToBoolean(Integer) (Math|Float|Round (Input|AxisValues|GetMoveRight)))))
      (if _output_get_2
        _))))

(event EventOnPlayerPickedUpGrapple
  (Variables|Default|SetbCanGrapple? true))

(event EventOnLanded
  (params (Hit :type Hit%20Result%20Structure%20%28by%20ref%29))
  (|CallParentFunction Hit)
  (if (Utilities|Enum|Equal(Enum) (Variables|Default|GetCurrentPlayerStance) "NewEnumerator5")
    (Variables|Default|SetCurrentPlayerStance "NewEnumerator0")))

(event EventMoveForwardInput
  (params (Axis :type Float%20%28single-precision%29))
  (|CallParentFunction Axis)
  (if (Utilities|Enum|Equal(Enum) (Variables|Default|GetCurrentPlayerStance) "NewEnumerator5")
    (Physics|AddImpulse (Variables|Character|GetCharacterMovement) (* (Math|Vector|GetForwardVector (Transformation|GetActorRotation)) (* Axis 5e+03)) false)))

(event EventAddNewObjective
  (params (NewObjective :type S%20Player%20Objective%20Structure) (NewObjectiveShortName :type String))
  (Default|AddNewObjective (Variables|Default|GetBP_ObjectiveComponent) NewObjectiveShortName NewObjective))

(event EventOnObjectiveComplete
  (params (ObjectiveShortName :type String))
  (Default|UpdateObjectiveStatus (Variables|Default|GetBP_ObjectiveComponent) ObjectiveShortName true))

(event EventAddNewCodexEntry
  (params (NewEntryShortName :type String) (NewCodexEntry :type S%20Player%20Objective%20Structure))
  (Default|AddNewCodexEntry (Variables|Default|GetBP_ObjectiveComponent) NewEntryShortName NewCodexEntry))

(event EventUpdateCurrentPower
  (params (InPower :type Magic%20Action%20Struct%20Structure))
  (Default|SetNewPower (Variables|Default|GetApolloPowerComponent) InPower))

(event EventUpdateCurrentAbility
  (params (InAbility :type Magic%20Action%20Struct%20Structure))
  (Default|SetNewAbility (Variables|Default|GetApolloPowerComponent) InAbility))

(event EventToggleSonarEffect?
  (params (bActivateEffect? :type Boolean))
  (bind _sonaroverlaptimeline (Variables|Default|GetSonarOverlapTimeline))
  (if bActivateEffect?
    (Components|Timeline|PlayfromStart _sonaroverlaptimeline)
    (else
      (Audio|Components|Audio|Stop _sonaroverlaptimeline))))

(event EventOnActivateCamo
  (params (CamoLevel :type Integer))
  (bind _aiperceptionstimulisource (Variables|Default|GetAIPerceptionStimuliSource))
  (Variables|Default|SetbIsInvisible? true)
  (switch int CamoLevel
    (:1
      (Class|AIPerceptionStimuliSourceComponent|UnregisterfromSense _aiperceptionstimulisource "/Script/AIModule.AISense_Sight"))
    (:2
      (Class|AIPerceptionStimuliSourceComponent|UnregisterfromSense _aiperceptionstimulisource "/Script/AIModule.AISense_Sight")
      (Class|AIPerceptionStimuliSourceComponent|UnregisterfromSense _aiperceptionstimulisource "/Script/AIModule.AISense_Hearing"))))

(event EventPlayerEquipWeapon
  (params (DesiredIndex :type Integer))
  (CallFunction|EquipWeapon(byKey) DesiredIndex))

(event EventAddLight
  (params (NewLight :type Light%20Base%20Object%20Reference))
  (Variables|Default|SetClosestLight NewLight))

(event EventRemoveLight
  (params (NewLight :type Light%20Base%20Object%20Reference))
  (Variables|Default|SetClosestLight (Variables|Default|GetEmptyLight)))

(event EventEquipWeapon
  (CallFunction|EquipWeapon(byKey) (Variables|Default|GetNewWeaponKey)))

(event EventUpdateSettingsfromConfig
  (Default|UpdatePlayerSettingsfromConfig (Variables|Default|GetPlayerSettingsManager))
  (Class|BPIPlayer|UpdateIcons(Message) (Game|GetPlayerController 0)))

(event Input|ActionEvents|InputActionPhotoMode
  (params (Key :type Key%20Structure :default "None"))
  (:Pressed
    (Default|PhotoMode (Variables|Default|GetPhotoModeComponent) Key)))

(event Input|ActionEvents|InputActionGallery
  (params (Key :type Key%20Structure :default "None"))
  (:Pressed
    (Default|OpenGallery (Variables|Default|GetPhotoModeComponent) Key)))

(event Input|ActionEvents|InputActionGrapple
  (params (Key :type Key%20Structure :default "None"))
  (bind _bcangrapple_ (Variables|Default|GetbCanGrapple?))
  (:Pressed
    (if _bcangrapple_
      (CallFunction|StartGrapple)))
  (:Released
    (if _bcangrapple_
      (CallFunction|CancelGrapple))))

(event Input|KeyboardEvents|B
  (params (Key :type Key%20Structure :default "None"))
  (:Pressed
    (Utilities|FlowControl|FlipFlop
      (:A
        (CallFunction|ActivateCloak))
      (:B
        (CallFunction|DeactivateCloak)))))

(event Input|KeyboardEvents|X
  (params (Key :type Key%20Structure :default "None"))
  (:Pressed
    (CallFunction|GetRelaxedState (not (Variables|Default|GetIsRelaxed)))))

(fn ConstructionScript
  (|CallParentFunction))

(fn CheckforCamoUpdates
  (bind _closestlight (Variables|Default|GetClosestLight))
  (bind _distancefromplayer (Variables|/Game/CheekyFPS/External/Environment/InteractiveLights/Blueprints/BaseElements/Light_Base.Light_Base_C|GetDistanceFromPlayer _closestlight))
  (Utilities|IsValid (Variables|Default|GetClosestLight)
    (:Is%20Valid
      (Utilities|FlowControl|Sequence
        (:then_0
          (Utilities|FlowControl|Sequence
            (:then_0
              (if (>= (Variables|Default|GetCurrentCamoIndex) 1.0)
                (Variables|Default|SetCurrentCamoIndex (Variables|Default|GetMaxCamoIndex))))
            (:then_1
              (if (<= (Variables|Default|GetCurrentCamoIndex) 0.0)
                (Variables|Default|SetCurrentCamoIndex 0.0)))))
        (:then_1
          (if (<= _distancefromplayer 0.4)
            (Variables|Default|SetCurrentCamoIndex _distancefromplayer)))))
    (:Is%20Not%20Valid
      (Variables|Default|SetCurrentCamoIndex (- (Variables|Default|GetCurrentCamoIndex) 0.025)))))

(fn GetEquippedWeaponInfo
  (return (Default|GetWeaponData (Variables|/Game/CheekyFPS/Blueprints/Components/BP_WeaponComponent.BP_WeaponComponent_C|GetCurrentWeapon (Variables|Default|GetBP_WeaponComponent)))))

(fn ActivateDash
  (bind _returnvalue (Transformation|GetActorRotation))
  (bind _charactermovement (Variables|Character|GetCharacterMovement))
  (bind _charactermovement_2 (Variables|Character|GetCharacterMovement))
  (bind _dashvectormultiplier (Variables|Default|GetDashVectorMultiplier))
  (bind _dashvectorinairmultiplier (Variables|Default|GetDashVectorInAirMultiplier))
  (bind _charactermovement_3 (Variables|Character|GetCharacterMovement))
  (bind _returnvalue_2 (Math|Vector|GetRightVector _returnvalue))
  (bind _returnvalue_3 (AI|Components|NavMovement|IsFalling _charactermovement_3))
  (bind _returnvalue_4 (select _returnvalue_3 _dashvectorinairmultiplier _dashvectormultiplier))
  (Utilities|FlowControl|Sequence
    (:then_0
      (if (Variables|Default|GetisMovingForward?)
        (if (< (Input|AxisValues|GetMoveForward) 0.0)
          (Physics|AddImpulse _charactermovement_2 (* (Math|Vector|NegateVector (Math|Vector|GetForwardVector (Transformation|GetActorRotation))) (select (AI|Components|NavMovement|IsFalling (Variables|Character|GetCharacterMovement)) (Variables|Default|GetDashVectorInAirMultiplier) (Variables|Default|GetDashVectorMultiplier))) true)
          (else
            (Physics|AddImpulse _charactermovement_2 (* (Math|Vector|GetForwardVector (Transformation|GetActorRotation)) (select (AI|Components|NavMovement|IsFalling (Variables|Character|GetCharacterMovement)) (Variables|Default|GetDashVectorInAirMultiplier) (Variables|Default|GetDashVectorMultiplier))) true)))
        (elif (Variables|Default|GetisMovingRight?)
          (if (< (Input|AxisValues|GetMoveRight) 0.0)
            (Physics|AddImpulse _charactermovement (* (Math|Vector|NegateVector _returnvalue_2) _returnvalue_4) true)
            (else
              (Physics|AddImpulse _charactermovement (* _returnvalue_2 _returnvalue_4) true)))
          (else
            (Physics|AddImpulse (Variables|Character|GetCharacterMovement) (* "0,1.000000, 0" (select (AI|Components|NavMovement|IsFalling (Variables|Character|GetCharacterMovement)) (Variables|Default|GetDashVectorInAirMultiplier) (Variables|Default|GetDashVectorMultiplier))) true)))))))

(fn ActivateCloak
  (Class|AIPerceptionStimuliSourceComponent|UnregisterfromSense (Variables|Default|GetAIPerceptionStimuliSource) "/Script/AIModule.AISense_Sight")
  (Rendering|Material|SetMaterial (Variables|Default|GetFPMesh) 0 (Variables|Default|GetCloakMeshMaterial)))

(fn DeactivateCloak
  (Class|AIPerceptionStimuliSourceComponent|RegisterforSense (Variables|Default|GetAIPerceptionStimuliSource) "/Script/AIModule.AISense_Sight")
  (Rendering|Material|SetMaterial (Variables|Default|GetFPMesh) 0 (Variables|Default|GetDefaultMeshMaterial)))

(fn EquipWeapon(byKey)
  (params (Key :type Integer))
  (if (!= Key 0)
    (|CallParentFunction Key)
    (CallFunction|ToggleRelaxState false)
    (else
      (CallFunction|PlayerUnequipWeapon))))

(fn MovetoGrappleLocation
  (bind _grappleouthit (Variables|Default|GetGrappleOutHit))
  (bind _charactermovement (Variables|Character|GetCharacterMovement))
  (bind (_bblockinghit _binitialoverlap _time _distance _location _impactpoint _normal _impactnormal _physmat _hitactor _hitcomponent) (Collision|BreakHitResult _grappleouthit))
  (if (Utilities|IsValid _hitactor)
    (if (and _bblockinghit (not (Actor|ActorHasTag _hitactor "Blocker")))
      (Class|NavMovementComponent|StopMovementKeepPathing (Variables|Character|GetCharacterMovement))
      (Class|PhysicsHandleComponent|GrabComponentatLocation (Variables|Default|GetPhysicsHandle) _hitcomponent "None" _impactpoint)
      (Class|MovementComponent|SetPlaneConstraintNormal _charactermovement "1.000000, 0,1.000000")
      (Class|MovementComponent|SetPlaneConstraintEnabled _charactermovement true)
      (bind _returnvalue (Transformation|SetActorLocation (Math|Interpolation|VInterpTo (Transformation|GetActorLocation) _impactpoint (Utilities|Time|GetWorldDeltaSeconds) 6.0) true false))
      (Variables|Default|SetCurrentPlayerStance "NewEnumerator5")
      (else
        (return)))
    (else
      (return))))

(fn CanJumpInternal
  (if (Utilities|Enum|Equal(Enum) (Variables|Default|GetCurrentPlayerStance) "NewEnumerator5")
    (if (<= (Variables|Default|GetJumpCurrentCount) (Variables|Default|GetJumpMaxCount))
      (return true)
      (else
        (return false)))
    (else
      (bind _returnvalue (|CallParentFunction))
      (return _returnvalue))))

(fn StartGrapple
  (bind _camera (Variables|Default|GetCamera))
  (bind _returnvalue (Transformation|GetWorldTransform _camera))
  (bind _outhit (Collision|LineTraceByChannel (.location _returnvalue) (+ (.location _returnvalue) (* (Math|Vector|GetForwardVector (.rotation _returnvalue)) 3e+03)) "TraceTypeQuery4" false 0 "ForDuration"))
  (Utilities|FlowControl|Sequence
    (:then_0
      (Variables|Default|SetGrappleOutHit _outhit)
      (bind _returnvalue_2 (Utilities|Time|SetTimerbyEvent (EventDispatchers|CreateEvent :!event MovetoGrappleLocation) 0.01 true))
      (Variables|Default|SetGrappleTimer _returnvalue_2)
      (bind _returnvalue_3 (Utilities|Time|SetTimerbyEvent (EventDispatchers|CreateEvent :!event ConsumeGrapple) 0.1 true))
      (Variables|Default|SetGripStrengthTimer _returnvalue_3))
    (:then_1
      (if (Utilities|IsValid (.HitActor (Collision|BreakHitResult _outhit)))
        (if (and (.bBlockingHit (Collision|BreakHitResult _outhit)) (not (Actor|ActorHasTag (.HitActor (Collision|BreakHitResult _outhit)) "Blocker")))
          (Audio|PlaySound2D "/Game/CheekyFPS/Sounds/Future_Crossbow_arrow_hit.Future_Crossbow_arrow_hit" 1.0 1.0 0.0 0 0))))))

(fn CancelGrapple
  (bind _charactermovement (Variables|Character|GetCharacterMovement))
  (Variables|/Script/Engine.CharacterMovementComponent|SetGravityScale _charactermovement 1.0)
  (Variables|/Script/Engine.CharacterMovementComponent|SetAirControl _charactermovement 0.5)
  (Class|MovementComponent|SetPlaneConstraintEnabled _charactermovement false)
  (Utilities|Time|ClearandInvalidateTimerbyHandle (Variables|Default|GetGrappleTimer))
  (CallFunction|StopGrappleConsume)
  (bind _returnvalue (Utilities|Time|SetTimerbyEvent (EventDispatchers|CreateEvent :!event RecoverGrapple) 0.1 true))
  (Variables|Default|SetRecoverGrappleTimer _returnvalue))

(fn ConsumeGrapple
  (if (Variables|Default|GetIsGrappling?)
    (bind _output_get (Variables|Default|SetCurrentGripStrength (- (Variables|Default|GetCurrentGripStrength) 0.1)))
    (Default|CallOnUpdateGrapple _output_get)
    (if (<= _output_get 0.0)
      (CallFunction|CancelGrapple))))

(fn StopGrappleConsume
  (if (or (Utilities|Enum|Equal(Enum) (Variables|Default|GetCurrentPlayerStance) "NewEnumerator0") (AI|Components|NavMovement|IsFalling))
    (Variables|Default|SetIsGrappling? false)))

(fn RecoverGrapple
  (if (not (Variables|Default|GetIsGrappling?))
    (if (AI|Components|NavMovement|IsMovingonGround)
      (bind _output_get (Variables|Default|SetCurrentGripStrength (+ (Variables|Default|GetCurrentGripStrength) 0.1)))
      (Default|CallOnUpdateGrapple _output_get)
      (if (>= _output_get (Variables|Default|GetMaxGripStrength))
        (Variables|Default|SetCurrentGripStrength (Variables|Default|GetMaxGripStrength))
        (Utilities|Time|ClearandInvalidateTimerbyHandle (Variables|Default|GetRecoverGrappleTimer))))))

(fn SearchforGrapplePoint
  (bind _camera (Variables|Default|GetCamera))
  (bind _returnvalue (Transformation|GetWorldTransform _camera))
  (if (Variables|Default|GetbCanGrapple?)
    (bind _returnvalue_2 (Collision|LineTraceByChannel (.location _returnvalue) (+ (.location _returnvalue) (* (Math|Vector|GetForwardVector (.rotation _returnvalue)) 3.5e+03)) "TraceTypeQuery4" false 0 "None"))
    (if _returnvalue_2
      (Development|PrintString "Can Grapple")
      (else
        (Development|PrintString "Can't Grapple")))))

(fn CanPlayerGrapple
  (return (Variables|Default|GetbCanGrapple?)))

(fn IsGrappleActive?
  (return (Variables|Default|GetIsGrappling?)))

(fn GetCurrentItem)

(fn GetGamepadIconDataTable
  (return 0))

(fn GetKBMIconDataTable
  (return 0))