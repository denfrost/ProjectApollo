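; Base player controller that handles gamepad detection and switching between gameplay and UI input.
; Any key press refreshes the gamepad icon set and records whether a gamepad is in use.
; The I key toggles an elevator panel widget, pausing on creation, while removal restores game-only input but leaves unpausing to OnRootWidgetRemoved.
; Menu navigation events are empty stubs, and a helper returns either stick's direction as a 2D vector.
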(event EventBeginPlay)

(event EventTick
  (params (DeltaSeconds :type Float%20%28single-precision%29)))

(event EventOnSelect)

(event EventOnRootWidgetRemoved
  (Variables|Default|SetbShowMouseCursor false)
  (Input|ResetIgnoreLookInput)
  (Input|ResetIgnoreMoveInput)
  (Input|SetInputModeGameOnly self)
  (Game|SetGamePaused false))

(event EventOnReturn)

(event EventOnPrevious)

(event EventOnNext)

(event EventOnNavigated
  (params (NavigationDirection :type ENavigationDirection%20Enum :default "None")))

(event EventOnInputChanged
  (params (From :type EInputType%20Enum :default "None") (To :type EInputType%20Enum :default "None")))

(event EventUpdateIcons
  (Class|ISSPlayerController|UpdateGamepadIconSet (Class|ApolloPlayerSettingsLibrary|GetPlayerGamepadType)))

(event Input|KeyboardEvents|I
  (params (Key :type Key%20Structure))
  (:Pressed
    (Utilities|IsValid (Variables|Default|GetElevatorWBP)
      (:Is%20Valid
        (CallFunction|RemoveWidget (Variables|Default|GetElevatorWBP)))
      (:Is%20Not%20Valid
        (bind _returnvalue (UserInterface|CreateWidget "/Game/CheekyFPS/Blueprints/UMG/WBP_ElevatorPanel.WBP_ElevatorPanel_C"))
        (bind _output_get (Variables|Default|SetElevatorWBP _returnvalue))
        (CallFunction|OnCreateNewWidget _output_get)))))

(event Input|KeyboardEvents|AnyKey
  (params (Key :type Key%20Structure))
  (:Pressed
    (Utilities|FlowControl|Sequence
      (:then_0
        (Class|ISSPlayerController|UpdateGamepadIconSet (Class|ApolloPlayerSettingsLibrary|GetPlayerGamepadType)))
      (:then_1
        (Variables|Default|SetIsUsingGamepad? (Class|KismetInputLibrary|KeyIsGamepadKey Key))))))

(fn ConstructionScript)

(fn OnCreateNewWidget
  (params (NewWidget :type User%20Widget%20Object%20Reference))
  (Input|SetInputModeGameandUI self 0 "DoNotLock" false)
  (Game|SetGamePaused true)
  (UserInterface|Viewport|AddtoViewport NewWidget 0))

(fn RemoveWidget
  (params (Widget :type Widget%20Object%20Reference))
  (Widget|RemovefromParent Widget)
  (Input|SetInputModeGameOnly self)
  (Class|Controller|ResetIgnoreInputFlags))

(fn GetJoystickDirection
  (params (Stick :type EJoystickTypes%20Enum :default "NewEnumerator0"))
  (switch Utilities|FlowControl|Switch|SwitchonEJoystickTypes Stick
    (:NewEnumerator0
      (return (Math|Vector2D|MakeVector2D (Class|Actor|GetInputAxisKeyValue) (* (Class|Actor|GetInputAxisKeyValue) -1.0))))
    (:NewEnumerator1
      (return (Math|Vector2D|MakeVector2D (Class|Actor|GetInputAxisKeyValue) (Class|Actor|GetInputAxisKeyValue))))))