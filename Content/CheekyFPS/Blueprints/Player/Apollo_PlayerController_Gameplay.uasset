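; Gameplay player controller that owns the HUD, pause menu, and weapon and item wheel widgets.
; BeginPlay creates the HUD; held wheel inputs pause the game and lock look until release plays a reverse animation and restores play.
; Hit and crit events drive timelines meant to tint the reticle red or gold, reversing after a retriggerable delay.
; Interact messages the item wheel to select, and the O key toggles a sonar effect through the game state.
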(event EventBeginPlay
  (bind _returnvalue (UserInterface|CreateWidget "/Game/CheekyFPS/Blueprints/UMG/WBP_GameplayHUD.WBP_GameplayHUD_C" 0 (.AsCheeky%20Character (Utilities|Casting|CastToCheekyCharacter (Game|GetPlayerCharacter 0)))))
  (bind _output_get (Variables|Default|SetGameplayHUD_WBP _returnvalue))
  (UserInterface|Viewport|AddtoViewport _returnvalue 0)
  (Variables|Default|SetMinimapWBP (Variables|/Game/CheekyFPS/Blueprints/UMG/WBP_GameplayHUD.WBP_GameplayHUD_C|GetWBP_Minimap _output_get)))

(event EventRegisterPlayerHit
  (bind _hittimeline (Variables|Default|GetHitTimeline))
  (Audio|Components|Audio|Play _hittimeline)
  (Utilities|FlowControl|RetriggerableDelay 0.6)
  (Utilities|String|Reverse _hittimeline))

(event EventUpdateWeaponHUD
  (Default|GetCurrentWeaponInfo (Variables|Default|GetGameplayHUD_WBP)))

(event EventRegisterPlayerCritHit
  (bind _crithittimeline (Variables|Default|GetCritHitTimeline))
  (Audio|Components|Audio|Play _crithittimeline)
  (Utilities|FlowControl|RetriggerableDelay 0.6)
  (Utilities|String|Reverse _crithittimeline))

(event EventOnRootWidgetRemoved
  (|CallParentFunction)
  (Utilities|IsValid (Variables|Default|GetPauseMenuWBP)
    (:Is%20Valid
      (CallFunction|RemoveWidget (Variables|Default|GetPauseMenuWBP))
      (Variables|Default|SetPauseMenuWBP 0))))

(event Input|ActionEvents|InputActionWeaponMenu
  (params (Key :type Key%20Structure :default "None"))
  (bind _self self)
  (:Pressed
    (Utilities|IsValid (Variables|Default|GetWeaponWheelWBP)
      (:Is%20Not%20Valid
        (if (not (Game|IsGamePaused))
          (bind _returnvalue (UserInterface|CreateWidget "/Game/CheekyFPS/Blueprints/UMG/WBP_WeaponWheel.WBP_WeaponWheel_C"))
          (Variables|Default|SetWeaponWheelWBP _returnvalue)
          (UserInterface|Viewport|AddtoViewport _returnvalue 0)
          (Game|SetGamePaused true)
          (Input|SetIgnoreLookInput true)
          (Input|SetInputModeGameandUI _self 0 "DoNotLock" true)))))
  (:Released
    (Class|UserWidget|PlayAnimationReverse (Variables|Default|GetWeaponWheelWBP) (Variables|/Game/CheekyFPS/Blueprints/UMG/WBP_WeaponWheel.WBP_WeaponWheel_C|GetStart (Variables|Default|GetWeaponWheelWBP)) 1.5 false)
    (Utilities|FlowControl|RetriggerableDelay 0.25)
    (Widget|RemovefromParent (Variables|Default|GetWeaponWheelWBP))
    (Game|SetGamePaused false)
    (Input|SetInputModeGameOnly _self)
    (Variables|Default|SetWeaponWheelWBP 0)
    (Input|ResetIgnoreLookInput)))

(event Input|ActionEvents|InputActionItemMenu
  (params (Key :type Key%20Structure :default "None"))
  (bind _self self)
  (:Pressed
    (Utilities|IsValid (Variables|Default|GetItemWheelWBP)
      (:Is%20Not%20Valid
        (if (not (Game|IsGamePaused))
          (bind _returnvalue (UserInterface|CreateWidget "/Game/CheekyFPS/Blueprints/UMG/WBP_ItemWheel.WBP_ItemWheel_C"))
          (Variables|Default|SetItemWheelWBP _returnvalue)
          (UserInterface|Viewport|AddtoViewport _returnvalue 0)
          (Input|SetIgnoreLookInput true)
          (Game|SetGamePaused true)
          (Input|SetInputModeGameandUI _self 0 "DoNotLock" true)))))
  (:Released
    (Class|UserWidget|PlayAnimationReverse (Variables|Default|GetItemWheelWBP) (Variables|/Game/CheekyFPS/Blueprints/UMG/WBP_ItemWheel.WBP_ItemWheel_C|GetStart (Variables|Default|GetItemWheelWBP)) 1.5 false)
    (Utilities|FlowControl|RetriggerableDelay 0.25)
    (Widget|RemovefromParent (Variables|Default|GetItemWheelWBP))
    (Game|SetGamePaused false)
    (Input|SetInputModeGameOnly _self)
    (Variables|Default|SetItemWheelWBP 0)
    (Input|ResetIgnoreLookInput)))

(event Input|ActionEvents|InputActionInteract
  (params (Key :type Key%20Structure :default "None"))
  (:Pressed
    (Class|BPIPlayer|PlayerSelect(Message) (Variables|Default|GetItemWheelWBP))))

(event Input|ActionEvents|InputActionPause
  (params (Key :type Key%20Structure :default "None"))
  (:Pressed
    (Utilities|IsValid (Variables|Default|GetPauseMenuWBP)
      (:Is%20Valid
        (CallFunction|RemoveWidget (Variables|Default|GetPauseMenuWBP))
        (Variables|Default|SetPauseMenuWBP 0))
      (:Is%20Not%20Valid
        (Variables|Default|SetbShowMouseCursor true)
        (Variables|Default|SetCurrentWBP (Variables|Default|GetPauseMenuWBP))
        (bind _returnvalue (UserInterface|CreateWidget "/Game/CheekyFPS/Blueprints/UMG/WBP_PauseMenu.WBP_PauseMenu_C"))
        (bind _output_get (Variables|Default|SetPauseMenuWBP _returnvalue))
        (UserInterface|Viewport|AddtoViewport _output_get 0)
        (Input|SetInputModeGameandUI self _output_get "DoNotLock" false)
        (Game|SetGamePaused true)))))

(event Input|KeyboardEvents|O
  (params (Key :type Key%20Structure :default "None"))
  (bind _returnvalue (Game|GetGameState))
  (:Pressed
    (Utilities|FlowControl|FlipFlop
      (:A
        (Class|BPIChameleon|ToggleSonarEffect?(Message) _returnvalue true))
      (:B
        (Class|BPIChameleon|ToggleSonarEffect?(Message) _returnvalue false)))))

(fn ConstructionScript
  (|CallParentFunction))