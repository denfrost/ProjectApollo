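; Base drone enemy that turns to face its blackboard CurrentEnemy and falls under physics on death, exploding when it hits something.
; Detection overlaps collect nearby friendly enemies, and SendMessage loops over them to store player or point-of-interest locations in PotentialPOILocation.
; A looping timer runs until death, while Tick calls RespondToPOIMessage.
; EMP damage enables mesh physics, and Stun zeroes AI sight range and starts a timer.
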(event OnThingDead(HealthComponent)
  (bind _bp_weaponcomponent (Variables|Default|GetBP_WeaponComponent))
  (bind _returnvalue (Default|GetCurrentWeapon _bp_weaponcomponent))
  (Utilities|Time|ClearandInvalidateTimerbyHandle (Variables|Default|GetMessageHandle))
  (Physics|SetSimulatePhysics (Variables|Default|GetDroneMesh) true)
  (Utilities|IsValid _returnvalue
    (:Is%20Valid
      (Physics|SetSimulatePhysics (Variables|/Game/CheekyFPS/Blueprints/Weapons/BP_BaseWeapon.BP_BaseWeapon_C|GetSkeletalMesh _returnvalue) true))))

(event OnComponentBeginOverlap(DetectionCollision)
  (params (OverlappedComponent :type Primitive%20Component%20Object%20Reference) (OtherActor :type Actor%20Object%20Reference) (OtherComp :type Primitive%20Component%20Object%20Reference) (OtherBodyIndex :type Integer) (bFromSweep :type Boolean) (SweepResult :type Hit%20Result%20Structure%20%28by%20ref%29))
  (bind _returnvalue (Actor|GetComponentbyClass OtherActor "/Game/CheekyFPS/Blueprints/Health/BP_CheekyHealthComponent.BP_CheekyHealthComponent_C"))
  (bind _asbp_base_enemy (Utilities|Casting|CastToBP_BaseEnemy OtherActor))
  (bind _charactertype (Variables|/Game/CheekyFPS/Blueprints/Health/BP_CheekyHealthComponent.BP_CheekyHealthComponent_C|GetCharacterType _returnvalue))
  (bind _returnvalue_2 (Utilities|Enum|Equal(Enum) _charactertype "NewEnumerator1"))
  (Utilities|IsValid _returnvalue
    (:Is%20Valid
      (if (and (!= OtherActor self) (not _returnvalue_2))
        (if (Utilities|IsValid _asbp_base_enemy)
          (Utilities|Array|AddUnique (Variables|Default|GetNearbyFriendlies) _asbp_base_enemy))
        (elif _returnvalue_2
          (if (== (AI|Components|Blackboard|GetValueasObject (CallFunction|GetAIBlackboard) (Utilities|Name|MakeLiteralName "CurrentEnemy")) 0)
            _))))))

(event OnComponentHit(DroneMesh)
  (params (HitComponent :type Primitive%20Component%20Object%20Reference) (OtherActor :type Actor%20Object%20Reference) (OtherComp :type Primitive%20Component%20Object%20Reference) (NormalImpulse :type Vector :default "0, 0, 0") (Hit :type Hit%20Result%20Structure%20%28by%20ref%29))
  (if (Default|IsDead? (Variables|Default|GetHealthComponent))
    (Effects|SpawnEmitteratLocation "/Game/CheekyFPS/External/VFX/FXVarietyPack/Particles/P_ky_explosion.P_ky_explosion" (Transformation|GetActorLocation))
    (Actor|SetLifeSpan 0.25)
    (Actor|Tick|SetActorTickEnabled false)))

(event EventBeginPlay
  (|CallParentFunction)
  (bind _returnvalue (Utilities|Time|SetTimerbyEvent (EventDispatchers|CreateEvent :!event SendMessage) 1.0 true))
  (Variables|Default|SetMessageHandle _returnvalue))

(event Collision|EventActorBeginOverlap
  (params (OtherActor :type Actor%20Object%20Reference)))

(event EventTick
  (params (DeltaSeconds :type Float%20%28single-precision%29))
  (bind (_outlocation _outrotation) (Actor|GetActorEyesViewPoint))
  (bind _returnvalue (Utilities|Name|MakeLiteralName "CurrentEnemy"))
  (bind _self self)
  (bind _returnvalue_2 (AI|GetAIController _self))
  (bind _returnvalue_3 (AI|GetBlackboard _returnvalue_2))
  (bind _returnvalue_4 (AI|Components|Blackboard|GetValueasObject _returnvalue_3 _returnvalue))
  (bind _asactor (Utilities|Casting|CastToActor _returnvalue_4))
  (CallFunction|HideWidgetwhenNotVisible (Variables|Default|GetDroneMesh))
  (CallFunction|RespondtoPOIMessage)
  (Utilities|FlowControl|Sequence
    (:then_0
      (if (Variables|Default|GetbEnableDebugMode?)
        (Collision|LineTraceByChannel _outlocation (+ _outlocation (* (Math|Vector|GetForwardVector _outrotation) 5e+03)) "TraceTypeQuery1" false 0 "ForOneFrame")))
    (:then_1
      (if (not (Default|IsDead? (Variables|Default|GetHealthComponent)))
        (Utilities|IsValid _asactor
          (:Is%20Valid
            (Transformation|SetActorRotation (Math|Rotator|FindLookatRotation (Transformation|GetActorLocation) (Transformation|GetActorLocation _asactor)))))))))

(event EventEndPlay
  (params (EndPlayReason :type EEndPlayReason%20Enum :default "Destroyed"))
  (Actor|Tick|SetActorTickEnabled false))

(fn ConstructionScript)

(fn ReportPlayerLocation
  (bind _returnvalue (Utilities|Name|MakeLiteralName "CurrentEnemy"))
  (bind _self self)
  (bind _returnvalue_2 (AI|GetAIController _self))
  (bind _returnvalue_3 (AI|GetBlackboard _returnvalue_2))
  (bind _returnvalue_4 (AI|Components|Blackboard|GetValueasObject _returnvalue_3 _returnvalue))
  (Utilities|IsValid _returnvalue_4
    (:Is%20Valid
      (if (== _returnvalue_4 (Game|GetPlayerCharacter 0))
        (return (AI|Components|Blackboard|GetValueasVector _returnvalue_3 (Utilities|Name|MakeLiteralName "PointOfInterest")))))))

(fn SendMessage
  (if (not (Default|IsDead? (Variables|Default|GetHealthComponent)))
    (Utilities|IsValid (AI|Components|Blackboard|GetValueasObject (CallFunction|GetAIBlackboard) (Utilities|Name|MakeLiteralName "CurrentEnemy"))
      (:Is%20Valid
        (for _array_element (Variables|Default|GetNearbyFriendlies)
          (bind _returnvalue (CallFunction|ReportPlayerLocation))
          (Utilities|IsValid (Default|GetAIBlackboard _array_element)
            (:Is%20Valid
              (Variables|Default|SetPotentialPOILocation _returnvalue)))))
      (:Is%20Not%20Valid
        (for _array_element_2 (Variables|Default|GetNearbyFriendlies)
          (bind _returnvalue_2 (CallFunction|ReportPOILocation))
          (Utilities|IsValid (Default|GetAIBlackboard _array_element_2)
            (:Is%20Valid
              (Variables|Default|SetPotentialPOILocation _returnvalue_2))))))
    (else
      (return))))

(fn ReportPOILocation
  (bind _returnvalue (CallFunction|GetAIBlackboard))
  (Utilities|IsValid _returnvalue
    (:Is%20Valid
      (if (Math|Vector|NotEqual(Vector) (AI|Components|Blackboard|GetValueasVector _returnvalue (Utilities|Name|MakeLiteralName "PointOfInterest")) "0, 0, 0" 0.0001)
        (return (AI|Components|Blackboard|GetValueasVector (AI|GetBlackboard (AI|GetAIController self)) (Utilities|Name|MakeLiteralName "PointOfInterest")))))))

(fn RespondtoDamage
  (params (DamageTypeRecieved :type BP%20Base%20Damage%20Type%20Object%20Reference))
  (|CallParentFunction DamageTypeRecieved)
  (switch Utilities|FlowControl|Switch|SwitchonE_DamageType (Variables|/Game/CheekyFPS/Blueprints/Weapons/DamageTypes/BP_BaseDamageType.BP_BaseDamageType_C|GetDamageType DamageTypeRecieved)
    (:NewEnumerator4
      (Physics|SetSimulatePhysics (Variables|Default|GetDroneMesh) true))
    (:NewEnumerator6
      (bind _returnvalue (Class|ApolloAIBlueprintLibrary|SetSightRange (AI|GetAIController self) 0.0))
      (if _returnvalue
        (Utilities|Time|SetTimerbyEvent (EventDispatchers|CreateEvent :!event ResetSightRange) 3e+01)))))