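; BP_AssaultDrone is an assault drone enemy in the Mechs set that carries a weapon.
; On BeginPlay it runs the parent logic, then snaps the current weapon from BPWeaponComponent onto its WeaponAttachPoint, if that weapon is valid.
; It adds no other active logic: the construction script only calls the parent, and the Tick and overlap events are disabled.
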(event EventBeginPlay
  (bind _bp_weaponcomponent (Variables|Default|GetBP_WeaponComponent))
  (bind _returnvalue (Default|GetCurrentWeapon _bp_weaponcomponent))
  (|CallParentFunction)
  (Utilities|IsValid _returnvalue
    (:Is%20Valid
      (Transformation|AttachComponentToComponent _returnvalue (Variables|Default|GetWeaponAttachPoint) "None" "SnapToTarget" "SnapToTarget" "SnapToTarget" true))))

(event Collision|EventActorBeginOverlap
  (params (OtherActor :type Actor%20Object%20Reference))
  (|CallParentFunction OtherActor) ; This node is disabled and will not be called.\nDrag off pins to build functionality.
)

(event EventTick
  (params (DeltaSeconds :type Float%20%28single-precision%29))
  (|CallParentFunction DeltaSeconds) ; This node is disabled and will not be called.\nDrag off pins to build functionality.
)

(fn ConstructionScript
  (|CallParentFunction))