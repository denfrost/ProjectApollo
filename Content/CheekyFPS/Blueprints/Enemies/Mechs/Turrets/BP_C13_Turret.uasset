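; Enemy mech turret that sweeps for targets and shoots them from twin guns.
; A rotation timeline drives sphere traces, briefly pausing on actors with health or destructible components and starting a looping fire timer.
; Firing applies point damage, turns toward the player and plays muzzle effects.
; Interaction or death disables it with sparks and sets a timer, with a reset event restoring scanning and, if dead, health.
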(event OnEndInteraction(CheekyInteractComponent)
  (params (Type :type EInteractionTypes%20Enum :default "NewEnumerator0"))
  (CallFunction|OnTurretDisabled)
  (Utilities|Time|SetTimerbyEvent (EventDispatchers|CreateEvent :!event Custom|ResetBehavior) 1e+01))

(event OnBeginInteraction(CheekyInteractComponent)
  (params (Type :type EInteractionTypes%20Enum :default "NewEnumerator0"))
  (Default|UpdateMessage (Variables|Default|GetCheekyInteractComponent) "Deactivate Turret"))

(event OnThingDead(CheekyHealthComponent)
  (CallFunction|OnTurretDisabled)
  (Utilities|Time|SetTimerbyEvent (EventDispatchers|CreateEvent :!event Custom|ResetBehavior) 3e+01))

(event Custom|DamagePlayer
  (bind _lgunvfxspawnpoint (Variables|Default|GetLGunVFXSpawnPoint))
  (bind _rgunvfxspawnpoint (Variables|Default|GetRGunVFXSpawnPoint))
  (bind _out_hit (Variables|Default|GetOut%20Hit))
  (bind (_bblockinghit _binitialoverlap _time _distance _location _impactpoint _normal _impactnormal _physmat _hitactor) (Collision|BreakHitResult _out_hit))
  (bind _returnvalue (Transformation|GetWorldTransform _rgunvfxspawnpoint))
  (bind _returnvalue_2 (Transformation|GetWorldTransform _lgunvfxspawnpoint))
  (bind _returnvalue_3 (Transformation|GetActorLocation _hitactor))
  (if (Variables|Status|GetbIsTurretActive?)
    (Game|Damage|ApplyPointDamage _hitactor 5.0 _impactpoint _out_hit 0 0 "/Game/CheekyFPS/Blueprints/Weapons/DamageTypes/BP_StandardDamageType.BP_StandardDamageType_C")
    (CallFunction|FacePlayer)
    (Effects|SpawnEmitteratLocation "/Game/CheekyFPS/External/Weapons/SciFiWeapDark/FX/Particles/P_AssaultRifle_MuzzleFlash_Dark.P_AssaultRifle_MuzzleFlash_Dark" (.location _returnvalue_2) (Math|Rotator|FindLookatRotation (.location _returnvalue_2) _returnvalue_3) "1.000000,1.000000,1.000000" true "AutoRelease")
    (Audio|PlaySoundatLocation "/Game/CheekyFPS/External/Audio/Ultimate_Sci_Fi_SFX/Sci_Fi_Weapon_Sounds/Cues/Sci_Fi_Blaster/Sci_Fi_Blaster_9_Cue.Sci_Fi_Blaster_9_Cue" (Transformation|GetActorLocation) "0, 0, 0" 1.0 1.0 0.0 0 0 0)
    (Utilities|FlowControl|RetriggerableDelay 0.2)
    (Effects|SpawnEmitteratLocation "/Game/CheekyFPS/External/Weapons/SciFiWeapDark/FX/Particles/P_AssaultRifle_MuzzleFlash_Dark.P_AssaultRifle_MuzzleFlash_Dark" (.location _returnvalue) (Math|Rotator|FindLookatRotation (.location _returnvalue) _returnvalue_3) "1.000000,1.000000,1.000000" true "AutoRelease")
    (Audio|PlaySoundatLocation "/Game/CheekyFPS/External/Audio/Ultimate_Sci_Fi_SFX/Sci_Fi_Weapon_Sounds/Cues/Sci_Fi_Blaster/Sci_Fi_Blaster_6_Cue.Sci_Fi_Blaster_6_Cue" (Transformation|GetActorLocation) "0, 0, 0" 1.0 1.0 0.0 0 0 0)))

(event Custom|FacePlayer
  (bind _returnvalue (Transformation|GetActorRotation))
  (Transformation|SetActorRotation (Math|Rotator|MakeRotator (.roll _returnvalue) (.pitch _returnvalue) (.yaw (Math|Rotator|FindLookatRotation (Transformation|GetActorLocation) (Transformation|GetActorLocation (Game|GetPlayerCharacter 0)))))))

(event Custom|ResetBehavior
  (bind _cheekyhealthcomponent (Variables|Default|GetCheekyHealthComponent))
  (Audio|Components|Audio|Play (Variables|Default|GetRotateTimeline))
  (Variables|Status|SetbIsTurretActive? true)
  (CallFunction|UpdateMessage)
  (if (Default|IsDead? _cheekyhealthcomponent)
    (Default|ResetHealth _cheekyhealthcomponent)))

(event EventBeginPlay
  (EventDispatchers|BindEventtoOnDamageRecieved (Variables|Default|GetCheekyHealthComponent) (EventDispatchers|CreateEvent :!event Custom|FacePlayer)))

(fn ConstructionScript
  (CallFunction|UpdateMessage))

(fn UpdateMessage
  (Default|UpdateMessage (Variables|Default|GetCheekyInteractComponent) (select (Variables|Status|GetbIsTurretActive?) "Deactivate Turret" "Activate Turret")))

(fn OnTurretDisabled
  (bind _scene (Variables|Default|GetScene))
  (bind _returnvalue (Transformation|GetWorldTransform _scene))
  (Variables|Status|SetbIsTurretActive? false)
  (Audio|Components|Audio|Stop (Variables|Default|GetRotateTimeline))
  (Utilities|Time|ClearandInvalidateTimerbyHandle (Variables|Default|GetFireTimer))
  (CallFunction|UpdateMessage)
  (Effects|SpawnEmitteratLocation "/Game/VFX_Toolkit_V1/ParticleSystems/356Days/Par_Voya_Sparks_01.Par_Voya_Sparks_01" (.location _returnvalue) (.rotation _returnvalue)))