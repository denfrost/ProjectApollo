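; Base enemy soldier for CheekyFPS, whose SoldierType selects its AI controller and, except for Boss, its default weapon.
; InitalizeAI caches controller and AnimBP, then binds health and alarm events, feeding health, ammo and player location into the Blackboard.
; A dynamic material color shows AI state; stun stops AI logic, and death or stun can drop an item.
; It also requests backup, opens doors by trace, and restores dead or stunned state through RamaSave.
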(event OnThingDead(HealthComponent)
  (bind _droppeditem (Variables|Default|GetDroppedItem))
  (CallFunction|PlayDeathAnimation)
  (if (Variables|Death|GetbShouldDropItem?)
    (Utilities|IsValid _droppeditem
      (:Is%20Valid
        (CallFunction|MoveDroppedItem _droppeditem (Transformation|GetActorTransform))))))

(event RamaSaveEventActorFullyLoaded(RamaSave)
  (params (RamaSaveComponent :type Rama%20Save%20Component%20Object%20Reference) (LevelPackageName :type String))
  (bind _healthcomponent (Variables|Default|GetHealthComponent))
  (Utilities|FlowControl|Sequence
    (:then_0
      (if (Variables|/Game/CheekyFPS/Blueprints/Health/CheekyHealthComponent.CheekyHealthComponent_C|GetbIsDead _healthcomponent)
        (CallFunction|PlayDeathAnimation)))
    (:then_1
      (if (Variables|/Game/CheekyFPS/Blueprints/Health/CheekyHealthComponent.CheekyHealthComponent_C|GetbIsStunned _healthcomponent)
        (Default|CallOnThingStunned _healthcomponent)))))

(event Custom|OnStunned
  (bind _droppeditem (Variables|Default|GetDroppedItem))
  (Utilities|FlowControl|Sequence
    (:then_0
      (Utilities|IsValid _droppeditem
        (:Is%20Valid
          (CallFunction|MoveDroppedItem _droppeditem (Transformation|GetActorTransform)))))
    (:then_1
      (Default|ClearPerception (Variables|Default|GetMyAICON) true)
      (CallFunction|UpdateStatusColor "(R=0.598958,G=0.598958,B=0.598958,A=1.000000)")
      (AI|Logic|StopLogic (Variables|/Script/AIModule.AIController|GetBrainComponent (Variables|Default|GetMyAICON)) "Stunned"))))

(event Custom|OnDeath
  (bind _returnvalue (Game|GetGameState))
  (bind _returnvalue_2 (Class|BPIGameEvents|GetReflexStatus(Message) _returnvalue))
  (if _returnvalue_2
    (Class|BPIGameEvents|StopReflexFX(Message) _returnvalue false))
  (Actor|SetLifeSpan 0.2)
  (Default|CallOnCharDeath self))

(event Custom|OnDamage
  (params (NewHealth :type Float%20%28single-precision%29))
  (bind _myaicon (Variables|Default|GetMyAICON))
  (bind _blackboard (Variables|/Script/AIModule.AIController|GetBlackboard _myaicon))
  (if (not (Variables|/Game/CheekyFPS/Blueprints/Health/CheekyHealthComponent.CheekyHealthComponent_C|GetbIsDead (Variables|Default|GetHealthComponent)))
    (AI|Components|Blackboard|SetValueasFloat _blackboard (Utilities|Name|MakeLiteralName "CurrentHealth") NewHealth)
    (AI|Components|Blackboard|SetValueasFloat _blackboard (Utilities|Name|MakeLiteralName "CurrentHealthPercent") (Default|GetHealthPercentage (Variables|Default|GetHealthComponent)))))

(event EventBeginPlay
  (CallFunction|AssignAIController)
  (CallFunction|AssignWeapon)
  (Utilities|FlowControl|Delay 0.2)
  (CallFunction|InitalizeAI))

(event EventOnWeaponFire
  (bind _bp_weaponcomponent (Variables|Default|GetBP_WeaponComponent))
  (bind _currentweapon (Variables|/Game/CheekyFPS/Blueprints/Components/BP_WeaponComponent.BP_WeaponComponent_C|GetCurrentWeapon _bp_weaponcomponent))
  (if (CallFunction|CheckStunStatus)
    (Utilities|IsValid _currentweapon
      (:Is%20Valid
        (CallFunction|UpdateAmmoCount)
        (Default|Fire _currentweapon)
        (Class|BPIAnimation|OnCharacterAttack(Message) (Variables|Default|GetMyABP) (Default|GetWeaponType _currentweapon))))))

(event EventHasDetectedEnemy?
  (params (bCanSeeEnemy? :type Boolean))
  (bind _myaicon (Variables|Default|GetMyAICON))
  (bind _returnvalue (AI|GetBlackboard _myaicon))
  (bind _poikey (Variables|/Game/CheekyFPS/Blueprints/AI/AIControllers/BP_AIController_Base.BP_AIController_Base_C|GetPOIKey _myaicon))
  (Utilities|IsValid _myaicon
    (:Is%20Valid
      (if bCanSeeEnemy?
        (AI|Components|Blackboard|SetValueasVector _returnvalue _poikey (Transformation|GetActorLocation (Game|Player|GetPlayerPawn 0)))
        (CallFunction|UpdateStatusColor "(R=1.000000,G=0.774480,B=0.000000,A=1.000000)")
        (else
          (AI|Components|Blackboard|ClearValue _returnvalue _poikey)
          (CallFunction|UpdateStatusColor "(R=0.000000,G=0.890520,B=1.000000,A=1.000000)"))))))

(event EventEndPlay
  (params (EndPlayReason :type EEndPlayReason%20Enum :default "Destroyed"))
  (Effects|SpawnEmitteratLocation "/Game/CheekyFPS/External/Weapons/SciFiWeapLight/FX/Particles/P_Grenade_Explosion_Dark.P_Grenade_Explosion_Dark" (Transformation|GetActorLocation)))

(event EventOnWeaponReload
  (bind _bp_weaponcomponent (Variables|Default|GetBP_WeaponComponent))
  (bind _currentweapon (Variables|/Game/CheekyFPS/Blueprints/Components/BP_WeaponComponent.BP_WeaponComponent_C|GetCurrentWeapon _bp_weaponcomponent))
  (if (CallFunction|CheckStunStatus)
    (Utilities|IsValid _currentweapon
      (:Is%20Valid
        (Default|Reload _currentweapon)
        (CallFunction|UpdateAmmoCount)))))

(event EventRequestBackup
  (bind _returnvalue (Class|BPISaveLoad|GetCurrentGameDifficulty(Message) (Game|GetGameInstance)))
  (Class|BPIGameEvents|ShouldSpawnBackup?(Message) (Game|GetGameState) (Math|Random|RandomBoolwithWeight (* (Default|GetHealthPercentage (Variables|Default|GetHealthComponent)) (Math|Conversions|ToFloat(Byte) _returnvalue))))
  (Development|PrintString (Utilities|String|ToString(Boolean) (Math|Random|RandomBoolwithWeight (* (Default|GetHealthPercentage (Variables|Default|GetHealthComponent)) (Math|Conversions|ToFloat(Byte) _returnvalue))))))

(fn ConstructionScript
  (bind _ramasave (Variables|Default|GetRamaSave))
  (CallFunction|AssignAIController)
  (CallFunction|AssignWeapon)
  (Variables|/Script/ApolloGame.PatrolRouteComponent|SetPatrolPoints (Variables|Default|GetPatrolRoute) (Variables|Nav|GetMyPatrolPoints))
  (if (not (Guid|IsValidGuid (Variables|/Script/RamaSaveSystem.RamaSaveComponent|GetRamaSave_PersistentActorUniqueID _ramasave)))
    (Variables|/Script/RamaSaveSystem.RamaSaveComponent|SetRamaSave_PersistentActorUniqueID _ramasave (Guid|NewGuid))
    (Development|PrintString (Utilities|String|Append (Utilities|GetDisplayName self) " " "Generated new GUID"))))

(fn FindInteractableObject
  (bind (_outlocation _outrotation) (Actor|GetActorEyesViewPoint))
  (bind _cheekytracecomponent (Variables|Default|GetCheekyTraceComponent))
  (bind _currentinteractioncomponent (Variables|/Game/CheekyFPS/Blueprints/Interaction/CheekyTraceComponent.CheekyTraceComponent_C|GetCurrentInteractionComponent _cheekytracecomponent))
  (bind _outhit (Collision|SphereTraceForObjects _outlocation (+ _outlocation (* (Math|Vector|GetForwardVector _outrotation) 5e+01)) 3.6e+02 (Utilities|Array|MakeArray "ObjectTypeQuery2") true 0 "ForDuration"))
  (if (.bBlockingHit (Collision|BreakHitResult _outhit))
    (Utilities|FlowControl|Sequence
      (:then_0
        (Utilities|IsValid (Actor|GetComponentbyClass (.HitActor (Collision|BreakHitResult _outhit)) "/Game/CheekyFPS/Blueprints/Interaction/CheekyInteractComponent.CheekyInteractComponent_C")
          (:Is%20Valid
            (Default|InteractInput _cheekytracecomponent true "NewEnumerator0")
            (Utilities|IsValid _currentinteractioncomponent
              (:Is%20Valid
                (Class|BPIDoors|AttemptDoorOpen(Message) _currentinteractioncomponent)
                (Development|PrintString "I opened a door!")))))))
    (else
      (Default|InteractInput _cheekytracecomponent false "NewEnumerator0"))))

(fn UpdateStatusColor
  (params (NewColor :type Linear%20Color%20Structure))
  (Rendering|Material|SetVectorParameterValue (Variables|Default|GetStatusDynMat) "Color" NewColor :!class /Script/Engine.MaterialInstanceDynamic))

(fn UpdateStatusColortoAlert
  (CallFunction|UpdateStatusColor "(R=1.000000,G=0.000000,B=0.000000,A=1.000000)"))

(fn CheckStunStatus
  (bind _myaicon (Variables|Default|GetMyAICON))
  (bind _returnvalue (AI|GetBlackboard _myaicon))
  (if (Utilities|IsValid _returnvalue)
    (return (not (ScalableFloat|GetValueasBool _returnvalue (Utilities|Name|MakeLiteralName "IsStunned"))))))

(fn UpdateAmmoCount
  (bind _myaicon (Variables|Default|GetMyAICON))
  (bind _returnvalue (AI|GetBlackboard _myaicon))
  (Utilities|IsValid _returnvalue
    (:Is%20Valid
      (Class|BlackboardComponent|SetValueasInt _returnvalue (Utilities|Name|MakeLiteralName "CurrentAmmo") (Default|GetCurrentAmmo (Variables|/Game/CheekyFPS/Blueprints/Components/BP_WeaponComponent.BP_WeaponComponent_C|GetCurrentWeapon (Variables|Default|GetBP_WeaponComponent)))))))

(fn AssignWeapon
  (bind _bp_weaponcomponent (Variables|Default|GetBP_WeaponComponent))
  (switch Utilities|FlowControl|Switch|SwitchonESoldierType (Variables|Default|GetSoldierType)
    (:NewEnumerator0
      (Default|UpdateDefaultWeapon _bp_weaponcomponent "/Game/CheekyFPS/Blueprints/Weapons/BP_Rifle.BP_Rifle_C"))
    (:NewEnumerator1
      (Default|UpdateDefaultWeapon _bp_weaponcomponent "/Game/CheekyFPS/Blueprints/Weapons/BP_Shotgun.BP_Shotgun_C"))
    (:NewEnumerator2
      (Default|UpdateDefaultWeapon _bp_weaponcomponent "/Game/CheekyFPS/Blueprints/Weapons/BP_SniperRifle.BP_SniperRifle_C"))))

(fn AssignAIController
  (switch Utilities|FlowControl|Switch|SwitchonESoldierType (Variables|Default|GetSoldierType)
    (:NewEnumerator0
      (Variables|Default|SetAIControllerClass "/Game/CheekyFPS/Blueprints/AI/AIControllers/BP_AIController_Grunt.BP_AIController_Grunt_C"))
    (:NewEnumerator1
      (Variables|Default|SetAIControllerClass "/Game/CheekyFPS/Blueprints/AI/AIControllers/BP_AIController_Enforcer.BP_AIController_Enforcer_C"))
    (:NewEnumerator2
      (Variables|Default|SetAIControllerClass "/Game/CheekyFPS/Blueprints/AI/AIControllers/BP_AIController_Sniper.BP_AIController_Sniper_C"))
    (:NewEnumerator5
      (Variables|Default|SetAIControllerClass "/Game/CheekyFPS/Blueprints/AI/AIControllers/BP_AIController_Sniper_Boss.BP_AIController_Sniper_Boss_C"))))

(fn InitalizeAI
  (bind _self self)
  (bind _bp_weaponcomponent (Variables|Default|GetBP_WeaponComponent))
  (bind _healthcomponent (Variables|Default|GetHealthComponent))
  (bind _healthcomponent_2 (Variables|Default|GetHealthComponent))
  (bind _returnvalue (AI|GetAIController _self))
  (bind _currentweapon (Variables|/Game/CheekyFPS/Blueprints/Components/BP_WeaponComponent.BP_WeaponComponent_C|GetCurrentWeapon _bp_weaponcomponent))
  (Utilities|FlowControl|Sequence
    (:then_0
      (Utilities|IsValid _returnvalue
        (:Is%20Valid
          (bind _output_get (Variables|Default|SetMyAICON (.AsBP%20AIController%20Base (Utilities|Casting|CastToBP_AIController_Base _returnvalue))))
          (Default|SetStartingStats _output_get (Variables|/Game/CheekyFPS/Blueprints/Health/CheekyHealthComponent.CheekyHealthComponent_C|GetCurrentHP (Variables|Default|GetHealthComponent)))
          (Variables|/Game/CheekyFPS/Blueprints/UMG/WBP_EnemyWidget.WBP_EnemyWidget_C|SetAIControllerRef (.AsWBP%20Enemy%20Widget (Utilities|Casting|CastToWBP_EnemyWidget (UserInterface|GetUserWidgetObject (Variables|Default|GetWidget)))) (Variables|Default|GetMyAICON)))))
    (:then_1
      (Variables|Default|SetMyABP (Components|SkeletalMesh|GetAnimInstance (Variables|Character|GetMesh)))
      (bind _returnvalue_2 (Rendering|Material|CreateDynamicMaterialInstance (Variables|Default|GetStaticMesh) 0 (Rendering|Material|GetMaterial (Variables|Default|GetStaticMesh) 0) "None" :!class /Script/Engine.PrimitiveComponent))
      (Variables|Default|SetStatusDynMat _returnvalue_2)
      (CallFunction|UpdateStatusColor "(R=0.000000,G=0.890520,B=1.000000,A=1.000000)")
      (EventDispatchers|BindEventtoOnAlarmActivate (.AsISSGame%20State%20Base (Utilities|Casting|CastToISSGameStateBase (Game|GetGameState))) (EventDispatchers|CreateEvent :!event UpdateStatusColortoAlert))
      (EventDispatchers|BindEventtoOnUpdateHealth _healthcomponent (EventDispatchers|CreateEvent :!event Custom|OnDamage))
      (EventDispatchers|BindEventtoOnThingDead _healthcomponent (EventDispatchers|CreateEvent :!event Custom|OnDeath))
      (Utilities|FlowControl|Sequence
        (:then_0
          (AI|Components|Blackboard|SetValueasFloat (Variables|/Script/AIModule.AIController|GetBlackboard (Variables|Default|GetMyAICON)) (Utilities|Name|MakeLiteralName "CurrentHealth") (Variables|/Game/CheekyFPS/Blueprints/Health/CheekyHealthComponent.CheekyHealthComponent_C|GetCurrentHP _healthcomponent_2))
          (AI|Components|Blackboard|SetValueasFloat (Variables|/Script/AIModule.AIController|GetBlackboard (Variables|Default|GetMyAICON)) (Utilities|Name|MakeLiteralName "CurrentHealthPercent") (Default|GetHealthPercentage _healthcomponent_2)))
        (:then_1
          (if (Utilities|IsValid _currentweapon)
            (CallFunction|EquipWeapon(byReference) _currentweapon)
            (Class|BPIAnimation|OnCharacterEquipWeapon(Message) (Variables|Default|GetMyABP) (Variables|/Game/CheekyFPS/Blueprints/Weapons/BP_BaseWeapon.BP_BaseWeapon_C|GetWeaponType _currentweapon))
            (CallFunction|UpdateAmmoCount)))
        (:then_2
          (CallFunction|ToggleCollisionStatus true)
          (EventDispatchers|BindEventtoOnThingStunned (Variables|Default|GetHealthComponent) (EventDispatchers|CreateEvent :!event Custom|OnStunned)))))))

(fn GetGenericTeamID
  (return 0))