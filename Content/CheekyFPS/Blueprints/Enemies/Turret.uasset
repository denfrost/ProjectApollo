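; Turret enemy Blueprint meant to sweep, spot the player and deal repeated damage, though its scan logic is never triggered.
; BeginPlay only binds to the health component's damage event.
; The unconnected timeline rotates yaw and line-traces, pausing on a player hit to start a looping timer.
; DamagePlayer applies damage to the traced actor, then calls FacePlayer, which copies the player's yaw rather than aiming at them.
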(event Custom|DamagePlayer
  (Game|Damage|ApplyDamage (.HitActor (Collision|BreakHitResult (Variables|Default|GetOut%20Hit))) 5.0 0 0 "/Game/CheekyFPS/Blueprints/Weapons/DamageTypes/BP_StandardDamageType.BP_StandardDamageType_C")
  (CallFunction|FacePlayer))

(event Custom|FacePlayer
  (bind _returnvalue (Transformation|GetActorRotation))
  (Transformation|SetActorRotation (Math|Rotator|MakeRotator (.roll _returnvalue) (.pitch _returnvalue) (.yaw (Transformation|GetActorRotation (Game|GetPlayerCharacter 0))))))

(event EventBeginPlay
  (EventDispatchers|BindEventtoOnDamageRecieved (Variables|Default|GetCheekyHealthComponent) (EventDispatchers|CreateEvent :!event Custom|FacePlayer)))

(event Collision|EventActorBeginOverlap
  (params (OtherActor :type Actor%20Object%20Reference)))

(event EventTick
  (params (DeltaSeconds :type Float%20%28single-precision%29)))

(fn ConstructionScript)