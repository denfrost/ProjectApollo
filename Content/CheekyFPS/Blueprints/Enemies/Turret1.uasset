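; Enemy turret Blueprint built to sweep for the player and fire on them, with its scanning logic currently disconnected.
; The unwired rotation timeline sphere-traces ahead, pauses on spotting the player and starts a looping timer.
; DamagePlayer damages the traced actor, turns to face the player and staggers left and right muzzle flashes.
; BeginPlay only binds a handler to the health component's damage event.
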(event Custom|DamagePlayer
  (bind _lgunvfxspawnpoint (Variables|Default|GetLGunVFXSpawnPoint))
  (bind _rgunvfxspawnpoint (Variables|Default|GetRGunVFXSpawnPoint))
  (bind _out_hit (Variables|Default|GetOut%20Hit))
  (bind _hitactor (Collision|BreakHitResult _out_hit))
  (bind _returnvalue (Transformation|GetWorldTransform _rgunvfxspawnpoint))
  (bind _returnvalue_2 (Transformation|GetWorldTransform _lgunvfxspawnpoint))
  (bind _returnvalue_3 (Transformation|GetActorLocation _hitactor))
  (Game|Damage|ApplyDamage _hitactor 5.0 0 0 "/Game/CheekyFPS/Blueprints/Weapons/DamageTypes/BP_StandardDamageType.BP_StandardDamageType_C")
  (CallFunction|FacePlayer)
  (Effects|SpawnEmitteratLocation "/Game/CheekyFPS/External/Weapons/SciFiWeapDark/FX/Particles/P_AssaultRifle_MuzzleFlash_Dark.P_AssaultRifle_MuzzleFlash_Dark" (.location _returnvalue_2) (Math|Rotator|FindLookatRotation (.location _returnvalue_2) _returnvalue_3) "1.000000,1.000000,1.000000" true "AutoRelease")
  (Utilities|FlowControl|RetriggerableDelay 0.2)
  (Effects|SpawnEmitteratLocation "/Game/CheekyFPS/External/Weapons/SciFiWeapDark/FX/Particles/P_AssaultRifle_MuzzleFlash_Dark.P_AssaultRifle_MuzzleFlash_Dark" (.location _returnvalue) (Math|Rotator|FindLookatRotation (.location _returnvalue) _returnvalue_3) "1.000000,1.000000,1.000000" true "AutoRelease"))

(event Custom|FacePlayer
  (Transformation|SetActorRotation (Math|Rotator|FindLookatRotation (Transformation|GetActorLocation) (Transformation|GetActorLocation (Game|GetPlayerCharacter 0)))))

(event EventBeginPlay
  (EventDispatchers|BindEventtoOnDamageRecieved (Variables|Default|GetCheekyHealthComponent) (EventDispatchers|CreateEvent :!event Custom|FacePlayer)))

(fn ConstructionScript)