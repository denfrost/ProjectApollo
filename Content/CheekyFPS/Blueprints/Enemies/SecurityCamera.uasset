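; Security camera enemy that sweeps its yaw and can be killed through its health component.
; Its AI controller receives starting HP and is linked to the enemy widget.
; StartMovement plays the rotation timeline and turns the widget toward the player; StopMovement halts the timeline and snaps the camera's yaw to the player.
; On death it detaches the controller and spawns an explosion.
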(event OnThingDead(CheekyHealthComponent)
  (Class|Pawn|DetachfromControllerPendingDestroy)
  (Effects|SpawnEmitteratLocation "/Game/StarterContent/Particles/P_Explosion.P_Explosion" (Transformation|GetActorLocation)))

(event EventBeginPlay
  (bind _output_get (Variables|Default|SetMyAICON (.AsBP%20Base%20AIController (Utilities|Casting|CastToBP_BaseAIController (AI|GetAIController self)))))
  (Default|SetStartingStats _output_get (Variables|/Game/CheekyFPS/Blueprints/Health/CheekyHealthComponent.CheekyHealthComponent_C|GetCurrentHP (Variables|Default|GetCheekyHealthComponent)))
  (Utilities|FlowControl|Sequence
    (:then_0
      (Variables|/Game/CheekyFPS/Blueprints/UI/WBP_EnemyWidget.WBP_EnemyWidget_C|SetAIControllerRef (.AsWBP%20Enemy%20Widget (Utilities|Casting|CastToWBP_EnemyWidget (UserInterface|GetUserWidgetObject (Variables|Default|GetWidget)))) (Variables|Default|GetMyAICON)))))

(event EventStartMovement
  (bind _rotatetimeline (Variables|Default|GetRotateTimeline))
  (if (Audio|Components|Audio|IsPlaying _rotatetimeline)
    _
    (else
      (Components|Timeline|PlayfromStart _rotatetimeline)))
  (Transformation|SetRelativeRotation (Variables|Default|GetWidget) (Math|Rotator|FindLookatRotation (Transformation|GetActorLocation) (Transformation|GetActorLocation (Game|GetPlayerCharacter 0))) false false))

(event EventStopMovement
  (bind _returnvalue (Transformation|GetActorRotation))
  (Audio|Components|Audio|Stop (Variables|Default|GetRotateTimeline))
  (Transformation|SetActorRotation (Math|Rotator|MakeRotator (.roll _returnvalue) (.pitch _returnvalue) (.yaw (Math|Rotator|FindLookatRotation (Transformation|GetActorLocation) (Transformation|GetActorLocation (Game|GetPlayerCharacter 0)))))))

(fn ConstructionScript)