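; Enemy alert component meant to track an AI's alert state, mirror it to the Blackboard and set character walk speed per state.
; The state write, Blackboard update and DoOnce entry are disconnected from the empty UpdateAlertState event, so none run, including the speed change behind the DoOnce.
; ResetAlertState only resets that DoOnce gate.
; GetGenericTeamID always returns team 0.
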(event EventBeginPlay)

(event EventTick
  (params (DeltaSeconds :type Float%20%28single-precision%29)))

(event EventUpdateAlertState
  (params (NewState :type E_EnemyAlertStatus%20Enum :default "NewEnumerator1")))

(event EventResetAlertState
  (Utilities|FlowControl|DoOnce false) ; enters at Reset
)

(fn GetGenericTeamID
  (return 0))