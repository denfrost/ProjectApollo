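; Debug actor for viewing a decal material and testing two scalar parameters on it.
; On BeginPlay it assigns the input material to the Decal, creates a dynamic instance from that material, sets both named parameters and prints their values.
; Tick reapplies both values to the instance every frame.
; The dynamic instance is never assigned to the Decal, which keeps the input material.
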(event EventBeginPlay
  (bind _indecalmaterial (Variables|Default|GetInDecalMaterial))
  (Rendering|Components|Decal|SetDecalMaterial (Variables|Decal|GetDecal) _indecalmaterial)
  (bind _returnvalue (Rendering|Material|CreateDynamicMaterialInstance _indecalmaterial "None" "None" :!class /Script/Engine.KismetMaterialLibrary))
  (bind _output_get (Variables|Default|SetNewDynamicMaterial _returnvalue))
  (Rendering|Material|SetScalarParameterValue _output_get (Variables|Default|GetNewScalarParamName1) (Variables|Default|GetNewScalarParam1_Value) :!class /Script/Engine.MaterialInstanceDynamic)
  (Rendering|Material|SetScalarParameterValue _output_get (Variables|Default|GetNewScalarParamName2) (Variables|Default|GetNewScalarParam2_Value) :!class /Script/Engine.MaterialInstanceDynamic)
  (bind _returnvalue_2 (Rendering|Material|GetScalarParameterValue _output_get (Variables|Default|GetNewScalarParamName1) :!class /Script/Engine.MaterialInstanceDynamic))
  (Development|PrintString (Utilities|String|ToString(Float) _returnvalue_2))
  (bind _returnvalue_3 (Rendering|Material|GetScalarParameterValue _output_get (Variables|Default|GetNewScalarParamName2) :!class /Script/Engine.MaterialInstanceDynamic))
  (Development|PrintString (Utilities|String|ToString(Float) _returnvalue_3)))

(event EventTick
  (params (DeltaSeconds :type Float%20%28single-precision%29))
  (bind _newdynamicmaterial (Variables|Default|GetNewDynamicMaterial))
  (Rendering|Material|SetScalarParameterValue _newdynamicmaterial (Variables|Default|GetNewScalarParamName1) (Variables|Default|GetNewScalarParam1_Value) :!class /Script/Engine.MaterialInstanceDynamic)
  (Rendering|Material|SetScalarParameterValue _newdynamicmaterial (Variables|Default|GetNewScalarParamName2) (Variables|Default|GetNewScalarParam2_Value) :!class /Script/Engine.MaterialInstanceDynamic))

(fn ConstructionScript)