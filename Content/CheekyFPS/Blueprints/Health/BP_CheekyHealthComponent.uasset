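; Actor component that manages health, stamina, dead/stunned states and optional curve-based character fall damage for CheekyFPS.
; It binds to owner damage and routes it by damage type: fire adds capped timer ticks, ice may freeze, tranq drains stamina, EMP varies by character type.
; Changes fire update events, and player hits trigger a camera pain modifier timed by severity.
; Optional health regeneration uses a retriggerable delay and looping timer.
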(event Custom|RegenHealth
  ;[1 0.7974 0] Health Regeneration
  (Utilities|Time|ClearTimerbyFunctionName 0 "RegenerateHealth") ; Make sure timer isn't running\nE.g. if the timer was running, and player\ntakes damage and triggers this event again\nthen stop regenerating
  (Utilities|FlowControl|RetriggerableDelay (Variables|Configuration|GetRegenerateDelay))
  (Utilities|Time|SetTimerbyFunctionName 0 "RegenerateHealth" 0.1 true))

(event Custom|EndPain
  (params (Delay :type Float%20%28single-precision%29))
  (bind _returnvalue (Game|Player|FindCameraModifierbyClass (Game|GetPlayerCameraManager 0) "/Game/CheekyFPS/Blueprints/CameraManager/CamModifiers/BP_CamModifier_Pain.BP_CamModifier_Pain_C"))
  (CameraModifier|DisableModifier _returnvalue false)
  (Utilities|FlowControl|Delay (Variables|/Script/Engine.CameraModifier|GetAlphaOutTime _returnvalue)))

(event Custom|RegenStamina
  (Utilities|Time|ClearTimerbyFunctionName 0 "RegenerateStamina") ; Make sure timer isn't running\nE.g. if the timer was running, and player\ntakes damage and triggers this event again\nthen stop regenerating
  (Utilities|FlowControl|RetriggerableDelay (Variables|Configuration|GetRegenerateDelay))
  (Utilities|Time|SetTimerbyFunctionName 0 "RegenerateStamina" 0.1 true))

(event EventBeginPlay
  (bind _returnvalue (Components|GetOwner))
  ;[0.9737 0 1] Beginplay Stuff
  (EventDispatchers|BindEventtoOnTakeAnyDamage _returnvalue (EventDispatchers|CreateEvent :!event OnTakeAnyDamage))
  (Variables|Runtime|SetCurrentHP (Variables|Configuration|GetMaxHP))
  (bind _ascharacter (Utilities|Casting|CastToCharacter _returnvalue)
    (:then
      (Variables|Runtime|SetCharacter _ascharacter)
      (Variables|Runtime|SetbIsCharacter true)
      (Variables|Runtime|SetCurrentStamina (Variables|Configuration|GetMaxStamina)))
    (:CastFailed
      (Variables|Runtime|SetbIsCharacter false))))

(event EventTick
  (params (DeltaSeconds :type Float%20%28single-precision%29))
  (bind _firedamagehandle (Variables|Default|GetFireDamageHandle))
  (if (Utilities|Time|IsTimerActivebyHandle _firedamagehandle)
    (if (>= (Variables|Runtime|GetDotHitCounter) (Variables|Default|GetDOTLimit))
      (Utilities|Time|ClearandInvalidateTimerbyHandle _firedamagehandle)
      (Variables|Runtime|SetDotHitCounter 0))))

(fn OnTakeAnyDamage
  (params (DamagedActor :type Actor%20Object%20Reference) (Damage :type Float%20%28single-precision%29) (DamageType :type Damage%20Type%20Object%20Reference) (InstigatedBy :type Controller%20Object%20Reference) (DamageCauser :type Actor%20Object%20Reference))
  (LocalVariables|SetLocalDamage Damage)
  (LocalVariables|SetLocalDamagedActor DamagedActor)
  (bind _output_get (LocalVariables|SetLocalDamageType (.AsBP%20Base%20Damage%20Type (Utilities|Casting|CastToBP_BaseDamageType DamageType))))
  (Utilities|IsValid _output_get
    (:Is%20Valid
      (switch Utilities|FlowControl|Switch|SwitchonE_DamageType (Variables|/Game/CheekyFPS/Blueprints/Weapons/DamageTypes/BP_BaseDamageType.BP_BaseDamageType_C|GetDamageType (LocalVariables|GetLocalDamageType))
        (:NewEnumerator0
          (CallFunction|RemoveHealth (LocalVariables|GetLocalDamage) (LocalVariables|GetLocalDamagedActor) (LocalVariables|GetLocalDamageType) :!label _label)
          (return))
        (:NewEnumerator1
          (goto _label))
        (:NewEnumerator2
          (CallFunction|RemoveHealth (LocalVariables|GetLocalDamage) (LocalVariables|GetLocalDamagedActor) (LocalVariables|GetLocalDamageType))
          (bind _returnvalue (Utilities|Time|SetTimerbyEvent (EventDispatchers|CreateEvent :!event DamageOverTime) 1.0 true))
          (Variables|Default|SetFireDamageHandle _returnvalue))
        (:NewEnumerator3
          (CallFunction|RemoveHealth (LocalVariables|GetLocalDamage) (LocalVariables|GetLocalDamagedActor) (LocalVariables|GetLocalDamageType))
          (CallFunction|TryFreezeOwner))
        (:NewEnumerator4
          (switch Utilities|FlowControl|Switch|SwitchonECharacterType (Variables|Configuration|GetCharacterType)
            (:NewEnumerator1
              (CallFunction|RemoveStamina (LocalVariables|GetLocalDamage) (LocalVariables|GetLocalDamagedActor) :!label _label_2)
              (return))
            (:NewEnumerator2
              (CallFunction|RemoveHealth (/ (LocalVariables|GetLocalDamage) 2.0) (LocalVariables|GetLocalDamagedActor) (LocalVariables|GetLocalDamageType))
              (return))
            (:NewEnumerator3
              (goto _label_2))
            (:NewEnumerator4
              (CallFunction|RemoveHealth (LocalVariables|GetLocalDamage) (LocalVariables|GetLocalDamagedActor) (LocalVariables|GetLocalDamageType)))))
        (:NewEnumerator5
          (CallFunction|RemoveStamina (LocalVariables|GetLocalDamage) (LocalVariables|GetLocalDamagedActor))
          (return))))
    (:Is%20Not%20Valid
      (return))))

(fn OnLanded
  (params (VelocityOnImpact :type Float%20%28single-precision%29))
  (bind _character (Variables|Runtime|GetCharacter))
  (if (Variables|Runtime|GetbIsCharacter)
    (if (Variables|Configuration|GetbUseFallDamage)
      (bind _output_get (LocalVariables|SetDamage (Math|Curves|GetFloatValue (Variables|Configuration|GetFallDamage) (Math|Float|Absolute(Float) VelocityOnImpact))))
      (if (< _output_get 1.0)
        (return)
        (else
          (Game|Damage|ApplyDamage _character (LocalVariables|GetDamage) 0 _character)
          (return))))
    (else
      ;[1 0.1073 0.02767] Error
      (Development|PrintString "(CheekyHealthComponent) OnLanded only works for Characters!")
      (return))))

(fn AddHealth
  (params (HealthAdd :type Float%20%28single-precision%29))
  (bind _output_get (Variables|Runtime|SetCurrentHP (Math|Conversions|ToFloat(Integer) (Math|Float|Round (Math|Float|Clamp(Float) (+ (Variables|Runtime|GetCurrentHP) HealthAdd) 0.0 (Variables|Configuration|GetMaxHP))))))
  (Variables|Runtime|SetHealthPercentage (CallFunction|GetHealthPercentage))
  (Default|CallOnUpdateHealth _output_get)
  (Default|CallOnThingHealed)
  (return))

(fn RemoveHealth
  (params (HealthLost :type Float%20%28single-precision%29) (DamagedActor :type Actor%20Object%20Reference) (DamageTypeRecieved :type BP%20Base%20Damage%20Type%20Object%20Reference))
  (if (not (Variables|Configuration|GetbIgnoresDamage?))
    (bind _output_get (Variables|Runtime|SetCurrentHP (Math|Conversions|ToFloat(Integer) (Math|Float|Round (Math|Float|Clamp(Float) (- (Variables|Runtime|GetCurrentHP) HealthLost) 0.0 (Variables|Configuration|GetMaxHP))))))
    (Variables|Runtime|SetHealthPercentage (CallFunction|GetHealthPercentage))
    (Default|CallOnUpdateHealth _output_get)
    (Default|CallOnDamageRecieved DamageTypeRecieved)
    (Utilities|FlowControl|Sequence
      (:then_0
        (if (Variables|Debug|GetbEnableDebugMode?)
          (Development|PrintString (Utilities|String|ToString(Float) (Variables|Runtime|GetCurrentHP)))))
      (:then_1
        (if (== DamagedActor (Game|GetPlayerCharacter 0))
          (CameraEffects|StartPainVisual HealthLost)))
      (:then_2
        (if (== (Variables|Runtime|GetCurrentHP) 0.0)
          (CallFunction|UpdateCharacterState "NewEnumerator6")
          (Default|CallOnThingDead)
          (return)
          (else
            ;[0.1277 0.2754 1] Regenerate Health (If Enabled)
            (if (and (< (Variables|Runtime|GetCurrentHP) (Variables|Configuration|GetMaxHP)) (Variables|Configuration|GetbRegenerateHealth))
              (CallFunction|RegenHealth))
            (return)))))))

(fn RegenerateHealth
  (CallFunction|AddHealth (/ (Variables|Configuration|GetRegenerateSpeed) 1e+01))
  ;[0.2842 0.2266 1] If we've healed the player, stop this running
  (Utilities|FlowControl|Sequence
    (:then_0
      (if (Variables|Debug|GetbEnableDebugMode?)
        (Development|PrintString (Utilities|String|ToString(Float) (Variables|Runtime|GetCurrentHP)))))
    (:then_1
      (if (or (== (Variables|Runtime|GetCurrentHP) (Variables|Configuration|GetMaxHP)) (>= (CallFunction|GetHealthPercentage) (Variables|Runtime|GetTargetHealthPercentage)))
        (Utilities|Time|ClearTimerbyFunctionName 0 "RegenerateHealth"))
      (return))))

(fn GetHealth
  (return (Variables|Runtime|GetCurrentHP) (Variables|Configuration|GetMaxHP)))

(fn StartPainVisual
  (params (Loss :type Float%20%28single-precision%29))
  (Utilities|IsValid (Variables|Runtime|GetPainCameraModifier)
    (:Is%20Valid
      (CameraModifier|EnableModifier (Variables|Runtime|GetPainCameraModifier)))
    (:Is%20Not%20Valid
      (bind _returnvalue (Game|Player|AddNewCameraModifier (Game|GetPlayerCameraManager 0) "/Game/CheekyFPS/Blueprints/CameraManager/CamModifiers/BP_CamModifier_Pain.BP_CamModifier_Pain_C"))
      (Variables|Runtime|SetPainCameraModifier _returnvalue)))
  (Utilities|Time|SetTimerbyFunctionName 0 "EndPainVisual" (Math|Float|Lerp 0.1 1.4 (Math|Float|Clamp(Float) (/ Loss (Variables|Configuration|GetMaxHP)))))
  (return))

(fn EndPainVisual
  (if (CallFunction|IsDead?)
    _
    (else
      (CameraModifier|DisableModifier (Variables|Runtime|GetPainCameraModifier) false)))
  (return))

(fn GetHealthPercentage
  (return (/ (Variables|Runtime|GetCurrentHP) (Variables|Configuration|GetMaxHP))))

(fn RegenerateStamina
  (CallFunction|AddStamina (/ (Variables|Configuration|GetRegenerateSpeed) 1e+01))
  ;[0.2842 0.2266 1] If we've healed the player, stop this running
  (if (== (Variables|Runtime|GetCurrentStamina) (Variables|Configuration|GetMaxStamina))
    (Utilities|Time|ClearTimerbyFunctionName 0 "RegenerateStamina"))
  (return))

(fn AddStamina
  (params (StaminaAdd :type Float%20%28single-precision%29))
  (bind _output_get (Variables|Runtime|SetCurrentStamina (Math|Conversions|ToFloat(Integer) (Math|Float|Round (Math|Float|Clamp(Float) (+ (Variables|Runtime|GetCurrentStamina) StaminaAdd) 0.0 (Variables|Configuration|GetMaxStamina))))))
  (Variables|Runtime|SetStaminaPercentage (CallFunction|GetStaminaPercentage))
  (Default|CallOnUpdateStamina _output_get)
  (return))

(fn GetStaminaPercentage
  (return (/ (Variables|Runtime|GetCurrentStamina) (Variables|Configuration|GetMaxStamina))))

(fn RemoveStamina
  (params (StaminaLost :type Float%20%28single-precision%29) (DamagedActor :type Actor%20Object%20Reference))
  (Default|CallOnUpdateStamina (Variables|Runtime|GetCurrentStamina))
  (Variables|Runtime|SetCurrentStamina (Math|Conversions|ToFloat(Integer) (Math|Float|Round (Math|Float|Clamp(Float) (- (Variables|Runtime|GetCurrentStamina) StaminaLost) 0.0 (Variables|Configuration|GetMaxStamina)))))
  (Variables|Runtime|SetStaminaPercentage (CallFunction|GetStaminaPercentage))
  (Utilities|FlowControl|Sequence
    (:then_0
      (if (== DamagedActor (Game|GetPlayerCharacter 0))
        (CameraEffects|StartPainVisual StaminaLost)))
    (:then_1
      (if (<= (Variables|Runtime|GetCurrentStamina) 0.0)
        (CallFunction|UpdateCharacterState "NewEnumerator4")
        (Default|CallOnThingStunned)
        (return)
        (else
          ;[0.1277 0.2754 1] Regenerate Health (If Enabled)
          (if (and (< (Variables|Runtime|GetCurrentStamina) (Variables|Configuration|GetMaxStamina)) (Variables|Configuration|GetbRegenerateStamina))
            (CallFunction|RegenerateStamina))
          (return))))))

(fn ToggleRegenHealthStatus
  (params (bRegenerateHealth :type Boolean))
  (bind _output_get (Variables|Configuration|SetbRegenerateHealth bRegenerateHealth))
  (if _output_get
    (CallFunction|RegenHealth)
    (else
      (Utilities|Time|ClearTimerbyFunctionName 0 "RegenerateHealth"))))

(fn IsDead?
  (return (Utilities|Enum|Equal(Enum) (CallFunction|GetCharacterState) "NewEnumerator6")))

(fn ResetHealth
  (Variables|Runtime|SetCurrentHP (Variables|Configuration|GetMaxHP)))

(fn UpdateMaximumHealth
  (params (NewMaxHealth :type Float%20%28single-precision%29))
  (bind _output_get (Variables|Configuration|SetMaxHP NewMaxHealth))
  (Variables|Runtime|SetCurrentHP _output_get))

(fn IsatHalfHealth?
  (return (<= (CallFunction|GetHealthPercentage) 0.5)))

(fn DamageOverTime
  (CallFunction|RemoveHealth (Math|Random|RandomFloatinRange 5.0 8.0) (Components|GetOwner))
  (Math|Integer|IncrementInt (Variables|Runtime|GetDotHitCounter)))

(fn TryFreezeOwner
  (bind _character (Variables|Runtime|GetCharacter))
  (Utilities|IsValid _character
    (:Is%20Valid
      (if (Math|Random|RandomBoolwithWeight 0.4)
        (Default|FreezeCharacter (.AsBP%20Cheeky%20Character (Utilities|Casting|CastToBP_CheekyCharacter _character)))
        (else
          (return))))))

(fn TryUnfreezeOwner
  (params (IsDelayed? :type Boolean) (Time :type Float%20%28single-precision%29))
  (bind _character (Variables|Runtime|GetCharacter))
  (bind _asbp_cheeky_character (Utilities|Casting|CastToBP_CheekyCharacter _character))
  (Utilities|IsValid _character
    (:Is%20Valid
      (if IsDelayed?
        (Default|DelayedUnfreezeCharacter _asbp_cheeky_character Time)
        (else
          (Default|UnFreezeCharacter _asbp_cheeky_character))))))

(fn GetCharacterState
  (return (Variables|Runtime|GetCurrentCharacterState)))

(fn UpdateCharacterState
  (params (NewCharacterState :type E_CharacterState%20Enum :default "NewEnumerator0"))
  (Variables|Runtime|SetCurrentCharacterState NewCharacterState))

(fn IsStunned?
  (return (Utilities|Enum|Equal(Enum) (CallFunction|GetCharacterState) "NewEnumerator4")))

(fn IsNotHumanoid?
  (bind _charactertype (Variables|Configuration|GetCharacterType))
  (return (or (Utilities|Enum|Equal(Enum) _charactertype "NewEnumerator3") (Utilities|Enum|Equal(Enum) _charactertype "NewEnumerator4"))))