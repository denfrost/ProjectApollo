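; Health and stamina component for any actor, broadcasting updates, death and stun events.
; Owner damage is routed by BP_BaseDamageType flags to stamina, or to health if humanoid targeting matches whether the owner is a Character.
; Health regenerates on a looping timer after a retriggerable delay, while stamina loss calls its regeneration step directly.
; Player hits trigger a camera pain modifier timed by loss, and OnLanded converts impact velocity to curve-based fall damage.
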(event Custom|RegenHealth
  ;[1 0.7974 0] Health Regeneration
  (Utilities|Time|ClearTimerbyFunctionName 0 "RegenerateHealth") ; Make sure timer isn't running\nE.g. if the timer was running, and player\ntakes damage and triggers this event again\nthen stop regenerating
  (Utilities|FlowControl|RetriggerableDelay (Variables|Configuration|GetRegenerateDelay))
  (Utilities|Time|SetTimerbyFunctionName 0 "RegenerateHealth" 0.1 true))

(event Custom|EndPain
  (params (Delay :type Float%20%28single-precision%29))
  (bind _returnvalue (Game|Player|FindCameraModifierbyClass (Game|GetPlayerCameraManager 0) "/Game/CheekyFPS/Blueprints/CameraManager/CamModifiers/CamModifier_Pain.CamModifier_Pain_C"))
  (CameraModifier|DisableModifier _returnvalue false)
  (Utilities|FlowControl|Delay (Variables|/Script/Engine.CameraModifier|GetAlphaOutTime _returnvalue)))

(event Custom|RegenStamina
  (Utilities|Time|ClearTimerbyFunctionName 0 "RegenerateStamina") ; Make sure timer isn't running\nE.g. if the timer was running, and player\ntakes damage and triggers this event again\nthen stop regenerating
  (Utilities|FlowControl|RetriggerableDelay (Variables|Configuration|GetRegenerateDelay))
  (Utilities|Time|SetTimerbyFunctionName 0 "RegenerateStamina" 0.1 true))

(event EventBeginPlay
  (bind _returnvalue (Components|GetOwner))
  ;[0.9737 0 1] Beginplay Stuff
  (EventDispatchers|BindEventtoOnTakeAnyDamage _returnvalue (EventDispatchers|CreateEvent :!event OnTakeAnyDamage))
  (Variables|Runtime|SetCurrentHP (Variables|Configuration|GetMaxHP))
  (bind _ascharacter (Utilities|Casting|CastToCharacter _returnvalue)
    (:then
      (Variables|Runtime|SetCharacter _ascharacter)
      (Variables|Runtime|SetbIsCharacter true)
      (Variables|Runtime|SetCurrentStamina (Variables|Configuration|GetMaxStamina)))
    (:CastFailed
      (Variables|Runtime|SetbIsCharacter false))))

(fn OnTakeAnyDamage
  (params (DamagedActor :type Actor%20Object%20Reference) (Damage :type Float%20%28single-precision%29) (DamageType :type Damage%20Type%20Object%20Reference) (InstigatedBy :type Controller%20Object%20Reference) (DamageCauser :type Actor%20Object%20Reference))
  (bind _asbp_base_damage_type (Utilities|Casting|CastToBP_BaseDamageType DamageType))
  (if (Variables|/Game/CheekyFPS/Blueprints/Weapons/DamageTypes/BP_BaseDamageType.BP_BaseDamageType_C|GetbDamagesStamina? _asbp_base_damage_type)
    (CallFunction|RemoveStamina Damage DamagedActor)
    (return)
    (elif (Variables|/Game/CheekyFPS/Blueprints/Weapons/DamageTypes/BP_BaseDamageType.BP_BaseDamageType_C|GetbAffectsHumanoids? _asbp_base_damage_type)
      (if (Variables|Runtime|GetbIsCharacter)
        (CallFunction|RemoveHealth Damage DamagedActor)
        (return))
      (elif (not (Variables|Runtime|GetbIsCharacter))
        (CallFunction|RemoveHealth Damage DamagedActor)
        (return)
        (else
          (return))))))

(fn OnLanded
  (params (VelocityOnImpact :type Float%20%28single-precision%29))
  (bind _character (Variables|Runtime|GetCharacter))
  (if (Variables|Runtime|GetbIsCharacter)
    (if (Variables|Configuration|GetbUseFallDamage)
      (bind _output_get (LocalVariables|SetDamage (Math|Curves|GetFloatValue (Variables|Configuration|GetFallDamage) (Math|Float|Absolute(Float) VelocityOnImpact))))
      (if (< _output_get 1.0)
        (return)
        (else
          (Game|Damage|ApplyDamage _character (LocalVariables|GetDamage) 0 _character)
          (return))))
    (else
      ;[1 0.1073 0.02767] Error
      (Development|PrintString "(CheekyHealthComponent) OnLanded only works for Characters!")
      (return))))

(fn AddHealth
  (params (HealthAdd :type Float%20%28single-precision%29))
  (bind _output_get (Variables|Runtime|SetCurrentHP (Math|Conversions|ToFloat(Integer) (Math|Float|Round (Math|Float|Clamp(Float) (+ (Variables|Runtime|GetCurrentHP) HealthAdd) 0.0 (Variables|Configuration|GetMaxHP))))))
  (Variables|Default|SetHealthPercentage (CallFunction|GetHealthPercentage))
  (Default|CallOnUpdateHealth _output_get)
  (return))

(fn RemoveHealth
  (params (HealthLost :type Float%20%28single-precision%29) (DamagedActor :type Actor%20Object%20Reference))
  (if (not (Variables|Default|GetbIgnoresDamage?))
    (bind _output_get (Variables|Runtime|SetCurrentHP (Math|Conversions|ToFloat(Integer) (Math|Float|Round (Math|Float|Clamp(Float) (- (Variables|Runtime|GetCurrentHP) HealthLost) 0.0 (Variables|Configuration|GetMaxHP))))))
    (Variables|Default|SetHealthPercentage (CallFunction|GetHealthPercentage))
    (Default|CallOnUpdateHealth _output_get)
    (Default|CallOnDamageRecieved)
    (Utilities|FlowControl|Sequence
      (:then_0
        (if (Variables|Default|GetbEnableDebugMode?)
          (Development|PrintString (Utilities|String|ToString(Float) (Variables|Runtime|GetCurrentHP)))))
      (:then_1
        (if (== DamagedActor (Game|GetPlayerCharacter 0))
          (CameraEffects|StartPainVisual HealthLost)))
      (:then_2
        (if (== (Variables|Runtime|GetCurrentHP) 0.0)
          (Variables|Runtime|SetbIsDead true)
          (Default|CallOnThingDead)
          (return)
          (else
            ;[0.1277 0.2754 1] Regenerate Health (If Enabled)
            (if (and (< (Variables|Runtime|GetCurrentHP) (Variables|Configuration|GetMaxHP)) (Variables|Configuration|GetbRegenerateHealth))
              (CallFunction|RegenHealth))
            (return)))))))

(fn RegenerateHealth
  (CallFunction|AddHealth (/ (Variables|Configuration|GetRegenerateSpeed) 1e+01))
  ;[0.2842 0.2266 1] If we've healed the player, stop this running
  (if (== (Variables|Runtime|GetCurrentHP) (Variables|Configuration|GetMaxHP))
    (Utilities|Time|ClearTimerbyFunctionName 0 "RegenerateHealth"))
  (return))

(fn GetHealth
  (return (Variables|Runtime|GetCurrentHP) (Variables|Configuration|GetMaxHP)))

(fn StartPainVisual
  (params (Loss :type Float%20%28single-precision%29))
  (Utilities|IsValid (Variables|Runtime|GetPainCameraModifier)
    (:Is%20Valid
      (CameraModifier|EnableModifier (Variables|Runtime|GetPainCameraModifier)))
    (:Is%20Not%20Valid
      (bind _returnvalue (Game|Player|AddNewCameraModifier (Game|GetPlayerCameraManager 0) "/Game/CheekyFPS/Blueprints/CameraManager/CamModifiers/CamModifier_Pain.CamModifier_Pain_C"))
      (Variables|Runtime|SetPainCameraModifier _returnvalue)))
  (Utilities|Time|SetTimerbyFunctionName 0 "EndPainVisual" (Math|Float|Lerp 0.1 1.4 (Math|Float|Clamp(Float) (/ Loss (Variables|Configuration|GetMaxHP)))))
  (return))

(fn EndPainVisual
  (if (Variables|Runtime|GetbIsDead)
    _
    (else
      (CameraModifier|DisableModifier (Variables|Runtime|GetPainCameraModifier) false)))
  (return))

(fn GetHealthPercentage
  (return (/ (Variables|Runtime|GetCurrentHP) (Variables|Configuration|GetMaxHP))))

(fn RegenerateStamina
  (CallFunction|AddStamina (/ (Variables|Configuration|GetRegenerateSpeed) 1e+01))
  ;[0.2842 0.2266 1] If we've healed the player, stop this running
  (if (== (Variables|Runtime|GetCurrentStamina) (Variables|Configuration|GetMaxStamina))
    (Utilities|Time|ClearTimerbyFunctionName 0 "RegenerateStamina"))
  (return))

(fn AddStamina
  (params (StaminaAdd :type Float%20%28single-precision%29))
  (bind _output_get (Variables|Runtime|SetCurrentStamina (Math|Conversions|ToFloat(Integer) (Math|Float|Round (Math|Float|Clamp(Float) (+ (Variables|Runtime|GetCurrentStamina) StaminaAdd) 0.0 (Variables|Configuration|GetMaxStamina))))))
  (Variables|Default|SetStaminaPercentage (CallFunction|GetStaminaPercentage))
  (Default|CallOnUpdateStamina _output_get)
  (return))

(fn GetStaminaPercentage
  (return (/ (Variables|Runtime|GetCurrentStamina) (Variables|Configuration|GetMaxStamina))))

(fn RemoveStamina
  (params (StaminaLost :type Float%20%28single-precision%29) (DamagedActor :type Actor%20Object%20Reference))
  (Default|CallOnUpdateStamina (Variables|Runtime|GetCurrentStamina))
  (Variables|Runtime|SetCurrentStamina (Math|Conversions|ToFloat(Integer) (Math|Float|Round (Math|Float|Clamp(Float) (- (Variables|Runtime|GetCurrentStamina) StaminaLost) 0.0 (Variables|Configuration|GetMaxStamina)))))
  (Variables|Default|SetStaminaPercentage (CallFunction|GetStaminaPercentage))
  (Utilities|FlowControl|Sequence
    (:then_0
      (if (== DamagedActor (Game|GetPlayerCharacter 0))
        (CameraEffects|StartPainVisual StaminaLost)))
    (:then_1
      (if (== (Variables|Runtime|GetCurrentStamina) 0.0)
        (Variables|Runtime|SetbIsStunned true)
        (Default|CallOnThingStunned)
        (return)
        (else
          ;[0.1277 0.2754 1] Regenerate Health (If Enabled)
          (if (and (< (Variables|Runtime|GetCurrentStamina) (Variables|Configuration|GetMaxStamina)) (Variables|Configuration|GetbRegenerateStamina))
            (CallFunction|RegenerateStamina))
          (return))))))

(fn ToggleRegenHealthStatus
  (params (bRegenerateHealth :type Boolean))
  (Variables|Configuration|SetbRegenerateHealth bRegenerateHealth))