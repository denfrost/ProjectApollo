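; Player power component that manages a magic pool spent on actions, currently Dash and Vision Cloak.
; AttemptAction checks unlock and remaining magic, spends it once or on a looping timer, then messages the player character to perform the action.
; Dash starts timed regeneration immediately, while looping powers stop via DeactivatePower, also called on empty magic, which regenerates if CanRecharge.
; Magic changes are rounded, clamped and broadcast through OnUpdateMagic.
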(event EventBeginPlay
  (CallFunction|SetStartingStats))

(event EventTick
  (params (DeltaSeconds :type Float%20%28single-precision%29)))

(fn UseMagic
  (params (ConsumeAmount :type Float%20%28single-precision%29))
  (bind _output_get (Variables|Default|SetCurrentMagic (Math|Conversions|ToFloat(Integer) (Math|Float|Round (Math|Float|Clamp(Float) (- (Variables|Default|GetCurrentMagic) ConsumeAmount) 0.0 (Variables|Default|GetMaxMagic))))))
  (Default|CallOnUpdateMagic _output_get)
  (bind _output_get_2 (Variables|Default|SetbOutOfMagic? (<= _output_get 0.0)))
  (if _output_get_2
    (CallFunction|DeactivatePower)))

(fn GetMagicPercentage
  (return (/ (Variables|Default|GetCurrentMagic) (Variables|Default|GetMaxMagic))))

(fn RecoverMagic
  (params (RecoverAmount :type Float%20%28single-precision%29))
  (bind _regenmagichandle (Variables|Default|GetRegenMagicHandle))
  (bind _output_get (Variables|Default|SetCurrentMagic (Math|Conversions|ToFloat(Integer) (Math|Float|Round (Math|Float|Clamp(Float) (+ (Variables|Default|GetCurrentMagic) RecoverAmount) 0.0 (Variables|Default|GetMaxMagic))))))
  (Default|CallOnUpdateMagic _output_get)
  (if (>= _output_get (Variables|Default|GetMaxMagic))
    (Variables|Default|SetCurrentMagic (Variables|Default|GetMaxMagic))
    (if (Utilities|Time|IsTimerActivebyHandle _regenmagichandle)
      (Utilities|Time|ClearandInvalidateTimerbyHandle _regenmagichandle))))

(fn AttemptAction
  (params (IncomingAction :type Magic%20Action%20Struct%20Structure))
  (bind (_bisactionunlocked_ _actionname _magicconsumeamount _bdoesactionusecooldown_ _cooldownlength _bdoesactionloop_) (Utilities|Struct|BreakMagicActionStruct IncomingAction))
  (bind _returnvalue (Game|GetPlayerCharacter 0))
  (if (and _bisactionunlocked_ (not (Variables|Default|GetbOutOfMagic?)))
    (Utilities|FlowControl|Sequence
      (:then_0
        (Utilities|Time|ClearandInvalidateTimerbyHandle (Variables|Default|GetRegenMagicHandle))
        (Variables|Default|SetActionCooldownLength _cooldownlength)
        (Variables|Default|SetbIsActionOnCooldown? _bdoesactionusecooldown_)
        (Variables|Default|SetbDoesActionLoop? _bdoesactionloop_))
      (:then_1
        (if (Variables|Default|GetbDoesActionLoop?)
          (Variables|Default|SetPowerConsumeAmount _magicconsumeamount)
          (CallFunction|StartMagicConsume)
          (else
            (CallFunction|UseMagic _magicconsumeamount))))
      (:then_2
        (Variables|Default|SetCurrentActionName _actionname)
        (switch string _actionname
          (:Dash
            (Class|BPIPlayer|AttemptDash(Message) _returnvalue)
            (CallFunction|StartMagicRegen))
          (:Vision%20Cloak
            (Class|BPIPlayer|AttemptCloak(Message) _returnvalue)
            (Variables|Default|SetbIsActionActivated? true)))))))

(fn ResetActionCooldown
  (Variables|Default|SetbIsActionOnCooldown? false))

(fn DeactivatePower
  (if (Variables|Default|GetbDoesActionLoop?)
    (Variables|Default|SetbIsActionActivated? false)
    (Utilities|FlowControl|Sequence
      (:then_0
        (if (Variables|Default|GetbCanRecharge?)
          (CallFunction|StartMagicRegen)))
      (:then_1
        (Utilities|Time|ClearandInvalidateTimerbyHandle (Variables|Default|GetConsumeMagicHandle))
        (switch string (Variables|Default|GetCurrentActionName)
          (:Vision%20Cloak
            (Class|BPIPlayer|StopCloak(Message) (Game|GetPlayerCharacter 0))))))))

(fn RegenMagic
  (CallFunction|RecoverMagic (Variables|Default|GetRegenAmount)))

(fn StartMagicRegen
  (if (or (Variables|Default|GetbOutOfMagic?) (< (Variables|Default|GetCurrentMagic) (Variables|Default|GetMaxMagic)))
    (bind _returnvalue (Utilities|Time|SetTimerbyEvent (EventDispatchers|CreateEvent :!event RegenMagic) (Variables|Default|GetRegenRate) true))
    (Variables|Default|SetRegenMagicHandle _returnvalue)))

(fn StartMagicConsume
  (bind _returnvalue (Utilities|Time|SetTimerbyEvent (EventDispatchers|CreateEvent :!event ConsumeMagic) (Variables|Default|GetPowerConsumeRate) true))
  (Variables|Default|SetConsumeMagicHandle _returnvalue))

(fn ConsumeMagic
  (CallFunction|UseMagic (Variables|Default|GetPowerConsumeAmount)))

(fn GetActionActiveStatus
  (return (Variables|Default|GetbIsActionActivated?)))

(fn SetStartingStats
  (bind _output_get (Variables|Default|SetCurrentMagic (Variables|Default|GetMaxMagic)))
  (Default|CallOnUpdateMagic _output_get))