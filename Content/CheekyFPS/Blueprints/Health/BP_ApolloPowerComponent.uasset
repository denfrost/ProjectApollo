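; Apollo power component that manages a character's magic pool and triggers powers: Dash, Vision Cloak, Slow Time and Hack.
; AttemptAction checks unlock and magic, spends it once or on a looping drain timer, then messages the player character.
; Deactivation stops looping powers and starts timed regen or refunds magic from damage.
; It also broadcasts magic updates and stores lookups and current selections for powers and abilities.
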(event EventBeginPlay
  (Setters|SetStartingStats))

(event EventTick
  (params (DeltaSeconds :type Float%20%28single-precision%29)))

(fn UseMagic
  (params (ConsumeAmount :type Float%20%28single-precision%29))
  (bind _output_get (Variables|Stats|SetCurrentMagic (Math|Conversions|ToFloat(Integer) (Math|Float|Round (Math|Float|Clamp(Float) (- (Variables|Stats|GetCurrentMagic) ConsumeAmount) 0.0 (Variables|Stats|GetMaxMagic))))))
  (Default|CallOnUpdateMagic _output_get)
  (bind _output_get_2 (Variables|Status|SetbOutOfMagic? (<= _output_get 0.0)))
  (if _output_get_2
    (Actions|DeactivateAction)))

(fn GetMagicPercentage
  (return (/ (Variables|Stats|GetCurrentMagic) (Variables|Stats|GetMaxMagic))))

(fn RecoverMagic
  (params (RecoverAmount :type Float%20%28single-precision%29))
  (bind _regenmagichandle (Variables|Runtime|GetRegenMagicHandle))
  (bind _output_get (Variables|Stats|SetCurrentMagic (Math|Conversions|ToFloat(Integer) (Math|Float|Round (Math|Float|Clamp(Float) (+ (Variables|Stats|GetCurrentMagic) RecoverAmount) 0.0 (Variables|Stats|GetMaxMagic))))))
  (Default|CallOnUpdateMagic _output_get)
  (if (>= _output_get (Variables|Stats|GetMaxMagic))
    (Variables|Stats|SetCurrentMagic (Variables|Stats|GetMaxMagic))
    (if (Utilities|Time|IsTimerActivebyHandle _regenmagichandle)
      (Utilities|Time|ClearandInvalidateTimerbyHandle _regenmagichandle))))

(fn AttemptAction
  (params (IncomingAction :type Magic%20Action%20Struct%20Structure))
  (bind (_bisactionunlocked_ _actionname _magicconsumeamount _bdoesactionusecooldown_ _cooldownlength _bdoesactionloop_) (Utilities|Struct|BreakMagicActionStruct IncomingAction))
  (bind _returnvalue (Game|GetPlayerCharacter 0))
  (if (and _bisactionunlocked_ (not (Variables|Status|GetbOutOfMagic?)))
    (Utilities|FlowControl|Sequence
      (:then_0
        (Utilities|Time|ClearandInvalidateTimerbyHandle (Variables|Runtime|GetRegenMagicHandle))
        (Variables|Stats|SetActionCooldownLength _cooldownlength)
        (Variables|Status|SetbIsActionOnCooldown? _bdoesactionusecooldown_)
        (Variables|Status|SetbDoesActionLoop? _bdoesactionloop_)
        (if (Variables|Status|GetbOutOfMagic?)
          (if (> (Variables|Stats|GetCurrentMagic) 0.0)
            (Variables|Status|SetbOutOfMagic? false))))
      (:then_1
        (if (Variables|Status|GetbDoesActionLoop?)
          (Variables|Stats|SetPowerConsumeAmount _magicconsumeamount)
          (Actions|StartMagicConsume)
          (else
            (Update|UseMagic _magicconsumeamount))))
      (:then_2
        (Variables|Runtime|SetCurrentActionName _actionname)
        (switch string _actionname
          (:Dash
            (Class|BPIPlayer|AttemptDash(Message) _returnvalue)
            (Update|Reset|StartMagicRegen))
          (:Vision%20Cloak
            (Class|BPIPlayer|AttemptCloak(Message) _returnvalue)
            (Variables|Status|SetbIsActionActivated? true :!label _label))
          (:Slow%20Time
            (Class|BPIPlayer|AttemptSlowTime(Message) _returnvalue)
            (goto _label))
          (:Hack
            (Class|BPIPlayer|AttemptHack(Message) _returnvalue)))))))

(fn ResetActionCooldown
  (Variables|Status|SetbIsActionOnCooldown? false))

(fn DeactivateAction
  (bind _returnvalue (Game|GetPlayerCharacter 0))
  (if (Variables|Status|GetbDoesActionLoop?)
    (Variables|Status|SetbIsActionActivated? false)
    (Utilities|FlowControl|Sequence
      (:then_0
        (if (Variables|Status|GetbCanRecharge?)
          (Update|Reset|StartMagicRegen)
          (elif (Variables|Status|GetbCanRechargeByDamage?)
            (Update|RecoverMagic (/ (Variables|/Game/CheekyFPS/Blueprints/BP_CheekyCharacter.BP_CheekyCharacter_C|GetIn%20Damage (.AsBP%20Cheeky%20Character (Utilities|Casting|CastToBP_CheekyCharacter (Components|GetOwner)))) 2.0)))))
      (:then_1
        (Utilities|Time|ClearandInvalidateTimerbyHandle (Variables|Runtime|GetConsumeMagicHandle))
        (switch string (Variables|Runtime|GetCurrentActionName)
          (:Slow%20Time
            (Class|BPIPlayer|StopSlowTime(Message) _returnvalue))
          (:Vision%20Cloak
            (Class|BPIPlayer|StopCloak(Message) _returnvalue)))))))

(fn RegenMagic
  (Update|RecoverMagic (Variables|Stats|GetRegenAmount)))

(fn StartMagicRegen
  (if (or (Variables|Status|GetbOutOfMagic?) (< (Variables|Stats|GetCurrentMagic) (Variables|Stats|GetMaxMagic)))
    (bind _returnvalue (Utilities|Time|SetTimerbyEvent (EventDispatchers|CreateEvent :!event RegenMagic) (Variables|Stats|GetRegenRate) true))
    (Variables|Runtime|SetRegenMagicHandle _returnvalue)))

(fn StartMagicConsume
  (bind _returnvalue (Utilities|Time|SetTimerbyEvent (EventDispatchers|CreateEvent :!event ConsumeMagic) (Variables|Stats|GetPowerConsumeRate) true))
  (Variables|Runtime|SetConsumeMagicHandle _returnvalue))

(fn ConsumeMagic
  (Update|UseMagic (Variables|Stats|GetPowerConsumeAmount)))

(fn GetActionActiveStatus
  (return (Variables|Status|GetbIsActionActivated?)))

(fn SetStartingStats
  (bind _output_get (Variables|Stats|SetCurrentMagic (Variables|Stats|GetMaxMagic)))
  (Default|CallOnUpdateMagic _output_get))

(fn FindPower
  (params (InPowerName :type String))
  (bind _availablepowers (Variables|Default|GetAvailablePowers))
  (bind (_value _returnvalue) (Utilities|Map|Find _availablepowers InPowerName))
  (if _returnvalue
    (Development|PrintString "Succeeded!")
    (return _value)
    (else
      (Development|PrintString "Failed"))))

(fn FindAbility
  (params (InAbilityName :type String%20%28by%20ref%29))
  (bind _availableabilities (Variables|Default|GetAvailableAbilities))
  (bind (_value _returnvalue) (Utilities|Map|Find _availableabilities InAbilityName))
  (if _returnvalue
    (return _value)))

(fn SetNewPower
  (params (InPower :type Magic%20Action%20Struct%20Structure))
  (Variables|Runtime|SetCurrentPower InPower))

(fn SetNewAbility
  (params (InAbility :type Magic%20Action%20Struct%20Structure))
  (Variables|Runtime|SetCurrentAbility InAbility))

(fn GetPowers
  (return (Variables|Default|GetAvailablePowers)))

(fn GetAbilities
  (return (Variables|Default|GetAvailableAbilities)))