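; BP_CheekyParkourHelper is a short-lived helper actor that moves the player character through a two-stage parkour move.
; On BeginPlay it records the character's location, disables capsule collision, then chains two fixed-length timelines that lerp the character to PositionA, then PositionB.
; When the second timeline finishes, it restores collision, fires the OnFinish dispatcher and destroys itself.
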(event EventBeginPlay
  (Variables|Default|SetStartLocation (Transformation|GetWorldLocation (Variables|/Script/Engine.Actor|GetRootComponent (Variables|Default|GetPlayerCharacter))))
  (CallFunction|SetTimelineDuration (Variables|Default|GetPosA) 0.3)
  (CallFunction|SetTimelineDuration (Variables|Default|GetPosB) 0.5)
  (Collision|SetCollisionEnabled (Variables|/Script/Engine.Character|GetCapsuleComponent (Variables|Default|GetPlayerCharacter)) "NoCollision")
  (bind _anim (Timeline|PosA PlayFromStart)
    (:Update
      (Transformation|SetActorLocation (Variables|Default|GetPlayerCharacter) (Math|Vector|Lerp(Vector) (Variables|Default|GetStartLocation) (Variables|Default|GetPositionA) _anim) false false))
    (:Finished
      (bind _anim_2 (Timeline|PosB PlayFromStart)
        (:Update
          (Transformation|SetActorLocation (Variables|Default|GetPlayerCharacter) (Math|Vector|Lerp(Vector) (Variables|Default|GetPositionA) (Variables|Default|GetPositionB) _anim_2) false false))
        (:Finished
          (Collision|SetCollisionEnabled (Variables|/Script/Engine.Character|GetCapsuleComponent (Variables|Default|GetPlayerCharacter)) "QueryAndPhysics")
          (Default|CallOnFinish)
          (Actor|DestroyActor))))))

(fn ConstructionScript)