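; ISSCheekyCharacter is a CheekyFPS character Blueprint that sets up health and attaches its weapon when play begins.
; After the parent BeginPlay, it turns off fall damage on the HealthComponent, raises max HP and fills current HP to match.
; It then has BPWeaponComponent attach the current weapon to WeaponAttachPoint, leaving all other behavior to the parent class and components.
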(event EventBeginPlay
  (bind _healthcomponent (Variables|Default|GetHealthComponent))
  (bind _bp_weaponcomponent (Variables|Default|GetBP_WeaponComponent))
  (|CallParentFunction)
  (Variables|/Game/CheekyFPS/Blueprints/Health/CheekyHealthComponent.CheekyHealthComponent_C|SetbUseFallDamage _healthcomponent false)
  (bind _output_get (Variables|/Game/CheekyFPS/Blueprints/Health/CheekyHealthComponent.CheekyHealthComponent_C|SetMaxHP _healthcomponent 2e+02))
  (Variables|/Game/CheekyFPS/Blueprints/Health/CheekyHealthComponent.CheekyHealthComponent_C|SetCurrentHP _healthcomponent _output_get)
  (Default|AttachtoOwner _bp_weaponcomponent (Variables|/Game/CheekyFPS/Blueprints/Weapons/BP_WeaponComponent.BP_WeaponComponent_C|GetCurrentWeapon _bp_weaponcomponent) (Variables|Default|GetWeaponAttachPoint) "None"))

(event Collision|EventActorBeginOverlap
  (params (OtherActor :type Actor%20Object%20Reference)))

(event EventTick
  (params (DeltaSeconds :type Float%20%28single-precision%29))
  (|CallParentFunction DeltaSeconds) ; This node is disabled and will not be called.\nDrag off pins to build functionality.
)

(fn ConstructionScript
  (|CallParentFunction))