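; Base Blueprint for grenade launcher weapons that fire a selectable type of grenade projectile.
; UpdateCurrentGrenade looks up CurrentGrenadeType in the Grenades map, synchronously loads that class asset and stores it as CurrentGrenade, cast to a BP_Grenade_Projectile class.
; The Fire event spawns CurrentGrenade at the skeletal mesh's WeaponMuzzlePoint socket when the class is valid.
; Nothing in this Blueprint calls UpdateCurrentGrenade.
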(event EventBeginPlay
  (|CallParentFunction) ; This node is disabled and will not be called.\nDrag off pins to build functionality.
)

(event Collision|EventActorBeginOverlap
  (params (OtherActor :type Actor%20Object%20Reference))
  (|CallParentFunction OtherActor) ; This node is disabled and will not be called.\nDrag off pins to build functionality.
)

(event EventTick
  (params (DeltaSeconds :type Float%20%28single-precision%29))
  (|CallParentFunction DeltaSeconds) ; This node is disabled and will not be called.\nDrag off pins to build functionality.
)

(event EventFire
  (bind _currentgrenade (Variables|Default|GetCurrentGrenade))
  (if (Utilities|IsValidClass _currentgrenade)
    (Game|SpawnActorfromClass _currentgrenade (Transformation|GetSocketTransform (Variables|Default|GetSkeletalMesh) (Variables|Default|GetWeaponMuzzlePoint) "RTS_World") "Undefined" 0 0)))

(fn ConstructionScript
  (|CallParentFunction))

(fn UpdateCurrentGrenade
  (bind _currentgrenadetype (Variables|Stats|GetCurrentGrenadeType))
  (bind _grenades (Variables|Default|GetGrenades))
  (bind (_value _returnvalue) (Utilities|Map|Find _grenades _currentgrenadetype))
  (if _returnvalue
    (bind _returnvalue_2 (Utilities|LoadClassAssetBlocking _value))
    (Variables|Default|SetCurrentGrenade (.AsBP%20Grenade%20Projectile (Utilities|Casting|CastToBP_Grenade_ProjectileClass _returnvalue_2)))))