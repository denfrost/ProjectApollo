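; Base hitscan weapon for CheekyFPS, used by the player and other characters, handling firing, ammo and reloading.
; Fire line-traces from the player camera or owner's eye view, repeating per shotgun pellet, with a looping timer for automatic fire.
; Hits apply team-checked point damage with head/pelvis crits and difficulty scaling that differs for player and non-player weapons.
; Shots trigger UI updates, surface impact effects and attachment-scaled noise events, while reload timing follows the sound's duration.
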(event Custom|GetPlaybackDuration
  (params (PlayingSoundWave :type Sound%20Wave%20Object%20Reference) (PlaybackPercent :type Float%20%28single-precision%29))
  (bind _output_get (Variables|Feedback|SetPlaybackPercent PlaybackPercent))
  (Variables|Feedback|SetPlaybackDuration (* _output_get (Variables|/Script/Engine.SoundBase|GetDuration PlayingSoundWave))))

(event EventBeginPlay
  (bind _returnvalue (Components|GetOwner))
  (bind _audio (Variables|Default|GetAudio))
  (bind _skeletalmesh (Variables|Default|GetSkeletalMesh))
  (Utilities|FlowControl|Sequence
    (:then_0
      (Variables|Ammo|SetInventoryAmmo (Variables|Ammo|GetMaxAmmoLimit))
      (Variables|Ammo|SetCurrentMagAmmo (Variables|Ammo|GetMagAmmoLimit))
      (Variables|Conditions|SetbCanFire? true)
      (bind _reloadsfx (Variables|Feedback|GetReloadSFX)
        (:then
          (Audio|Components|Audio|SetSound _audio _reloadsfx)
          (Variables|Feedback|SetPlaybackDuration (Variables|/Script/Engine.SoundBase|GetDuration (Variables|/Script/Engine.AudioComponent|GetSound _audio))))
        (:else
          _))
      (EventDispatchers|BindEventtoOnAudioPlaybackPercent (Variables|Default|GetAudio) (EventDispatchers|CreateEvent :!event Custom|GetPlaybackDuration))
      (Variables|Conditions|SetbCanReload? true)
      ;[1 1 1] Attach scene component for easier FX spawning
      (CallFunction|StartReload)
      (Transformation|AttachComponentToComponent (Variables|Default|GetScene) (Variables|Default|GetSkeletalMesh) (Variables|Feedback|GetWeaponMuzzlePoint) "SnapToTarget" "SnapToTarget" "SnapToTarget" true)
      (Transformation|AttachComponentToComponent (Variables|Default|GetAudio) (Variables|/Script/Engine.Actor|GetRootComponent (Components|GetOwner)) "None" "SnapToTarget" "SnapToTarget" "SnapToTarget" true))
    (:then_1
      (Variables|Default|SetWeaponOwner _returnvalue)
      (bind _output_get (Variables|Conditions|SetbIsPlayerWeapon? (== _returnvalue (Game|Player|GetPlayerPawn 0))))
      (Variables|Conditions|SetbIsLethal? (== (Variables|Damage|GetCurrentDamageTypeClass) "/Game/CheekyFPS/Blueprints/Weapons/DamageTypes/BP_StandardDamageType.BP_StandardDamageType_C"))
      (Utilities|Array|AddUnique (Variables|Default|GetIgnoredActors) (Variables|Default|GetWeaponOwner))
      (if _output_get
        (Utilities|Time|SetTimerbyEvent (EventDispatchers|CreateEvent :!event CheckforIgnoredActors) 1e+01 true)
        (Class|PrimitiveComponent|SetOwnerNoSee _skeletalmesh true)
        (Rendering|SetCastShadow _skeletalmesh false)))))

(fn ConstructionScript
  (Utilities|Struct|SetmembersinST_Weapon (Variables|Stats|GetWeaponData) (Variables|Feedback|GetWeaponName) (Variables|Ammo|GetCurrentMagAmmo) (Variables|Ammo|GetInventoryAmmo) (Variables|Feedback|GetTime%20to%20Equip) (Variables|Feedback|GetTime%20to%20Unequip) (Variables|Feedback|GetTime%20to%20Enter%20ADS) (Variables|Feedback|GetTime%20to%20Exit%20ADS) (Variables|Feedback|GetADS%20FOV%20Modifier) (Variables|/Script/Engine.SkinnedMeshComponent|GetSkeletalMesh (Variables|Default|GetSkeletalMesh))))

(fn Fire
  (bind (_startlocation _endlocation) (CallFunction|GetOwnerTraceLocations))
  (bind _bisplayerweapon_ (Variables|Conditions|GetbIsPlayerWeapon?))
  (CallFunction|UpdateOwner)
  ;[1 1 1] Does the user have enough rounds to fire the weapon?
  (if (Variables|Conditions|GetbCanFire?)
    ;[1 1 1] Does this weapon use the ammo in the mag?
    (if (Variables|Conditions|GetbConsumesAmmo?)
      (CallFunction|ConsumeAmmo 1))
    (if (Utilities|Enum|Equal(Enum) (Variables|Stats|GetWeaponType) "NewEnumerator2")
      (Variables|Conditions|SetisFiring? true)
      ;[1 1 1] Run the same function for the shotgun, but multiple times per "pellet"
      (CallFunction|ShotgunFire)
      (else
        (Variables|Conditions|SetisFiring? true)
        (bind _outhit (Collision|LineTraceByChannel _startlocation _endlocation "TraceTypeQuery3" true (Variables|Default|GetIgnoredActors) (select (Variables|Conditions|GetbEnableDebugMode?) "ForDuration" "None") true (Math|Color|SelectColor "(R=1.000000,G=0.774480,B=0.000000,A=1.000000)" "(R=1.000000,G=0.000000,B=0.000000,A=1.000000)" _bisplayerweapon_) (Math|Color|SelectColor "(R=0.736302,G=0.000000,B=1.000000,A=1.000000)" "(R=0.111099,G=1.000000,B=0.000000,A=1.000000)" _bisplayerweapon_)))
        (CallFunction|HandleFireTrace _outhit)))))

(fn Reload
  ;[1 1 1] Has the user fired at least one shot and has enough ammo to reload?
  (if (Variables|Conditions|GetbCanReload?)
    (Variables|Conditions|SetbCanFire? false)
    (Variables|Conditions|SetisFiring? false)
    (if (Variables|Conditions|GetbHasInfiniteAmmo?)
      ;[1 1 1] Update HUD
      (bind _output_get (Variables|Ammo|SetInventoryAmmo (Variables|Ammo|GetMaxAmmoLimit)))
      (Default|CallOnReloadMag _output_get)
      (bind _output_get_2 (Variables|Ammo|SetCurrentMagAmmo (Variables|Ammo|GetMagAmmoLimit)))
      (Default|CallOnConsumeAmmo _output_get_2)
      ;[1 1 1] Allow user to fire now that reload has finished
      (bind _output_get_3 (Variables|Conditions|SetbCanFire? true))
      (Variables|Conditions|SetbCanReload? (not _output_get_3))
      (else
        (bind _output_get_4 (LocalVariables|SetAmmoRemainder (- (Variables|Ammo|GetMagAmmoLimit) (Variables|Ammo|GetCurrentMagAmmo))))
        (bind _output_get_5 (Variables|Ammo|SetInventoryAmmo (- (Variables|Ammo|GetInventoryAmmo) _output_get_4)))
        (Default|CallOnReloadMag _output_get_5)
        (bind _output_get_6 (Variables|Ammo|SetCurrentMagAmmo (Variables|Ammo|GetMagAmmoLimit)))
        (Default|CallOnConsumeAmmo _output_get_6)
        (bind _output_get_7 (Variables|Conditions|SetbCanFire? true))
        (Variables|Conditions|SetbCanReload? (not _output_get_7))))
    (Default|CallOnReloadedWeapon (.AsCheeky%20Character (Utilities|Casting|CastToCheekyCharacter (Components|GetOwner))) (Variables|Ammo|GetCurrentMagAmmo) (Variables|Ammo|GetInventoryAmmo))
    (return)))

(fn ConsumeAmmo
  (params (DecrementAmount :type Integer))
  (bind _output_get (Variables|Ammo|SetCurrentMagAmmo (- (Variables|Ammo|GetCurrentMagAmmo) DecrementAmount)))
  (Default|CallOnConsumeAmmo _output_get)
  (Utilities|FlowControl|Sequence
    (:then_0
      (Variables|Conditions|SetbCanReload? (< _output_get (Variables|Ammo|GetMagAmmoLimit))))
    (:then_1
      (if (<= _output_get 0)
        (Variables|Ammo|SetCurrentMagAmmo 0)
        (Variables|Conditions|SetbCanFire? false)
        (Variables|Conditions|SetbIsOutOfAmmo? true)))))

(fn GetWeaponType
  (return (Variables|Stats|GetWeaponType)))

(fn GetWeaponData
  (return (Variables|Stats|GetWeaponData)))

(fn GetWeaponAnimationData
  (bind _weapondata (Variables|Stats|GetWeaponData))
  (bind _animationset (Utilities|Struct|BreakST_Weapon _weapondata))
  (if (Utilities|IsValidClass (.Arms_AnimBP (Utilities|Struct|BreakST_AnimationSet _animationset)))
    (return _animationset)
    (else
      (return (Variables|Default|GetAnimation%20Set)))))

(fn ResetRoundsFired
  (Variables|Default|SetRoundsFired 0))

(fn StartAutoFire
  (bind _returnvalue (Utilities|Time|SetTimerbyEvent (EventDispatchers|CreateEvent :!event Fire) (Variables|Stats|GetFireRate) true))
  (Variables|Stats|SetAutoFireHandle _returnvalue))

(fn EndAutoFire
  (bind _autofirehandle (Variables|Stats|GetAutoFireHandle))
  ;[1 1 1] Clear timer once player has let go of fire button
  (if (or (Utilities|Time|IsTimerActivebyHandle _autofirehandle) (Class|KismetSystemLibrary|TimerExistsHandle _autofirehandle))
    (Utilities|Time|ClearandInvalidateTimerbyHandle _autofirehandle)))

(fn StartFire
  (if (Variables|Stats|GetbIsAutomatic?)
    ;[1 1 1] Allow player to fire at least one shot before auto fire
    (CallFunction|Fire)
    (CallFunction|StartAutoFire)
    (else
      (CallFunction|Fire))))

(fn EndFire
  (CallFunction|ResetRoundsFired)
  (Variables|Conditions|SetisFiring? false)
  (if (Variables|Stats|GetbIsAutomatic?)
    (CallFunction|EndAutoFire)))

(fn ShotgunFire
  (bind (_startlocation _endlocation) (CallFunction|GetOwnerTraceLocations))
  (bind _returnvalue (Game|GetPlayerCharacter 0))
  (while (< (Variables|Default|GetRoundsFired) (Variables|Damage|GetShotgunPellets))
    (bind _outhit (Collision|LineTraceByChannel _startlocation _endlocation "TraceTypeQuery3" true (Variables|Default|GetIgnoredActors) (select (Variables|Conditions|GetbEnableDebugMode?) "ForDuration" "None")))
    (bind _output_get (LocalVariables|SetShotgunHit _outhit))
    (Utilities|FlowControl|Sequence
      (:then_0
        (CallFunction|HandleFireTrace _output_get)
        (bind _result (Math|Integer|IncrementInt (Variables|Default|GetRoundsFired))
          (:%20%20
            (Variables|Default|SetRoundsFired _result))))))
  (CallFunction|ReportWeaponFire (Variables|Feedback|GetFireSFX) (Transformation|GetActorLocation (Components|GetOwner)) (select (Utilities|IsValid (.PhysMat (Collision|BreakHitResult (LocalVariables|GetShotgunHit)))) (Variables|/Script/PhysicsCore.PhysicalMaterial|GetSurfaceType (.PhysMat (Collision|BreakHitResult (LocalVariables|GetShotgunHit)))) "SurfaceType_Default"))
  (if (== (Components|GetOwner) _returnvalue)
    (Class|BPIPlayer|UpdateWeaponAmmoCount(Message) _returnvalue (Variables|Ammo|GetCurrentMagAmmo))))

(fn StartReload
  (bind _audio (Variables|Default|GetAudio))
  (bind _playbackduration (Variables|Feedback|GetPlaybackDuration))
  (Audio|Components|Audio|SetSound _audio (Variables|Feedback|GetReloadSFX))
  (if (Variables|Conditions|GetbCanReload?)
    (Default|CallOnWeaponReload)
    (Audio|Components|Audio|Play _audio 0.0)
    (bind _returnvalue (Utilities|Time|SetTimerbyEvent (EventDispatchers|CreateEvent :!event Reload) (select (> _playbackduration 0.0) _playbackduration 0.25)))
    (Variables|Default|SetReloadHandle _returnvalue)))

(fn ReportWeaponFire
  (params (Sound :type Sound%20Base%20Object%20Reference) (HitLocation :type Vector) (HitSurface :type EPhysicalSurface%20Enum :default "SurfaceType_Default"))
  (bind _weaponowner (Variables|Default|GetWeaponOwner))
  ;[1 1 1] Set variables we need
  (Utilities|FlowControl|Sequence
    (:then_0
      (if (== (Variables|Default|GetWeaponOwner) (Game|GetPlayerCharacter 0))
        (Class|BPIAnimation|OnCharacterFireWeapon(Message) _weaponowner)
        (Class|BPIPlayer|UpdateWeaponAmmoCount(Message) _weaponowner (Variables|Ammo|GetCurrentMagAmmo))))
    (:then_1
      (LocalVariables|SetLocalSoundToPlay Sound)
      (LocalVariables|SetLocalHitLocation HitLocation)
      (LocalVariables|SetLocalHitSurface HitSurface)
      (LocalVariables|SetLocalOwnerLocation (Transformation|GetActorLocation (Components|GetOwner)))
      (LocalVariables|SetLocalLoudnessLevel (Utilities|Select :Index (Variables|Attachments|GetAttachmentSlot2) :NewEnumerator0 1.0 :NewEnumerator1 0.0 :NewEnumerator2 0.1 :NewEnumerator3 0.0 :NewEnumerator4 0.0 :NewEnumerator5 0.0 :NewEnumerator6 0.0))
      ;[1 1 1] Tell Player UI to Update
      (Default|CallOnWeaponFire)
      ;[1 1 1] Play Visual and Audio feedback
      (Audio|PlaySoundatLocation (LocalVariables|GetLocalSoundToPlay) (LocalVariables|GetLocalOwnerLocation) "0, 0, 0" 1.0 1.0 0.0 0 0 0)
      (Class|AISenseHearing|ReportNoiseEvent (LocalVariables|GetLocalOwnerLocation) (LocalVariables|GetLocalLoudnessLevel) (Components|GetOwner) 0.0 "Weapon")
      (Utilities|FlowControl|Sequence
        (:then_0
          (CallFunction|HandleBulletVFX (LocalVariables|GetLocalHitSurface) (LocalVariables|GetLocalHitLocation)))
        (:then_1
          (if (Variables|Conditions|GetbEnableDebugMode?)
            (Development|PrintString (Utilities|String|EnumtoString (LocalVariables|GetLocalHitSurface)))))))))

(fn GetOwnerTraceLocations
  (bind _weaponowner (Variables|Default|GetWeaponOwner))
  (bind _bisplayerweapon_ (Variables|Conditions|GetbIsPlayerWeapon?))
  (bind (_outlocation _outrotation) (Actor|GetActorEyesViewPoint _weaponowner))
  (bind _returnvalue (Actor|GetComponentbyClass _weaponowner "/Script/Engine.CameraComponent"))
  (bind _returnvalue_2 (Transformation|GetWorldTransform _returnvalue))
  (bind _returnvalue_3 (Math|Vector|GetForwardVector (.rotation _returnvalue_2)))
  (return (select _bisplayerweapon_ (.location _returnvalue_2) _outlocation) (select (and (Utilities|Enum|Equal(Enum) (Variables|Stats|GetWeaponType) "NewEnumerator2") _bisplayerweapon_) (+ (.location _returnvalue_2) (* (Math|Random|RandomUnitVectorinConeinDegrees _returnvalue_3 12.0) (Variables|Damage|GetWeaponRange))) (select _bisplayerweapon_ (+ (.location _returnvalue_2) (* _returnvalue_3 (Variables|Damage|GetWeaponRange))) (+ _outlocation (* (Math|Random|RandomUnitVectorinConeinDegrees (Math|Vector|GetForwardVector _outrotation) (Utilities|Select :Index (CallFunction|GetWeaponType) :NewEnumerator0 3.0 :NewEnumerator1 6.0 :NewEnumerator2 6.0 :NewEnumerator3 3.0 :NewEnumerator4 15.0)) (Variables|Damage|GetWeaponRange)))))))

(fn HandleFireTrace
  (params (Hit :type Hit%20Result%20Structure%20%28by%20ref%29))
  ;[1 1 1] Set the commonly used values at the start to make it easier to track/read
  (LocalVariables|SetInstigatorController (Game|GetInstigatorController))
  (bind _output_get (LocalVariables|SetLocalOwner (Components|GetOwner)))
  (LocalVariables|SetOwnerTeamID (Default|GetOwnerTeamID (Actor|GetComponentbyClass _output_get "/Game/CheekyFPS/Blueprints/Components/IdentificationComponent.IdentificationComponent_C")))
  (bind _output_get_2 (LocalVariables|SetLocalHitResult Hit))
  (LocalVariables|SetHitComp (.HitComponent (Collision|BreakHitResult _output_get_2)))
  (LocalVariables|SetbWasHitBlocked? (.bBlockingHit (Collision|BreakHitResult _output_get_2)))
  (LocalVariables|SetHitLocation (.Location (Collision|BreakHitResult _output_get_2)))
  (LocalVariables|SetHitImpactPoint (.ImpactPoint (Collision|BreakHitResult _output_get_2)))
  (LocalVariables|SetHitBoneName (.HitBoneName (Collision|BreakHitResult _output_get_2)))
  (LocalVariables|SetHitSurfaceType (Variables|/Script/PhysicsCore.PhysicalMaterial|GetSurfaceType (select (Utilities|IsValid (.PhysMat (Collision|BreakHitResult _output_get_2))) (.PhysMat (Collision|BreakHitResult _output_get_2)) "/Game/CheekyFPS/Data/PhysicalMaterials/PM_Concrete.PM_Concrete")))
  (bind _output_get_3 (LocalVariables|SetHitActor (.HitActor (Collision|BreakHitResult _output_get_2))))
  (Utilities|IsValid _output_get_3
    (:Is%20Valid
      (Utilities|FlowControl|Sequence
        (:then_0
          (Utilities|IsValid (Actor|GetComponentbyClass _output_get_3 "/Game/CheekyFPS/Blueprints/Components/IdentificationComponent.IdentificationComponent_C")
            (:Is%20Valid
              (if (!= (Default|GetOwnerTeamID (Actor|GetComponentbyClass _output_get_3 "/Game/CheekyFPS/Blueprints/Components/IdentificationComponent.IdentificationComponent_C")) 0)
                (LocalVariables|SetTargetTeamID (Default|GetOwnerTeamID (Actor|GetComponentbyClass _output_get_3 "/Game/CheekyFPS/Blueprints/Components/IdentificationComponent.IdentificationComponent_C")))
                (LocalVariables|SetCanBeDamaged? (Utilities|IsValid (Actor|GetComponentbyClass (LocalVariables|GetHitActor) "/Game/CheekyFPS/Blueprints/Health/CheekyHealthComponent.CheekyHealthComponent_C")))
                (else
                  (LocalVariables|SetTargetTeamID 0)
                  (Utilities|FlowControl|Sequence :!label _label
                    (:then_0
                      ;[1 1 1] Check that the line trace doesn't hit us, and that our target is valid
                      (if (LocalVariables|GetbWasHitBlocked?)
                        (if (Math|Boolean|ANDBoolean (!= (LocalVariables|GetHitActor) (LocalVariables|GetLocalOwner)) (Utilities|IsValid (LocalVariables|GetHitActor)) (!= (LocalVariables|GetOwnerTeamID) (LocalVariables|GetTargetTeamID)))
                          (if (Math|Boolean|ORBoolean (Utilities|Name|Equal(Name) (LocalVariables|GetHitBoneName) "head") (Utilities|Name|Equal(Name) (LocalVariables|GetHitBoneName) "pelvis") (or (Components|ComponentHasTag (LocalVariables|GetHitComp) "head") (Components|ComponentHasTag (LocalVariables|GetHitComp) "pelvis")))
                            ;[1 1 1] Apply crit damage as necessary
                            (bind _returnvalue (Game|Damage|ApplyPointDamage (LocalVariables|GetHitActor) (* (CallFunction|GetWeaponDamage) 1e+01) (LocalVariables|GetHitImpactPoint) (LocalVariables|GetLocalHitResult) (LocalVariables|GetInstigatorController) self (Variables|Damage|GetCurrentDamageTypeClass)))
                            (bind _output_get_4 (LocalVariables|SetActualDamage _returnvalue))
                            (Class|AISenseDamage|ReportDamageEvent (LocalVariables|GetHitActor) (LocalVariables|GetInstigatorController) _output_get_4 (LocalVariables|GetHitLocation) (LocalVariables|GetHitImpactPoint))
                            (if (and (== (Components|GetOwner) (Game|GetPlayerCharacter 0)) (LocalVariables|GetCanBeDamaged?))
                              (Class|BPIPlayer|RegisterPlayerCritHit(Message) (Game|GetPlayerController 0))
                              (Development|PrintString "Crit!" true true "(R=1.000000,G=0.116864,B=0.000000,A=1.000000)")
                              (if (Variables|Conditions|GetbEnableDebugMode?) :!label _label_2
                                (Development|PrintString (Utilities|String|ToString(Name) (LocalVariables|GetHitBoneName)) true true "(R=1.000000,G=0.116864,B=0.000000,A=1.000000)")))
                            (else
                              (bind _returnvalue_2 (Game|Damage|ApplyPointDamage (LocalVariables|GetHitActor) (CallFunction|GetWeaponDamage) (LocalVariables|GetHitImpactPoint) (LocalVariables|GetLocalHitResult) (LocalVariables|GetInstigatorController) (LocalVariables|GetLocalOwner) (Variables|Damage|GetCurrentDamageTypeClass)))
                              (Class|AISenseDamage|ReportDamageEvent (LocalVariables|GetHitActor) (LocalVariables|GetInstigatorController) _returnvalue_2 (LocalVariables|GetHitLocation) (LocalVariables|GetHitImpactPoint))
                              ;[1 1 1] Update player UI Crosshair
                              (if (and (== (Components|GetOwner) (Game|GetPlayerCharacter 0)) (LocalVariables|GetCanBeDamaged?))
                                (Class|BPIPlayer|RegisterPlayerHit(Message) (Game|GetPlayerController 0))
                                (goto _label_2)))))))
                    (:then_1
                      ;[1 1 1] We don't want the shotgun to play sounds multiple times
                      (if (Utilities|Enum|NotEqual(Enum) (Variables|Stats|GetWeaponType) "NewEnumerator2")
                        ;[1 1 1] Provide feedback for player
                        (CallFunction|ReportWeaponFire (Variables|Feedback|GetFireSFX) (LocalVariables|GetHitImpactPoint) (LocalVariables|GetHitSurfaceType))))
                    (:then_2
                      (return))))))
            (:Is%20Not%20Valid
              (CallFunction|ReportWeaponFire (Variables|Feedback|GetFireSFX) (LocalVariables|GetHitImpactPoint) (LocalVariables|GetHitSurfaceType) :!label _label_3)
              (return))))
        (:then_1
          (goto _label))))
    (:Is%20Not%20Valid
      (goto _label_3))))

(fn HandleBulletVFX
  (params (HitSurface :type EPhysicalSurface%20Enum :default "SurfaceType_Default") (HitLocation :type Vector))
  (LocalVariables|SetLocalHitLocation HitLocation)
  (LocalVariables|SetLocalHitSurface HitSurface)
  (Rendering|Decal|SpawnDecalatLocation (Utilities|Select :Index HitSurface :SurfaceType_Default (Variables|Default|GetDefault) :SurfaceType1 "/Game/CheekyFPS/External/Weapons/UWC_Bullet_Holes/Instances/Decals/Concrete/MI_Concrete_4.MI_Concrete_4" :SurfaceType2 "/Game/CheekyFPS/External/Weapons/UWC_Bullet_Holes/Instances/Decals/Metal_Solid/MI_Metal_Solid_2.MI_Metal_Solid_2" :SurfaceType3 0 :SurfaceType4 0 :SurfaceType5 0 :SurfaceType6 0 :SurfaceType7 0 :SurfaceType8 "/Game/CheekyFPS/External/Weapons/UWC_Bullet_Holes/Instances/Decals/Flesh/MI_Flesh_3.MI_Flesh_3") "1.000000,1.000000,1.000000" (LocalVariables|GetLocalHitLocation) "0.000000,0.000000,0.000000" 1e+01)
  (switch Utilities|FlowControl|Switch|SwitchonEPhysicalSurface (LocalVariables|GetLocalHitSurface)
    (:SurfaceType_Default
      (Effects|SpawnEmitteratLocation (select (Variables|Conditions|GetbIsLethal?) "/Game/CheekyFPS/External/Weapons/SciFiWeapLight/FX/Particles/P_Impact_Metal_Medium_Dark.P_Impact_Metal_Medium_Dark" "/Game/CheekyFPS/External/Weapons/SciFiWeapLight/FX/Particles/P_Impact_Metal_Medium_Light.P_Impact_Metal_Medium_Light") (LocalVariables|GetLocalHitLocation))
      (Audio|PlaySoundatLocation (Variables|Feedback|GetHitSurfaceSFX) (LocalVariables|GetLocalHitLocation) "0, 0, 0" 1.0 1.0 0.0 0 0 0))
    (:SurfaceType7
      (Effects|SpawnEmitteratLocation (select (Variables|Conditions|GetbIsLethal?) "/Game/CheekyFPS/External/Weapons/SciFiWeapLight/FX/Particles/P_Impact_Stone_Medium_Dark.P_Impact_Stone_Medium_Dark" "/Game/CheekyFPS/External/Weapons/SciFiWeapLight/FX/Particles/P_Impact_Stone_Medium_Light.P_Impact_Stone_Medium_Light") "0, 0, 0"))
    (:SurfaceType8
      (Audio|PlaySoundatLocation (Variables|Feedback|GetHitBodySFX) (LocalVariables|GetLocalHitLocation) "0, 0, 0" 1.0 1.0 0.0 0 0 0)
      (Effects|SpawnEmitteratLocation (select (Variables|Conditions|GetbIsLethal?) "/Game/CheekyFPS/External/Weapons/SciFiWeapLight/FX/Particles/P_Impact_Metal_Large_Dark.P_Impact_Metal_Large_Dark" "/Game/CheekyFPS/External/Weapons/SciFiWeapLight/FX/Particles/P_Impact_Metal_Large_Light.P_Impact_Metal_Large_Light") (LocalVariables|GetLocalHitLocation)))))

(fn CheckforIgnoredActors
  (if (Variables|Conditions|GetbIsPlayerWeapon?)
    (bind _outactors (Actor|GetAllActorswithTag "IGTrace"))
    (for _array_element _outactors
      (Utilities|Array|AddUnique (Variables|Default|GetIgnoredActors) _array_element))
    (Development|PrintString "Updated Ignore actor array!")))

(fn UpdateOwner
  (bind _ignoredactors (Variables|Default|GetIgnoredActors))
  ;[1 1 1] For whatever reason the BP will reset all of it's values if adjusted in editor
  (if (Variables|Conditions|GetbIsPlayerWeapon?)
    (bind _output_get (Variables|Default|SetWeaponOwner (Game|GetPlayerCharacter 0)))
    (Actor|SetOwner _output_get)
    (if (not (Utilities|Array|ContainsItem _ignoredactors _output_get))
      (Utilities|Array|Clear _ignoredactors)
      (Utilities|Array|AddUnique _ignoredactors _output_get))))

(fn GetCurrentAmmo
  (return (Variables|Ammo|GetCurrentMagAmmo)))

(fn GetMaxAmmo
  (if (not (or (not (Variables|Conditions|GetbConsumesAmmo?)) (Variables|Conditions|GetbHasInfiniteAmmo?)))
    (return (Variables|Ammo|GetMaxAmmoLimit))))

(fn GetWeaponDamage
  (bind _weapondamage (Variables|Damage|GetWeaponDamage))
  (bind _weapondamage_2 (Variables|Damage|GetWeaponDamage))
  (bind _returnvalue (* _weapondamage_2 1.0))
  (bind _returnvalue_2 (Class|BPISaveLoad|GetCurrentGameDifficulty(Message) (Game|GetGameInstance)))
  (LocalVariables|SetLocalGameDifficulty _returnvalue_2)
  (if (Variables|Conditions|GetbIsPlayerWeapon?)
    (return (Utilities|Select :Index (LocalVariables|GetLocalGameDifficulty) :Beginner (* _weapondamage_2 2.0) :Easy (* _weapondamage_2 1.5) :Medium _returnvalue :Hard _returnvalue :VeryHard (* _weapondamage_2 0.5) :Extreme (* _weapondamage_2 0.25)))
    (else
      (return (Utilities|Select :Index (LocalVariables|GetLocalGameDifficulty) :Beginner (* _weapondamage 0.25) :Easy (* _weapondamage 0.5) :Medium (* _weapondamage 1.0) :Hard (* _weapondamage 1.5) :VeryHard (* _weapondamage 1.75) :Extreme (* _weapondamage 2.0))))))