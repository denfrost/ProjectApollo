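; Smoke grenade projectile actor that releases an area smoke effect when it detonates.
; On BeginPlay it binds to the OnGrenadeDetonated event to spawn a BP_GrenadeFX_AOE_Smoke actor at its location, leaving the smoke to that actor.
; The affected-characters list is unused, and an unconnected branch that spawned NS_GrenadeSmoke directly with a colour parameter never runs.
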(event Custom|SpawnSmokeEffect
  (params (AffectedCharacters :type Array%20of%20Character%20Object%20References))
  (Game|SpawnActorfromClass "/Game/CheekyFPS/Blueprints/VisualFX/BP_GrenadeFX_AOE_Smoke.BP_GrenadeFX_AOE_Smoke_C" (Math|Transform|MakeTransform (Transformation|GetActorLocation) "0, 0, 0" "1,1,1") "Undefined" 0 0))

(event EventBeginPlay
  (|CallParentFunction)
  (EventDispatchers|BindEventtoOnGrenadeDetonated (EventDispatchers|CreateEvent :!event Custom|SpawnSmokeEffect)))

(event Collision|EventActorBeginOverlap
  (params (OtherActor :type Actor%20Object%20Reference)))

(event EventTick
  (params (DeltaSeconds :type Float%20%28single-precision%29))
  (|CallParentFunction DeltaSeconds) ; This node is disabled and will not be called.\nDrag off pins to build functionality.
)

(fn ConstructionScript
  (|CallParentFunction))