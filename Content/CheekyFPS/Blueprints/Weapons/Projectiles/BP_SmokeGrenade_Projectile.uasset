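; Smoke grenade projectile that spawns a smoke effect and interferes with AI sight.
; ApplyExplosionEffect spawns a tripled-scale smoke emitter at the grenade's transform, while its Explode event is empty.
; Sphere overlap finds the actor's AI sight config and attempts to shrink its sight range.
; Only when that call fails does it send the controller a sight-reset message after a short delay.
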(event OnComponentBeginOverlap(Sphere)
  (params (OverlappedComponent :type Primitive%20Component%20Object%20Reference) (OtherActor :type Actor%20Object%20Reference) (OtherComp :type Primitive%20Component%20Object%20Reference) (OtherBodyIndex :type Integer) (bFromSweep :type Boolean) (SweepResult :type Hit%20Result%20Structure%20%28by%20ref%29))
  (bind _returnvalue (AI|GetAIController OtherActor))
  (Utilities|IsValid (Class|ApolloAIBlueprintLibrary|GetPerceptionSenseConfig _returnvalue "/Script/AIModule.AISense_Sight")
    (:Is%20Valid
      (bind _returnvalue_2 (Class|ApolloAIBlueprintLibrary|SetSightRange _returnvalue 5e+01))
      (if _returnvalue_2
        (Development|PrintString "Modified Sight Range!")
        (else
          (Utilities|FlowControl|Delay 2.0)
          (Class|BPIEnemy|OnResetSight(Message) _returnvalue))))))

(event EventBeginPlay
  (|CallParentFunction) ; This node is disabled and will not be called.\nDrag off pins to build functionality.
)

(event Collision|EventActorBeginOverlap
  (params (OtherActor :type Actor%20Object%20Reference))
  (|CallParentFunction OtherActor) ; This node is disabled and will not be called.\nDrag off pins to build functionality.
)

(event EventTick
  (params (DeltaSeconds :type Float%20%28single-precision%29))
  (|CallParentFunction DeltaSeconds) ; This node is disabled and will not be called.\nDrag off pins to build functionality.
)

(event EventExplode)

(event EventApplyExplosionEffect
  (Effects|SpawnEmitteratLocation "/Game/CheekyFPS/External/StarterContent/Particles/P_Smoke.P_Smoke" (Transformation|GetActorLocation) (Transformation|GetActorRotation) "3.000000,3.000000,3.000000"))

(fn ConstructionScript
  (|CallParentFunction))