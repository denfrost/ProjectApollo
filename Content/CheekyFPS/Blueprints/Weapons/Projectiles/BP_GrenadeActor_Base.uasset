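; Base Blueprint for thrown grenade actors, adding sound and decal feedback to the grenade's cook, throw and detonation.
; On BeginPlay it binds handlers to those three grenade events, which play sounds at the grenade, or at its owner for the throw.
; It also waits until half a second before the fuze time elapses, then sets a blink parameter on a dynamic decal material.
; Nodes for decal blink frequency and radius are unconnected.
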(event EventBeginPlay
  (Utilities|FlowControl|Sequence
    (:then_0
      (Utilities|FlowControl|Delay (- (Class|GrenadeActor|GetFuzeTime) 0.5))
      (bind _returnvalue (Rendering|Material|CreateDynamicMaterialInstance (Variables|Default|Getm_DecalComponent) :!class /Script/Engine.DecalComponent))
      (Rendering|Material|SetScalarParameterValue _returnvalue "blink" 1.0 :!class /Script/Engine.MaterialInstanceDynamic))
    (:then_1
      (EventDispatchers|BindEventtoOnGrenadeDetonated (EventDispatchers|CreateEvent :!event Explode))
      (EventDispatchers|BindEventtoOnGrenadeCook (EventDispatchers|CreateEvent :!event OnCookGrenade))
      (EventDispatchers|BindEventtoOnGrenadeThrown (EventDispatchers|CreateEvent :!event OnThrowGrenade)))))

(event EventTick
  (params (DeltaSeconds :type Float%20%28single-precision%29)))

(fn ConstructionScript)

(fn Explode
  (params (AffectedCharacters :type Array%20of%20Character%20Object%20References))
  (Audio|PlaySoundatLocation (Variables|Default|GetExplodeSFX) (Transformation|GetActorLocation) "0, 0, 0" 1.0 1.0 0.0 0 0 0)
  (return))

(fn OnCookGrenade
  (Audio|PlaySoundatLocation (Variables|Default|GetCookSFX) (Transformation|GetActorLocation) "0, 0, 0" 1.0 1.0 0.0 0 0 0))

(fn OnThrowGrenade
  (Audio|PlaySoundatLocation (Variables|Default|GetThrowSFX) (Transformation|GetActorLocation (Components|GetOwner)) "0, 0, 0" 1.0 1.0 0.0 0 0 0))