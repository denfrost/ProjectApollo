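; Grenade projectile Blueprint that deals radial damage and plays explosion effects.
; Explode applies falloff damage at ExplosionOrigin, then sets a short lifespan; nothing in this file calls it.
; ExplosionOrigin is cached at BeginPlay, so damage centers on the starting location rather than the current one.
; EndPlay triggers the explosion particle and sound at the actor's current transform, however the actor ends.
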(event EventBeginPlay
  (|CallParentFunction)
  (Variables|Default|SetExplosionOrigin (Transformation|GetActorLocation)))

(event Collision|EventActorBeginOverlap
  (params (OtherActor :type Actor%20Object%20Reference))
  (|CallParentFunction OtherActor) ; This node is disabled and will not be called.\nDrag off pins to build functionality.
)

(event EventTick
  (params (DeltaSeconds :type Float%20%28single-precision%29))
  (|CallParentFunction DeltaSeconds) ; This node is disabled and will not be called.\nDrag off pins to build functionality.
)

(event EventExplode
  (Class|GameplayStatics|ApplyRadialDamagewithFalloff (Variables|Default|GetBase%20Damage) (Variables|Default|GetMinimum%20Damage) (Variables|Default|GetExplosionOrigin) (Variables|Default|GetDamage%20Inner%20Radius) (Variables|Default|GetDamage%20Outer%20Radius) (Variables|Default|GetDamage%20Falloff) 0 0 0 0 "ECC_Visibility")
  (Actor|SetLifeSpan 0.2))

(event EventApplyExplosionEffect
  (bind _returnvalue (Transformation|GetActorLocation))
  (Effects|SpawnEmitteratLocation (Variables|Default|GetExplosionVFX) _returnvalue (Transformation|GetActorRotation))
  (Audio|PlaySoundatLocation (Variables|Default|GetExplosionSFX) _returnvalue "0, 0, 0" 1.0 1.0 0.0 0 0 0))

(event EventEndPlay
  (params (EndPlayReason :type EEndPlayReason%20Enum :default "Destroyed"))
  (CallFunction|ApplyExplosionEffect))

(fn ConstructionScript
  (|CallParentFunction))