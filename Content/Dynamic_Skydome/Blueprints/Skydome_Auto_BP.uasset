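; Skydome actor that drives sky, lighting, fog and atmosphere, with an optional day-night cycle that pitches the directional light on Tick.
; RefreshSkydome runs on construction and each cycle tick, mapping actor pitch to SunHeight to sample color curves for sun, sky and fog.
; It creates a new dynamic material instance each call for sun, clouds, stars, moon and aurora, optionally recapturing the skylight.
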(event EventTick
  (params (DeltaSeconds :type Float%20%28single-precision%29))
  (if (Variables|Sun|GetEnable%20Day-Night-Cycle)
    (Transformation|AddLocalRotation (Variables|Default|GetDirectionalLight) (Math|Rotator|MakeRotator 0.0 (* (/ (* DeltaSeconds 3.6e+02) (Variables|Sun|GetDay-Night-Cycle%20Length)) (Math|Conversions|ToFloat(Integer) (Variables|Sun|GetDay-Night-Cycle%20Factor))) 0.0) false false)
    (CallFunction|RefreshSkydome)))

(fn ConstructionScript
  (CallFunction|RefreshSkydome))

(fn RefreshSkydome
  (bind _returnvalue (Transformation|GetActorRotation))
  (bind _directionallight (Variables|Default|GetDirectionalLight))
  (bind _skylight (Variables|Default|GetSkyLight))
  (bind _skyatmosphere (Variables|Default|GetSkyAtmosphere))
  (bind _directionallight_2 (Variables|Default|GetDirectionalLight))
  (bind _moon_direction (Variables|Moon|GetMoon%20Direction))
  (bind _exponentialheightfog (Variables|Default|GetExponentialHeightFog))
  (bind (_x _y) (Math|Vector2D|BreakVector2D _moon_direction))
  (Utilities|FlowControl|Sequence
    (:then_0
      ;[1 1 1] Material Instance and BP Rotation
      (Transformation|SetWorldRotation (Variables|Components|GetStaticMeshComponent0) "0, 0, 0" false false)
      (Variables|Sun|SetSun%20Inclination (.Roll (Math|Rotator|BreakRotator (Transformation|GetActorRotation))))
      (bind _returnvalue_2 (Rendering|Material|CreateDynamicMaterialInstance (Variables|Components|GetStaticMeshComponent0) 0 "/Game/Dynamic_Skydome/Materials/Skydome_inst.Skydome_inst" "None" :!class /Script/Engine.PrimitiveComponent)))
    (:then_1
      ;[1 1 1] Sun
      (Rendering|Material|SetVectorParameterValue _returnvalue_2 "Sun Direction" (Math|Conversions|ToLinearColor(Vector) (Math|Rotator|GetRotationXVector _returnvalue)) :!class /Script/Engine.MaterialInstanceDynamic)
      (bind _output_get (Variables|Sun|SetSun%20Height (Math|Float|MapRangeUnclamped (.Pitch (Math|Rotator|BreakRotator _returnvalue)) 0.0 -9e+01 0.0 1.0)))
      (Rendering|Material|SetVectorParameterValue _returnvalue_2 "Sun Color" (* (Rendering|Components|Light|GetLightColor (Variables|Default|GetDirectionalLight)) (Math|Curves|GetLinearColorValue (Variables|Sun|GetSun%20Curve) _output_get)) :!class /Script/Engine.MaterialInstanceDynamic)
      (Rendering|Material|SetScalarParameterValue _returnvalue_2 "Sun Brightness" (Variables|Sun|GetSun%20Brightness) :!class /Script/Engine.MaterialInstanceDynamic)
      (Rendering|Material|SetScalarParameterValue _returnvalue_2 "Sun Hardness" (Variables|Sun|GetSun%20Hardness) :!class /Script/Engine.MaterialInstanceDynamic)
      (Rendering|Material|SetScalarParameterValue _returnvalue_2 "Sun Radius" (Variables|Sun|GetSun%20Radius) :!class /Script/Engine.MaterialInstanceDynamic)
      (Rendering|Material|SetScalarParameterValue _returnvalue_2 "Use Sun" (Math|Conversions|ToFloat(Boolean) (Variables|Sun|GetEnable%20Sun)) :!class /Script/Engine.MaterialInstanceDynamic)
      (Rendering|Material|SetVectorParameterValue _returnvalue_2 "Sun Tint" (Math|Conversions|ToLinearColor(Color) (Variables|Sun|GetSun%20Tint)) :!class /Script/Engine.MaterialInstanceDynamic)
      (if (Variables|Sun|GetEnable%20Sun)
        (Rendering|Components|Light|SetLightColor _directionallight (Math|Curves|GetLinearColorValue (Variables|Sun|GetSun%20Curve) (Variables|Sun|GetSun%20Height)) false)
        (Rendering|Components|Light|SetIntensity _directionallight (* (Variables|Sun|GetSun%20Light%20Intensity) (.R (Math|Color|BreakColor (Math|Curves|GetLinearColorValue (Variables|Stars|GetNight%20Color%20Ramp) (Variables|Sun|GetSun%20Height))))))
        (else
          (Rendering|Components|Light|SetIntensity _directionallight 0.0)))
      (Rendering|Components|Light|SetIntensity _skylight (Variables|Sun|GetSky%20Light%20Intensity))
      (Rendering|Components|Light|SetLightColor _skylight (Math|Color|Lerp(LinearColor) (Math|Curves|GetLinearColorValue (Variables|Atmosphere|GetZenith%20Color%20Ramp) (Variables|Sun|GetSun%20Height)) (Math|Conversions|ToLinearColor(Color) (Variables|Sun|GetSky%20Light%20Color%20Tint)) (Variables|Sun|GetSky%20Light%20Color%20Override)))
      (Class|DirectionalLightComponent|SetDynamicShadowCascades _directionallight_2 (Variables|Sun|GetShadow%20Cascades))
      (Class|DirectionalLightComponent|SetDynamicShadowDistanceMovableLight _directionallight_2 (Variables|Sun|GetShadow%20Distance))
      (Class|LightComponent|SetBloomScale _directionallight_2 (Variables|Sun|GetSun%20Shafts))
      (if (Variables|Sun|GetAuto%20Update%20Skylight)
        (Class|SkyLightComponent|RecaptureSky _skylight)))
    (:then_2
      ;[1 1 1] Clouds
      (Rendering|Material|SetVectorParameterValue _returnvalue_2 "Horizon Cloud Color" (Math|Curves|GetLinearColorValue (Variables|Clouds|GetCloud%20Color%20Ramp) (Variables|Sun|GetSun%20Height)) :!class /Script/Engine.MaterialInstanceDynamic)
      (Rendering|Material|SetVectorParameterValue _returnvalue_2 "High Cloud Color" (Math|Curves|GetLinearColorValue (Variables|Clouds|GetCloud%20Color%20Ramp) (Variables|Sun|GetSun%20Height)) :!class /Script/Engine.MaterialInstanceDynamic)
      (Rendering|Material|SetScalarParameterValue _returnvalue_2 "Cloud Distortion" (Variables|Clouds|GetCloud%20Distortion) :!class /Script/Engine.MaterialInstanceDynamic)
      (Rendering|Material|SetScalarParameterValue _returnvalue_2 "High Cloud Brightness" (Variables|Clouds|GetHigh%20Clouds%20Brightness) :!class /Script/Engine.MaterialInstanceDynamic)
      (Rendering|Material|SetScalarParameterValue _returnvalue_2 "High Cloud Density" (Variables|Clouds|GetHigh%20Clouds%20Density) :!class /Script/Engine.MaterialInstanceDynamic)
      (Rendering|Material|SetScalarParameterValue _returnvalue_2 "Horizon Cloud Brightness" (Variables|Clouds|GetHorizon%20Clouds%20Brightness) :!class /Script/Engine.MaterialInstanceDynamic)
      (Rendering|Material|SetScalarParameterValue _returnvalue_2 "Horizon Cloud Density" (Variables|Clouds|GetHorizon%20Clouds%20Density) :!class /Script/Engine.MaterialInstanceDynamic)
      (Rendering|Material|SetScalarParameterValue _returnvalue_2 "Wind Speed" (Variables|Clouds|GetWind%20Speed) :!class /Script/Engine.MaterialInstanceDynamic)
      (Rendering|Material|SetScalarParameterValue _returnvalue_2 "Cloud Saturation" (Variables|Clouds|GetCloud%20Saturation) :!class /Script/Engine.MaterialInstanceDynamic)
      (Rendering|Material|SetScalarParameterValue _returnvalue_2 "Cloud Coverage" (Variables|Clouds|GetCloud%20Coverage) :!class /Script/Engine.MaterialInstanceDynamic)
      (Rendering|Material|SetScalarParameterValue _returnvalue_2 "Background Speed" (Variables|Clouds|GetBackground%20Rotation%20Speed) :!class /Script/Engine.MaterialInstanceDynamic)
      (Rendering|Material|SetScalarParameterValue _returnvalue_2 "Background Coverage" (Variables|Clouds|GetBackground%20Coverage) :!class /Script/Engine.MaterialInstanceDynamic)
      (Rendering|Material|SetScalarParameterValue _returnvalue_2 "Night Background Intensity" (Variables|Clouds|GetBackground%20Night%20Intensity) :!class /Script/Engine.MaterialInstanceDynamic)
      (Rendering|Material|SetScalarParameterValue _returnvalue_2 "Background Intensity" (Variables|Clouds|GetBackground%20Intensity) :!class /Script/Engine.MaterialInstanceDynamic)
      (Rendering|Material|SetTextureParameterValue _returnvalue_2 "Background" (Variables|Clouds|GetBackground)))
    (:then_3
      ;[1 1 1] Atmosphere
      (Class|SkyAtmosphereComponent|SetRayleighScatteringScale _skyatmosphere (Variables|Atmosphere|GetRayleigh%20Scattering))
      (Class|SkyAtmosphereComponent|SetMieScatteringScale _skyatmosphere (Variables|Atmosphere|GetMie%20Scattering))
      (Class|SkyAtmosphereComponent|SetMieAbsorptionScale _skyatmosphere (Variables|Atmosphere|GetMie%20Absorbtion))
      (Class|SkyAtmosphereComponent|SetOtherAbsorptionScale _skyatmosphere (Variables|Atmosphere|GetAtmosphere%20Absorbtion))
      (Class|ExponentialHeightFogComponent|SetVolumetricFog _exponentialheightfog (Variables|Atmosphere|GetVolumetric%20Fog))
      (Class|ExponentialHeightFogComponent|SetVolumetricFogDistance _exponentialheightfog (Variables|Atmosphere|GetVolumetric%20Fog%20Distance))
      (Class|ExponentialHeightFogComponent|SetVolumetricFogExtinctionScale _exponentialheightfog (Variables|Atmosphere|GetVolumetric%20Fog%20Extinction))
      (Class|ExponentialHeightFogComponent|SetFogDensity _exponentialheightfog (Variables|Atmosphere|GetFog%20Intensity))
      (Class|ExponentialHeightFogComponent|SetFogInscatteringColor _exponentialheightfog (Class|KismetMathLibrary|HSVtoRGBVector (Math|Conversions|ToLinearColor(Vector) (Math|Vector|MakeVector (.X (Math|Vector|BreakVector (Math|Conversions|ToVector(LinearColor) (Class|KismetMathLibrary|RGBtoHSVVector (Math|Curves|GetLinearColorValue (Variables|Atmosphere|GetHorizon%20Color%20Ramp) (Variables|Sun|GetSun%20Height)))))) (* (.Y (Math|Vector|BreakVector (Math|Conversions|ToVector(LinearColor) (Class|KismetMathLibrary|RGBtoHSVVector (Math|Curves|GetLinearColorValue (Variables|Atmosphere|GetHorizon%20Color%20Ramp) (Variables|Sun|GetSun%20Height)))))) (Variables|Atmosphere|GetFog%20Saturation)) (* (Variables|Atmosphere|GetFog%20Brightness) (.Z (Math|Vector|BreakVector (Math|Conversions|ToVector(LinearColor) (Class|KismetMathLibrary|RGBtoHSVVector (Math|Curves|GetLinearColorValue (Variables|Atmosphere|GetHorizon%20Color%20Ramp) (Variables|Sun|GetSun%20Height)))))))))))
      (Class|ExponentialHeightFogComponent|SetFogHeightFalloff _exponentialheightfog (Variables|Atmosphere|GetFog%20Falloff))
      (Rendering|Material|SetVectorParameterValue _returnvalue_2 "Zenith Color" (Math|Curves|GetLinearColorValue (Variables|Atmosphere|GetZenith%20Color%20Ramp) (Variables|Sun|GetSun%20Height)) :!class /Script/Engine.MaterialInstanceDynamic)
      (Rendering|Material|SetVectorParameterValue _returnvalue_2 "Horizon Color" (Math|Curves|GetLinearColorValue (Variables|Atmosphere|GetHorizon%20Color%20Ramp) (Variables|Sun|GetSun%20Height)) :!class /Script/Engine.MaterialInstanceDynamic)
      (Rendering|Material|SetVectorParameterValue _returnvalue_2 "Ground Color" (Math|Conversions|ToLinearColor(Color) (Variables|Atmosphere|GetGround%20Color)) :!class /Script/Engine.MaterialInstanceDynamic)
      (Rendering|Material|SetVectorParameterValue _returnvalue_2 "Overall Color" (Math|Conversions|ToLinearColor(Color) (Variables|Atmosphere|GetOverall%20Color)) :!class /Script/Engine.MaterialInstanceDynamic)
      (Rendering|Material|SetScalarParameterValue _returnvalue_2 "Ground Alpha" (Variables|Atmosphere|GetGround%20Alpha) :!class /Script/Engine.MaterialInstanceDynamic)
      (Rendering|Material|SetScalarParameterValue _returnvalue_2 "Ground Falloff" (Variables|Atmosphere|GetGround%20Falloff) :!class /Script/Engine.MaterialInstanceDynamic)
      (Rendering|Material|SetScalarParameterValue _returnvalue_2 "Ground Level" (Variables|Atmosphere|GetGround%20Level) :!class /Script/Engine.MaterialInstanceDynamic)
      (Rendering|Material|SetScalarParameterValue _returnvalue_2 "Horizon Falloff" (Variables|Atmosphere|GetHorizon%20Falloff) :!class /Script/Engine.MaterialInstanceDynamic)
      (Rendering|Material|SetScalarParameterValue _returnvalue_2 "Overall Contrast" (Variables|Atmosphere|GetOverall%20Contrast) :!class /Script/Engine.MaterialInstanceDynamic)
      (Rendering|Material|SetScalarParameterValue _returnvalue_2 "Overall Saturation" (Variables|Atmosphere|GetOverall%20Saturation) :!class /Script/Engine.MaterialInstanceDynamic)
      (Rendering|Material|SetScalarParameterValue _returnvalue_2 "Horizon Falloff Contrast" (Variables|Atmosphere|GetHorizon%20Falloff%20Contrast) :!class /Script/Engine.MaterialInstanceDynamic))
    (:then_4
      ;[1 1 1] Stars
      (Rendering|Material|SetVectorParameterValue _returnvalue_2 "Stars Color" (Math|Curves|GetLinearColorValue (Variables|Stars|GetStars%20Color%20Ramp) (Variables|Sun|GetSun%20Height)) :!class /Script/Engine.MaterialInstanceDynamic)
      (Rendering|Material|SetScalarParameterValue _returnvalue_2 "Stars Rotation" (Variables|Stars|GetStars%20Rotation%20Speed) :!class /Script/Engine.MaterialInstanceDynamic)
      (Rendering|Material|SetScalarParameterValue _returnvalue_2 "Stars Brightness" (Variables|Stars|GetStars%20Brightness) :!class /Script/Engine.MaterialInstanceDynamic)
      (Rendering|Material|SetVectorParameterValue _returnvalue_2 "Night Color" (Math|Curves|GetLinearColorValue (Variables|Stars|GetNight%20Color%20Ramp) (Variables|Sun|GetSun%20Height)) :!class /Script/Engine.MaterialInstanceDynamic)
      (Rendering|Material|SetTextureParameterValue _returnvalue_2 "Star Texture" (Variables|Stars|GetStar%20Texture)))
    (:then_5
      ;[1 1 1] Moon
      (if (Variables|Moon|GetShow%20Moon)
        (Rendering|Material|SetVectorParameterValue _returnvalue_2 "Moon Direction" (Math|Conversions|ToLinearColor(Vector) (Math|Rotator|GetRotationXVector (Math|Rotator|MakeRotator 0.0 _x _y))) :!class /Script/Engine.MaterialInstanceDynamic)
        (Rendering|Material|SetScalarParameterValue _returnvalue_2 "Moon Scale" (Variables|Moon|GetMoon%20Scale) :!class /Script/Engine.MaterialInstanceDynamic)
        (Rendering|Material|SetScalarParameterValue _returnvalue_2 "Moon Intensity" (Variables|Moon|GetMoon%20Intensity) :!class /Script/Engine.MaterialInstanceDynamic)
        (Rendering|Material|SetScalarParameterValue _returnvalue_2 "Moon Phase" (Variables|Moon|GetMoon%20Phase) :!class /Script/Engine.MaterialInstanceDynamic)
        (Rendering|Material|SetScalarParameterValue _returnvalue_2 "Moon Phase Rotation" (Variables|Moon|GetMoon%20Phase%20Rotation) :!class /Script/Engine.MaterialInstanceDynamic)
        (Rendering|Material|SetVectorParameterValue _returnvalue_2 "Moon Tint" (Math|Conversions|ToLinearColor(Color) (Variables|Moon|GetMoon%20Tint)) :!class /Script/Engine.MaterialInstanceDynamic)
        (Rendering|Material|SetTextureParameterValue _returnvalue_2 "Moon Texture" (Variables|Moon|GetMoon%20Texture))
        (else
          (Rendering|Material|SetScalarParameterValue _returnvalue_2 "Moon Intensity" 0.0 :!class /Script/Engine.MaterialInstanceDynamic))))
    (:then_6
      ;[1 1 1] Aurora
      (Rendering|Material|SetScalarParameterValue _returnvalue_2 "Aurora Speed" (Variables|Aurora|GetAurora%20Speed) :!class /Script/Engine.MaterialInstanceDynamic)
      (Rendering|Material|SetScalarParameterValue _returnvalue_2 "Aurora Intensity" (Variables|Aurora|GetAurora%20Intensity) :!class /Script/Engine.MaterialInstanceDynamic)
      (Rendering|Material|SetScalarParameterValue _returnvalue_2 "Aurora Color Variation" (Variables|Aurora|GetAurora%20Color%20Variation) :!class /Script/Engine.MaterialInstanceDynamic)
      (Rendering|Material|SetVectorParameterValue _returnvalue_2 "Aurora Color" (Math|Conversions|ToLinearColor(Color) (Variables|Aurora|GetAurora%20Color%20Tint)) :!class /Script/Engine.MaterialInstanceDynamic))))