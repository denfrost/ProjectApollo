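; Volumetric cloud actor for a dynamic skydome that renders clouds through a material on a scaled CloudBounds component.
; RefreshClouds runs on construction and every Tick, placing the bounds, creating a new dynamic material instance and pushing shape, motion and color parameters.
; Cloud color comes from a color ramp sampled by the sun actor's pitch, with an optional override.
; Construction also issues console commands for volumetric fog grid resolution.
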(event EventTick
  (params (DeltaSeconds :type Float%20%28single-precision%29))
  (CallFunction|RefreshClouds))

(fn ConstructionScript
  (CallFunction|RefreshClouds)
  (Development|ExecuteConsoleCommand (Utilities|String|Append "r.VolumetricFog.GridPixelSize " (Utilities|String|ToString(Integer) (Variables|CloudSettings|GetPixel%20Resolution))) 0)
  (Development|ExecuteConsoleCommand (Utilities|String|Append "r.VolumetricFog.GridSizeZ " (Utilities|String|ToString(Integer) (Variables|CloudSettings|GetGrid%20Resolution))) 0))

(fn RefreshClouds
  (bind _cloud_bounds (Variables|Default|GetCloud%20Bounds))
  (bind _cloud_area (Variables|GeometryandSpeed|GetCloud%20Area))
  (Utilities|FlowControl|Sequence
    (:then_0
      ;[1 1 1] Material Instance and BP Transform
      (Transformation|SetWorldRotation (Variables|Default|GetCloud%20Bounds) "0, 0, 0" false false)
      (Transformation|SetWorldLocation _cloud_bounds (Math|Vector|MakeVector 0.0 0.0 (Variables|GeometryandSpeed|GetCloud%20Height)) false false)
      (Transformation|SetWorldScale3D _cloud_bounds (Math|Vector|MakeVector _cloud_area _cloud_area (Variables|GeometryandSpeed|GetCloud%20Depth)))
      (bind _returnvalue (Rendering|Material|CreateDynamicMaterialInstance (Variables|Default|GetCloud%20Bounds) 0 "/Game/Dynamic_Skydome/Materials/Clouds_inst.Clouds_inst" "None" :!class /Script/Engine.PrimitiveComponent)))
    (:then_1
      ;[1 1 1] Cloud Settings
      (Rendering|Material|SetScalarParameterValue _returnvalue "Density" (Variables|CloudSettings|GetDensity) :!class /Script/Engine.MaterialInstanceDynamic)
      (Rendering|Material|SetScalarParameterValue _returnvalue "Detail" (Variables|CloudSettings|GetDetail%20Intensity) :!class /Script/Engine.MaterialInstanceDynamic)
      (Rendering|Material|SetScalarParameterValue _returnvalue "Scale" (Variables|CloudSettings|GetScale) :!class /Script/Engine.MaterialInstanceDynamic)
      (Rendering|Material|SetScalarParameterValue _returnvalue "Detail Scale" (Variables|CloudSettings|GetDetail%20Scale) :!class /Script/Engine.MaterialInstanceDynamic)
      (Rendering|Material|SetScalarParameterValue _returnvalue "Amount" (Variables|CloudSettings|GetCloud%20Amount) :!class /Script/Engine.MaterialInstanceDynamic))
    (:then_2
      ;[1 1 1] Position and Speed
      (Rendering|Material|SetScalarParameterValue _returnvalue "Position X" (Variables|GeometryandSpeed|GetPosition%20X) :!class /Script/Engine.MaterialInstanceDynamic)
      (Rendering|Material|SetScalarParameterValue _returnvalue "Position Y" (Variables|GeometryandSpeed|GetPosition%20Y) :!class /Script/Engine.MaterialInstanceDynamic)
      (Rendering|Material|SetScalarParameterValue _returnvalue "Speed X" (Variables|GeometryandSpeed|GetSpeed%20X) :!class /Script/Engine.MaterialInstanceDynamic)
      (Rendering|Material|SetScalarParameterValue _returnvalue "Speed Y" (Variables|GeometryandSpeed|GetSpeed%20Y) :!class /Script/Engine.MaterialInstanceDynamic))
    (:then_3
      ;[1 1 1] Color Settings
      (Variables|ColorSettings|SetSun%20Height (Math|Float|MapRangeUnclamped (.Pitch (Math|Rotator|BreakRotator (Transformation|GetActorRotation (Variables|ColorSettings|GetSun%20/%20Sky%20Actor)))) 0.0 -9e+01 0.0 1.0))
      (Rendering|Material|SetVectorParameterValue _returnvalue "Color" (Math|Curves|GetLinearColorValue (Variables|ColorSettings|GetCloud%20Color%20Ramp) (Variables|ColorSettings|GetSun%20Height)) :!class /Script/Engine.MaterialInstanceDynamic)
      (Rendering|Material|SetVectorParameterValue _returnvalue "Custom Color" (Math|Conversions|ToLinearColor(Color) (Variables|ColorSettings|GetOverride%20Color)) :!class /Script/Engine.MaterialInstanceDynamic)
      (Rendering|Material|SetScalarParameterValue _returnvalue "Override Color" (Variables|ColorSettings|GetOverride%20Factor) :!class /Script/Engine.MaterialInstanceDynamic)
      (Rendering|Material|SetScalarParameterValue _returnvalue "Fake Volume" (Variables|ColorSettings|GetFake%20Volume) :!class /Script/Engine.MaterialInstanceDynamic)
      (Rendering|Material|SetScalarParameterValue _returnvalue "Saturation" (Variables|ColorSettings|GetSaturation) :!class /Script/Engine.MaterialInstanceDynamic))))